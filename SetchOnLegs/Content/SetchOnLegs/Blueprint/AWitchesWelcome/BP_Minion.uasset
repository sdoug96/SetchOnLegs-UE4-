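; BP_Minion is a turret-like minion that repeatedly fires BP_Orb projectiles at a rate set by BP_WickedWitch's state.
; Every Tick it looks up the first witch in the level and branches on her State, with a shorter Delay for each successive state.
; The latent Delay acts as the fire timer, after which an orb spawns at the Arrow component's transform and a 2D turret sound plays.
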(event EventTick
  (params (DeltaSeconds :type Float%20%28single-precision%29))
  (bind _outactors (Actor|GetAllActorsOfClass "/Game/SetchOnLegs/Blueprint/AWitchesWelcome/BP_WickedWitch.BP_WickedWitch_C"))
  (bind _asbp_wicked_witch (Utilities|Casting|CastToBP_WickedWitch (Utilities|Array|Get(acopy) _outactors)))
  (if (Utilities|Enum|Equal(Enum) (Variables|/Game/SetchOnLegs/Blueprint/AWitchesWelcome/BP_WickedWitch.BP_WickedWitch_C|GetState _asbp_wicked_witch) "NewEnumerator0")
    (Utilities|FlowControl|Delay 3.0)
    (Game|SpawnActorfromClass "/Game/SetchOnLegs/Blueprint/AWitchesWelcome/BP_Orb.BP_Orb_C" (Transformation|GetWorldTransform (Variables|Default|GetArrow)) "Undefined" 0 0)
    (Audio|PlaySound2D "/Game/SetchOnLegs/Audio/GreasyGrove/Turret.Turret" 1.0 1.0 0.0 0 0 :!label _label)
    (elif (Utilities|Enum|Equal(Enum) (Variables|/Game/SetchOnLegs/Blueprint/AWitchesWelcome/BP_WickedWitch.BP_WickedWitch_C|GetState _asbp_wicked_witch) "NewEnumerator1")
      (Utilities|FlowControl|Delay 2.5)
      (Game|SpawnActorfromClass "/Game/SetchOnLegs/Blueprint/AWitchesWelcome/BP_Orb.BP_Orb_C" (Transformation|GetWorldTransform (Variables|Default|GetArrow)) "Undefined" 0 0)
      (goto _label)
      (elif (Utilities|Enum|Equal(Enum) (Variables|/Game/SetchOnLegs/Blueprint/AWitchesWelcome/BP_WickedWitch.BP_WickedWitch_C|GetState _asbp_wicked_witch) "NewEnumerator2")
        (Utilities|FlowControl|Delay 2.0)
        (Game|SpawnActorfromClass "/Game/SetchOnLegs/Blueprint/AWitchesWelcome/BP_Orb.BP_Orb_C" (Transformation|GetWorldTransform (Variables|Default|GetArrow)) "Undefined" 0 0)
        (goto _label)))))

(fn ConstructionScript)
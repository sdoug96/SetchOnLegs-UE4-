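; BP_Bat is a flying enemy that chases the player, BP_Spike, and dies when its health runs out.
; A homing projectile movement component targets Spike's capsule, and Tick flips the bat by comparing X positions.
; Its HitSpike overlap damages Spike without knockback, scaled down by armor level and skipped in one player state.
; Its TakeHit overlap destroys normal and charged bullets and applies their damage to the bat.
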(event OnComponentBeginOverlap(HitSpike)
  (params (OverlappedComponent :type Primitive%20Component%20Object%20Reference) (OtherActor :type Actor%20Object%20Reference) (OtherComp :type Primitive%20Component%20Object%20Reference) (OtherBodyIndex :type Integer) (bFromSweep :type Boolean) (SweepResult :type Hit%20Result%20Structure%20%28by%20ref%29))
  ;[1 1 1] Hit Player
  (bind _asbp_spike (Utilities|Casting|CastToBP_Spike OtherActor))
  (if (Utilities|Enum|NotEqual(Enum) (Variables|/Game/SetchOnLegs/Blueprint/Spike/BP_Spike.BP_Spike_C|GetState _asbp_spike) "NewEnumerator5")
    (switch int (Variables|/Game/SetchOnLegs/Blueprint/Spike/BP_Spike.BP_Spike_C|GetArmorLevel _asbp_spike)
      (:0
        (Default|DamageSytsem _asbp_spike (Variables|Default|GetDamage) 0.0))
      (:1
        (Default|DamageSytsem _asbp_spike (* (Variables|Default|GetDamage) 0.9) 0.0))
      (:2
        (Default|DamageSytsem _asbp_spike (* (Variables|Default|GetDamage) 0.8) 0.0))
      (:3
        (Default|DamageSytsem _asbp_spike (* (Variables|Default|GetDamage) 0.7) 0.0))
      (:4
        (Default|DamageSytsem _asbp_spike (* (Variables|Default|GetDamage) 0.6) 0.0))
      (:5
        (Default|DamageSytsem _asbp_spike (* (Variables|Default|GetDamage) 0.5) 0.0)))
    (Audio|PlaySound2D "/Game/SetchOnLegs/Audio/Misc/Ouch.Ouch" 1.0 1.0 0.0 0 0)))

(event OnComponentBeginOverlap(TakeHit)
  (params (OverlappedComponent :type Primitive%20Component%20Object%20Reference) (OtherActor :type Actor%20Object%20Reference) (OtherComp :type Primitive%20Component%20Object%20Reference) (OtherBodyIndex :type Integer) (bFromSweep :type Boolean) (SweepResult :type Hit%20Result%20Structure%20%28by%20ref%29))
  ;[1 1 1] Bullet Collision
  (Utilities|FlowControl|Sequence
    (:then_0
      (bind _asbp_bullet (Utilities|Casting|CastToBP_Bullet OtherActor))
      (Actor|DestroyActor _asbp_bullet)
      (if (not (Variables|Default|GetIsDead))
        (CallFunction|DamageSytsem (Variables|Default|GetBulletDamage))))
    (:then_1
      (bind _asbp_charged_bullet (Utilities|Casting|CastToBP_ChargedBullet OtherActor))
      (Actor|DestroyActor _asbp_charged_bullet)
      (if (not (Variables|Default|GetIsDead))
        (CallFunction|DamageSytsem (Variables|Default|GetChargedBulletDamage))))))

(event Custom|Damage%20Sytsem
  (params (DamageIn :type Float%20%28single-precision%29))
  ;[1 1 1] Damage & Death System
  (bind _output_get (Variables|Default|SetCurrentHealth (- (Variables|Default|GetCurrentHealth) DamageIn)))
  (if (<= _output_get 0.0)
    (Variables|Default|SetIsDead true)
    (Actor|DestroyActor)))

(event EventBeginPlay
  (bind _projectilemovement (Variables|Default|GetProjectileMovement))
  ;[1 1 1] Move towards Spike
  (bind _asbp_spike (Utilities|Casting|CastToBP_Spike (Game|GetPlayerCharacter 0)))
  (Variables|/Script/Engine.ProjectileMovementComponent|SetbIsHomingProjectile _projectilemovement true)
  (Variables|/Script/Engine.ProjectileMovementComponent|SetHomingTargetComponent _projectilemovement (Variables|/Script/Engine.Character|GetCapsuleComponent _asbp_spike)))

(event EventTick
  (params (DeltaSeconds :type Float%20%28single-precision%29))
  ;[1 1 1] Rotate according to position
  (bind _asbp_spike (Utilities|Casting|CastToBP_Spike (Game|GetPlayerCharacter 0)))
  (if (> (.x (Transformation|GetActorLocation _asbp_spike)) (.x (Transformation|GetActorLocation)))
    (Transformation|SetActorRotation "0,180.000000, 0")
    (else
      (Transformation|SetActorRotation "0, 0, 0"))))

(fn ConstructionScript)
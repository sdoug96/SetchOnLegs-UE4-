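; Wicked Witch boss with a health widget, flipbook forms and a looping timeline that moves it between two points.
; As health drops, delay-gated Tick logic switches forms and spawns random-X flameballs, adding shadows in the final form.
; Bullet overlaps deal damage with a timer-driven blink, though charged bullets only do so once IsDead is set.
; Death destroys minions, hazards and the witch, with a delayed LevelSelect load on Tick.
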(event OnComponentBeginOverlap(BulletBox)
  (params (OverlappedComponent :type Primitive%20Component%20Object%20Reference) (OtherActor :type Actor%20Object%20Reference) (OtherComp :type Primitive%20Component%20Object%20Reference) (OtherBodyIndex :type Integer) (bFromSweep :type Boolean) (SweepResult :type Hit%20Result%20Structure%20%28by%20ref%29))
  ;[1 1 1] Bullet Collision
  (Utilities|FlowControl|Sequence
    (:then_0
      (bind _asbp_bullet (Utilities|Casting|CastToBP_Bullet OtherActor))
      (Actor|DestroyActor _asbp_bullet)
      (if (not (Variables|Default|GetIsDead))
        (CallFunction|DamageSytsem (Variables|Default|GetBulletDamage))))
    (:then_1
      (bind _asbp_charged_bullet (Utilities|Casting|CastToBP_ChargedBullet OtherActor))
      (Actor|DestroyActor _asbp_charged_bullet)
      (if (Variables|Default|GetIsDead)
        (CallFunction|DamageSytsem (Variables|Default|GetChargedBulletDamage))))))

(event Custom|Blink
  (bind _sprite (Variables|Default|GetSprite))
  ;[1 1 1] Damage & Death System
  (Development|SetHiddeninGame _sprite (not (Variables|/Script/Engine.SceneComponent|GetbHiddenInGame _sprite)) false))

(event Custom|Damage%20Sytsem
  (params (DamageIn :type Float%20%28single-precision%29))
  ;[1 1 1] Damage & Death System
  (bind _output_get (Variables|Default|SetCurrentHealth (- (Variables|Default|GetCurrentHealth) DamageIn)))
  (if (<= _output_get 0.0)
    (Variables|Default|SetState "NewEnumerator3")
    (Variables|Default|SetIsDead true)
    (Widget|RemovefromParent (stale EventBeginPlay _returnvalue))
    (CallFunction|UpdateAnimation)
    (Utilities|FlowControl|Delay 1.0)
    (Actor|DestroyActor)
    (else
      (Utilities|Time|SetTimerbyFunctionName 0 "Blink" 0.05 true)
      (Utilities|FlowControl|Delay 0.2)
      (Utilities|Time|ClearTimerbyFunctionName 0 "Blink")
      (Development|SetHiddeninGame (Variables|Default|GetSprite) false false))))

(event Custom|UpdateAnimation
  ;[1 1 1] Handle Animation
  (switch Utilities|FlowControl|Switch|SwitchonEnum_WickedWitchState (Variables|Default|GetState)
    (:NewEnumerator0
      (Sprite|SetFlipbook (Variables|Default|GetSprite) "/Game/SetchOnLegs/Sprites/AWitchesWelcome/WickedWitch/Form1/A_Form1.A_Form1"))
    (:NewEnumerator1
      (Sprite|SetFlipbook (Variables|Default|GetSprite) "/Game/SetchOnLegs/Sprites/AWitchesWelcome/WickedWitch/Form2/A_Form2.A_Form2"))
    (:NewEnumerator2
      (Sprite|SetFlipbook (Variables|Default|GetSprite) "/Game/SetchOnLegs/Sprites/AWitchesWelcome/WickedWitch/Form3/A_Form3.A_Form3"))
    (:NewEnumerator3
      (Sprite|SetFlipbook (Variables|Default|GetSprite) "/Game/SetchOnLegs/Sprites/AWitchesWelcome/WickedWitch/A_Death.A_Death"))))

(event EventBeginPlay
  ;[1 1 1] Initialise
  (Utilities|FlowControl|Sequence
    (:then_0
      (Variables|Default|SetState "NewEnumerator0")
      (CallFunction|UpdateAnimation)
      (bind _returnvalue (UserInterface|CreateWidget "/Game/SetchOnLegs/Blueprint/AWitchesWelcome/Widget_WickedWitch.Widget_WickedWitch_C"))
      (UserInterface|Viewport|AddtoViewport _returnvalue 0)
      (bind _asbp_game_instance (Utilities|Casting|CastToBP_GameInstance (Game|GetGameInstance)))
      (if (Variables|/Game/SetchOnLegs/Blueprint/Misc/BP_GameInstance.BP_GameInstance_C|GetMegaCannon _asbp_game_instance)
        (Variables|Default|SetBulletDamage 4.0)))
    (:then_1
      (bind _output_get (Variables|Default|SetInitialLocation (Transformation|GetActorLocation)))
      (Variables|Default|SetEndLocation (+ _output_get (Math|Vector|MakeVector (Variables|Default|GetPosDiffX) 0.0 (Variables|Default|GetPosDiffZ))))
      (bind _newtrack_0 (Timeline|Timeline_0 Play)
        (:Update
          (Transformation|SetActorLocation (Math|Vector|Lerp(Vector) (Variables|Default|GetInitialLocation) (Variables|Default|GetEndLocation) _newtrack_0) false false))
        (:Finished
          (if (Variables|Default|GetTimeFactor)
            (Variables|Default|SetTimeFactor false)
            (Timeline|Timeline_0 ReverseFromEnd)
            (else
              (Variables|Default|SetTimeFactor true)
              (Timeline|Timeline_0 PlayFromStart))))))))

(event EventTick
  (params (DeltaSeconds :type Float%20%28single-precision%29))
  (bind _currenthealth (Variables|Default|GetCurrentHealth))
  ;[1 1 1] Tick
  (Utilities|FlowControl|Sequence
    (:then_0
      (if (< _currenthealth 1.5e+03)
        (if (> _currenthealth 5e+02)
          (Variables|Default|SetState "NewEnumerator1")
          (CallFunction|UpdateAnimation)
          (Utilities|FlowControl|Delay 0.5)
          (Game|SpawnActorfromClass "/Game/SetchOnLegs/Blueprint/AWitchesWelcome/BP_Flameball.BP_Flameball_C" (Math|Transform|MakeTransform (Math|Vector|MakeVector (Math|Random|RandomFloatinRange -725.0 2e+03) 0.0 1013.0) "0, 0, 0" "1,1,1") "Undefined" 0 0)
          (Audio|PlaySound2D "/Game/SetchOnLegs/Audio/Menus/Fire.Fire" 1.0 1.0 0.0 0 0))))
    (:then_1
      (if (< _currenthealth 5e+02)
        (if (> _currenthealth 0.0)
          (Variables|Default|SetState "NewEnumerator2")
          (CallFunction|UpdateAnimation)
          (Utilities|FlowControl|Delay 0.35)
          (Game|SpawnActorfromClass "/Game/SetchOnLegs/Blueprint/AWitchesWelcome/BP_Flameball.BP_Flameball_C" (Math|Transform|MakeTransform (Math|Vector|MakeVector (Math|Random|RandomFloatinRange -725.0 2e+03) 0.0 1013.0) "0, 0, 0" "1,1,1") "Undefined" 0 0)
          (Audio|PlaySound2D "/Game/SetchOnLegs/Audio/Menus/Fire.Fire" 1.0 1.0 0.0 0 0)
          (Utilities|FlowControl|Delay 2.5)
          (Utilities|Casting|CastToBP_Spike (Game|GetPlayerCharacter 0))
          (Game|SpawnActorfromClass "/Game/SetchOnLegs/Blueprint/AWitchesWelcome/BP_Shadow.BP_Shadow_C" (Math|Transform|MakeTransform (Math|Vector|MakeVector 1.8e+03 0.0 -3.5e+02) "0, 0, 0" "2.125000,1.000000,1.812500") "Undefined" 0 0))))
    (:then_3
      (if (Variables|Default|GetIsDead)
        (bind _outactors (Actor|GetAllActorsOfClass "/Game/SetchOnLegs/Blueprint/AWitchesWelcome/BP_Minion.BP_Minion_C"))
        (Actor|DestroyActor _outactors)
        (bind _outactors_2 (Actor|GetAllActorsOfClass "/Game/SetchOnLegs/Blueprint/AWitchesWelcome/BP_Flameball.BP_Flameball_C"))
        (Actor|DestroyActor _outactors_2)
        (bind _outactors_3 (Actor|GetAllActorsOfClass "/Game/SetchOnLegs/Blueprint/AWitchesWelcome/BP_Shadow.BP_Shadow_C"))
        (Actor|DestroyActor _outactors_3)
        (bind _outactors_4 (Actor|GetAllActorsOfClass "/Game/SetchOnLegs/Blueprint/Misc/BP_Killpad.BP_Killpad_C"))
        (Actor|DestroyActor _outactors_4)
        (bind _outactors_5 (Actor|GetAllActorsOfClass "/Game/SetchOnLegs/Blueprint/AWitchesWelcome/BP_Orb.BP_Orb_C"))
        (Actor|DestroyActor _outactors_5)
        (Utilities|FlowControl|Delay 7.0)
        (Game|OpenLevel(byName) "LevelSelect")))))

(fn ConstructionScript)
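; GBWF boss enemy for Greasy Grove: a flipbook character that chases Spike along X and lunges to swipe on proximity.
; A state enum drives animation, while overlap volumes take bullet hits and deal armor-scaled damage with directional knockback.
; Tick steers movement and activates three turrets below a health threshold.
; Death shuts off turrets, clears killpads, replaces bouncepads with a new one, and destroys the boss after a delay.
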(event OnComponentBeginOverlap(Sphere)
  (params (OverlappedComponent :type Primitive%20Component%20Object%20Reference) (OtherActor :type Actor%20Object%20Reference) (OtherComp :type Primitive%20Component%20Object%20Reference) (OtherBodyIndex :type Integer) (bFromSweep :type Boolean) (SweepResult :type Hit%20Result%20Structure%20%28by%20ref%29))
  (bind _lunge (Variables|Default|GetLunge))
  ;[1 1 1] Hit Spike
  (if (not (Variables|Default|GetIsDead))
    (Utilities|Casting|CastToBP_Spike OtherActor)
    (Components|Movement|StopMovementImmediately (Variables|Character|GetCharacterMovement))
    (Variables|Default|SetState "NewEnumerator1")
    (CallFunction|UpdateAnimation)
    (if (== (.yaw (Transformation|GetActorRotation)) 0.0)
      (Character|LaunchCharacter _lunge false false)
      (else
        (Character|LaunchCharacter (* _lunge "-1.000000, 0, 0") false false)))))

(event OnComponentEndOverlap(Sphere)
  (params (OverlappedComponent :type Primitive%20Component%20Object%20Reference) (OtherActor :type Actor%20Object%20Reference) (OtherComp :type Primitive%20Component%20Object%20Reference) (OtherBodyIndex :type Integer))
  ;[1 1 1] Hit Spike
  (if (not (Variables|Default|GetIsDead))
    (Utilities|Casting|CastToBP_Spike OtherActor)
    (Variables|/Script/Engine.MovementComponent|SetVelocity (Variables|Character|GetCharacterMovement) "275.000000, 0, 0")
    (Variables|Default|SetState "NewEnumerator2")
    (CallFunction|UpdateAnimation)))

(event OnComponentBeginOverlap(Box)
  (params (OverlappedComponent :type Primitive%20Component%20Object%20Reference) (OtherActor :type Actor%20Object%20Reference) (OtherComp :type Primitive%20Component%20Object%20Reference) (OtherBodyIndex :type Integer) (bFromSweep :type Boolean) (SweepResult :type Hit%20Result%20Structure%20%28by%20ref%29))
  (bind _spikeknockback (Variables|Default|GetSpikeKnockBack))
  (bind _damage (Variables|Default|GetDamage))
  ;[1 1 1] Hit Spike
  (if (not (Variables|Default|GetIsDead))
    (Utilities|FlowControl|Delay 0.5)
    (bind _asbp_spike (Utilities|Casting|CastToBP_Spike OtherActor))
    (if (Utilities|Enum|NotEqual(Enum) (Variables|/Game/SetchOnLegs/Blueprint/Spike/BP_Spike.BP_Spike_C|GetState _asbp_spike) "NewEnumerator5")
      (switch int (Variables|/Game/SetchOnLegs/Blueprint/Spike/BP_Spike.BP_Spike_C|GetArmorLevel _asbp_spike)
        (:0
          (Default|DamageSytsem _asbp_spike _damage _spikeknockback))
        (:1
          (Default|DamageSytsem _asbp_spike (* _damage 0.9) _spikeknockback))
        (:2
          (Default|DamageSytsem _asbp_spike (* _damage 0.8) _spikeknockback))
        (:3
          (Default|DamageSytsem _asbp_spike (* _damage 0.7) _spikeknockback))
        (:4
          (Default|DamageSytsem _asbp_spike (* _damage 0.6) _spikeknockback))
        (:5
          (Default|DamageSytsem _asbp_spike (* _damage 0.5) _spikeknockback))))))

(event OnComponentBeginOverlap(BulletBox)
  (params (OverlappedComponent :type Primitive%20Component%20Object%20Reference) (OtherActor :type Actor%20Object%20Reference) (OtherComp :type Primitive%20Component%20Object%20Reference) (OtherBodyIndex :type Integer) (bFromSweep :type Boolean) (SweepResult :type Hit%20Result%20Structure%20%28by%20ref%29))
  ;[1 1 1] Bullet Collision
  (Utilities|FlowControl|Sequence
    (:then_0
      (bind _asbp_bullet (Utilities|Casting|CastToBP_Bullet OtherActor))
      (Actor|DestroyActor _asbp_bullet)
      (if (not (Variables|Default|GetIsDead))
        (CallFunction|DamageSytsem (Variables|Default|GetBulletDamage))
        (Utilities|Casting|CastToBP_Spike (Game|GetPlayerCharacter 0))))
    (:then_1
      (bind _asbp_charged_bullet (Utilities|Casting|CastToBP_ChargedBullet OtherActor))
      (Actor|DestroyActor _asbp_charged_bullet)
      (if (not (Variables|Default|GetIsDead))
        (Utilities|Casting|CastToBP_Spike (Game|GetPlayerCharacter 0))
        (CallFunction|DamageSytsem (Variables|Default|GetChargedBulletDamage))))))

(event Custom|Blink
  (bind _sprite (Variables|Default|GetSprite))
  ;[1 1 1] Damage & Death System
  (Development|SetHiddeninGame _sprite (not (Variables|/Script/Engine.SceneComponent|GetbHiddenInGame _sprite)) false))

(event Custom|Damage%20Sytsem
  (params (DamageIn :type Float%20%28single-precision%29))
  ;[1 1 1] Damage & Death System
  (bind _output_get (Variables|Default|SetCurrentHealth (- (Variables|Default|GetCurrentHealth) DamageIn)))
  (if (<= _output_get 0.0)
    (Variables|Default|SetState "NewEnumerator3")
    (Variables|Default|SetIsDead true)
    (Widget|RemovefromParent (stale EventBeginPlay _returnvalue))
    (CallFunction|UpdateAnimation)
    (Utilities|FlowControl|Delay 5.0)
    (Actor|DestroyActor)
    (else
      (Utilities|Time|SetTimerbyFunctionName 0 "Blink" 0.05 true)
      (Utilities|FlowControl|Delay 0.2)
      (Utilities|Time|ClearTimerbyFunctionName 0 "Blink")
      (Development|SetHiddeninGame (Variables|Default|GetSprite) false false))))

(event Custom|UpdateAnimation
  ;[1 1 1] Handle Animation
  (switch Utilities|FlowControl|Switch|SwitchonGBWF_State (Variables|Default|GetState)
    (:NewEnumerator0
      (Sprite|SetFlipbook (Variables|Default|GetSprite) "/Game/SetchOnLegs/Sprites/GreasyGrove/GBWFCharacter/Animations/A_Idle.A_Idle"))
    (:NewEnumerator1
      (Sprite|SetFlipbook (Variables|Default|GetSprite) "/Game/SetchOnLegs/Sprites/GreasyGrove/GBWFCharacter/Animations/A_Swipe.A_Swipe"))
    (:NewEnumerator2
      (Sprite|SetFlipbook (Variables|Default|GetSprite) "/Game/SetchOnLegs/Sprites/GreasyGrove/GBWFCharacter/Animations/A_Run.A_Run"))
    (:NewEnumerator3
      (Sprite|SetFlipbook (Variables|Default|GetSprite) "/Game/SetchOnLegs/Sprites/GreasyGrove/GBWFCharacter/Animations/A_Dead.A_Dead"))))

(event EventBeginPlay
  ;[1 1 1] Initialise
  (Utilities|FlowControl|Sequence
    (:then_0
      (Variables|Default|SetState "NewEnumerator2")
      (Pawn|Components|CharacterMovement|SetMovementMode (Variables|Character|GetCharacterMovement) "MOVE_Walking" 0)
      (CallFunction|UpdateAnimation))
    (:then_1
      (bind _asbp_game_instance (Utilities|Casting|CastToBP_GameInstance (Game|GetGameInstance)))
      (if (Variables|/Game/SetchOnLegs/Blueprint/Misc/BP_GameInstance.BP_GameInstance_C|GetMegaCannon _asbp_game_instance)
        (Variables|Default|SetBulletDamage 4.0)))
    (:then_2
      (if (Variables|Default|GetPhase2)
        (bind _returnvalue (UserInterface|CreateWidget "/Game/SetchOnLegs/Blueprint/GreasyGrove/Widget_GBWF.Widget_GBWF_C"))
        (UserInterface|Viewport|AddtoViewport _returnvalue 0)))))

(event EventTick
  (params (DeltaSeconds :type Float%20%28single-precision%29))
  (bind _charactermovement (Variables|Character|GetCharacterMovement))
  (bind _state (Variables|Default|GetState))
  (bind _currenthealth (Variables|Default|GetCurrentHealth))
  ;[1 1 1] Tick
  (Utilities|FlowControl|Sequence
    (:then_0
      (if (Utilities|Enum|NotEqual(Enum) _state "NewEnumerator3")
        (if (Utilities|Enum|Equal(Enum) _state "NewEnumerator1")
          (Utilities|FlowControl|Delay 0.75)
          (Audio|PlaySound2D "/Game/SetchOnLegs/Audio/GreasyGrove/Swipe.Swipe" 1.0 1.0 0.0 0 0)
          (else
            (bind _asbp_spike (Utilities|Casting|CastToBP_Spike (Game|GetPlayerCharacter 0)))
            (if (> (.x (Transformation|GetActorLocation)) (.x (Transformation|GetActorLocation _asbp_spike)))
              (Pawn|Input|AddMovementInput "-1.000000, 0, 0" 1.0 false)
              (Transformation|SetActorRotation "0,180.000000, 0")
              (Variables|Default|SetSpikeKnockBack -2.5e+07)
              (else
                (Pawn|Input|AddMovementInput "1.000000, 0, 0" 1.0 false)
                (Transformation|SetActorRotation "0, 0, 0")
                (Variables|Default|SetSpikeKnockBack 2.5e+07)))))))
    (:then_1
      (if (Variables|Default|GetIsDead)
        (Components|Movement|StopMovementImmediately _charactermovement)
        (Variables|/Script/Engine.MovementComponent|SetVelocity _charactermovement "0, 0, 0")
        (bind _outactors (Actor|GetAllActorsOfClass "/Game/SetchOnLegs/Blueprint/Misc/BP_Killpad.BP_Killpad_C"))
        (Actor|DestroyActor _outactors)
        (bind _outactors_2 (Actor|GetAllActorsOfClass "/Game/SetchOnLegs/Blueprint/GreasyGrove/BP_TurretKillpad.BP_TurretKillpad_C"))
        (Actor|DestroyActor _outactors_2)
        (if (Variables|Default|GetDoOnce)
          (bind _outactors_3 (Actor|GetAllActorsOfClass "/Game/SetchOnLegs/Blueprint/Misc/BP_Bouncepad.BP_Bouncepad_C"))
          (Actor|DestroyActor _outactors_3))))
    (:then_2
      (if (< _currenthealth 3.5e+02)
        (if (> _currenthealth 0.0)
          (bind _outactors_4 (Actor|GetAllActorsOfClass "/Game/SetchOnLegs/Blueprint/GreasyGrove/BP_Turret.BP_Turret_C"))
          (Variables|/Game/SetchOnLegs/Blueprint/GreasyGrove/BP_Turret.BP_Turret_C|SetActive (Utilities|Array|Get(acopy) _outactors_4) true)
          (Variables|/Game/SetchOnLegs/Blueprint/GreasyGrove/BP_Turret.BP_Turret_C|SetActive (Utilities|Array|Get(acopy) _outactors_4 1) true)
          (Variables|/Game/SetchOnLegs/Blueprint/GreasyGrove/BP_Turret.BP_Turret_C|SetActive (Utilities|Array|Get(acopy) _outactors_4 2) true)
          (else
            (bind _outactors_5 (Actor|GetAllActorsOfClass "/Game/SetchOnLegs/Blueprint/GreasyGrove/BP_Turret.BP_Turret_C"))
            (Variables|/Game/SetchOnLegs/Blueprint/GreasyGrove/BP_Turret.BP_Turret_C|SetActive (Utilities|Array|Get(acopy) _outactors_5) false)
            (Variables|/Game/SetchOnLegs/Blueprint/GreasyGrove/BP_Turret.BP_Turret_C|SetActive (Utilities|Array|Get(acopy) _outactors_5 1) false)
            (Variables|/Game/SetchOnLegs/Blueprint/GreasyGrove/BP_Turret.BP_Turret_C|SetActive (Utilities|Array|Get(acopy) _outactors_5 2) false)))))
    (:then_3
      (if (Variables|Default|GetIsDead)
        (if (Variables|Default|GetDoOnce)
          (Game|SpawnActorfromClass "/Game/SetchOnLegs/Blueprint/Misc/BP_Bouncepad.BP_Bouncepad_C" (Math|Transform|MakeTransform "-19.000000, 0,-6481.000000" "0, 0, 0" "0.750000,1,0.218750") "Undefined" 0 "0.000000,0.000000,2100.000000" 0)
          (Variables|Default|SetDoOnce false))))))

(fn ConstructionScript)
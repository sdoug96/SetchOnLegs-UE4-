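; BP_MiniGBWF is a flipbook-animated enemy that wakes and throws rocks while BP_Spike is inside its WakeTrigger.
; Overlap plays the wake and attack animations, then a looping timer spawns BP_Rock with a throw force; leaving clears it and returns to sleep.
; While active, two bullet spheres consume BP_Bullet and apply the player's BulletDamage.
; Damage blinks the sprite via a timer toggling visibility, and zero health destroys the actor.
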(event OnComponentBeginOverlap(WakeTrigger)
  (params (OverlappedComponent :type Primitive%20Component%20Object%20Reference) (OtherActor :type Actor%20Object%20Reference) (OtherComp :type Primitive%20Component%20Object%20Reference) (OtherBodyIndex :type Integer) (bFromSweep :type Boolean) (SweepResult :type Hit%20Result%20Structure%20%28by%20ref%29))
  ;[1 1 1] Wake up and throw rocks
  (Utilities|Casting|CastToBP_Spike OtherActor)
  (Variables|Default|SetActive true)
  (Sprite|SetFlipbook (Variables|Default|GetMiniGBWF) "/Game/SetchOnLegs/Sprites/02GreasyGrove/MiniCharacter/Animations/A_MiniGBWFWake.A_MiniGBWFWake")
  (Utilities|FlowControl|Delay 0.7)
  (if (Variables|Default|GetActive)
    (Sprite|SetFlipbook (Variables|Default|GetMiniGBWF) "/Game/SetchOnLegs/Sprites/02GreasyGrove/MiniCharacter/Animations/A_MiniGBWFAttack.A_MiniGBWFAttack")
    (Utilities|FlowControl|Delay (Variables|Default|GetInitialThrowDelay))
    (if (Variables|Default|GetActive)
      (CallFunction|ThrowRock)
      (Utilities|Time|SetTimerbyFunctionName 0 "ThrowRock" (Variables|Default|GetThrowDelay) true))))

(event OnComponentEndOverlap(WakeTrigger)
  (params (OverlappedComponent :type Primitive%20Component%20Object%20Reference) (OtherActor :type Actor%20Object%20Reference) (OtherComp :type Primitive%20Component%20Object%20Reference) (OtherBodyIndex :type Integer))
  ;[1 1 1] Wake up and throw rocks
  (Utilities|Casting|CastToBP_Spike OtherActor)
  (Variables|Default|SetActive false)
  (Sprite|SetFlipbook (Variables|Default|GetMiniGBWF) "/Game/SetchOnLegs/Sprites/02GreasyGrove/MiniCharacter/Animations/A_MiniGBWFSleep.A_MiniGBWFSleep")
  (Utilities|Time|ClearTimerbyFunctionName 0 "ThrowRock")
  (Utilities|FlowControl|Delay 0.5)
  (Sprite|SetFlipbook (Variables|Default|GetMiniGBWF)))

(event OnComponentBeginOverlap(BulletSphere1)
  (params (OverlappedComponent :type Primitive%20Component%20Object%20Reference) (OtherActor :type Actor%20Object%20Reference) (OtherComp :type Primitive%20Component%20Object%20Reference) (OtherBodyIndex :type Integer) (bFromSweep :type Boolean) (SweepResult :type Hit%20Result%20Structure%20%28by%20ref%29))
  ;[1 1 1] Bullet Collision
  (bind _asbp_bullet (Utilities|Casting|CastToBP_Bullet OtherActor))
  (if (Variables|Default|GetActive)
    (Actor|DestroyActor _asbp_bullet)
    (if (not (Variables|Default|GetIsDead))
      (CallFunction|DamageSytsem (Variables|/Game/SetchOnLegs/Blueprint/08Spike/BP_Spike.BP_Spike_C|GetBulletDamage (Variables|Default|GetPlayer))))))

(event OnComponentBeginOverlap(BulletSphere2)
  (params (OverlappedComponent :type Primitive%20Component%20Object%20Reference) (OtherActor :type Actor%20Object%20Reference) (OtherComp :type Primitive%20Component%20Object%20Reference) (OtherBodyIndex :type Integer) (bFromSweep :type Boolean) (SweepResult :type Hit%20Result%20Structure%20%28by%20ref%29))
  ;[1 1 1] Bullet Collision
  (bind _asbp_bullet (Utilities|Casting|CastToBP_Bullet OtherActor))
  (if (Variables|Default|GetActive)
    (Actor|DestroyActor _asbp_bullet)
    (if (not (Variables|Default|GetIsDead))
      (CallFunction|DamageSytsem (Variables|/Game/SetchOnLegs/Blueprint/08Spike/BP_Spike.BP_Spike_C|GetBulletDamage (Variables|Default|GetPlayer))))))

(event Custom|Blink
  (bind _minigbwf (Variables|Default|GetMiniGBWF))
  ;[1 1 1] Damage & Death System
  (Development|SetHiddeninGame _minigbwf (not (Variables|/Script/Engine.SceneComponent|GetbHiddenInGame _minigbwf)) false))

(event Custom|Damage%20Sytsem
  (params (DamageIn :type Float%20%28single-precision%29))
  ;[1 1 1] Damage & Death System
  (bind _output_get (Variables|Default|SetCurrentHealth (- (Variables|Default|GetCurrentHealth) DamageIn)))
  (if (<= _output_get 0.0)
    (Variables|Default|SetIsDead true)
    (Actor|DestroyActor)
    (else
      (Utilities|Time|SetTimerbyFunctionName 0 "Blink" 0.05 true)
      (Utilities|FlowControl|Delay 0.2)
      (Utilities|Time|ClearTimerbyFunctionName 0 "Blink")
      (Development|SetHiddeninGame (Variables|Default|GetMiniGBWF) false false))))

(event Custom|ThrowRock
  ;[1 1 1] Throw rock function
  (if (Variables|Default|GetActive)
    (Game|SpawnActorfromClass "/Game/SetchOnLegs/Blueprint/02GreasyGrove/BP_Rock.BP_Rock_C" (Math|Transform|MakeTransform (Transformation|GetWorldLocation (Variables|Default|GetRockSpawn)) "0, 0, 0" "0.187500,0.187500,0.187500") "Undefined" 0 (Variables|Default|GetThrowForce) 0)
    (Audio|PlaySound2D "/Game/SetchOnLegs/Audio/02GreasyGrove/Dir.Dir" 1.0 1.0 0.0 0 0)))

(event EventBeginPlay
  (bind _asbp_spike (Utilities|Casting|CastToBP_Spike (Game|GetPlayerCharacter 0)))
  (Variables|Default|SetPlayer _asbp_spike))

(fn ConstructionScript)
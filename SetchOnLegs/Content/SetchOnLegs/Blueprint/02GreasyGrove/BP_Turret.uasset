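; BP_Turret is a turret actor that fires BP_TurretKillpad projectiles at a set interval while Active.
; Tick runs through a Delay of BulletDelay to throttle fire, spawning each killpad at the Arrow's location and rotation with a flattened scale and playing a 2D sound.
; When Rotator is also set, Tick accumulates a timer and sets the actor's pitch from it times Rotation, zeroing roll and yaw.
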(event EventTick
  (params (DeltaSeconds :type Float%20%28single-precision%29))
  (bind _arrow (Variables|Default|GetArrow))
  (bind _returnvalue (Transformation|GetWorldTransform _arrow))
  ;[1 1 1] Spawn Bullets
  (Utilities|FlowControl|Sequence
    (:then_0
      (Utilities|FlowControl|Delay (Variables|Default|GetBulletDelay))
      (if (Variables|Default|GetActive)
        (Game|SpawnActorfromClass "/Game/SetchOnLegs/Blueprint/02GreasyGrove/BP_TurretKillpad.BP_TurretKillpad_C" (Math|Transform|MakeTransform (.location _returnvalue) (.rotation _returnvalue) "0.500000,1,0.200000") "Undefined" 0 0)
        (Audio|PlaySound2D "/Game/SetchOnLegs/Audio/GreasyGrove/Turret.Turret" 1.0 1.0 0.0 0 0)))
    (:then_1
      ;[1 1 1] Rotate
      (if (Variables|Default|GetActive)
        (if (Variables|Default|GetRotator)
          (Variables|Default|SetTimer (+ DeltaSeconds (Variables|Default|GetTimer)))
          (Transformation|SetActorRotation (Math|Rotator|MakeRotator 0.0 (* (Variables|Default|GetTimer) (Variables|Default|GetRotation)) 0.0)))))))

(fn ConstructionScript)
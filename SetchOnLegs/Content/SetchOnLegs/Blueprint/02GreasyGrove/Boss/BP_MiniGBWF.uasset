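; BP_MiniGBWF is a flipbook-animated enemy in the Greasy Grove boss folder that runs at the player, BP_Spike.
; Tick steers it along X and sets the knockback direction; once dead, it stops, loses capsule collision and is destroyed after a delay.
; Its hitbox takes bullet and charged-shot damage against randomized health, and deals armor-scaled contact damage to Spike.
; Non-lethal hits blink the sprite via a timer, while a state enum selects animations.
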(event OnComponentBeginOverlap(HitBox)
  (params (OverlappedComponent :type Primitive%20Component%20Object%20Reference) (OtherActor :type Actor%20Object%20Reference) (OtherComp :type Primitive%20Component%20Object%20Reference) (OtherBodyIndex :type Integer) (bFromSweep :type Boolean) (SweepResult :type Hit%20Result%20Structure%20%28by%20ref%29))
  (bind _spikeknockback (Variables|Default|GetSpikeKnockBack))
  (bind _damage (Variables|Default|GetDamage))
  ;[1 1 1] Hitbox logic
  (Utilities|FlowControl|Sequence
    (:then_0
      (bind _asbp_bullet (Utilities|Casting|CastToBP_Bullet OtherActor))
      (Actor|DestroyActor _asbp_bullet)
      (if (not (Variables|Default|GetIsDead))
        (bind _asbp_spike (Utilities|Casting|CastToBP_Spike (Game|GetPlayerCharacter 0)))
        (CallFunction|DamageSytsem (Variables|/Game/SetchOnLegs/Blueprint/08Spike/BP_Spike.BP_Spike_C|GetBulletDamage _asbp_spike))))
    (:then_1
      (bind _asbp_charged_bullet (Utilities|Casting|CastToBP_ChargedBullet OtherActor))
      (Actor|DestroyActor _asbp_charged_bullet)
      (if (not (Variables|Default|GetIsDead))
        (bind _asbp_spike_2 (Utilities|Casting|CastToBP_Spike (Game|GetPlayerCharacter 0)))
        (CallFunction|DamageSytsem (Variables|/Game/SetchOnLegs/Blueprint/08Spike/BP_Spike.BP_Spike_C|GetChargedShotDamage _asbp_spike_2))))
    (:then_2
      (bind _asbp_spike_3 (Utilities|Casting|CastToBP_Spike OtherActor))
      (if (not (Variables|Default|GetIsDead))
        (if (not (Variables|/Game/SetchOnLegs/Blueprint/08Spike/BP_Spike.BP_Spike_C|GetIsDead _asbp_spike_3))
          (switch int (Variables|/Game/SetchOnLegs/Blueprint/08Spike/BP_Spike.BP_Spike_C|GetArmorLevel _asbp_spike_3)
            (:0
              (Default|DamageSytsem _asbp_spike_3 _damage _spikeknockback))
            (:1
              (Default|DamageSytsem _asbp_spike_3 (* _damage 0.9) _spikeknockback))
            (:2
              (Default|DamageSytsem _asbp_spike_3 (* _damage 0.8) _spikeknockback))
            (:3
              (Default|DamageSytsem _asbp_spike_3 (* _damage 0.7) _spikeknockback))
            (:4
              (Default|DamageSytsem _asbp_spike_3 (* _damage 0.6) _spikeknockback))
            (:5
              (Default|DamageSytsem _asbp_spike_3 (* _damage 0.5) _spikeknockback))))))))

(event Custom|Blink
  (bind _sprite (Variables|Default|GetSprite))
  ;[1 1 1] Damage & Death System
  (Development|SetHiddeninGame _sprite (not (Variables|/Script/Engine.SceneComponent|GetbHiddenInGame _sprite)) false))

(event Custom|Damage%20Sytsem
  (params (DamageIn :type Float%20%28single-precision%29))
  ;[1 1 1] Damage & Death System
  (bind _output_get (Variables|Default|SetCurrentHealth (- (Variables|Default|GetCurrentHealth) DamageIn)))
  (if (<= _output_get 0.0)
    (Variables|Default|SetState "NewEnumerator3")
    (Variables|Default|SetIsDead true)
    (CallFunction|UpdateAnimation)
    (else
      (Utilities|Time|SetTimerbyFunctionName 0 "Blink" 0.05 true)
      (Utilities|FlowControl|Delay 0.2)
      (Utilities|Time|ClearTimerbyFunctionName 0 "Blink")
      (Development|SetHiddeninGame (Variables|Default|GetSprite) false false))))

(event Custom|UpdateAnimation
  ;[1 1 1] Handle Animation
  (switch Utilities|FlowControl|Switch|SwitchonGBWF_State (Variables|Default|GetState)
    (:NewEnumerator0
      (Sprite|SetFlipbook (Variables|Default|GetSprite) "/Game/SetchOnLegs/Sprites/02GreasyGrove/GBWFCharacter/Animations/A_Idle.A_Idle"))
    (:NewEnumerator1
      (Sprite|SetFlipbook (Variables|Default|GetSprite) "/Game/SetchOnLegs/Sprites/02GreasyGrove/GBWFCharacter/Animations/A_Swipe.A_Swipe"))
    (:NewEnumerator2
      (Sprite|SetFlipbook (Variables|Default|GetSprite) "/Game/SetchOnLegs/Sprites/02GreasyGrove/GBWFCharacter/Animations/A_Run.A_Run"))
    (:NewEnumerator3
      (Sprite|SetFlipbook (Variables|Default|GetSprite) "/Game/SetchOnLegs/Sprites/02GreasyGrove/GBWFCharacter/Animations/A_QuickDeath.A_QuickDeath"))))

(event EventBeginPlay
  ;[1 1 1] Initialise
  (Variables|Default|SetState "NewEnumerator2")
  (Pawn|Components|CharacterMovement|SetMovementMode (Variables|Character|GetCharacterMovement) "MOVE_Walking" 0)
  (CallFunction|UpdateAnimation)
  (Variables|Default|SetCurrentHealth (Math|Random|RandomFloatinRange 1e+01 2e+01)))

(event EventTick
  (params (DeltaSeconds :type Float%20%28single-precision%29))
  (bind _charactermovement (Variables|Character|GetCharacterMovement))
  ;[1 1 1] Tick
  (if (Variables|Default|GetIsDead)
    (Components|Movement|StopMovementImmediately _charactermovement)
    (Variables|/Script/Engine.MovementComponent|SetVelocity _charactermovement "0, 0, 0")
    (Collision|SetCollisionEnabled (Variables|Collision|GetCapsuleComponent) "NoCollision")
    (Utilities|FlowControl|Delay 2.0)
    (Actor|DestroyActor)
    (else
      (bind _asbp_spike (Utilities|Casting|CastToBP_Spike (Game|GetPlayerCharacter 0)))
      (if (> (.x (Transformation|GetActorLocation)) (.x (Transformation|GetActorLocation _asbp_spike)))
        (Pawn|Input|AddMovementInput "-1.000000, 0, 0" 1.0 false)
        (Transformation|SetActorRotation "0,180.000000, 0")
        (Variables|Default|SetSpikeKnockBack -1.5e+07)
        (else
          (Pawn|Input|AddMovementInput "1.000000, 0, 0" 1.0 false)
          (Transformation|SetActorRotation "0, 0, 0")
          (Variables|Default|SetSpikeKnockBack 1.5e+07))))))

(fn ConstructionScript)
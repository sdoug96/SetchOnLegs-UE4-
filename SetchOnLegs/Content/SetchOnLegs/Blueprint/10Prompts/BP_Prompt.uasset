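; BP_Prompt is a trigger volume that shows a configurable prompt widget when BP_Spike enters its Box.
; Begin overlap waits for a set delay, then casts the overlapping actor to BP_Spike, creates WidgetToPrompt and adds it to the viewport.
; End overlap removes the stored widget only when Respawner is true and the leaving actor is BP_Spike.
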(event OnComponentBeginOverlap(Box)
  (params (OverlappedComponent :type Primitive%20Component%20Object%20Reference) (OtherActor :type Actor%20Object%20Reference) (OtherComp :type Primitive%20Component%20Object%20Reference) (OtherBodyIndex :type Integer) (bFromSweep :type Boolean) (SweepResult :type Hit%20Result%20Structure%20%28by%20ref%29))
  ;[1 1 1] Show widget then kill prompt
  (Utilities|FlowControl|Delay (Variables|Default|GetDelay))
  (Utilities|Casting|CastToBP_Spike OtherActor)
  (bind _returnvalue (UserInterface|CreateWidget (Variables|Default|GetWidgetToPrompt)))
  (bind _output_get (Variables|Default|SetWidget _returnvalue))
  (UserInterface|Viewport|AddtoViewport _output_get 0))

(event OnComponentEndOverlap(Box)
  (params (OverlappedComponent :type Primitive%20Component%20Object%20Reference) (OtherActor :type Actor%20Object%20Reference) (OtherComp :type Primitive%20Component%20Object%20Reference) (OtherBodyIndex :type Integer))
  ;[1 1 1] Show widget then kill prompt
  (if (Variables|Default|GetRespawner)
    (Utilities|Casting|CastToBP_Spike OtherActor)
    (Widget|RemovefromParent (Variables|Default|GetWidget))))

(fn ConstructionScript)
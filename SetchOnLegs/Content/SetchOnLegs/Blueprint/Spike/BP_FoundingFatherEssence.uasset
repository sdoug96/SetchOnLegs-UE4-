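; BP_FoundingFatherEssence is a short-lived attack actor that deals heavy damage to BP_TheCreatorEnraged.
; On BeginPlay it adds its Widget_FoundingFatherEssence to the viewport, then destroys itself after a brief delay.
; When HitSphere overlaps the enraged Creator, a delayed loop repeatedly plays a hit sound and calls DamageSytsem on the first Creator instance found in the level.
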(event OnComponentBeginOverlap(HitSphere)
  (params (OverlappedComponent :type Primitive%20Component%20Object%20Reference) (OtherActor :type Actor%20Object%20Reference) (OtherComp :type Primitive%20Component%20Object%20Reference) (OtherBodyIndex :type Integer) (bFromSweep :type Boolean) (SweepResult :type Hit%20Result%20Structure%20%28by%20ref%29))
  ;[1 1 1] Damage Creator Enraged and play audio 10x
  (Utilities|Casting|CastToBP_TheCreatorEnraged OtherActor)
  (bind _outactors (Actor|GetAllActorsOfClass "/Game/SetchOnLegs/Blueprint/06TheCreator/Enraged/BP_TheCreatorEnraged.BP_TheCreatorEnraged_C"))
  (Utilities|ForLoopwithDelay 0 10 :!label _label
    (:LoopBody
      (Audio|PlaySound2D "/Game/SetchOnLegs/Audio/Misc/FoundingFatherEssenceHit.FoundingFatherEssenceHit" 1.0 1.0 0.0 0 0)
      (Default|DamageSytsem (Utilities|Array|Get(acopy) _outactors) 5e+05))
    (:DelayOut
      (Utilities|FlowControl|Delay 0.25)
      (goto _label DelayIn))))

(event EventBeginPlay
  ;[1 1 1] Initialise
  (bind _returnvalue (UserInterface|CreateWidget "/Game/SetchOnLegs/Blueprint/Spike/Widget_FoundingFatherEssence.Widget_FoundingFatherEssence_C"))
  (UserInterface|Viewport|AddtoViewport _returnvalue 0)
  (Utilities|FlowControl|Delay 2.7)
  (Actor|DestroyActor))

(fn ConstructionScript)
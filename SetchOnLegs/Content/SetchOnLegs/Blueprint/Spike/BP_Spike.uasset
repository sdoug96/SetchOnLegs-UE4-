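; BP_Spike is the player's 2D side-scrolling flipbook character, handling walking, jumping, ladder climbing, shooting, pausing and placeable checkpoints.
; On BeginPlay it creates the HUD and copies stats and upgrades from BP_GameInstance.
; Shots aim at the mouse via screen projection, with spread upgrades and a shot-charged blast that launches Spike.
; Damage applies knockback and timer-driven blinking; death reloads listed boss levels or restores the saved checkpoint location.
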(event Custom|Blink
  (bind _sprite (Variables|Default|GetSprite))
  ;[1 1 1] Damage & Death System
  (Development|SetHiddeninGame _sprite (not (Variables|/Script/Engine.SceneComponent|GetbHiddenInGame _sprite)) false))

(event Custom|Damage%20Sytsem
  (params (DamageIn :type Float%20%28single-precision%29) (KnockBack :type Float%20%28single-precision%29))
  ;[1 1 1] Damage & Death System
  (if (Utilities|Enum|NotEqual(Enum) (Variables|Default|GetState) "NewEnumerator5")
    (if (!= (Class|PaperFlipbookComponent|GetFlipbook (Variables|Default|GetSprite)) "/Game/SetchOnLegs/Sprites/Spike/Character/A_Dead.A_Dead")
      (bind _output_get (Variables|Default|SetCurrentHealth (- (Variables|Default|GetCurrentHealth) DamageIn)))
      (if (<= _output_get 0.0)
        (Variables|Default|SetState "NewEnumerator5")
        (Variables|Default|SetDeathCount (+ (Variables|Default|GetDeathCount) 1))
        (Input|DisableInput (Game|GetPlayerController 0))
        (CallFunction|UpdateAnimation)
        (Utilities|FlowControl|Delay 2.0)
        (Variables|Default|SetIsDead true)
        (if (Variables|Default|GetIsDead)
          (bind _returnvalue (Game|GetCurrentLevelName true))
          (if (Utilities|Enum|Equal(Enum) _returnvalue "HinceInHellBoss")
            (Utilities|FlowControl|Delay 2.0)
            (bind _asbp_game_instance (Utilities|Casting|CastToBP_GameInstance (Game|GetGameInstance)))
            (Variables|/Game/SetchOnLegs/Blueprint/Misc/BP_GameInstance.BP_GameInstance_C|SetDeathCount _asbp_game_instance (Variables|Default|GetDeathCount))
            (Game|OpenLevel(byName) "HinceInHellBoss")
            (else
              (bind _returnvalue_2 (Game|GetCurrentLevelName true))
              (if (Utilities|Enum|Equal(Enum) _returnvalue_2 "GreasyGroveBossChase")
                (Utilities|FlowControl|Delay 2.0)
                (bind _asbp_game_instance_2 (Utilities|Casting|CastToBP_GameInstance (Game|GetGameInstance)))
                (Variables|/Game/SetchOnLegs/Blueprint/Misc/BP_GameInstance.BP_GameInstance_C|SetDeathCount _asbp_game_instance_2 (Variables|Default|GetDeathCount))
                (Game|OpenLevel(byName) "GreasyGroveBossChase")
                (else
                  (bind _returnvalue_3 (Game|GetCurrentLevelName true))
                  (if (Utilities|Enum|Equal(Enum) _returnvalue_3 "GreasyGroveBoss")
                    (Utilities|FlowControl|Delay 2.0)
                    (bind _asbp_game_instance_3 (Utilities|Casting|CastToBP_GameInstance (Game|GetGameInstance)))
                    (Variables|/Game/SetchOnLegs/Blueprint/Misc/BP_GameInstance.BP_GameInstance_C|SetDeathCount _asbp_game_instance_3 (Variables|Default|GetDeathCount))
                    (Game|OpenLevel(byName) "GreasyGroveBoss")
                    (else
                      (bind _returnvalue_4 (Game|GetCurrentLevelName true))
                      (if (Utilities|Enum|Equal(Enum) _returnvalue_4 "TheButcherBoss")
                        (Utilities|FlowControl|Delay 2.0)
                        (bind _asbp_game_instance_4 (Utilities|Casting|CastToBP_GameInstance (Game|GetGameInstance)))
                        (Variables|/Game/SetchOnLegs/Blueprint/Misc/BP_GameInstance.BP_GameInstance_C|SetDeathCount _asbp_game_instance_4 (Variables|Default|GetDeathCount))
                        (Game|OpenLevel(byName) "TheButcherBoss")
                        (else
                          (bind _returnvalue_5 (Game|GetCurrentLevelName true))
                          (if (Utilities|Enum|Equal(Enum) _returnvalue_5 "AWitchesWelcomeBoss")
                            (Utilities|FlowControl|Delay 2.0)
                            (bind _asbp_game_instance_5 (Utilities|Casting|CastToBP_GameInstance (Game|GetGameInstance)))
                            (Variables|/Game/SetchOnLegs/Blueprint/Misc/BP_GameInstance.BP_GameInstance_C|SetDeathCount _asbp_game_instance_5 (Variables|Default|GetDeathCount))
                            (Game|OpenLevel(byName) "AWitchesWelcomeBoss")
                            (else
                              (bind _returnvalue_6 (Game|GetCurrentLevelName true))
                              (if (Utilities|Enum|Equal(Enum) _returnvalue_6 "TheCreatorBoss")
                                (Utilities|FlowControl|Delay 2.0)
                                (bind _asbp_game_instance_6 (Utilities|Casting|CastToBP_GameInstance (Game|GetGameInstance)))
                                (Variables|/Game/SetchOnLegs/Blueprint/Misc/BP_GameInstance.BP_GameInstance_C|SetDeathCount _asbp_game_instance_6 (Variables|Default|GetDeathCount))
                                (Game|OpenLevel(byName) "TheCreatorBoss")
                                (else
                                  (bind _returnvalue_7 (SaveGame|LoadGamefromSlot "Location"))
                                  (bind _asbp_save_info (Utilities|Casting|CastToBP_SaveInfo _returnvalue_7))
                                  (Transformation|SetActorRelativeLocation (Variables|/Game/SetchOnLegs/Blueprint/Misc/BP_SaveInfo.BP_SaveInfo_C|GetcheckLocation _asbp_save_info))
                                  (Variables|Default|SetCurrentHealth 5e+01)
                                  (Input|EnableInput 0)
                                  (Variables|Default|SetState "NewEnumerator0")
                                  (CallFunction|UpdateAnimation))))))))))))))
        (else
          (Variables|Default|SetState "NewEnumerator4")
          (Physics|AddForce (Variables|Character|GetCharacterMovement) (Math|Vector|MakeVector KnockBack 0.0 2.5e+06))
          (Utilities|Time|SetTimerbyFunctionName 0 "Blink" 0.15 true)
          (Utilities|FlowControl|Delay 1.0)
          (Utilities|Time|ClearTimerbyFunctionName 0 "Blink")
          (Development|SetHiddeninGame (Variables|Default|GetSprite) false false))))))

(event Custom|UpdateAnimation
  (bind _sprite (Variables|Default|GetSprite))
  (bind _sprite_2 (Variables|Default|GetSprite))
  ;[1 1 1] Handle Animation
  (switch Utilities|FlowControl|Switch|SwitchonSpikeState (Variables|Default|GetState)
    (:NewEnumerator0
      (Sprite|SetFlipbook (Variables|Default|GetSprite) (select (> (Math|Vector|VectorLength (Transformation|GetVelocity)) 0.0) "/Game/SetchOnLegs/Sprites/Spike/Character/A_SpikeWalking.A_SpikeWalking" "/Game/SetchOnLegs/Sprites/Spike/Character/A_Idle.A_Idle"))
      (goto _label Reset))
    (:NewEnumerator2
      (Sprite|SetFlipbook (Variables|Default|GetSprite) "/Game/SetchOnLegs/Sprites/Spike/Character/A_Jumping.A_Jumping")
      (Utilities|FlowControl|DoOnce false :!label _label
        (:Completed
          (Audio|PlaySound2D "/Game/SetchOnLegs/Audio/Misc/jump.jump" 1.0 1.0 0.0 0 0))))
    (:NewEnumerator3
      (Sprite|SetFlipbook (Variables|Default|GetSprite) "/Game/SetchOnLegs/Sprites/Spike/Character/A_Crouching.A_Crouching"))
    (:NewEnumerator4
      (Sprite|SetFlipbook (Variables|Default|GetSprite) "/Game/SetchOnLegs/Sprites/Spike/Character/A_Hit.A_Hit"))
    (:NewEnumerator5
      (Sprite|SetFlipbook _sprite "/Game/SetchOnLegs/Sprites/Spike/Character/A_Dead.A_Dead")
      (Transformation|SetRelativeScale3D _sprite "0.500000,0.500000,0.500000")
      (Pawn|Components|CharacterMovement|DisableMovement (Variables|Character|GetCharacterMovement)))
    (:NewEnumerator6
      (Sprite|SetFlipbook (Variables|Default|GetSprite) "/Game/SetchOnLegs/Sprites/Spike/Character/A_Fire.A_Fire"))
    (:NewEnumerator7
      (Sprite|SetFlipbook _sprite_2 "/Game/SetchOnLegs/Sprites/Spike/Character/A_Climbing.A_Climbing")
      (if (Math|Float|InRange(Float) (Math|Vector|VectorLength (Transformation|GetVelocity)) -0.1 0.1)
        (Components|Timeline|SetPlayRate _sprite_2 1.0)
        (else
          (Components|Timeline|SetPlayRate _sprite_2 1.0))))))

(event Custom|ClimbingEnd
  ;[1 1 1] Ladder Logic
  (Variables|Default|SetState "NewEnumerator0")
  (CallFunction|UpdateAnimation)
  (Pawn|Components|CharacterMovement|SetMovementMode (Variables|Character|GetCharacterMovement) "MOVE_Walking" 0)
  (Variables|Default|SetCanJump_0 true))

(event EventOnLanded
  (params (Hit :type Hit%20Result%20Structure%20%28by%20ref%29))
  ;[1 1 1] Handle Jump
  (if (Utilities|Enum|Equal(Enum) (Variables|Default|GetState) "NewEnumerator5")
    (Sprite|SetFlipbook (Variables|Default|GetSprite) "/Game/SetchOnLegs/Sprites/Spike/Character/A_Dead.A_Dead")
    (else
      (Variables|Default|SetState "NewEnumerator0"))))

(event EventTick
  (params (DeltaSeconds :type Float%20%28single-precision%29))
  ;[1 1 1] Handle Abilities
  (Utilities|FlowControl|Sequence
    (:then_0
      (if (Variables|Default|GetMegaCannon)
        (Variables|Default|SetBulletScale "2.000000,2.000000,2.000000")))
    (:then_1
      (if (Variables|Default|GetHasFlashlight)
        (Rendering|SetVisibility (Variables|Default|GetFlashlight) true false)))
    (:then_2
      (if (Variables|Default|GetOnDragpad)
        (if (Utilities|Enum|NotEqual(Enum) (Variables|Default|GetState) "NewEnumerator5")
          (Pawn|Input|AddMovementInput "0.750000, 0, 0" 1.0 false))))))

(event EventBeginPlay
  ;[1 1 1] Initialise
  (Utilities|FlowControl|Sequence
    (:then_0
      (Variables|/Script/Engine.PlayerController|SetbShowMouseCursor (Game|GetPlayerController 0) true)
      (Class|ActorComponent|SetIsReplicated (Variables|Default|GetSprite) true))
    (:then_1
      (bind _returnvalue (UserInterface|CreateWidget "/Game/SetchOnLegs/Blueprint/Spike/Widget_HUD.Widget_HUD_C" (Game|GetPlayerController 0)))
      (bind _output_get (Variables|Default|SetHealthBar _returnvalue))
      (UserInterface|Viewport|AddtoViewport _output_get 0))
    (:then_2
      (bind _asbp_game_instance (Utilities|Casting|CastToBP_GameInstance (Game|GetGameInstance)))
      (Utilities|FlowControl|Sequence
        (:then_0
          (Variables|Default|SetCurrentHealth (Variables|/Game/SetchOnLegs/Blueprint/Misc/BP_GameInstance.BP_GameInstance_C|GetHealth _asbp_game_instance)))
        (:then_1
          (Variables|Default|SetMasterBalls (Variables|/Game/SetchOnLegs/Blueprint/Misc/BP_GameInstance.BP_GameInstance_C|GetCurrency _asbp_game_instance)))
        (:then_2
          (Variables|Default|SetDeathCount (Variables|/Game/SetchOnLegs/Blueprint/Misc/BP_GameInstance.BP_GameInstance_C|GetDeathCount _asbp_game_instance)))
        (:then_3
          (Variables|Default|SetChargedShot (Variables|/Game/SetchOnLegs/Blueprint/Misc/BP_GameInstance.BP_GameInstance_C|GetChargedShot _asbp_game_instance)))
        (:then_4
          (Variables|Default|SetHealthLevel (Variables|/Game/SetchOnLegs/Blueprint/Misc/BP_GameInstance.BP_GameInstance_C|GetHealthLevel _asbp_game_instance)))
        (:then_5
          (Variables|Default|Set3Bullet (Variables|/Game/SetchOnLegs/Blueprint/Misc/BP_GameInstance.BP_GameInstance_C|Get3BulletSpread _asbp_game_instance)))
        (:then_6
          (Variables|Default|Set5Bullet (Variables|/Game/SetchOnLegs/Blueprint/Misc/BP_GameInstance.BP_GameInstance_C|Get5BulletSpread _asbp_game_instance)))
        (:then_7
          (Variables|Default|SetMegaCannon (Variables|/Game/SetchOnLegs/Blueprint/Misc/BP_GameInstance.BP_GameInstance_C|GetMegaCannon _asbp_game_instance)))
        (:then_8
          (Variables|Default|SetArmorLevel (Variables|/Game/SetchOnLegs/Blueprint/Misc/BP_GameInstance.BP_GameInstance_C|GetArmorLevel _asbp_game_instance)))
        (:then_9
          (Variables|Default|SetMaxHealth (Variables|/Game/SetchOnLegs/Blueprint/Misc/BP_GameInstance.BP_GameInstance_C|GetMaxHealth _asbp_game_instance)))
        (:then_10
          (Variables|Default|SetCheckpoints (Variables|/Game/SetchOnLegs/Blueprint/Misc/BP_GameInstance.BP_GameInstance_C|GetCheckpoints _asbp_game_instance)))))))

(event Input|ActionEvents|InputActionSpawnCheckpoint
  (params (Key :type Key%20Structure))
  (bind _returnvalue (Transformation|GetActorLocation))
  ;[1 1 1] Spawn Checkpoint
  (:Pressed
    (bind _returnvalue_2 (Game|GetCurrentLevelName true))
    (if (Utilities|Enum|NotEqual(Enum) _returnvalue_2 "HinceInHellBoss")
      (if (Utilities|Enum|NotEqual(Enum) _returnvalue_2 "GreasyGroveChase")
        (if (Utilities|Enum|NotEqual(Enum) _returnvalue_2 "GreasyGroveBoss")
          (if (> (Variables|Default|GetCheckpoints) 0)
            (Game|SpawnActorfromClass "/Game/SetchOnLegs/Blueprint/Misc/BP_Checkpoint.BP_Checkpoint_C" (Math|Transform|MakeTransform (Math|Vector|MakeVector (.x _returnvalue) (.y _returnvalue) (.z _returnvalue)) "0, 0, 0" "1,1,1") "Undefined" 0 0)
            (Variables|Default|SetCheckpoints (- (Variables|Default|GetCheckpoints) 1))))))))

(event Input|ActionEvents|InputActionChargedShoot
  (params (Key :type Key%20Structure))
  (bind _returnvalue (Game|GetPlayerController 0))
  (bind _returnvalue_2 (Game|GetPlayerController 0))
  (bind _returnvalue_3 (Game|GetPlayerController 0))
  (bind _returnvalue_4 (Pawn|GetControlledPawn _returnvalue_3))
  (bind (_locationx _locationy) (Game|Player|GetMousePosition _returnvalue_2))
  (bind _returnvalue_5 (Transformation|GetActorLocation _returnvalue_4))
  (bind _screenlocation (Class|PlayerController|ProjectWorldLocationtoScreen _returnvalue _returnvalue_5 false))
  (bind (_x _y _z) (Math|Vector|BreakVector _returnvalue_5))
  (bind (_x_2 _y_2) (Math|Vector2D|BreakVector2D _screenlocation))
  ;[1 1 1] Handle Charged Shoot
  (:Pressed
    (if (Variables|Default|GetChargedShot)
      (if (== (Variables|Default|GetShots) 25.0)
        (Variables|Default|SetShots 0.0)
        (Audio|PlaySound2D "/Game/SetchOnLegs/Audio/Misc/ChargedShoot.ChargedShoot" 1.0 1.0 0.0 0 0)
        (Variables|Default|SetCanMove false)
        (Variables|Default|SetState "NewEnumerator6")
        (bind _output_get (Variables|Default|SetBulletMouseRotation (Math|Rotator|FindLookatRotation _returnvalue_5 (Math|Vector|MakeVector (+ _x (- _locationx _x_2)) 0.0 (+ _z (- _y_2 _locationy))))))
        (Game|SpawnActorfromClass "/Game/SetchOnLegs/Blueprint/Spike/BP_ChargedBullet.BP_ChargedBullet_C" (Math|Transform|MakeTransform (.location (Transformation|GetWorldTransform (Variables|Default|GetArrow1))) _output_get "1,1,1") "AlwaysSpawn" 0 0)
        (CallFunction|UpdateAnimation)
        (Character|LaunchCharacter (Math|Vector|MakeVector (Math|Conversions|ToFloat(Integer) (* (Variables|Default|GetFacing) 1500)) 0.0 0.0) false false))))
  (:Released
    (Utilities|FlowControl|Delay 0.2)
    (Variables|Default|SetState "NewEnumerator0")
    (Variables|Default|SetCanMove true)
    (CallFunction|UpdateAnimation)))

(event Input|ActionEvents|InputActionShoot
  (params (Key :type Key%20Structure))
  (bind _returnvalue (Game|GetPlayerController 0))
  (bind _returnvalue_2 (Game|GetPlayerController 0))
  (bind _returnvalue_3 (Game|GetPlayerController 0))
  (bind _arrow1 (Variables|Default|GetArrow1))
  (bind _returnvalue_4 (Transformation|GetWorldTransform _arrow1))
  (bind _returnvalue_5 (Pawn|GetControlledPawn _returnvalue_3))
  (bind (_locationx _locationy) (Game|Player|GetMousePosition _returnvalue_2))
  (bind _returnvalue_6 (Transformation|GetActorLocation _returnvalue_5))
  (bind _screenlocation (Class|PlayerController|ProjectWorldLocationtoScreen _returnvalue _returnvalue_6 false))
  (bind (_x _y _z) (Math|Vector|BreakVector _returnvalue_6))
  (bind (_x_2 _y_2) (Math|Vector2D|BreakVector2D _screenlocation))
  ;[1 1 1] Handle Shoot
  (:Pressed
    (Variables|Default|SetCanMove false)
    (Variables|Default|SetState "NewEnumerator6")
    (if (< (Variables|Default|GetShots) 25.0)
      (if (Variables|Default|GetChargedShot)
        (Variables|Default|SetShots (+ (Variables|Default|GetShots) 1.0))))
    (Audio|PlaySound2D "/Game/SetchOnLegs/Audio/Misc/Shoot.Shoot" 1.0 1.0 0.0 0 0)
    (bind _output_get (Variables|Default|SetBulletMouseRotation (Math|Rotator|FindLookatRotation _returnvalue_6 (Math|Vector|MakeVector (+ _x (- _locationx _x_2)) 0.0 (+ _z (- _y_2 _locationy))))))
    (Game|SpawnActorfromClass "/Game/SetchOnLegs/Blueprint/Spike/BP_Bullet.BP_Bullet_C" (Math|Transform|MakeTransform (.location _returnvalue_4) _output_get (Variables|Default|GetBulletScale)) "AlwaysSpawn" 0 0)
    (CallFunction|UpdateAnimation)
    (if (Variables|Default|Get3Bullet)
      (Game|SpawnActorfromClass "/Game/SetchOnLegs/Blueprint/Spike/BP_Bullet.BP_Bullet_C" (Math|Transform|MakeTransform (.location _returnvalue_4) (Math|Rotator|MakeRotator (.roll (Variables|Default|GetBulletMouseRotation)) (+ (.pitch (Variables|Default|GetBulletMouseRotation)) 3.0) (.yaw (Variables|Default|GetBulletMouseRotation))) (Variables|Default|GetBulletScale)) "AlwaysSpawn" 0 0)
      (Game|SpawnActorfromClass "/Game/SetchOnLegs/Blueprint/Spike/BP_Bullet.BP_Bullet_C" (Math|Transform|MakeTransform (.location _returnvalue_4) (Math|Rotator|MakeRotator (.roll (Variables|Default|GetBulletMouseRotation)) (- (.pitch (Variables|Default|GetBulletMouseRotation)) 3.0) (.yaw (Variables|Default|GetBulletMouseRotation))) (Variables|Default|GetBulletScale)) "AlwaysSpawn" 0 0)
      (CallFunction|UpdateAnimation)
      (if (Variables|Default|Get5Bullet)
        (Game|SpawnActorfromClass "/Game/SetchOnLegs/Blueprint/Spike/BP_Bullet.BP_Bullet_C" (Math|Transform|MakeTransform (.location _returnvalue_4) (Math|Rotator|MakeRotator (.roll (Variables|Default|GetBulletMouseRotation)) (+ (.pitch (Variables|Default|GetBulletMouseRotation)) 6.0) (.yaw (Variables|Default|GetBulletMouseRotation))) (Variables|Default|GetBulletScale)) "AlwaysSpawn" 0 0)
        (Game|SpawnActorfromClass "/Game/SetchOnLegs/Blueprint/Spike/BP_Bullet.BP_Bullet_C" (Math|Transform|MakeTransform (.location _returnvalue_4) (Math|Rotator|MakeRotator (.roll (Variables|Default|GetBulletMouseRotation)) (- (.pitch (Variables|Default|GetBulletMouseRotation)) 6.0) (.yaw (Variables|Default|GetBulletMouseRotation))) (Variables|Default|GetBulletScale)) "AlwaysSpawn" 0 0)
        (CallFunction|UpdateAnimation))))
  (:Released
    (Utilities|FlowControl|Delay 0.2)
    (Variables|Default|SetState "NewEnumerator0")
    (Variables|Default|SetCanMove true)
    (CallFunction|UpdateAnimation)))

(event Input|ActionEvents|InputActionPause
  (params (Key :type Key%20Structure))
  ;[1 1 1] Handle Pause Menu
  (:Pressed
    (bind _returnvalue (UserInterface|CreateWidget "/Game/SetchOnLegs/Blueprint/Menus/Widget_PauseMenu.Widget_PauseMenu_C"))
    (UserInterface|Viewport|AddtoViewport _returnvalue 0)
    (Game|SetGamePaused true)))

(event Input|ActionEvents|InputActionJump
  (params (Key :type Key%20Structure))
  ;[1 1 1] Handle Jump
  (:Pressed
    (if (Variables|Default|GetCanClimb)
      (Transformation|AddActorLocalOffset (Math|Vector|MakeVector 0.0 0.0 (* (stale Input|AxisEvents|InputAxisClimb AxisValue) (Variables|Default|GetClimbSpeed))) false false)
      (else
        (Character|Jump)
        (Variables|Default|SetState "NewEnumerator2")
        (Utilities|FlowControl|Delay 0.3)
        (Variables|Default|SetState "NewEnumerator0"))))
  (:Released
    (Character|StopJumping)))

(event Input|AxisEvents|InputAxisClimb
  (params (AxisValue :type Float%20%28single-precision%29))
  ;[1 1 1] Handle Jump
  (if (>= AxisValue 0.1)
    (if (Variables|Default|GetCanClimb)
      (Transformation|AddActorLocalOffset (Math|Vector|MakeVector 0.0 0.0 (* AxisValue (Variables|Default|GetClimbSpeed))) false false)
      (else
        (Character|Jump)
        (Variables|Default|SetState "NewEnumerator2")
        (Utilities|FlowControl|Delay 0.3)
        (Variables|Default|SetState "NewEnumerator0")))))

(event Input|AxisEvents|InputAxisMoveRight
  (params (AxisValue :type Float%20%28single-precision%29))
  ;[1 1 1] Handle movement
  (if (Variables|Default|GetCanMove)
    (if (> AxisValue 0.0)
      (Variables|Default|SetIsMovingRight true)
      (elif (< AxisValue 0.0)
        (Variables|Default|SetIsMovingRight false)))
    (Pawn|Input|AddMovementInput "1.000000, 0, 0" AxisValue false)
    ;[1 1 1] Tick - Updates animation
    (CallFunction|UpdateAnimation)
    (Math|Float|CompareFloat (.X (Math|Vector|BreakVector (Variables|/Script/Engine.MovementComponent|GetVelocity (Pawn|GetMovementComponent)))) AxisValue
      (:>
        (Pawn|SetControlRotation (Pawn|GetController) (Math|Rotator|MakeRotator 0.0 0.0 0.0) :!label _label)
        (Variables|Default|SetFacing -1))
      (:==
        (if (Variables|Default|GetIsMovingRight)
          (goto _label)
          (else
            (Pawn|SetControlRotation (Pawn|GetController) (Math|Rotator|MakeRotator 0.0 0.0 1.8e+02) :!label _label_2)
            (Variables|Default|SetFacing 1))))
      (:<
        (goto _label_2)))))

(event Input|AxisEvents|InputAxisClimb
  (params (AxisValue :type Float%20%28single-precision%29))
  ;[1 1 1] Ladder Logic
  (if (Variables|Default|GetCanClimb)
    (if (not (Math|Float|InRange(Float) AxisValue -0.1 0.1))
      (Variables|Default|SetState "NewEnumerator7")
      (CallFunction|UpdateAnimation)
      (Pawn|Components|CharacterMovement|SetMovementMode (Variables|Character|GetCharacterMovement) "MOVE_Flying" 0)
      (Pawn|Input|AddMovementInput (Math|Vector|MakeVector 0.0 0.0 0.5) AxisValue false)
      (Variables|Default|SetCanJump_0 false))))

(event Input|TouchEvents|InputTouch
  (params (Location :type Vector) (FingerIndex :type ETouchIndex%20Enum))
  ;[1 1 1] Handle Jump
  (:Pressed
    (Character|Jump)
    (Variables|Default|SetState "NewEnumerator2")
    (Utilities|FlowControl|Delay 0.3)
    (Variables|Default|SetState "NewEnumerator0"))
  (:Released
    (Character|StopJumping)))

(fn ConstructionScript)
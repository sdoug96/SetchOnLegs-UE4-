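; BP_SpinBlade is a moving, spinning blade hazard that damages the player character, BP_Spike, on contact.
; A timeline lerps it between its start location and an X/Z offset, with a flag on finish choosing reverse or replay to keep it moving.
; Tick sets its pitch from accumulated time times a rotation rate.
; Sphere begin-overlap passes Damage to BP_Spike's DamageSytsem function.
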(event OnComponentBeginOverlap(Sphere)
  (params (OverlappedComponent :type Primitive%20Component%20Object%20Reference) (OtherActor :type Actor%20Object%20Reference) (OtherComp :type Primitive%20Component%20Object%20Reference) (OtherBodyIndex :type Integer) (bFromSweep :type Boolean) (SweepResult :type Hit%20Result%20Structure%20%28by%20ref%29))
  ;[1 1 1] Player Collision
  (bind _asbp_spike (Utilities|Casting|CastToBP_Spike OtherActor))
  (Default|DamageSytsem _asbp_spike (Variables|Default|GetDamage)))

(event EventBeginPlay
  ;[1 1 1] Movement
  (bind _output_get (Variables|Default|SetinitialLocation (Transformation|GetActorLocation)))
  (Variables|Default|SetendLocation (+ _output_get (Math|Vector|MakeVector (Variables|Default|GetposDiffX) 0.0 (Variables|Default|GetposDiffZ))))
  (bind _newtrack_0 (Timeline|Timeline_0 Play)
    (:Update
      (Transformation|SetActorLocation (Math|Vector|Lerp(Vector) (Variables|Default|GetinitialLocation) (Variables|Default|GetendLocation) _newtrack_0) false false))
    (:Finished
      (if (Variables|Default|GettimeFactor)
        (Variables|Default|SettimeFactor false)
        (Timeline|Timeline_0 ReverseFromEnd)
        (else
          (Variables|Default|SettimeFactor true)
          (Timeline|Timeline_0 PlayFromStart))))))

(event Collision|EventActorBeginOverlap
  (params (OtherActor :type Actor%20Object%20Reference)))

(event EventTick
  (params (DeltaSeconds :type Float%20%28single-precision%29))
  ;[1 1 1] Rotate
  (Variables|Default|Settimer (+ DeltaSeconds (Variables|Default|Gettimer)))
  (Transformation|SetActorRotation (Math|Rotator|MakeRotator 0.0 (* (Variables|Default|Gettimer) (Variables|Default|Getrotation)) 0.0)))

(fn ConstructionScript)
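; BP_EnergyBall is a short-lived energy ball hazard, apparently an attack of BP_TheCreator, that damages BP_Spike.
; On spawn it plays a camera shake at the player's side-view camera and a low rumble, then destroys itself after a brief delay.
; HitSphere overlaps skip one Spike state, otherwise apply damage reduced by armor level.
; A horizontal launch then knocks Spike away from the Creator, based on their relative X positions.
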(event OnComponentBeginOverlap(HitSphere)
  (params (OverlappedComponent :type Primitive%20Component%20Object%20Reference) (OtherActor :type Actor%20Object%20Reference) (OtherComp :type Primitive%20Component%20Object%20Reference) (OtherBodyIndex :type Integer) (bFromSweep :type Boolean) (SweepResult :type Hit%20Result%20Structure%20%28by%20ref%29))
  (bind _damage (Variables|Default|GetDamage))
  ;[1 1 1] Hitsphere
  (bind _asbp_spike (Utilities|Casting|CastToBP_Spike OtherActor))
  (if (Utilities|Enum|NotEqual(Enum) (Variables|/Game/SetchOnLegs/Blueprint/08Spike/BP_Spike.BP_Spike_C|GetState _asbp_spike) "NewEnumerator5")
    (bind _outactors (Actor|GetAllActorsOfClass "/Game/SetchOnLegs/Blueprint/06TheCreator/Regular/BP_TheCreator.BP_TheCreator_C"))
    (if (< (.x (Transformation|GetActorLocation _asbp_spike)) (.x (Transformation|GetActorLocation (Utilities|Array|Get(acopy) _outactors))))
      (Variables|Default|SetKnockback -5e+03)
      (else
        (Variables|Default|SetKnockback 5e+03)))
    (switch int (Variables|/Game/SetchOnLegs/Blueprint/08Spike/BP_Spike.BP_Spike_C|GetArmorLevel _asbp_spike)
      (:0
        (Default|DamageSytsem _asbp_spike _damage 0.0))
      (:1
        (Default|DamageSytsem _asbp_spike (* _damage 0.9) 0.0))
      (:2
        (Default|DamageSytsem _asbp_spike (* _damage 0.8) 0.0))
      (:3
        (Default|DamageSytsem _asbp_spike (* _damage 0.7) 0.0))
      (:4
        (Default|DamageSytsem _asbp_spike (* _damage 0.6) 0.0))
      (:5
        (Default|DamageSytsem _asbp_spike (* _damage 0.5) 0.0)))
    (Character|LaunchCharacter _asbp_spike (Math|Vector|MakeVector (Variables|Default|GetKnockback) 0.0 0.0) false false)))

(event EventBeginPlay
  ;[1 1 1] Initialise
  (bind _asbp_spike (Utilities|Casting|CastToBP_Spike (Game|GetPlayerCharacter 0)))
  (Camera|PlayWorldCameraShake "/Game/SetchOnLegs/Blueprint/06TheCreator/Regular/BP_EnergyBallShake.BP_EnergyBallShake_C" (Transformation|GetWorldLocation (Variables|/Game/SetchOnLegs/Blueprint/08Spike/BP_Spike.BP_Spike_C|GetSideViewCameraComponent _asbp_spike)) 0.0 5e+02)
  (Audio|PlaySound2D "/Game/SetchOnLegs/Audio/06Creator/LowRumble.LowRumble" 1.0 1.0 0.0 0 0)
  (Utilities|FlowControl|Delay 2.7)
  (Actor|DestroyActor))

(fn ConstructionScript)
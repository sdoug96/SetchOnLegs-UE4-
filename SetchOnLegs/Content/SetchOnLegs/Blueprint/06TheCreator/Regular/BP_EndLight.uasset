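; BP_EndLight is a light actor that brightens into a blinding glare and hands over to a white screen fade.
; Tick raises the EndLight intensity by a large fixed step every frame, without delta-time scaling, so the ramp depends on frame rate.
; BeginPlay runs a timed chain: it waits, adds the Widget_FadeToWhite overlay to the viewport, later hides the light, then destroys the actor.
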(event EventBeginPlay
  (Utilities|FlowControl|Delay 3.0)
  (bind _returnvalue (UserInterface|CreateWidget "/Game/SetchOnLegs/Blueprint/06TheCreator/Regular/Widget_FadeToWhite.Widget_FadeToWhite_C"))
  (UserInterface|Viewport|AddtoViewport _returnvalue 0)
  (Utilities|FlowControl|Delay 3.9)
  (Rendering|SetVisibility (Variables|Default|GetEndLight) false false)
  (Utilities|FlowControl|Delay 0.6)
  (Actor|DestroyActor))

(event EventTick
  (params (DeltaSeconds :type Float%20%28single-precision%29))
  (bind _endlight (Variables|Default|GetEndLight))
  (Rendering|Components|Light|SetIntensity _endlight (+ (Variables|/Script/Engine.LightComponentBase|GetIntensity _endlight) 2.5e+05)))

(fn ConstructionScript)
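; BP_FireBomb is a lobbed, spinning projectile tied to the enraged Creator fight that bursts into BP_MiniFireBombs after a short fuse, then destroys itself.
; Tick spins it and polls BP_TheCreatorEnraged's phase flags to raise the mini-bomb count in later phases.
; Overlapping BP_Spike outside one excluded state deals damage reduced by armor level and destroys the bomb.
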(event OnComponentBeginOverlap(HitSphere)
  (params (OverlappedComponent :type Primitive%20Component%20Object%20Reference) (OtherActor :type Actor%20Object%20Reference) (OtherComp :type Primitive%20Component%20Object%20Reference) (OtherBodyIndex :type Integer) (bFromSweep :type Boolean) (SweepResult :type Hit%20Result%20Structure%20%28by%20ref%29))
  ;[1 1 1] Player Collision
  (bind _asbp_spike (Utilities|Casting|CastToBP_Spike OtherActor))
  (if (Utilities|Enum|NotEqual(Enum) (Variables|/Game/SetchOnLegs/Blueprint/Spike/BP_Spike.BP_Spike_C|GetState _asbp_spike) "NewEnumerator5")
    (switch int (Variables|/Game/SetchOnLegs/Blueprint/Spike/BP_Spike.BP_Spike_C|GetArmorLevel _asbp_spike)
      (:0
        (Default|DamageSytsem _asbp_spike (Variables|Default|GetDamage) 0.0))
      (:1
        (Default|DamageSytsem _asbp_spike (* (Variables|Default|GetDamage) 0.9) 0.0))
      (:2
        (Default|DamageSytsem _asbp_spike (* (Variables|Default|GetDamage) 0.8) 0.0))
      (:3
        (Default|DamageSytsem _asbp_spike (* (Variables|Default|GetDamage) 0.7) 0.0))
      (:4
        (Default|DamageSytsem _asbp_spike (* (Variables|Default|GetDamage) 0.6) 0.0))
      (:5
        (Default|DamageSytsem _asbp_spike (* (Variables|Default|GetDamage) 0.5) 0.0)))
    (Actor|DestroyActor)
    (Audio|PlaySound2D "/Game/SetchOnLegs/Audio/Misc/Ouch.Ouch" 1.0 1.0 0.0 0 0)))

(event EventBeginPlay
  ;[1 1 1] Initialise
  (Variables|/Script/Engine.MovementComponent|SetVelocity (Variables|Default|GetProjectileMovement) (Math|Vector|MakeVector -8.5e+02 0.0 7.5e+02))
  (Audio|PlaySound2D "/Game/SetchOnLegs/Audio/Menus/Fire.Fire" 1.0 1.0 0.0 0 0)
  (Utilities|FlowControl|Delay 0.9)
  (Audio|PlaySound2D "/Game/SetchOnLegs/Audio/Creator/CreatorBombExplosion.CreatorBombExplosion" 1.0 1.0 0.0 0 0)
  (for _index (range 0 (Variables|Default|GetBombsToSpawn))
    (Game|SpawnActorfromClass "/Game/SetchOnLegs/Blueprint/06TheCreator/Enraged/BP_MiniFireBomb.BP_MiniFireBomb_C" (Math|Transform|MakeTransform (Transformation|GetActorLocation) "0, 0, 0" "1,1,1") "Undefined" 0 0)
    (Utilities|FlowControl|Delay 0.1)
    (Actor|DestroyActor)))

(event EventTick
  (params (DeltaSeconds :type Float%20%28single-precision%29))
  ;[1 1 1] Rotate
  (Utilities|FlowControl|Sequence
    (:then_0
      (Variables|Default|SetTimer (+ DeltaSeconds (Variables|Default|GetTimer)))
      (Transformation|SetActorRotation (Math|Rotator|MakeRotator 0.0 (* (Variables|Default|GetTimer) (Variables|Default|GetRotation)) 0.0)))
    (:then_1
      (bind _outactors (Actor|GetAllActorsOfClass "/Game/SetchOnLegs/Blueprint/06TheCreator/Enraged/BP_TheCreatorEnraged.BP_TheCreatorEnraged_C"))
      (Utilities|IsValid (Utilities|Array|Get(acopy) _outactors)
        (:Is%20Valid
          (Utilities|FlowControl|Sequence
            (:then_0
              (if (Variables|/Game/SetchOnLegs/Blueprint/06TheCreator/Enraged/BP_TheCreatorEnraged.BP_TheCreatorEnraged_C|GetPhase1 (Utilities|Array|Get(acopy) _outactors))
                (Variables|Default|SetBombsToSpawn 2)))
            (:then_1
              (if (Variables|/Game/SetchOnLegs/Blueprint/06TheCreator/Enraged/BP_TheCreatorEnraged.BP_TheCreatorEnraged_C|GetPhase2 (Utilities|Array|Get(acopy) _outactors))
                (Variables|Default|SetBombsToSpawn 4)))
            (:then_2
              (if (Variables|/Game/SetchOnLegs/Blueprint/06TheCreator/Enraged/BP_TheCreatorEnraged.BP_TheCreatorEnraged_C|GetPhase3 (Utilities|Array|Get(acopy) _outactors))
                (Variables|Default|SetBombsToSpawn 6)))
            (:then_3
              (if (Variables|/Game/SetchOnLegs/Blueprint/06TheCreator/Enraged/BP_TheCreatorEnraged.BP_TheCreatorEnraged_C|GetPhase4 (Utilities|Array|Get(acopy) _outactors))
                (Variables|Default|SetBombsToSpawn 8)))
            (:then_4
              (if (Variables|/Game/SetchOnLegs/Blueprint/06TheCreator/Enraged/BP_TheCreatorEnraged.BP_TheCreatorEnraged_C|GetPhase5 (Utilities|Array|Get(acopy) _outactors))
                (Variables|Default|SetBombsToSpawn 9)))))))))

(fn ConstructionScript)
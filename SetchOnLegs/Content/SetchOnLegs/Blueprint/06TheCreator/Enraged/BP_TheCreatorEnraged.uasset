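; Enraged Creator boss, a flipbook character with an intro roar, boss HUD and death sequence ending in a screen fade.
; Tick derives five phases from health bands, tightening attack counts and delays, and uses Delay to pace attacks.
; Flags rotate attacks through bombs, random-X fireballs and pillars at the player's X, spawned via delayed-loop macros.
; HitSphere overlaps apply the player's normal or charged bullet damage, blinking the sprite until death.
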(event OnComponentBeginOverlap(HitSphere)
  (params (OverlappedComponent :type Primitive%20Component%20Object%20Reference) (OtherActor :type Actor%20Object%20Reference) (OtherComp :type Primitive%20Component%20Object%20Reference) (OtherBodyIndex :type Integer) (bFromSweep :type Boolean) (SweepResult :type Hit%20Result%20Structure%20%28by%20ref%29))
  ;[1 1 1] Bullet Collision
  (bind _asbp_spike (Utilities|Casting|CastToBP_Spike (Game|GetPlayerCharacter 0)))
  (Utilities|FlowControl|Sequence
    (:then_0
      (bind _asbp_bullet (Utilities|Casting|CastToBP_Bullet OtherActor))
      (Actor|DestroyActor _asbp_bullet)
      (if (not (Variables|Default|GetIsDead))
        (CallFunction|DamageSytsem (Variables|/Game/SetchOnLegs/Blueprint/Spike/BP_Spike.BP_Spike_C|GetBulletDamage _asbp_spike))))
    (:then_1
      (bind _asbp_charged_bullet (Utilities|Casting|CastToBP_ChargedBullet OtherActor))
      (Actor|DestroyActor _asbp_charged_bullet)
      (if (not (Variables|Default|GetIsDead))
        (CallFunction|DamageSytsem (Variables|/Game/SetchOnLegs/Blueprint/Spike/BP_Spike.BP_Spike_C|GetChargedShotDamage _asbp_spike))))))

(event Custom|Blink
  (bind _sprite (Variables|Default|GetSprite))
  ;[1 1 1] Damage & Death System
  (Development|SetHiddeninGame _sprite (not (Variables|/Script/Engine.SceneComponent|GetbHiddenInGame _sprite)) false))

(event Custom|Damage%20Sytsem
  (params (DamageIn :type Float%20%28single-precision%29))
  ;[1 1 1] Damage & Death System
  (bind _output_get (Variables|Default|SetCurrentHealth (- (Variables|Default|GetCurrentHealth) DamageIn)))
  (if (<= _output_get 0.0)
    (Variables|Default|SetIsDead true)
    (Sprite|SetFlipbook (Variables|Default|GetSprite) "/Game/SetchOnLegs/Sprites/06TheCreator/Enraged/Character/Death/A_Death.A_Death")
    (Character|LaunchCharacter "1500.000000, 0,350.000000" false false)
    (Utilities|FlowControl|Delay 2.0)
    (Widget|RemovefromParent (Variables|Default|GetWidgetHUD))
    (Utilities|FlowControl|Delay 3.0)
    (bind _returnvalue (UserInterface|CreateWidget "/Game/SetchOnLegs/Blueprint/Misc/Widget_FadeOutFadeIn.Widget_FadeOutFadeIn_C"))
    (UserInterface|Viewport|AddtoViewport _returnvalue 0)
    (Utilities|FlowControl|Delay 4.0)
    (Widget|RemovefromParent _returnvalue)
    (else
      (Utilities|Time|SetTimerbyFunctionName 0 "Blink" 0.05 true)
      (Utilities|FlowControl|Delay 0.2)
      (Utilities|Time|ClearTimerbyFunctionName 0 "Blink")
      (Development|SetHiddeninGame (Variables|Default|GetSprite) false false))))

(event Custom|IntroCutscene
  ;[1 1 1] Intro Logic
  (Variables|Default|SetIntro true)
  (bind _asbp_spike (Utilities|Casting|CastToBP_Spike (Game|GetPlayerCharacter 0)))
  (Sprite|SetFlipbook (Variables|/Script/Paper2D.PaperCharacter|GetSprite _asbp_spike) "/Game/SetchOnLegs/Sprites/Spike/Character/A_Idle.A_Idle")
  (Utilities|FlowControl|Delay 1.5)
  (Audio|PlaySound2D "/Game/SetchOnLegs/Audio/Creator/CreatorRoar.CreatorRoar" 1.0 1.0 0.0 0 0)
  (Camera|PlayWorldCameraShake "/Game/SetchOnLegs/Blueprint/06TheCreator/Enraged/BP_CreatorRoarShake.BP_CreatorRoarShake_C" (Transformation|GetWorldLocation (Variables|/Game/SetchOnLegs/Blueprint/Spike/BP_Spike.BP_Spike_C|GetSideViewCameraComponent _asbp_spike)) 0.0 5e+02)
  (Utilities|FlowControl|Delay 5.0)
  (Variables|/Game/SetchOnLegs/Blueprint/Spike/BP_Spike.BP_Spike_C|SetChargedShotIncrement _asbp_spike true)
  (Audio|SpawnSound2D "/Game/SetchOnLegs/Audio/Creator/CreatorEnraged.CreatorEnraged" 1.0 1.0 0.0 0)
  (bind _returnvalue (UserInterface|CreateWidget "/Game/SetchOnLegs/Blueprint/06TheCreator/Enraged/Widget_TheCreatorEnraged.Widget_TheCreatorEnraged_C"))
  (bind _output_get (Variables|Default|SetWidgetHUD _returnvalue))
  (UserInterface|Viewport|AddtoViewport _output_get 0)
  (Variables|Default|SetIntro false))

(event Custom|Attack
  ;[1 1 1] Attack Logic
  (Utilities|FlowControl|Sequence
    (:then_0
      (if (Variables|Default|GetBombs)
        (Sprite|SetFlipbook (Variables|Default|GetSprite) "/Game/SetchOnLegs/Sprites/06TheCreator/Enraged/Character/BombFire/A_BombFire.A_BombFire")
        (Utilities|ForLoopwithDelay 0 (Variables|Default|GetBombsAmount) :!label _label
          (:LoopBody
            (Game|SpawnActorfromClass "/Game/SetchOnLegs/Blueprint/06TheCreator/Enraged/BP_FireBomb.BP_FireBomb_C" (Transformation|GetWorldTransform (Variables|Default|GetBombSpawn)) "Undefined" 0 0))
          (:Completed
            (Variables|Default|SetBombs false)
            (Variables|Default|SetFireballs true)
            (Sprite|SetFlipbook (Variables|Default|GetSprite) "/Game/SetchOnLegs/Sprites/06TheCreator/Enraged/Character/Idle/A_Idle.A_Idle"))
          (:DelayOut
            (Utilities|FlowControl|Delay (Variables|Default|GetBombDelay))
            (goto _label DelayIn)))))
    (:then_1
      (if (Variables|Default|GetFireballs)
        (Sprite|SetFlipbook (Variables|Default|GetSprite) "/Game/SetchOnLegs/Sprites/06TheCreator/Enraged/Character/Fireballs/A_Fireballs.A_Fireballs")
        (Utilities|ForLoopwithDelay 0 (Variables|Default|GetFireballsAmount) :!label _label_2
          (:LoopBody
            (Game|SpawnActorfromClass "/Game/SetchOnLegs/Blueprint/06TheCreator/Enraged/BP_FireBall.BP_FireBall_C" (Math|Transform|MakeTransform (Math|Vector|MakeVector (Math|Random|RandomFloatinRange 7435.0 9743.0) 0.1 611.0) "0, 0, 0" "1,1,1") "Undefined" 0 0))
          (:Completed
            (Variables|Default|SetFireballs false)
            (Variables|Default|SetFirePillars true)
            (Sprite|SetFlipbook (Variables|Default|GetSprite) "/Game/SetchOnLegs/Sprites/06TheCreator/Enraged/Character/Idle/A_Idle.A_Idle"))
          (:DelayOut
            (Utilities|FlowControl|Delay (Variables|Default|GetFireballsDelay))
            (goto _label_2 DelayIn)))))
    (:then_2
      (if (Variables|Default|GetFirePillars)
        (Sprite|SetFlipbook (Variables|Default|GetSprite) "/Game/SetchOnLegs/Sprites/06TheCreator/Enraged/Character/FirePillars/A_FirePillars.A_FirePillars")
        (Utilities|ForLoopwithDelay 0 (Variables|Default|GetFirePillarsAmount) :!label _label_3
          (:LoopBody
            (bind _asbp_spike (Utilities|Casting|CastToBP_Spike (Game|GetPlayerCharacter 0)))
            (Game|SpawnActorfromClass "/Game/SetchOnLegs/Blueprint/06TheCreator/Enraged/BP_FirePillar.BP_FirePillar_C" (Math|Transform|MakeTransform (Math|Vector|MakeVector (.x (Transformation|GetWorldLocation (Variables|/Script/Paper2D.PaperCharacter|GetSprite _asbp_spike))) 0.0 1.05e+03) "0, 0, 0" "1,1,1") "Undefined" 0 0))
          (:Completed
            (Variables|Default|SetFirePillars false)
            (Variables|Default|SetBombs true)
            (Sprite|SetFlipbook (Variables|Default|GetSprite) "/Game/SetchOnLegs/Sprites/06TheCreator/Enraged/Character/Idle/A_Idle.A_Idle"))
          (:DelayOut
            (Utilities|FlowControl|Delay (Variables|Default|GetFirePillarDelay))
            (goto _label_3 DelayIn)))))))

(event Custom|SetPhase
  ;[1 1 1] Set phase based on current health
  (Utilities|FlowControl|Sequence
    (:then_0
      (if (Math|Float|InRange(Float) (Variables|Default|GetCurrentHealth) 2.1e+07 2.5e+07)
        (Variables|Default|SetPhase1 true)))
    (:then_1
      (if (Math|Float|InRange(Float) (Variables|Default|GetCurrentHealth) 1.6e+07 2e+07)
        (Variables|Default|SetPhase2 true)
        (Variables|Default|SetPhase1 false)))
    (:then_2
      (if (Math|Float|InRange(Float) (Variables|Default|GetCurrentHealth) 1.1e+07 1.5e+07)
        (Variables|Default|SetPhase3 true)
        (Variables|Default|SetPhase2 false)))
    (:then_3
      (if (Math|Float|InRange(Float) (Variables|Default|GetCurrentHealth) 6e+06 1e+07)
        (Variables|Default|SetPhase4 true)
        (Variables|Default|SetPhase3 false)))
    (:then_4
      (if (Math|Float|InRange(Float) (Variables|Default|GetCurrentHealth) 1.0 5e+06)
        (Variables|Default|SetPhase5 true)
        (Variables|Default|SetPhase4 false)))))

(event Custom|SetAttacks
  ;[1 1 1] Set Attacks
  (Utilities|FlowControl|Sequence
    (:then_0
      (if (Variables|Default|GetPhase1)
        (Variables|Default|SetFirePillarsAmount 2)
        (Variables|Default|SetFirePillarDelay 3.0)
        (Variables|Default|SetFireballsAmount 9)
        (Variables|Default|SetFireballsDelay 0.9)
        (Variables|Default|SetBombsAmount 1)
        (Variables|Default|SetBombDelay 4.0)
        (Variables|Default|SetAttackDelay 1e+01)))
    (:then_1
      (if (Variables|Default|GetPhase2)
        (Variables|Default|SetFirePillarsAmount 3)
        (Variables|Default|SetFirePillarDelay 1.5)
        (Variables|Default|SetFireballsAmount 12)
        (Variables|Default|SetFireballsDelay 0.4)
        (Variables|Default|SetBombsAmount 2)
        (Variables|Default|SetBombDelay 2.0)
        (Variables|Default|SetAttackDelay 7.0)))
    (:then_2
      (if (Variables|Default|GetPhase3)
        (Variables|Default|SetFirePillarsAmount 4)
        (Variables|Default|SetFirePillarDelay 1.2)
        (Variables|Default|SetFireballsAmount 14)
        (Variables|Default|SetFireballsDelay 0.3)
        (Variables|Default|SetBombsAmount 3)
        (Variables|Default|SetBombDelay 1.5)
        (Variables|Default|SetAttackDelay 7.0)))
    (:then_3
      (if (Variables|Default|GetPhase4)
        (Variables|Default|SetFirePillarsAmount 5)
        (Variables|Default|SetFirePillarDelay 1.0)
        (Variables|Default|SetFireballsAmount 17)
        (Variables|Default|SetFireballsDelay 0.25)
        (Variables|Default|SetBombsAmount 4)
        (Variables|Default|SetBombDelay 1.2)
        (Variables|Default|SetAttackDelay 7.0)))
    (:then_4
      (if (Variables|Default|GetPhase5)
        (Variables|Default|SetFirePillarsAmount 6)
        (Variables|Default|SetFirePillarDelay 0.6)
        (Variables|Default|SetFireballsAmount 19)
        (Variables|Default|SetFireballsDelay 0.2)
        (Variables|Default|SetBombsAmount 4)
        (Variables|Default|SetBombDelay 0.8)
        (Variables|Default|SetAttackDelay 5.0)))))

(event EventBeginPlay
  ;[1 1 1] Initialise
  (Utilities|FlowControl|Sequence
    (:then_0
      (CallFunction|IntroCutscene)
      (Variables|Default|SetPhase1 true))
    (:then_1
      (Sprite|SetFlipbook (Variables|Default|GetSprite) "/Game/SetchOnLegs/Sprites/06TheCreator/Enraged/Character/Spawn/A_Spawn.A_Spawn")
      (Audio|PlaySound2D "/Game/SetchOnLegs/Audio/Creator/CreatorSpawn.CreatorSpawn" 1.0 1.0 0.0 0 0)
      (Utilities|FlowControl|Delay 0.5)
      (Sprite|SetFlipbook (Variables|Default|GetSprite) "/Game/SetchOnLegs/Sprites/06TheCreator/Enraged/Character/Idle/A_Idle.A_Idle")
      (Utilities|FlowControl|Delay 1.0)
      (Sprite|SetFlipbook (Variables|Default|GetSprite) "/Game/SetchOnLegs/Sprites/06TheCreator/Enraged/Character/Roar/A_Roar.A_Roar")
      (Utilities|FlowControl|Delay 5.0)
      (Sprite|SetFlipbook (Variables|Default|GetSprite) "/Game/SetchOnLegs/Sprites/06TheCreator/Enraged/Character/Idle/A_Idle.A_Idle"))))

(event EventTick
  (params (DeltaSeconds :type Float%20%28single-precision%29))
  ;[1 1 1] Attack every attack delay
  (Utilities|FlowControl|Sequence
    (:then_0
      (CallFunction|SetPhase)
      (CallFunction|SetAttacks))
    (:then_1
      (if (not (Variables|Default|GetIsDead))
        (if (not (Variables|Default|GetIntro))
          (Utilities|FlowControl|Delay (Variables|Default|GetAttackDelay))
          (CallFunction|Attack))))))

(fn ConstructionScript)
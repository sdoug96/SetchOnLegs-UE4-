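; BP_FFEPickup is a collectible that sets the FFE flag on the player's BP_Spike character.
; When a BP_Spike overlaps its box and is not in one specific state, the pickup destroys itself, plays a 2D collectible sound and sets FFE on player 0's BP_Spike.
; The construction script assigns its Paper2D sprite.
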(event OnComponentBeginOverlap(Box)
  (params (OverlappedComponent :type Primitive%20Component%20Object%20Reference) (OtherActor :type Actor%20Object%20Reference) (OtherComp :type Primitive%20Component%20Object%20Reference) (OtherBodyIndex :type Integer) (bFromSweep :type Boolean) (SweepResult :type Hit%20Result%20Structure%20%28by%20ref%29))
  ;[1 1 1] When hit
  (bind _asbp_spike (Utilities|Casting|CastToBP_Spike OtherActor))
  (if (Utilities|Enum|NotEqual(Enum) (Variables|/Game/SetchOnLegs/Blueprint/08Spike/BP_Spike.BP_Spike_C|GetState _asbp_spike) "NewEnumerator5")
    (Actor|DestroyActor)
    (Audio|PlaySound2D "/Game/SetchOnLegs/Audio/07Misc/Collectible.Collectible" 1.0 1.0 0.0 0 0)
    (bind _asbp_spike_2 (Utilities|Casting|CastToBP_Spike (Game|GetPlayerCharacter 0)))
    (Variables|/Game/SetchOnLegs/Blueprint/08Spike/BP_Spike.BP_Spike_C|SetFFE _asbp_spike_2 true)))

(fn ConstructionScript
  (Rendering|Components|Sprite|SetSprite (Variables|Default|GetPaperSprite) (Variables|Default|GetNewPaperSprite)))
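; Thunder disc projectile for The Creator's attacks that bursts into a ring of mini discs.
; On spawn it plays a spark sound and moves along X at a configurable velocity.
; After a short delay it spawns the mini discs at its spawn point, stepping pitch by an equal share of a full circle for each.
; It then replays the spark and destroys itself.
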(event EventBeginPlay
  (bind _spawnpoint (Variables|Default|GetSpawnPoint))
  (bind _returnvalue (Transformation|GetWorldTransform _spawnpoint))
  ;[1 1 1] Initialise
  (Audio|PlaySound2D "/Game/SetchOnLegs/Audio/06Creator/Spark.Spark" 1.0 1.0 0.0 0 0)
  (Variables|/Script/Engine.MovementComponent|SetVelocity (Variables|Default|GetProjectileMovement) (Math|Vector|MakeVector (Variables|Default|GetXVelocity) 0.0 0.0))
  (Utilities|FlowControl|Delay 0.5)
  (for _index (range 0 (- (Variables|Default|GetMiniDiscs) 1))
    (Game|SpawnActorfromClass "/Game/SetchOnLegs/Blueprint/06TheCreator/Attacks/BP_MiniThunderDisc.BP_MiniThunderDisc_C" (Math|Transform|MakeTransform (.location _returnvalue) (Math|Rotator|MakeRotator (.roll (.rotation _returnvalue)) (+ (.pitch (.rotation _returnvalue)) (Variables|Default|GetRotationIncrement)) (.yaw (.rotation _returnvalue))) (.scale _returnvalue)) "Undefined" 0 0)
    (Variables|Default|SetRotationIncrement (+ (Variables|Default|GetRotationIncrement) (Math|Conversions|ToFloat(Integer) (/ 360 (Variables|Default|GetMiniDiscs))))))
  (Audio|PlaySound2D "/Game/SetchOnLegs/Audio/06Creator/Spark.Spark" 1.0 1.0 0.0 0 0)
  (Actor|DestroyActor))

(fn ConstructionScript)
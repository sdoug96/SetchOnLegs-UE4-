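; BP_CutsceneThunder is a one-shot cutscene actor that plays a lightning strike when spawned and then removes itself.
; After a short delay it flashes its point light on, plays 2D thunder and triggers a world camera shake at the side-view camera of the BP_Spike player.
; It then hides the light and destroys itself; if the player is not BP_Spike, the sequence stops with the light left on.
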(event EventBeginPlay
  ;[1 1 1] Initialise
  (Utilities|FlowControl|Delay 0.4)
  (Rendering|SetVisibility (Variables|Default|GetPointLight) true false)
  (Audio|PlaySound2D "/Game/SetchOnLegs/Audio/06Creator/Thunder.Thunder" 1.0 1.0 0.0 0 0)
  (bind _asbp_spike (Utilities|Casting|CastToBP_Spike (Game|GetPlayerCharacter 0)))
  (Camera|PlayWorldCameraShake "/Game/SetchOnLegs/Blueprint/06TheCreator/Attacks/BP_ThunderShake.BP_ThunderShake_C" (Transformation|GetWorldLocation (Variables|/Game/SetchOnLegs/Blueprint/08Spike/BP_Spike.BP_Spike_C|GetSideViewCameraComponent _asbp_spike)) 0.0 5e+02)
  (Utilities|FlowControl|Delay 0.1)
  (Rendering|SetVisibility (Variables|Default|GetPointLight) false false)
  (Utilities|FlowControl|Delay 0.2)
  (Actor|DestroyActor))

(fn ConstructionScript)
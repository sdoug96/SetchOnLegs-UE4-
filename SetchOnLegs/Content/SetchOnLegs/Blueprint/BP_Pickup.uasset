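; BP_Pickup is a sprite-based collectible that adds to the MasterBalls count of a BP_Spike actor on touch.
; When a BP_Spike overlaps its Box, the pickup destroys itself, plays PickupSound in 2D and increases that actor's MasterBalls by Value.
; The construction script applies NewPaperSprite to the PaperSprite component, so the look comes from a variable.
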(event OnComponentBeginOverlap(Box)
  (params (OverlappedComponent :type Primitive%20Component%20Object%20Reference) (OtherActor :type Actor%20Object%20Reference) (OtherComp :type Primitive%20Component%20Object%20Reference) (OtherBodyIndex :type Integer) (bFromSweep :type Boolean) (SweepResult :type Hit%20Result%20Structure%20%28by%20ref%29))
  (bind _asbp_spike (Utilities|Casting|CastToBP_Spike OtherActor))
  (Actor|DestroyActor)
  (Audio|PlaySound2D (Variables|Default|GetPickupSound) 1.0 1.0 0.0 0 0)
  (Variables|/Game/SetchOnLegs/Blueprint/Spike/BP_Spike.BP_Spike_C|SetMasterBalls _asbp_spike (+ (Variables|/Game/SetchOnLegs/Blueprint/Spike/BP_Spike.BP_Spike_C|GetMasterBalls _asbp_spike) (Variables|Default|GetValue))))

(fn ConstructionScript
  (Rendering|Components|Sprite|SetSprite (Variables|Default|GetPaperSprite) (Variables|Default|GetNewPaperSprite)))
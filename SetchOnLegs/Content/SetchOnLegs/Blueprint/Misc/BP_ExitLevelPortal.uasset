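; Level exit portal that sends the BP_Spike character to a configurable next level when it overlaps the portal's box.
; On overlap it copies the character's progress, such as health, currency, deaths, upgrades and checkpoints, into BP_GameInstance so it survives the level change.
; It then plays a portal sound and opens the LevelToOpen level by name after a one-second delay.
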(event OnComponentBeginOverlap(Box)
  (params (OverlappedComponent :type Primitive%20Component%20Object%20Reference) (OtherActor :type Actor%20Object%20Reference) (OtherComp :type Primitive%20Component%20Object%20Reference) (OtherBodyIndex :type Integer) (bFromSweep :type Boolean) (SweepResult :type Hit%20Result%20Structure%20%28by%20ref%29))
  ;[1 1 1] Exit Level Logic
  (bind _asbp_spike (Utilities|Casting|CastToBP_Spike OtherActor))
  (Utilities|FlowControl|Sequence
    (:then_0
      (bind _asbp_game_instance (Utilities|Casting|CastToBP_GameInstance (Game|GetGameInstance)))
      (Utilities|FlowControl|Sequence
        (:then_0
          (Variables|/Game/SetchOnLegs/Blueprint/Misc/BP_GameInstance.BP_GameInstance_C|SetHealth _asbp_game_instance (Variables|/Game/SetchOnLegs/Blueprint/Spike/BP_Spike.BP_Spike_C|GetCurrentHealth _asbp_spike)))
        (:then_1
          (Variables|/Game/SetchOnLegs/Blueprint/Misc/BP_GameInstance.BP_GameInstance_C|SetCurrency _asbp_game_instance (Variables|/Game/SetchOnLegs/Blueprint/Spike/BP_Spike.BP_Spike_C|GetMasterBalls _asbp_spike)))
        (:then_2
          (Variables|/Game/SetchOnLegs/Blueprint/Misc/BP_GameInstance.BP_GameInstance_C|SetDeathCount _asbp_game_instance (Variables|/Game/SetchOnLegs/Blueprint/Spike/BP_Spike.BP_Spike_C|GetDeathCount _asbp_spike)))
        (:then_3
          (Variables|/Game/SetchOnLegs/Blueprint/Misc/BP_GameInstance.BP_GameInstance_C|SetChargedShot _asbp_game_instance (Variables|/Game/SetchOnLegs/Blueprint/Spike/BP_Spike.BP_Spike_C|GetChargedShot _asbp_spike)))
        (:then_4
          (Variables|/Game/SetchOnLegs/Blueprint/Misc/BP_GameInstance.BP_GameInstance_C|Set3BulletSpread _asbp_game_instance (Variables|/Game/SetchOnLegs/Blueprint/Spike/BP_Spike.BP_Spike_C|Get3Bullet _asbp_spike)))
        (:then_5
          (Variables|/Game/SetchOnLegs/Blueprint/Misc/BP_GameInstance.BP_GameInstance_C|Set5BulletSpread _asbp_game_instance (Variables|/Game/SetchOnLegs/Blueprint/Spike/BP_Spike.BP_Spike_C|Get5Bullet _asbp_spike)))
        (:then_6
          (Variables|/Game/SetchOnLegs/Blueprint/Misc/BP_GameInstance.BP_GameInstance_C|SetMaxHealth _asbp_game_instance (Variables|/Game/SetchOnLegs/Blueprint/Spike/BP_Spike.BP_Spike_C|GetMaxHealth _asbp_spike)))
        (:then_7
          (Variables|/Game/SetchOnLegs/Blueprint/Misc/BP_GameInstance.BP_GameInstance_C|SetHealthLevel _asbp_game_instance (Variables|/Game/SetchOnLegs/Blueprint/Spike/BP_Spike.BP_Spike_C|GetHealthLevel _asbp_spike)))
        (:then_8
          (Variables|/Game/SetchOnLegs/Blueprint/Misc/BP_GameInstance.BP_GameInstance_C|SetCheckpoints _asbp_game_instance (Variables|/Game/SetchOnLegs/Blueprint/Spike/BP_Spike.BP_Spike_C|GetCheckpoints _asbp_spike)))
        (:then_9
          (Variables|/Game/SetchOnLegs/Blueprint/Misc/BP_GameInstance.BP_GameInstance_C|SetArmorLevel _asbp_game_instance (Variables|/Game/SetchOnLegs/Blueprint/Spike/BP_Spike.BP_Spike_C|GetArmorLevel _asbp_spike)))))
    (:then_1
      (Audio|PlaySound2D "/Game/SetchOnLegs/Audio/Misc/portal.Portal" 1.0 1.0 0.0 0 0)
      (Utilities|FlowControl|Delay 1.0)
      (Game|OpenLevel(byName) (Variables|Default|GetLevelToOpen)))))

(fn ConstructionScript)
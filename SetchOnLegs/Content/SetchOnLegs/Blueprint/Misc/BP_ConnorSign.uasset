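; BP_ConnorSign is a sign with a Paper2D sprite that can face one of four directions.
; On BeginPlay it checks the Left, Up and Down flags in that priority order and sets the sprite's relative rotation in quarter-turn steps, keeping zero rotation when none is set.
; The construction script is empty, so the chosen direction is applied only when play begins.
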(event EventBeginPlay
  (if (Variables|Default|GetLeft)
    (Transformation|SetRelativeRotation (Variables|Default|GetPaperSprite1) "180.000000, 0,0.000000" false false)
    (elif (Variables|Default|GetUp)
      (Transformation|SetRelativeRotation (Variables|Default|GetPaperSprite1) "90.000000, 0,0.000000" false false)
      (elif (Variables|Default|GetDown)
        (Transformation|SetRelativeRotation (Variables|Default|GetPaperSprite1) "270.000000, 0,0.000000" false false)
        (else
          (Transformation|SetRelativeRotation (Variables|Default|GetPaperSprite1) "0.000000, 0,0.000000" false false))))))

(fn ConstructionScript)
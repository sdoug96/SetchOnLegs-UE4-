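; BP_Ladder is a climbable 2D sprite ladder for the BP_Spike character.
; The construction script stacks collision-free Paper sprite rungs at RungOffset intervals over the height between LadderBottom and LadderTop.
; It also scales and raises a Box trigger based on that height.
; Overlapping the Box sets CanClimb on BP_Spike, and leaving it clears the flag and calls ClimbingEnd.
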(event OnComponentBeginOverlap(Box)
  (params (OverlappedComponent :type Primitive%20Component%20Object%20Reference) (OtherActor :type Actor%20Object%20Reference) (OtherComp :type Primitive%20Component%20Object%20Reference) (OtherBodyIndex :type Integer) (bFromSweep :type Boolean) (SweepResult :type Hit%20Result%20Structure%20%28by%20ref%29))
  (bind _asbp_spike (Utilities|Casting|CastToBP_Spike OtherActor))
  (Variables|/Game/SetchOnLegs/Blueprint/Spike/BP_Spike.BP_Spike_C|SetCanClimb _asbp_spike true))

(event OnComponentEndOverlap(Box)
  (params (OverlappedComponent :type Primitive%20Component%20Object%20Reference) (OtherActor :type Actor%20Object%20Reference) (OtherComp :type Primitive%20Component%20Object%20Reference) (OtherBodyIndex :type Integer))
  (bind _asbp_spike (Utilities|Casting|CastToBP_Spike OtherActor))
  (Variables|/Game/SetchOnLegs/Blueprint/Spike/BP_Spike.BP_Spike_C|SetCanClimb _asbp_spike false)
  (Default|ClimbingEnd _asbp_spike))

(fn ConstructionScript
  (bind _ladderbottom (Variables|Default|GetLadderBottom))
  (bind _laddertop (Variables|Default|GetLadderTop))
  (bind _rungoffset (Variables|Default|GetRungOffset))
  (bind _returnvalue (- _laddertop _ladderbottom))
  (bind _returnvalue_2 (/ (.z _returnvalue) 2.0))
  (for _index (range 0 (Math|Float|Truncate (/ (.z _returnvalue) _rungoffset)))
    (bind _returnvalue_3 (AddComponent|AddPaperSpriteComponent false (Math|Transform|MakeTransform (Math|Vector|MakeVector 0.0 0.0 (* _index _rungoffset)) "0, 0, 0" "1,1,1")))
    (Rendering|Components|Sprite|SetSprite _returnvalue_3 (Variables|Default|GetLadderSprite))
    (Collision|SetCollisionEnabled _returnvalue_3 "NoCollision"))
  (Transformation|SetRelativeScale3D (Variables|Default|GetBox) (Math|Vector|MakeVector 1.0 1.0 _returnvalue_2))
  (Transformation|AddRelativeLocation (Variables|Default|GetBox) (Math|Vector|MakeVector 0.0 0.0 _returnvalue_2) false false))
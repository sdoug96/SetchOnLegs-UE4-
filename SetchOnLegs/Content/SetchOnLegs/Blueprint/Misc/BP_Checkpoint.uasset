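; BP_Checkpoint is a checkpoint trigger actor that saves the player's location when a player-tagged actor overlaps it.
; Each overlap creates a new BP_SaveInfo, stores the BP_Spike character's position and writes the "Location" slot, identically on both Checkpoint branches.
; A flag limits the checkpoint sound to one play.
; The construction script sizes the hit box and picks the got or not-got sprite from Checkpoint, with no runtime sprite change.
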(event Collision|EventActorBeginOverlap
  (params (OtherActor :type Actor%20Object%20Reference))
  (if (Actor|ActorHasTag OtherActor "PlayerTag")
    (bind _returnvalue (SaveGame|CreateSaveGameObject "/Game/SetchOnLegs/Blueprint/Misc/BP_SaveInfo.BP_SaveInfo_C"))
    (bind _asbp_save_info (Utilities|Casting|CastToBP_SaveInfo _returnvalue))
    (Variables|Default|SetSaveInfo _asbp_save_info)
    (bind _asbp_spike (Utilities|Casting|CastToBP_Spike (Game|GetPlayerCharacter 0)))
    (Variables|Default|SetCharacterInfo _asbp_spike)
    (if (Variables|Default|GetCheckpoint)
      (Variables|/Game/SetchOnLegs/Blueprint/Misc/BP_SaveInfo.BP_SaveInfo_C|SetcheckLocation (Variables|Default|GetSaveInfo) (Transformation|GetActorLocation (Variables|Default|GetCharacterInfo)))
      (SaveGame|SaveGametoSlot (Variables|Default|GetSaveInfo) "Location")
      (else
        (Variables|/Game/SetchOnLegs/Blueprint/Misc/BP_SaveInfo.BP_SaveInfo_C|SetcheckLocation (Variables|Default|GetSaveInfo) (Transformation|GetActorLocation (Variables|Default|GetCharacterInfo)))
        (SaveGame|SaveGametoSlot (Variables|Default|GetSaveInfo) "Location")))
    (if (Variables|Default|GetPlayCheckpointMusic)
      (Audio|PlaySound2D "/Game/SetchOnLegs/Audio/Checkpoint.Checkpoint" 1.0 1.0 0.0 0 0)
      (Variables|Default|SetPlayCheckpointMusic false))))

(fn ConstructionScript
  (Components|Box|SetBoxExtent (Variables|Default|GetBox) (Variables|Default|GetchangeHitBox) true)
  (if (Variables|Default|GetCheckpoint)
    (Rendering|Components|Sprite|SetSprite (Variables|Default|GetNotGot) "/Game/SetchOnLegs/Sprites/Map/CheckpointNot.CheckpointNot")
    (else
      (Rendering|Components|Sprite|SetSprite (Variables|Default|GetNotGot) "/Game/SetchOnLegs/Sprites/Map/CheckpointGot.CheckpointGot"))))
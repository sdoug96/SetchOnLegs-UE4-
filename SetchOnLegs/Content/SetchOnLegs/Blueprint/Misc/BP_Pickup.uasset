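; BP_Pickup is a collectible item that adds its Value to the player's MasterBalls when BP_Spike overlaps its Box, unless Spike shows the dead flipbook.
; On pickup it destroys itself, plays a sound and also adds Value to the total in BP_GameInstance.
; Pickups flagged IsCollectible set the GameInstance's collectible flag, handled only for the HinceInHell level.
; The construction script applies a configurable sprite.
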(event OnComponentBeginOverlap(Box)
  (params (OverlappedComponent :type Primitive%20Component%20Object%20Reference) (OtherActor :type Actor%20Object%20Reference) (OtherComp :type Primitive%20Component%20Object%20Reference) (OtherBodyIndex :type Integer) (bFromSweep :type Boolean) (SweepResult :type Hit%20Result%20Structure%20%28by%20ref%29))
  (bind _asbp_spike (Utilities|Casting|CastToBP_Spike OtherActor))
  (if (!= (Class|PaperFlipbookComponent|GetFlipbook (Variables|/Script/Paper2D.PaperCharacter|GetSprite _asbp_spike)) "/Game/SetchOnLegs/Sprites/Spike/Character/A_Dead.A_Dead")
    (Actor|DestroyActor)
    (Audio|PlaySound2D (Variables|Default|GetPickupSound) 1.0 1.0 0.0 0 0)
    (Variables|/Game/SetchOnLegs/Blueprint/Spike/BP_Spike.BP_Spike_C|SetMasterBalls _asbp_spike (+ (Variables|/Game/SetchOnLegs/Blueprint/Spike/BP_Spike.BP_Spike_C|GetMasterBalls _asbp_spike) (Variables|Default|GetValue)))
    (bind _asbp_game_instance (Utilities|Casting|CastToBP_GameInstance (Game|GetGameInstance)))
    (Variables|/Game/SetchOnLegs/Blueprint/Misc/BP_GameInstance.BP_GameInstance_C|SetTotalMasterBalls _asbp_game_instance (+ (Variables|/Game/SetchOnLegs/Blueprint/Misc/BP_GameInstance.BP_GameInstance_C|GetTotalMasterBalls _asbp_game_instance) (Variables|Default|GetValue)))
    (if (Variables|Default|GetIsCollectible)
      (bind _returnvalue (Game|GetCurrentLevelName true))
      (if (Utilities|Enum|Equal(Enum) _returnvalue "HinceInHell")
        (bind _asbp_game_instance_2 (Utilities|Casting|CastToBP_GameInstance (Game|GetGameInstance)))
        (Variables|/Game/SetchOnLegs/Blueprint/Misc/BP_GameInstance.BP_GameInstance_C|SetHinceInHellCollectible _asbp_game_instance_2 true)))))

(fn ConstructionScript
  (Rendering|Components|Sprite|SetSprite (Variables|Default|GetPaperSprite) (Variables|Default|GetNewPaperSprite)))
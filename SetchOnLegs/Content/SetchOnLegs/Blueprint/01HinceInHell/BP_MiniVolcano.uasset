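; BP_MiniVolcano is a hazard that shoots fireballs while a BP_Spike actor is inside its ActiveTrigger volume.
; Entering the trigger fires at once and starts a looping Fire timer spaced by SpawnDelay, and leaving clears that timer.
; Each shot spawns a scaled-down BP_Fireball at the Arrow component's location and rotation and plays a 2D fire sound.
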(event OnComponentBeginOverlap(ActiveTrigger)
  (params (OverlappedComponent :type Primitive%20Component%20Object%20Reference) (OtherActor :type Actor%20Object%20Reference) (OtherComp :type Primitive%20Component%20Object%20Reference) (OtherBodyIndex :type Integer) (bFromSweep :type Boolean) (SweepResult :type Hit%20Result%20Structure%20%28by%20ref%29))
  ;[1 1 1] Set active an inactive
  (Utilities|Casting|CastToBP_Spike OtherActor)
  (CallFunction|Fire)
  (Utilities|Time|SetTimerbyFunctionName 0 "Fire" (Variables|Default|GetSpawnDelay) true))

(event OnComponentEndOverlap(ActiveTrigger)
  (params (OverlappedComponent :type Primitive%20Component%20Object%20Reference) (OtherActor :type Actor%20Object%20Reference) (OtherComp :type Primitive%20Component%20Object%20Reference) (OtherBodyIndex :type Integer))
  ;[1 1 1] Set active an inactive
  (Utilities|Casting|CastToBP_Spike OtherActor)
  (Utilities|Time|ClearTimerbyFunctionName 0 "Fire"))

(event Custom|Fire
  (bind _arrow (Variables|Default|GetArrow))
  (bind _returnvalue (Transformation|GetWorldTransform _arrow))
  ;[1 1 1] Spawn fireball every delay if active
  (Game|SpawnActorfromClass "/Game/SetchOnLegs/Blueprint/01HinceInHell/BP_Fireball.BP_Fireball_C" (Math|Transform|MakeTransform (.location _returnvalue) (.rotation _returnvalue) "0.050000,0.050000,0.050000") "Undefined" 0 1e+03 0)
  (Audio|PlaySound2D "/Game/SetchOnLegs/Audio/00Menus/Fire.Fire" 1.0 1.0 0.0 0 0))

(fn ConstructionScript)
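; BP_Chest is a shootable chest that opens and releases pickups when its health runs out.
; It starts with random health within a range, and bullets hitting its HitBox are destroyed and deal the BP_Spike player's bullet damage.
; Tick watches health and, once depleted, swaps to the open sprite a single time.
; A delayed loop macro then spawns BP_Pickup actors one after another at PickupSpawn, with sounds.
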(event OnComponentBeginOverlap(HitBox)
  (params (OverlappedComponent :type Primitive%20Component%20Object%20Reference) (OtherActor :type Actor%20Object%20Reference) (OtherComp :type Primitive%20Component%20Object%20Reference) (OtherBodyIndex :type Integer) (bFromSweep :type Boolean) (SweepResult :type Hit%20Result%20Structure%20%28by%20ref%29))
  (bind _asbp_bullet (Utilities|Casting|CastToBP_Bullet OtherActor))
  (Actor|DestroyActor _asbp_bullet)
  (bind _asbp_spike (Utilities|Casting|CastToBP_Spike (Game|GetPlayerCharacter 0)))
  (Variables|Default|SetCurrentHealth (- (Variables|Default|GetCurrentHealth) (Variables|/Game/SetchOnLegs/Blueprint/08Spike/BP_Spike.BP_Spike_C|GetBulletDamage _asbp_spike)))
  (Audio|PlaySound2D "/Game/SetchOnLegs/Audio/07Misc/ChestHit.ChestHit" 1.0 1.0 0.0 0 0))

(event Custom|SpawnPickups
  (Utilities|ForLoopwithDelay 0 (- (Variables|Default|GetValue) 1) :!label _label
    (:Loop%20Body
      (Game|SpawnActorfromClass "/Game/SetchOnLegs/Blueprint/07Misc/BP_Pickup.BP_Pickup_C" (Math|Transform|MakeTransform (Transformation|GetWorldLocation (Variables|Default|GetPickupSpawn)) "0, 0, 0" "1,1,1") "Undefined" 0 0)
      (Audio|PlaySound2D "/Game/SetchOnLegs/Audio/07Misc/Pickup.Pickup" 1.0 1.0 0.0 0 0))
    (:Delay%20Out
      (Utilities|FlowControl|Delay (Variables|Default|GetSpawnDelay))
      (goto _label Delay%20In))))

(event EventBeginPlay
  (Variables|Default|SetCurrentHealth (Math|Random|RandomFloatinRange (Variables|Default|GetHealthMin) (Variables|Default|GetHealthMax))))

(event EventTick
  (params (DeltaSeconds :type Float%20%28single-precision%29))
  (if (<= (Variables|Default|GetCurrentHealth) 0.0)
    (Utilities|FlowControl|DoOnce false
      (:Completed
        (Rendering|Components|Sprite|SetSprite (Variables|Default|GetChest) "/Game/SetchOnLegs/Sprites/Misc/SilverChestOpen.SilverChestOpen")
        (Audio|PlaySound2D "/Game/SetchOnLegs/Audio/07Misc/ChestOpen.ChestOpen" 1.0 1.0 0.0 0 0)
        (CallFunction|SpawnPickups)))))

(fn ConstructionScript)
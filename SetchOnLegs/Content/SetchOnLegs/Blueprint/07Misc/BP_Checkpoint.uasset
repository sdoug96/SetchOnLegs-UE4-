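; BP_Checkpoint is a level checkpoint that saves the player's position when BP_Spike enters its trigger box.
; If its PointLight is off, it turns off every checkpoint's light, lights its own and plays a sound, so only the latest stays lit.
; Each overlap writes the player's location to a fresh BP_SaveInfo in the "Checkpoint" save slot.
; The construction script sizes the box from the ChangeHitBox variable.
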(event OnComponentBeginOverlap(Box)
  (params (OverlappedComponent :type Primitive%20Component%20Object%20Reference) (OtherActor :type Actor%20Object%20Reference) (OtherComp :type Primitive%20Component%20Object%20Reference) (OtherBodyIndex :type Integer) (bFromSweep :type Boolean) (SweepResult :type Hit%20Result%20Structure%20%28by%20ref%29))
  (Utilities|Casting|CastToBP_Spike OtherActor)
  (if (Variables|/Script/Engine.SceneComponent|GetbVisible (Variables|Default|GetPointLight))
    _
    (else
      (bind _outactors (Actor|GetAllActorsOfClass "BP_Checkpoint_C"))
      (for _array_element _outactors
        (Rendering|SetVisibility (Variables|BP_Checkpoint_C|GetPointLight _array_element) false false))
      (Rendering|ToggleVisibility (Variables|Default|GetPointLight) false)
      (Audio|PlaySound2D "/Game/SetchOnLegs/Audio/07Misc/Checkpoint.Checkpoint" 1.0 1.0 0.0 0 0)))
  (bind _returnvalue (SaveGame|CreateSaveGameObject "/Game/SetchOnLegs/Blueprint/07Misc/BP_SaveInfo.BP_SaveInfo_C"))
  (Variables|Default|SetSaveInfo _returnvalue)
  (bind _asbp_spike (Utilities|Casting|CastToBP_Spike (Game|GetPlayerCharacter 0)))
  (Variables|Default|SetCharacterInfo _asbp_spike)
  (CallFunction|SetSaveLocation)
  (SaveGame|SaveGametoSlot (Variables|Default|GetSaveInfo) "Checkpoint"))

(event Custom|SetSaveLocation
  (Variables|/Game/SetchOnLegs/Blueprint/07Misc/BP_SaveInfo.BP_SaveInfo_C|SetcheckLocation (Variables|Default|GetSaveInfo) (Transformation|GetActorLocation (Variables|Default|GetCharacterInfo))))

(fn ConstructionScript
  (Components|Box|SetBoxExtent (Variables|Default|GetBox) (Variables|Default|GetchangeHitBox) true))
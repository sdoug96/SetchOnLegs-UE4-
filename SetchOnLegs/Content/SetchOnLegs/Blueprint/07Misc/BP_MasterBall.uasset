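; BP_MasterBall is a collectible pickup that adds its Value to BP_Spike's master ball count.
; On BeginPlay it enables gravity and pops upward with a random impulse to either side along X.
; Overlap with BP_Spike, unless Spike is in one excluded state, destroys it and plays a pickup sound.
; It also updates BP_GameInstance's total and the per-level count, indexed by the current GameState.
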(event OnComponentBeginOverlap(HitSphere)
  (params (OverlappedComponent :type Primitive%20Component%20Object%20Reference) (OtherActor :type Actor%20Object%20Reference) (OtherComp :type Primitive%20Component%20Object%20Reference) (OtherBodyIndex :type Integer) (bFromSweep :type Boolean) (SweepResult :type Hit%20Result%20Structure%20%28by%20ref%29))
  ;[1 1 1] When hit
  (bind _asbp_spike (Utilities|Casting|CastToBP_Spike OtherActor))
  (if (Utilities|Enum|NotEqual(Enum) (Variables|/Game/SetchOnLegs/Blueprint/08Spike/BP_Spike.BP_Spike_C|GetState _asbp_spike) "NewEnumerator5")
    (Actor|DestroyActor)
    (Audio|PlaySound2D (Variables|Default|GetPickupSound) 1.0 1.0 0.0 0 0)
    (Variables|/Game/SetchOnLegs/Blueprint/08Spike/BP_Spike.BP_Spike_C|SetMasterBalls _asbp_spike (+ (Variables|/Game/SetchOnLegs/Blueprint/08Spike/BP_Spike.BP_Spike_C|GetMasterBalls _asbp_spike) (Variables|Default|GetValue)))
    (CallFunction|SetMasterBalls)))

(event Custom|SetMasterBalls
  (bind _value (Variables|Default|GetValue))
  ;[1 1 1] Set master balls for individual levels
  (bind _asbp_game_instance (Utilities|Casting|CastToBP_GameInstance (Game|GetGameInstance)))
  (Variables|/Game/SetchOnLegs/Blueprint/07Misc/BP_GameInstance.BP_GameInstance_C|SetTotalMasterBalls _asbp_game_instance (+ (Variables|/Game/SetchOnLegs/Blueprint/07Misc/BP_GameInstance.BP_GameInstance_C|GetTotalMasterBalls _asbp_game_instance) (Variables|Default|GetValue)))
  (switch Utilities|FlowControl|Switch|SwitchonGameState (Variables|/Game/SetchOnLegs/Blueprint/07Misc/BP_GameInstance.BP_GameInstance_C|GetGameState _asbp_game_instance)
    (:NewEnumerator2
      (Utilities|Array|SetArrayElem (Variables|/Game/SetchOnLegs/Blueprint/07Misc/BP_GameInstance.BP_GameInstance_C|GetLevelsMasterBalls _asbp_game_instance) 0 (+ (Utilities|Array|Get(acopy) (Variables|/Game/SetchOnLegs/Blueprint/07Misc/BP_GameInstance.BP_GameInstance_C|GetLevelsMasterBalls _asbp_game_instance)) _value) true))
    (:NewEnumerator3
      (Utilities|Array|SetArrayElem (Variables|/Game/SetchOnLegs/Blueprint/07Misc/BP_GameInstance.BP_GameInstance_C|GetLevelsMasterBalls _asbp_game_instance) 1 (+ (Utilities|Array|Get(acopy) (Variables|/Game/SetchOnLegs/Blueprint/07Misc/BP_GameInstance.BP_GameInstance_C|GetLevelsMasterBalls _asbp_game_instance) 1) _value) true))
    (:NewEnumerator4
      (Utilities|Array|SetArrayElem (Variables|/Game/SetchOnLegs/Blueprint/07Misc/BP_GameInstance.BP_GameInstance_C|GetLevelsMasterBalls _asbp_game_instance) 2 (+ (Utilities|Array|Get(acopy) (Variables|/Game/SetchOnLegs/Blueprint/07Misc/BP_GameInstance.BP_GameInstance_C|GetLevelsMasterBalls _asbp_game_instance) 2) _value) true))
    (:NewEnumerator5
      (Utilities|Array|SetArrayElem (Variables|/Game/SetchOnLegs/Blueprint/07Misc/BP_GameInstance.BP_GameInstance_C|GetLevelsMasterBalls _asbp_game_instance) 3 (+ (Utilities|Array|Get(acopy) (Variables|/Game/SetchOnLegs/Blueprint/07Misc/BP_GameInstance.BP_GameInstance_C|GetLevelsMasterBalls _asbp_game_instance) 3) _value) true))
    (:NewEnumerator8
      (Utilities|Array|SetArrayElem (Variables|/Game/SetchOnLegs/Blueprint/07Misc/BP_GameInstance.BP_GameInstance_C|GetLevelsMasterBalls _asbp_game_instance) 4 (+ (Utilities|Array|Get(acopy) (Variables|/Game/SetchOnLegs/Blueprint/07Misc/BP_GameInstance.BP_GameInstance_C|GetLevelsMasterBalls _asbp_game_instance) 4) _value) true))
    (:NewEnumerator6
      (Utilities|Array|SetArrayElem (Variables|/Game/SetchOnLegs/Blueprint/07Misc/BP_GameInstance.BP_GameInstance_C|GetLevelsMasterBalls _asbp_game_instance) 5 (+ (Utilities|Array|Get(acopy) (Variables|/Game/SetchOnLegs/Blueprint/07Misc/BP_GameInstance.BP_GameInstance_C|GetLevelsMasterBalls _asbp_game_instance) 5) _value) true))))

(event EventBeginPlay
  (bind _returnvalue (Math|Random|RandomFloatinRange 5e+02 7.5e+02))
  (bind _pickup (Variables|Default|GetPickup))
  ;[1 1 1] Begin Play
  (Variables|/Script/Engine.ProjectileMovementComponent|SetProjectileGravityScale (Variables|Default|GetProjectileMovement) 1.0)
  (if (== (Math|Random|RandomInteger 2) 0)
    (Physics|AddImpulse _pickup (Math|Vector|MakeVector (Math|Random|RandomFloatinRange -3e+02 -2e+02) 0.0 _returnvalue) "None" true)
    (else
      (Physics|AddImpulse _pickup (Math|Vector|MakeVector (Math|Random|RandomFloatinRange 2e+02 3e+02) 0.0 _returnvalue) "None" true))))

(fn ConstructionScript)
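; The Butcher is a sprite-based boss that throws randomly aimed cleavers and shows a health widget or similar HUD while alive.
; Tick-driven Delays pace the throws, switching to smaller paired cleavers below a health threshold.
; Bullet overlaps apply damage, boosted by the MegaCannon upgrade, with timer-driven blinking; charged bullets deal damage only if IsDead is set.
; Death clears the widget, cleavers, spin blades and drag pads, then destroys the boss.
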(event OnComponentBeginOverlap(BulletBox)
  (params (OverlappedComponent :type Primitive%20Component%20Object%20Reference) (OtherActor :type Actor%20Object%20Reference) (OtherComp :type Primitive%20Component%20Object%20Reference) (OtherBodyIndex :type Integer) (bFromSweep :type Boolean) (SweepResult :type Hit%20Result%20Structure%20%28by%20ref%29))
  ;[1 1 1] Bullet Collision
  (Utilities|FlowControl|Sequence
    (:then_0
      (bind _asbp_bullet (Utilities|Casting|CastToBP_Bullet OtherActor))
      (Actor|DestroyActor _asbp_bullet)
      (if (not (Variables|Default|GetIsDead))
        (CallFunction|DamageSytsem (Variables|Default|GetBulletDamage))))
    (:then_1
      (bind _asbp_charged_bullet (Utilities|Casting|CastToBP_ChargedBullet OtherActor))
      (Actor|DestroyActor _asbp_charged_bullet)
      (if (Variables|Default|GetIsDead)
        (CallFunction|DamageSytsem (Variables|Default|GetChargedBulletDamage))))))

(event Custom|Blink
  (bind _sprite (Variables|Default|GetSprite))
  ;[1 1 1] Damage & Death System
  (Development|SetHiddeninGame _sprite (not (Variables|/Script/Engine.SceneComponent|GetbHiddenInGame _sprite)) false))

(event Custom|Damage%20Sytsem
  (params (DamageIn :type Float%20%28single-precision%29))
  ;[1 1 1] Damage & Death System
  (bind _output_get (Variables|Default|SetCurrentHealth (- (Variables|Default|GetCurrentHealth) DamageIn)))
  (if (<= _output_get 0.0)
    (Variables|Default|SetIsDead true)
    (Widget|RemovefromParent (stale EventBeginPlay _returnvalue))
    (Utilities|FlowControl|Delay 5.0)
    (Actor|DestroyActor)
    (else
      (Utilities|Time|SetTimerbyFunctionName 0 "Blink" 0.05 true)
      (Utilities|FlowControl|Delay 0.2)
      (Utilities|Time|ClearTimerbyFunctionName 0 "Blink")
      (Development|SetHiddeninGame (Variables|Default|GetSprite) false false))))

(event EventBeginPlay
  ;[1 1 1] Initialise
  (bind _returnvalue (UserInterface|CreateWidget "/Game/SetchOnLegs/Blueprint/TheButcher/Widget_TheButcher.Widget_TheButcher_C"))
  (UserInterface|Viewport|AddtoViewport _returnvalue 0)
  (bind _asbp_game_instance (Utilities|Casting|CastToBP_GameInstance (Game|GetGameInstance)))
  (if (Variables|/Game/SetchOnLegs/Blueprint/Misc/BP_GameInstance.BP_GameInstance_C|GetMegaCannon _asbp_game_instance)
    (Variables|Default|SetBulletDamage 4.0)))

(event EventTick
  (params (DeltaSeconds :type Float%20%28single-precision%29))
  (bind _arrow1 (Variables|Default|GetArrow1))
  (bind _currenthealth (Variables|Default|GetCurrentHealth))
  (bind _arrow1_2 (Variables|Default|GetArrow1))
  (bind _returnvalue (Transformation|GetWorldTransform _arrow1_2))
  (bind _returnvalue_2 (Transformation|GetWorldTransform _arrow1))
  ;[1 1 1] Throw Cleavers
  (Utilities|FlowControl|Sequence
    (:then_0
      (if (not (Variables|Default|GetIsDead))
        (if (> _currenthealth 5e+02)
          (Utilities|FlowControl|Delay 1.5)
          (bind _returnvalue_3 (Game|SpawnActorfromClass "/Game/SetchOnLegs/Blueprint/TheButcher/BP_Cleaver.BP_Cleaver_C" (Transformation|GetWorldTransform (Variables|Default|GetArrow1)) "Undefined" 0 0))
          (Variables|/Script/Engine.MovementComponent|SetVelocity (Variables|/Game/SetchOnLegs/Blueprint/TheButcher/BP_Cleaver.BP_Cleaver_C|GetProjectileMovement _returnvalue_3) (Math|Vector|MakeVector (Math|Random|RandomFloatinRange -1e+02 -1.1e+03) 0.0 (Math|Random|RandomFloatinRange 1e+02 -1e+02))))))
    (:then_1
      (if (not (Variables|Default|GetIsDead))
        (if (< _currenthealth 5e+02)
          (if (> _currenthealth 0.0)
            (Utilities|FlowControl|Delay 1.5)
            (bind _returnvalue_4 (Game|SpawnActorfromClass "/Game/SetchOnLegs/Blueprint/TheButcher/BP_Cleaver.BP_Cleaver_C" (Math|Transform|MakeTransform (.location _returnvalue_2) (.rotation _returnvalue_2) "0.300000,0.300000,0.300000") "Undefined" 0 0))
            (Variables|/Script/Engine.MovementComponent|SetVelocity (Variables|/Game/SetchOnLegs/Blueprint/TheButcher/BP_Cleaver.BP_Cleaver_C|GetProjectileMovement _returnvalue_4) (Math|Vector|MakeVector (Math|Random|RandomFloatinRange -1e+02 -1.1e+03) 0.0 (Math|Random|RandomFloatinRange 1e+02 -1e+02)))
            (bind _returnvalue_5 (Game|SpawnActorfromClass "/Game/SetchOnLegs/Blueprint/TheButcher/BP_Cleaver.BP_Cleaver_C" (Math|Transform|MakeTransform (.location _returnvalue) (.rotation _returnvalue) "0.300000,0.300000,0.300000") "Undefined" 0 0))
            (Variables|/Script/Engine.MovementComponent|SetVelocity (Variables|/Game/SetchOnLegs/Blueprint/TheButcher/BP_Cleaver.BP_Cleaver_C|GetProjectileMovement _returnvalue_5) (Math|Vector|MakeVector (Math|Random|RandomFloatinRange -1e+02 -1.1e+03) 0.0 (Math|Random|RandomFloatinRange 1e+02 -1e+02)))))))
    (:then_2
      (if (Variables|Default|GetIsDead)
        (bind _outactors (Actor|GetAllActorsOfClass "/Game/SetchOnLegs/Blueprint/HinceInHell/BP_SpinBlade.BP_SpinBlade_C"))
        (Actor|DestroyActor _outactors)
        (bind _outactors_2 (Actor|GetAllActorsOfClass "/Game/SetchOnLegs/Blueprint/Misc/BP_DragPad.BP_DragPad_C"))
        (Actor|DestroyActor _outactors_2)
        (bind _outactors_3 (Actor|GetAllActorsOfClass "/Game/SetchOnLegs/Blueprint/TheButcher/BP_Cleaver.BP_Cleaver_C"))
        (Actor|DestroyActor _outactors_3)))))

(fn ConstructionScript)
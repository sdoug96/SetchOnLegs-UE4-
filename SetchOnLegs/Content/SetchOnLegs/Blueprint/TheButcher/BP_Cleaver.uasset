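; BP_Cleaver is a spinning cleaver hazard from The Butcher's asset set that damages the player, BP_Spike.
; Tick accumulates time and multiplies it by Rotation to set the actor's pitch.
; Box overlap skips Spike in one excluded state, otherwise calls its damage function with no knockback, scaling Damage down as ArmorLevel rises.
; The cleaver destroys itself after dealing that damage.
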(event OnComponentBeginOverlap(Box)
  (params (OverlappedComponent :type Primitive%20Component%20Object%20Reference) (OtherActor :type Actor%20Object%20Reference) (OtherComp :type Primitive%20Component%20Object%20Reference) (OtherBodyIndex :type Integer) (bFromSweep :type Boolean) (SweepResult :type Hit%20Result%20Structure%20%28by%20ref%29))
  ;[1 1 1] Player Collision
  (bind _asbp_spike (Utilities|Casting|CastToBP_Spike OtherActor))
  (if (Utilities|Enum|NotEqual(Enum) (Variables|/Game/SetchOnLegs/Blueprint/Spike/BP_Spike.BP_Spike_C|GetState _asbp_spike) "NewEnumerator5")
    (switch int (Variables|/Game/SetchOnLegs/Blueprint/Spike/BP_Spike.BP_Spike_C|GetArmorLevel _asbp_spike)
      (:0
        (Default|DamageSytsem _asbp_spike (Variables|Default|GetDamage) 0.0))
      (:1
        (Default|DamageSytsem _asbp_spike (* (Variables|Default|GetDamage) 0.9) 0.0))
      (:2
        (Default|DamageSytsem _asbp_spike (* (Variables|Default|GetDamage) 0.8) 0.0))
      (:3
        (Default|DamageSytsem _asbp_spike (* (Variables|Default|GetDamage) 0.7) 0.0))
      (:4
        (Default|DamageSytsem _asbp_spike (* (Variables|Default|GetDamage) 0.6) 0.0))
      (:5
        (Default|DamageSytsem _asbp_spike (* (Variables|Default|GetDamage) 0.5) 0.0)))
    (Actor|DestroyActor)))

(event EventTick
  (params (DeltaSeconds :type Float%20%28single-precision%29))
  ;[1 1 1] Rotate
  (Variables|Default|SetTimer (+ DeltaSeconds (Variables|Default|GetTimer)))
  (Transformation|SetActorRotation (Math|Rotator|MakeRotator 0.0 (* (Variables|Default|GetTimer) (Variables|Default|GetRotation)) 0.0)))

(fn ConstructionScript)
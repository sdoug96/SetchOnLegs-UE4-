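; The Butcher boss enemy, which takes damage from the player's bullets and has its own health HUD widget.
; Bullet overlaps subtract normal or charged damage read from BP_Spike, blinking the sprite, or on death removing the HUD and destroying the boss after a delay.
; Tick retunes cleaver and blade variables at low health and clears spawned hazards once dead.
; The cleaver-throwing logic is disconnected and never runs.
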(event OnComponentBeginOverlap(BulletBox)
  (params (OverlappedComponent :type Primitive%20Component%20Object%20Reference) (OtherActor :type Actor%20Object%20Reference) (OtherComp :type Primitive%20Component%20Object%20Reference) (OtherBodyIndex :type Integer) (bFromSweep :type Boolean) (SweepResult :type Hit%20Result%20Structure%20%28by%20ref%29))
  ;[1 1 1] Bullet Collision
  (Utilities|FlowControl|Sequence
    (:then_0
      (bind _asbp_bullet (Utilities|Casting|CastToBP_Bullet OtherActor))
      (Actor|DestroyActor _asbp_bullet)
      (if (not (Variables|Default|GetIsDead))
        (bind _asbp_spike (Utilities|Casting|CastToBP_Spike (Game|GetPlayerCharacter 0)))
        (CallFunction|DamageSytsem (Variables|/Game/SetchOnLegs/Blueprint/08Spike/BP_Spike.BP_Spike_C|GetBulletDamage _asbp_spike))))
    (:then_1
      (bind _asbp_charged_bullet (Utilities|Casting|CastToBP_ChargedBullet OtherActor))
      (Actor|DestroyActor _asbp_charged_bullet)
      (if (not (Variables|Default|GetIsDead))
        (bind _asbp_spike_2 (Utilities|Casting|CastToBP_Spike (Game|GetPlayerCharacter 0)))
        (CallFunction|DamageSytsem (Variables|/Game/SetchOnLegs/Blueprint/08Spike/BP_Spike.BP_Spike_C|GetChargedShotDamage _asbp_spike_2))))))

(event Custom|Blink
  (bind _sprite (Variables|Default|GetSprite))
  ;[1 1 1] Damage & Death System
  (Development|SetHiddeninGame _sprite (not (Variables|/Script/Engine.SceneComponent|GetbHiddenInGame _sprite)) false))

(event Custom|Damage%20Sytsem
  (params (DamageIn :type Float%20%28single-precision%29))
  ;[1 1 1] Damage & Death System
  (bind _output_get (Variables|Default|SetCurrentHealth (- (Variables|Default|GetCurrentHealth) DamageIn)))
  (if (<= _output_get 0.0)
    (Variables|Default|SetIsDead true)
    (Widget|RemovefromParent (Variables|Default|GetHUD))
    (Utilities|FlowControl|Delay 5.0)
    (Actor|DestroyActor)
    (else
      (Utilities|Time|SetTimerbyFunctionName 0 "Blink" 0.05 true)
      (Utilities|FlowControl|Delay 0.2)
      (Utilities|Time|ClearTimerbyFunctionName 0 "Blink")
      (Development|SetHiddeninGame (Variables|Default|GetSprite) false false))))

(event Custom|ShowHUD
  ;[1 1 1] Show HUD function
  (bind _returnvalue (UserInterface|CreateWidget "/Game/SetchOnLegs/Blueprint/03TheButcher/Widget_TheButcher.Widget_TheButcher_C"))
  (bind _output_get (Variables|Default|SetHUD _returnvalue))
  (UserInterface|Viewport|AddtoViewport _output_get 0))

(event EventBeginPlay
  ;[1 1 1] Initialise
)

(event EventTick
  (params (DeltaSeconds :type Float%20%28single-precision%29))
  (bind _currenthealth (Variables|Default|GetCurrentHealth))
  ;[1 1 1] Throw Cleavers
  (Utilities|FlowControl|Sequence
    (:then_1
      (if (not (Variables|Default|GetIsDead))
        (if (Math|Float|InRange(Float) (Variables|Default|GetCurrentHealth) 0.0 1.0)
          _)))
    (:then_2
      (if (not (Variables|Default|GetIsDead))
        (if (< _currenthealth 1e+03)
          (if (> _currenthealth 0.0)
            (Variables|Default|SetCleaverDelay 1.0)
            (Variables|Default|SetFallingBladeSpeed -5e+02)
            (Variables|Default|SetBladeDelay 1.5)))))
    (:then_3
      (if (Variables|Default|GetIsDead)
        (bind _outactors (Actor|GetAllActorsOfClass "/Game/SetchOnLegs/Blueprint/03TheButcher/BP_SpinBlade.BP_SpinBlade_C"))
        (Actor|DestroyActor _outactors)
        (bind _outactors_2 (Actor|GetAllActorsOfClass "/Game/SetchOnLegs/Blueprint/03TheButcher/BP_DragPad.BP_DragPad_C"))
        (Actor|DestroyActor _outactors_2)
        (bind _outactors_3 (Actor|GetAllActorsOfClass "/Game/SetchOnLegs/Blueprint/03TheButcher/BP_Cleaver.BP_Cleaver_C"))
        (Actor|DestroyActor _outactors_3)))))

(fn ConstructionScript)
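; BP_MazePortal is a maze portal that teleports the BP_Spike character to a linked portal.
; On box overlap it moves Spike to PortalToWarpTo, offset by XDiff along X and lowered in Z, and plays a portal sound.
; It also sets Spike's flipbook to idle and disables input for a short delay.
; The Left flag makes the X offset negative at BeginPlay.
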(event OnComponentBeginOverlap(Box)
  (params (OverlappedComponent :type Primitive%20Component%20Object%20Reference) (OtherActor :type Actor%20Object%20Reference) (OtherComp :type Primitive%20Component%20Object%20Reference) (OtherBodyIndex :type Integer) (bFromSweep :type Boolean) (SweepResult :type Hit%20Result%20Structure%20%28by%20ref%29))
  (bind _portaltowarpto (Variables|Default|GetPortalToWarpTo))
  (bind _returnvalue (Transformation|GetActorLocation _portaltowarpto))
  ;[1 1 1] Portal Logic
  (bind _asbp_spike (Utilities|Casting|CastToBP_Spike OtherActor))
  (Transformation|SetActorLocation _asbp_spike (Math|Vector|MakeVector (+ (.x _returnvalue) (Variables|Default|GetXDiff)) (.y _returnvalue) (- (.z _returnvalue) 5e+01)) false false)
  (Audio|PlaySound2D "/Game/SetchOnLegs/Audio/Misc/portal.Portal" 1.0 1.0 0.0 0 0)
  (Sprite|SetFlipbook (Variables|/Script/Paper2D.PaperCharacter|GetSprite _asbp_spike) "/Game/SetchOnLegs/Sprites/Spike/Character/A_Idle.A_Idle")
  (Input|DisableInput _asbp_spike 0)
  (Utilities|FlowControl|Delay 0.75)
  (Input|EnableInput _asbp_spike 0))

(event EventBeginPlay
  (if (Variables|Default|GetLeft)
    (Variables|Default|SetXDiff -1e+02)))

(fn ConstructionScript)
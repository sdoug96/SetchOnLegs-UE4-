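; BP_ShopPrompt is a trigger volume that switches between level music and shop music as BP_Spike enters or leaves it.
; Box overlap events cast to BP_Spike, then set volume multipliers, making one track full and the other near-silent.
; The switch is instant with no fade, and neither track is stopped or started here.
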(event OnComponentBeginOverlap(Box)
  (params (OverlappedComponent :type Primitive%20Component%20Object%20Reference) (OtherActor :type Actor%20Object%20Reference) (OtherComp :type Primitive%20Component%20Object%20Reference) (OtherBodyIndex :type Integer) (bFromSweep :type Boolean) (SweepResult :type Hit%20Result%20Structure%20%28by%20ref%29))
  (Utilities|Casting|CastToBP_Spike OtherActor)
  (Audio|Components|Audio|SetVolumeMultiplier (Variables|Default|GetLevelMusic) 0.001 :!class /Script/Engine.AudioComponent)
  (Audio|Components|Audio|SetVolumeMultiplier (Variables|Default|GetShopMusic) 1.0 :!class /Script/Engine.AudioComponent))

(event OnComponentEndOverlap(Box)
  (params (OverlappedComponent :type Primitive%20Component%20Object%20Reference) (OtherActor :type Actor%20Object%20Reference) (OtherComp :type Primitive%20Component%20Object%20Reference) (OtherBodyIndex :type Integer))
  (Utilities|Casting|CastToBP_Spike OtherActor)
  (Audio|Components|Audio|SetVolumeMultiplier (Variables|Default|GetLevelMusic) 1.0 :!class /Script/Engine.AudioComponent)
  (Audio|Components|Audio|SetVolumeMultiplier (Variables|Default|GetShopMusic) 0.0001 :!class /Script/Engine.AudioComponent))

(fn ConstructionScript)
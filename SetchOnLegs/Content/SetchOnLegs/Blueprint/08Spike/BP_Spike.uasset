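; Player character Blueprint for Spike, a 2D flipbook side-scroller hero with jump, dash, climbing, shooting, shields and placeable checkpoints.
; Stats and upgrades load from BP_GameInstance on BeginPlay, and a State enum selects the flipbook in UpdateAnimation.
; Tick converts mouse screen position into X/Z aim for spread and charged shots, and updates dragpad push, cooldown and shield visuals.
; Death records per-level counts, then reloads boss levels or respawns at the saved location.
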(event Custom|Blink
  (bind _sprite (Variables|Default|GetSprite))
  ;[1 1 1] Damage & Death System
  (Development|SetHiddeninGame _sprite (not (Variables|/Script/Engine.SceneComponent|GetbHiddenInGame _sprite)) false))

(event Custom|Damage%20Sytsem
  (params (DamageIn :type Float%20%28single-precision%29) (KnockBack :type Float%20%28single-precision%29))
  ;[1 1 1] Damage & Death System
  (if (Utilities|Enum|NotEqual(Enum) (Variables|Default|GetState) "NewEnumerator5")
    (if (!= (Class|PaperFlipbookComponent|GetFlipbook (Variables|Default|GetSprite)) "/Game/SetchOnLegs/Sprites/Spike/Character/A_Dead.A_Dead")
      (bind _output_get (Variables|Default|SetCurrentHealth (- (Variables|Default|GetCurrentHealth) DamageIn)))
      (if (<= _output_get 0.0)
        (Audio|PlaySound2D "/Game/SetchOnLegs/Audio/00Menus/Splat.Splat" 1.0 1.0 0.0 0 0)
        (Variables|Default|SetState "NewEnumerator5")
        (Variables|Default|SetDeathCount (+ (Variables|Default|GetDeathCount) 1))
        (CallFunction|SetDeaths)
        (Input|DisableInput (Game|GetPlayerController 0))
        (CallFunction|UpdateAnimation)
        (Variables|Default|SetIsDead true)
        (Utilities|Time|ClearTimerbyFunctionName 0 "Shoot")
        (Rendering|SetVisibility (Variables|Default|GetShield) false false)
        (Utilities|FlowControl|Delay 2.0)
        (if (Variables|Default|GetIsDead)
          (if (Variables|Default|GetBossFight)
            (bind _asbp_game_instance (Utilities|Casting|CastToBP_GameInstance (Game|GetGameInstance)))
            (Variables|/Game/SetchOnLegs/Blueprint/07Misc/BP_GameInstance.BP_GameInstance_C|SetDeathCount _asbp_game_instance (Variables|Default|GetDeathCount))
            (Variables|Default|SetOnDragpad false)
            (Components|Movement|StopMovementImmediately (Variables|Character|GetCharacterMovement))
            (bind _returnvalue (Game|GetCurrentLevelName true))
            (Game|OpenLevel(byName) (Utilities|String|StringToName _returnvalue))
            (else
              (bind _asbp_game_instance_2 (Utilities|Casting|CastToBP_GameInstance (Game|GetGameInstance)))
              (Transformation|SetActorRelativeLocation (Variables|/Game/SetchOnLegs/Blueprint/07Misc/BP_GameInstance.BP_GameInstance_C|GetSpawnLocation _asbp_game_instance_2))
              (Variables|Default|SetCurrentHealth (* (Variables|Default|GetMaxHealth) 0.75))
              (Input|EnableInput 0)
              (Variables|Default|SetState "NewEnumerator0")
              (CallFunction|UpdateAnimation)
              (Variables|Default|SetIsDead false)
              (Variables|Default|SetOnDragpad false)
              (Components|Movement|StopMovementImmediately (Variables|Character|GetCharacterMovement)))))
        (else
          (Variables|Default|SetState "NewEnumerator4")
          (Audio|PlaySound2D "/Game/SetchOnLegs/Audio/07Misc/Ouch.Ouch" 1.0 1.0 0.0 0 0)
          (Physics|AddForce (Variables|Character|GetCharacterMovement) (Math|Vector|MakeVector KnockBack 0.0 2.5e+06))
          (Utilities|Time|SetTimerbyFunctionName 0 "Blink" 0.15 true)
          (Utilities|FlowControl|Delay 1.0)
          (Utilities|Time|ClearTimerbyFunctionName 0 "Blink")
          (Development|SetHiddeninGame (Variables|Default|GetSprite) false false))))))

(event Custom|UpdateAnimation
  (bind _sprite (Variables|Default|GetSprite))
  (bind _sprite_2 (Variables|Default|GetSprite))
  ;[1 1 1] Handle Animation
  (switch Utilities|FlowControl|Switch|SwitchonSpikeState (Variables|Default|GetState)
    (:NewEnumerator0
      (if (Variables|Default|GetCanJump_0)
        (Sprite|SetFlipbook (Variables|Default|GetSprite) (select (> (Math|Vector|VectorLength (Transformation|GetVelocity)) 0.0) "/Game/SetchOnLegs/Sprites/Spike/Character/A_SpikeWalking.A_SpikeWalking" "/Game/SetchOnLegs/Sprites/Spike/Character/A_Idle.A_Idle"))
        (goto _label Reset)))
    (:NewEnumerator2
      (Sprite|SetFlipbook (Variables|Default|GetSprite) "/Game/SetchOnLegs/Sprites/Spike/Character/A_Jumping.A_Jumping")
      (Utilities|FlowControl|DoOnce false :!label _label))
    (:NewEnumerator4
      (Sprite|SetFlipbook (Variables|Default|GetSprite) "/Game/SetchOnLegs/Sprites/Spike/Character/A_Hit.A_Hit"))
    (:NewEnumerator5
      (Sprite|SetFlipbook _sprite "/Game/SetchOnLegs/Sprites/Spike/Character/A_Dead.A_Dead")
      (Transformation|SetRelativeScale3D _sprite "0.500000,0.500000,0.500000")
      (Pawn|Components|CharacterMovement|DisableMovement (Variables|Character|GetCharacterMovement))
      (Utilities|FlowControl|Delay 2.0)
      (Transformation|SetRelativeScale3D _sprite "1.375000,1.000000,1.375000")
      (Utilities|FlowControl|Delay 0.2)
      (Pawn|Components|CharacterMovement|SetMovementMode (Variables|Character|GetCharacterMovement) "MOVE_Walking" 0))
    (:NewEnumerator6
      (Sprite|SetFlipbook (Variables|Default|GetSprite) "/Game/SetchOnLegs/Sprites/Spike/Character/A_Fire.A_Fire"))
    (:NewEnumerator7
      (Sprite|SetFlipbook _sprite_2 "/Game/SetchOnLegs/Sprites/Spike/Character/A_Climbing.A_Climbing")
      (if (Math|Float|InRange(Float) (Math|Vector|VectorLength (Transformation|GetVelocity)) -0.1 0.1)
        (Components|Timeline|SetPlayRate _sprite_2 1.0)
        (else
          (Components|Timeline|SetPlayRate _sprite_2 1.0))))
    (:NewEnumerator8
      (Sprite|SetFlipbook (Variables|Default|GetSprite) "/Game/SetchOnLegs/Sprites/Spike/Character/A_Jumping.A_Jumping"))))

(event Custom|Dragpad
  ;[1 1 1] Movement Logic
  ;;[1 1 1] Dragpad logic
  (if (Variables|Default|GetOnDragpad)
    (if (Utilities|Enum|NotEqual(Enum) (Variables|Default|GetState) "NewEnumerator5")
      (Pawn|Input|AddMovementInput "0.750000, 0, 0" 1.0 false))))

(event Custom|Shoot
  (bind _bulletmouserotation (Variables|Default|GetBulletMouseRotation))
  ;[1 1 1] Shoot Logic
  ;;[1 1 1] Handle Shoot
  (Variables|Default|SetCanMove false)
  (Variables|Default|SetState "NewEnumerator6")
  (for _index (range 0 (Variables|Default|GetBullets))
    (Game|SpawnActorfromClass "/Game/SetchOnLegs/Blueprint/08Spike/BP_Bullet.BP_Bullet_C" (Math|Transform|MakeTransform (.location (Transformation|GetWorldTransform (Variables|Default|GetBulletSpawn))) (Math|Rotator|MakeRotator (.roll _bulletmouserotation) (+ (.pitch _bulletmouserotation) (Variables|Default|GetBulletIncrement)) (.yaw _bulletmouserotation)) "1,1,1") "AlwaysSpawn" 0 0)
    (Utilities|FlowControl|Sequence
      (:then_0
        (if (Variables|Default|Get3Bullet)
          (Variables|Default|SetBulletIncrement (+ (Variables|Default|GetBulletIncrement) 3.0))))))
  (Audio|PlaySound2D "/Game/SetchOnLegs/Audio/07Misc/Shoot.Shoot" 1.0 1.0 0.0 0 0)
  (CallFunction|UpdateAnimation)
  (Variables|Default|SetBulletIncrement 0.0))

(event Custom|ClimbingEnd
  ;[1 1 1] Movement Logic
  ;;[1 1 1] Ladder Logic
  (Variables|Default|SetState "NewEnumerator0")
  (CallFunction|UpdateAnimation)
  (Pawn|Components|CharacterMovement|SetMovementMode (Variables|Character|GetCharacterMovement) "MOVE_Walking" 0)
  (Variables|Default|SetCanJump_0 true)
  (Variables|Default|SetIsClimbing false)
  (Variables|Default|SetJumpCount 0))

(event Custom|ChargedShootCooldown
  ;[1 1 1] Shoot Logic
  ;;[1 1 1] Charged Shot Cooldown
  (if (Variables|Default|GetChargedShot)
    (if (Variables|Default|GetChargedShotIncrement)
      (if (!= (Variables|Default|GetChargedShotCooldown) (Variables|Default|GetMaxChargedShotCooldown))
        (Utilities|FlowControl|Delay 1.0)
        (Variables|Default|SetChargedShotCooldown (+ (Variables|Default|GetChargedShotCooldown) 1.0))))))

(event Custom|SetGameInstanceValues
  ;[1 1 1] Set Game Instance Values
  (bind _asbp_game_instance (Utilities|Casting|CastToBP_GameInstance (Game|GetGameInstance)))
  (Utilities|FlowControl|Sequence
    (:then_0
      (Variables|Default|SetCurrentHealth (Variables|/Game/SetchOnLegs/Blueprint/07Misc/BP_GameInstance.BP_GameInstance_C|GetHealth _asbp_game_instance)))
    (:then_1
      (Variables|Default|SetMasterBalls (Variables|/Game/SetchOnLegs/Blueprint/07Misc/BP_GameInstance.BP_GameInstance_C|GetCurrency _asbp_game_instance)))
    (:then_2
      (Variables|Default|SetDeathCount (Variables|/Game/SetchOnLegs/Blueprint/07Misc/BP_GameInstance.BP_GameInstance_C|GetDeathCount _asbp_game_instance)))
    (:then_3
      (Variables|Default|SetHealthLevel (Variables|/Game/SetchOnLegs/Blueprint/07Misc/BP_GameInstance.BP_GameInstance_C|GetHealthLevel _asbp_game_instance)))
    (:then_4
      (Variables|Default|SetArmorLevel (Variables|/Game/SetchOnLegs/Blueprint/07Misc/BP_GameInstance.BP_GameInstance_C|GetArmorLevel _asbp_game_instance)))
    (:then_5
      (Variables|Default|SetCheckpoints (Variables|/Game/SetchOnLegs/Blueprint/07Misc/BP_GameInstance.BP_GameInstance_C|GetCheckpoints _asbp_game_instance)))
    (:then_6
      (Variables|Default|SetShields (Variables|/Game/SetchOnLegs/Blueprint/07Misc/BP_GameInstance.BP_GameInstance_C|GetShields _asbp_game_instance)))
    (:then_7
      (Variables|Default|SetChargedShot (Variables|/Game/SetchOnLegs/Blueprint/07Misc/BP_GameInstance.BP_GameInstance_C|GetChargedShot _asbp_game_instance)))
    (:then_8
      (Variables|Default|Set3Bullet (Variables|/Game/SetchOnLegs/Blueprint/07Misc/BP_GameInstance.BP_GameInstance_C|Get3BulletSpread _asbp_game_instance)))
    (:then_9
      (Variables|Default|Set5Bullet (Variables|/Game/SetchOnLegs/Blueprint/07Misc/BP_GameInstance.BP_GameInstance_C|Get5BulletSpread _asbp_game_instance)))
    (:then_10
      (Variables|Default|SetMaxHealth (Variables|/Game/SetchOnLegs/Blueprint/07Misc/BP_GameInstance.BP_GameInstance_C|GetMaxHealth _asbp_game_instance)))
    (:then_11
      (Variables|Default|SetBulletDamage (Variables|/Game/SetchOnLegs/Blueprint/07Misc/BP_GameInstance.BP_GameInstance_C|GetBulletDamage _asbp_game_instance)))
    (:then_12
      (Variables|Default|SetChargedShotDamage (Variables|/Game/SetchOnLegs/Blueprint/07Misc/BP_GameInstance.BP_GameInstance_C|GetChargedBulletDamage _asbp_game_instance)))
    (:then_13
      (Variables|Default|SetMaxChargedShotCooldown (Variables|/Game/SetchOnLegs/Blueprint/07Misc/BP_GameInstance.BP_GameInstance_C|GetChargedBulletCooldown _asbp_game_instance)))
    (:then_14
      (Variables|Default|SetGunner (Variables|/Game/SetchOnLegs/Blueprint/07Misc/BP_GameInstance.BP_GameInstance_C|GetGunner _asbp_game_instance)))))

(event Custom|SetDeaths
  ;[1 1 1] Set individual death counts based on current level
  (bind _asbp_game_instance (Utilities|Casting|CastToBP_GameInstance (Game|GetGameInstance)))
  (switch Utilities|FlowControl|Switch|SwitchonGameState (Variables|/Game/SetchOnLegs/Blueprint/07Misc/BP_GameInstance.BP_GameInstance_C|GetGameState _asbp_game_instance)
    (:NewEnumerator2
      (Utilities|Array|SetArrayElem (Variables|/Game/SetchOnLegs/Blueprint/07Misc/BP_GameInstance.BP_GameInstance_C|GetLevelsDeaths _asbp_game_instance) 0 (+ (Utilities|Array|Get(acopy) (Variables|/Game/SetchOnLegs/Blueprint/07Misc/BP_GameInstance.BP_GameInstance_C|GetLevelsDeaths _asbp_game_instance)) 1) true))
    (:NewEnumerator3
      (Utilities|Array|SetArrayElem (Variables|/Game/SetchOnLegs/Blueprint/07Misc/BP_GameInstance.BP_GameInstance_C|GetLevelsDeaths _asbp_game_instance) 1 (+ (Utilities|Array|Get(acopy) (Variables|/Game/SetchOnLegs/Blueprint/07Misc/BP_GameInstance.BP_GameInstance_C|GetLevelsDeaths _asbp_game_instance) 1) 1) true))
    (:NewEnumerator4
      (Utilities|Array|SetArrayElem (Variables|/Game/SetchOnLegs/Blueprint/07Misc/BP_GameInstance.BP_GameInstance_C|GetLevelsDeaths _asbp_game_instance) 2 (+ (Utilities|Array|Get(acopy) (Variables|/Game/SetchOnLegs/Blueprint/07Misc/BP_GameInstance.BP_GameInstance_C|GetLevelsDeaths _asbp_game_instance) 2) 1) true))
    (:NewEnumerator5
      (Utilities|Array|SetArrayElem (Variables|/Game/SetchOnLegs/Blueprint/07Misc/BP_GameInstance.BP_GameInstance_C|GetLevelsDeaths _asbp_game_instance) 3 (+ (Utilities|Array|Get(acopy) (Variables|/Game/SetchOnLegs/Blueprint/07Misc/BP_GameInstance.BP_GameInstance_C|GetLevelsDeaths _asbp_game_instance) 3) 1) true))
    (:NewEnumerator8
      (Utilities|Array|SetArrayElem (Variables|/Game/SetchOnLegs/Blueprint/07Misc/BP_GameInstance.BP_GameInstance_C|GetLevelsDeaths _asbp_game_instance) 4 (+ (Utilities|Array|Get(acopy) (Variables|/Game/SetchOnLegs/Blueprint/07Misc/BP_GameInstance.BP_GameInstance_C|GetLevelsDeaths _asbp_game_instance) 4) 1) true))
    (:NewEnumerator6
      (Utilities|Array|SetArrayElem (Variables|/Game/SetchOnLegs/Blueprint/07Misc/BP_GameInstance.BP_GameInstance_C|GetLevelsDeaths _asbp_game_instance) 5 (+ (Utilities|Array|Get(acopy) (Variables|/Game/SetchOnLegs/Blueprint/07Misc/BP_GameInstance.BP_GameInstance_C|GetLevelsDeaths _asbp_game_instance) 5) 1) true))))

(event Custom|GetFireRotation
  (bind _returnvalue (Game|GetPlayerController 0))
  (bind _returnvalue_2 (Game|GetPlayerController 0))
  (bind _bulletspawn (Variables|Default|GetBulletSpawn))
  (bind _returnvalue_3 (Transformation|GetWorldLocation _bulletspawn))
  (bind (_locationx _locationy) (Game|Player|GetMousePosition _returnvalue_2))
  (bind _screenlocation (Class|PlayerController|ProjectWorldLocationtoScreen _returnvalue _returnvalue_3 false))
  (bind (_x _y _z) (Math|Vector|BreakVector _returnvalue_3))
  (bind (_x_2 _y_2) (Math|Vector2D|BreakVector2D _screenlocation))
  ;[1 1 1] Shoot Logic
  ;;[1 1 1] Get Fire Rotation
  (bind _output_get (Variables|Default|SetBulletMouseRotation (Math|Rotator|FindLookatRotation _returnvalue_3 (Math|Vector|MakeVector (+ _x (- _locationx _x_2)) 0.0 (+ _z (- _y_2 _locationy))))))
  (if (Variables|Default|Get3Bullet)
    (if (Variables|Default|Get5Bullet)
      (Variables|Default|SetBulletMouseRotation (Math|Rotator|MakeRotator (.roll _output_get) (- (.pitch _output_get) 6.0) (.yaw _output_get)))
      (else
        (Variables|Default|SetBulletMouseRotation (Math|Rotator|MakeRotator (.roll _output_get) (- (.pitch _output_get) 3.0) (.yaw _output_get)))))))

(event Custom|ShootEnd
  ;[1 1 1] Shoot Logic
  ;;[1 1 1] Handle Shoot
  (if (not (Variables|Default|GetCutScene))
    (if (Variables|Default|GetIsDead)
      (Sprite|SetFlipbook (Variables|Default|GetSprite) "/Game/SetchOnLegs/Sprites/Spike/Character/A_Dead.A_Dead")
      (else
        (Utilities|FlowControl|Delay 0.2)
        (Variables|Default|SetState "NewEnumerator0")
        (Variables|Default|SetCanMove true)
        (CallFunction|UpdateAnimation)))))

(event EventOnLanded
  (params (Hit :type Hit%20Result%20Structure%20%28by%20ref%29))
  ;[1 1 1] Movement Logic
  ;;[1 1 1] Handle Jump
  (if (Utilities|Enum|Equal(Enum) (Variables|Default|GetState) "NewEnumerator5")
    (Sprite|SetFlipbook (Variables|Default|GetSprite) "/Game/SetchOnLegs/Sprites/Spike/Character/A_Dead.A_Dead")
    (else
      (Variables|Default|SetState "NewEnumerator0")
      (Variables|Default|SetCanJump_0 true)
      (Variables|Default|SetJumpCount 0))))

(event EventTick
  (params (DeltaSeconds :type Float%20%28single-precision%29))
  ;[1 1 1] Handle Abilities
  (Utilities|FlowControl|Sequence
    (:then_0
      (CallFunction|GetFireRotation)
      (if (< (Variables|Default|GetCurrentHealth) 0.0)
        (Variables|Default|SetCurrentHealth 0.0)))
    (:then_1
      (if (Variables|Default|Get3Bullet)
        (if (Variables|Default|Get5Bullet)
          (Variables|Default|SetBullets 4)
          (else
            (Variables|Default|SetBullets 2)))))
    (:then_2
      (CallFunction|Dragpad)
      (CallFunction|ChargedShootCooldown)
      (if (Variables|Default|GetShielded)
        (Rendering|SetVisibility (Variables|Default|GetShield) true false)
        (else
          (Rendering|SetVisibility (Variables|Default|GetShield1) false false))))))

(event EventBeginPlay
  ;[1 1 1] Initialise
  (Utilities|FlowControl|Sequence
    (:then_0
      (Class|ActorComponent|SetIsReplicated (Variables|Default|GetSprite) true)
      (Variables|Default|SetState "NewEnumerator0")
      (CallFunction|UpdateAnimation)
      (Variables|Default|SetJumpMaxCount 2))
    (:then_1
      (if (Variables|Default|GetShowHUD)
        (Utilities|FlowControl|Delay (Variables|Default|GetHUDDelay))
        (bind _returnvalue (UserInterface|CreateWidget "/Game/SetchOnLegs/Blueprint/08Spike/Widget_HUD.Widget_HUD_C" (Game|GetPlayerController 0)))
        (bind _output_get (Variables|Default|SetHUD _returnvalue))
        (UserInterface|Viewport|AddtoViewport _output_get 0)
        (Variables|/Script/Engine.PlayerController|SetbShowMouseCursor (Game|GetPlayerController 0) true)))
    (:then_2
      (CallFunction|SetGameInstanceValues))))

(event Input|ActionEvents|InputActionSpawnCheckpoint
  (params (Key :type Key%20Structure))
  (bind _returnvalue (Transformation|GetActorLocation))
  ;[1 1 1] Spawn Checkpoint
  (:Pressed
    (if (not (Variables|Default|GetBossFight))
      (if (> (Variables|Default|GetCheckpoints) 0)
        (Input|DisableInput 0)
        (bind _returnvalue_2 (UserInterface|CreateWidget "/Game/SetchOnLegs/Blueprint/07Misc/Fades/Widget_QuickFadeOutFadeIn.Widget_QuickFadeOutFadeIn_C"))
        (UserInterface|Viewport|AddtoViewport _returnvalue_2 0)
        (Utilities|FlowControl|Delay 0.9)
        (Audio|PlaySound2D "/Game/SetchOnLegs/Audio/07Misc/BuildCheckpoint.BuildCheckpoint" 1.0 1.0 0.0 0 0)
        (Utilities|FlowControl|Delay 1.1)
        (Game|SpawnActorfromClass "/Game/SetchOnLegs/Blueprint/07Misc/BP_Checkpoint.BP_Checkpoint_C" (Math|Transform|MakeTransform (Math|Vector|MakeVector (.x _returnvalue) -0.1 (+ (.z _returnvalue) 145.0)) "0, 0, 0" "1,1,1") "Undefined" 0 0)
        (Variables|Default|SetCheckpoints (- (Variables|Default|GetCheckpoints) 1))
        (Utilities|FlowControl|Delay 2.0)
        (Input|EnableInput 0)))))

(event Input|ActionEvents|InputActionJournal
  (params (Key :type Key%20Structure))
  ;[1 1 1] Handle Journal Menu
  (:Pressed
    (bind _returnvalue (UserInterface|CreateWidget "/Game/SetchOnLegs/Blueprint/00Menus/Journal/Widget_JournalDefault.Widget_JournalDefault_C"))
    (UserInterface|Viewport|AddtoViewport _returnvalue 0)
    (Game|SetGamePaused true)))

(event Input|ActionEvents|InputActionChargedShoot
  (params (Key :type Key%20Structure))
  ;[1 1 1] Shoot Logic
  ;;[1 1 1] Handle Charged Shoot
  (:Pressed
    (if (Variables|Default|GetChargedShot)
      (if (== (Variables|Default|GetChargedShotCooldown) (Variables|Default|GetMaxChargedShotCooldown))
        (Variables|Default|SetChargedShotCooldown 0.0)
        (Audio|PlaySound2D "/Game/SetchOnLegs/Audio/07Misc/ChargedShoot.ChargedShoot" 1.0 1.0 0.0 0 0)
        (Variables|Default|SetCanMove false)
        (Variables|Default|SetState "NewEnumerator6")
        (Game|SpawnActorfromClass "/Game/SetchOnLegs/Blueprint/08Spike/BP_ChargedBullet.BP_ChargedBullet_C" (Math|Transform|MakeTransform (.location (Transformation|GetWorldTransform (Variables|Default|GetBulletSpawn))) (Variables|Default|GetBulletMouseRotation) "1,1,1") "AlwaysSpawn" 0 0)
        (CallFunction|UpdateAnimation)
        (Character|LaunchCharacter (Math|Vector|MakeVector (Math|Conversions|ToFloat(Integer) (* (Variables|Default|GetFacing) 1500)) 0.0 0.0) false false))))
  (:Released
    (Utilities|FlowControl|Delay 0.2)
    (Variables|Default|SetState "NewEnumerator0")
    (Variables|Default|SetCanMove true)
    (CallFunction|UpdateAnimation)))

(event Input|ActionEvents|InputActionDash
  (params (Key :type Key%20Structure))
  ;[1 1 1] Handle Abilities
  (:Pressed
    (if (Variables|Default|GetDash)
      (if (not (AI|Components|NavMovement|IsFalling (Variables|Character|GetCharacterMovement)))
        (if (Variables|Default|GetCanDash)
          (Character|LaunchCharacter (Math|Vector|MakeVector (Math|Conversions|ToFloat(Integer) (* (Variables|Default|GetDashSpeed) (Variables|Default|GetFacing))) 0.0 0.0) false false)
          (Audio|PlaySound2D "/Game/SetchOnLegs/Audio/07Misc/Dash.Dash" 1.0 1.0 0.0 0 0)
          (Variables|Default|SetCanDash false)
          (Variables|Default|SetCanJump_0 false)
          (Rendering|SetVisibility (Variables|Default|GetSprite) false false)
          (Utilities|FlowControl|Delay 0.2)
          (Variables|Default|SetCanJump_0 true)
          (Utilities|FlowControl|Delay 0.1)
          (Rendering|SetVisibility (Variables|Default|GetSprite) true false)
          (Utilities|FlowControl|Delay 0.45)
          (Variables|Default|SetCanDash true))))))

(event Input|ActionEvents|InputActionInteract
  (params (Key :type Key%20Structure))
  ;[1 1 1] Interact
  (:Pressed
    (bind _outactors (Actor|GetAllActorswithInterface "/Game/SetchOnLegs/Blueprint/07Misc/Interface_Interact.Interface_Interact_C"))
    (for _array_element _outactors
      (if (Collision|IsOverlappingActor _array_element self :!class /Script/Engine.Actor)
        (Class|InterfaceInteract|Interact(Message) _array_element)))))

(event Input|ActionEvents|InputActionFlashlight
  (params (Key :type Key%20Structure))
  ;[1 1 1] Handle Abilities
  (:Pressed
    (if (Variables|Default|GetHasFlashlight)
      (Rendering|ToggleVisibility (Variables|Default|GetFlashlight) false))))

(event Input|ActionEvents|InputActionShoot
  (params (Key :type Key%20Structure))
  ;[1 1 1] Shoot Logic
  ;;[1 1 1] Handle Shoot
  (:Pressed
    (if (Variables|Default|GetShowHUD)
      (if (Variables|Default|GetGunner)
        (CallFunction|Shoot)
        (Utilities|Time|SetTimerbyEvent (delegate Custom|Shoot) (Variables|Default|GetGunnerDelay) true)
        (else
          (CallFunction|Shoot)))))
  (:Released
    (CallFunction|ShootEnd)
    (Utilities|Time|ClearTimerbyFunctionName 0 "Shoot")))

(event Input|ActionEvents|InputActionJump
  (params (Key :type Key%20Structure))
  ;[1 1 1] Movement Logic
  ;;[1 1 1] Handle Jump
  (:Pressed
    (Utilities|FlowControl|Sequence
      (:then_0
        (if (not (Variables|Default|GetCanClimb))
          (if (<= (Variables|Default|GetJumpCount) 1)
            (Audio|PlaySound2D "/Game/SetchOnLegs/Audio/07Misc/jump.jump" 1.0 1.0 0.0 0 0))))
      (:then_1
        (if (Variables|Default|GetCanJump_0)
          (if (Variables|Default|GetShowHUD)
            (Character|Jump)
            (Variables|Default|SetJumpCount (+ (Variables|Default|GetJumpCount) 1))
            (Variables|Default|SetState "NewEnumerator2")
            (CallFunction|UpdateAnimation)))))))

(event Input|ActionEvents|InputActionSpawnShield
  (params (Key :type Key%20Structure))
  ;[1 1 1] Spawn Shield
  (:Pressed
    (if (Variables|Default|GetChargedShotIncrement)
      (if (> (Variables|Default|GetShields) 0)
        (Variables|Default|SetShields (- (Variables|Default|GetShields) 1))
        (Audio|PlaySound2D "/Game/SetchOnLegs/Audio/07Misc/Shield.Shield" 1.0 1.0 0.0 0 0)
        (Variables|Default|SetShielded true)))))

(event Input|AxisEvents|InputAxisClimb
  (params (AxisValue :type Float%20%28single-precision%29))
  ;[1 1 1] Movement Logic
  ;;[1 1 1] Handle Jump
  (if (>= AxisValue 0.1)
    (if (Variables|Default|GetCanClimb)
      (Transformation|AddActorLocalOffset (Math|Vector|MakeVector 0.0 0.0 (* AxisValue (Variables|Default|GetClimbSpeed))) false false))))

(event Input|AxisEvents|InputAxisMove
  (params (AxisValue :type Float%20%28single-precision%29))
  ;[1 1 1] Movement Logic
  ;;[1 1 1] Handle movement
  (if (Variables|Default|GetCanMove)
    (if (>= AxisValue 0.0)
      (Variables|Default|SetIsMovingRight true)
      (else
        (Variables|Default|SetIsMovingRight false)))
    (Pawn|Input|AddMovementInput "1.000000, 0,0.000000" AxisValue false)
    (CallFunction|UpdateAnimation)
    (Math|Float|CompareFloat (.X (Math|Vector|BreakVector (Variables|/Script/Engine.MovementComponent|GetVelocity (Pawn|GetMovementComponent)))) AxisValue
      (:>
        (Pawn|SetControlRotation (Pawn|GetController) (Math|Rotator|MakeRotator 0.0 0.0 0.0) :!label _label)
        (Variables|Default|SetFacing -1))
      (:==
        (if (Variables|Default|GetIsMovingRight)
          (goto _label)
          (else
            (Pawn|SetControlRotation (Pawn|GetController) (Math|Rotator|MakeRotator 0.0 0.0 1.8e+02) :!label _label_2)
            (Variables|Default|SetFacing 1))))
      (:<
        (goto _label_2)))))

(event Input|AxisEvents|InputAxisClimb
  (params (AxisValue :type Float%20%28single-precision%29))
  ;[1 1 1] Movement Logic
  ;;[1 1 1] Ladder Logic
  (if (Variables|Default|GetCanClimb)
    (if (not (Math|Float|InRange(Float) AxisValue -0.1 0.1))
      (Variables|Default|SetState "NewEnumerator7")
      (CallFunction|UpdateAnimation)
      (Pawn|Components|CharacterMovement|SetMovementMode (Variables|Character|GetCharacterMovement) "MOVE_Flying" 0)
      (Pawn|Input|AddMovementInput (Math|Vector|MakeVector 0.0 0.0 0.5) AxisValue false)
      (Variables|Default|SetCanJump_0 false)
      (Variables|Default|SetIsClimbing true))))

(fn ConstructionScript)
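; The Creator is a Paper2D boss with a health widget, flipbook attack animations and a timed shield that periodically drops into a resting window.
; While shielded, Tick uses Delays to alternate a thunder strike at the player's position with a thunder disc shower, and low health adds cross spawns.
; The shield sphere destroys bullets while up, and BulletBox hits reduce health with a timer-driven sprite blink until death.
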(event OnComponentBeginOverlap(BulletBox)
  (params (OverlappedComponent :type Primitive%20Component%20Object%20Reference) (OtherActor :type Actor%20Object%20Reference) (OtherComp :type Primitive%20Component%20Object%20Reference) (OtherBodyIndex :type Integer) (bFromSweep :type Boolean) (SweepResult :type Hit%20Result%20Structure%20%28by%20ref%29))
  ;[1 1 1] Bullet Collision
  (Utilities|FlowControl|Sequence
    (:then_0
      (bind _asbp_bullet (Utilities|Casting|CastToBP_Bullet OtherActor))
      (Actor|DestroyActor _asbp_bullet)
      (if (not (Variables|Default|GetIsDead))
        (CallFunction|DamageSytsem (Variables|Default|GetBulletDamage))))
    (:then_1
      (bind _asbp_charged_bullet (Utilities|Casting|CastToBP_ChargedBullet OtherActor))
      (Actor|DestroyActor _asbp_charged_bullet)
      (if (not (Variables|Default|GetIsDead))
        (CallFunction|DamageSytsem (Variables|Default|GetChargedBulletDamage))))))

(event OnComponentBeginOverlap(Sphere)
  (params (OverlappedComponent :type Primitive%20Component%20Object%20Reference) (OtherActor :type Actor%20Object%20Reference) (OtherComp :type Primitive%20Component%20Object%20Reference) (OtherBodyIndex :type Integer) (bFromSweep :type Boolean) (SweepResult :type Hit%20Result%20Structure%20%28by%20ref%29))
  (bind _shielded (Variables|Default|GetShielded))
  ;[1 1 1] Bullet Collision
  (Utilities|FlowControl|Sequence
    (:then_0
      (if _shielded
        (bind _asbp_bullet (Utilities|Casting|CastToBP_Bullet OtherActor))
        (Actor|DestroyActor _asbp_bullet)))
    (:then_1
      (if _shielded
        (bind _asbp_charged_bullet (Utilities|Casting|CastToBP_ChargedBullet OtherActor))
        (Actor|DestroyActor _asbp_charged_bullet)))))

(event Custom|Blink
  (bind _sprite (Variables|Default|GetSprite))
  ;[1 1 1] Damage & Death System
  (Development|SetHiddeninGame _sprite (not (Variables|/Script/Engine.SceneComponent|GetbHiddenInGame _sprite)) false))

(event Custom|Damage%20Sytsem
  (params (DamageIn :type Float%20%28single-precision%29))
  ;[1 1 1] Damage & Death System
  (bind _output_get (Variables|Default|SetCurrentHealth (- (Variables|Default|GetCurrentHealth) DamageIn)))
  (if (<= _output_get 0.0)
    (Variables|Default|SetIsDead true)
    (Widget|RemovefromParent (stale EventBeginPlay _returnvalue))
    (Utilities|FlowControl|Delay 5.0)
    (Actor|DestroyActor)
    (else
      (Utilities|Time|SetTimerbyFunctionName 0 "Blink" 0.05 true)
      (Utilities|FlowControl|Delay 0.2)
      (Utilities|Time|ClearTimerbyFunctionName 0 "Blink")
      (Development|SetHiddeninGame (Variables|Default|GetSprite) false false))))

(event Custom|Thunder
  ;[1 1 1] Thunder Attack
  (if (Variables|Default|GetShielded)
    (Sprite|SetFlipbook (Variables|Default|GetSprite) "/Game/SetchOnLegs/Sprites/Creator/Character/Thunder/A_Thunder.A_Thunder")
    (bind _asbp_spike (Utilities|Casting|CastToBP_Spike (Game|GetPlayerCharacter 0)))
    (Game|SpawnActorfromClass "/Game/SetchOnLegs/Blueprint/Creator/BP_Thunder.BP_Thunder_C" (Math|Transform|MakeTransform (Math|Vector|MakeVector (.x (.location (Transformation|GetWorldTransform (Variables|/Script/Paper2D.PaperCharacter|GetSprite _asbp_spike)))) (.y (.location (Transformation|GetWorldTransform (Variables|/Script/Paper2D.PaperCharacter|GetSprite _asbp_spike)))) -1371.0) "0, 0, 0" "1,1,1") "Undefined" 0 0)
    (Utilities|FlowControl|Delay 5.0)
    (Sprite|SetFlipbook (Variables|Default|GetSprite) "/Game/SetchOnLegs/Sprites/Creator/Character/Idle/A_Idle.A_Idle")))

(event Custom|ThunderDiscShower
  (bind _returnvalue (Transformation|GetActorLocation))
  ;[1 1 1] Thunder Disc Shower
  (if (Variables|Default|GetShielded)
    (Sprite|SetFlipbook (Variables|Default|GetSprite) "/Game/SetchOnLegs/Sprites/Creator/Character/Blast/A_DiscShower.A_DiscShower")
    (Utilities|FlowControl|Delay 4.0)
    (Audio|PlaySound2D "/Game/SetchOnLegs/Audio/Creator/CreatorDiscShower.CreatorDiscShower" 1.0 1.0 0.0 0 0)
    (for _index (range 0 5)
      (Game|SpawnActorfromClass "/Game/SetchOnLegs/Blueprint/Creator/BP_ThunderDisc.BP_ThunderDisc_C" (Math|Transform|MakeTransform (Math|Vector|MakeVector (+ (.x _returnvalue) (Variables|Default|GetDiscIncrement)) (.y _returnvalue) (- (.z _returnvalue) 265.0)) "0, 0, 0" "1,1,1") "Undefined" 0 0)
      (Variables|Default|SetDiscIncrement (+ (Variables|Default|GetDiscIncrement) 1e+03))
      (Utilities|FlowControl|Delay 11.0)
      (Sprite|SetFlipbook (Variables|Default|GetSprite) "/Game/SetchOnLegs/Sprites/Creator/Character/Idle/A_Idle.A_Idle"))
    (Variables|Default|SetDiscIncrement 7.5e+02)))

(event Custom|ShieldDown
  ;[1 1 1] Initialise
  (Variables|Default|SetShielded false)
  (Utilities|FlowControl|Delay 7.0)
  (Variables|Default|SetShielded true)
  (Sprite|SetFlipbook (Variables|Default|GetSprite) "/Game/SetchOnLegs/Sprites/Creator/Character/Idle/A_Idle.A_Idle"))

(event EventBeginPlay
  ;[1 1 1] Initialise
  (Utilities|FlowControl|Sequence
    (:then_0
      (bind _returnvalue (UserInterface|CreateWidget "/Game/SetchOnLegs/Blueprint/Creator/Widget_TheCreator.Widget_TheCreator_C"))
      (UserInterface|Viewport|AddtoViewport _returnvalue 0)
      (bind _asbp_game_instance (Utilities|Casting|CastToBP_GameInstance (Game|GetGameInstance)))
      (if (Variables|/Game/SetchOnLegs/Blueprint/Misc/BP_GameInstance.BP_GameInstance_C|GetMegaCannon _asbp_game_instance)
        (Variables|Default|SetBulletDamage 4.0)))
    (:then_1
      (Utilities|Time|SetTimerbyEvent (delegate Custom|ShieldDown) 45.0 true))))

(event EventTick
  (params (DeltaSeconds :type Float%20%28single-precision%29))
  ;[1 1 1] Attacks
  (Utilities|FlowControl|Sequence
    (:then_0
      (if (Variables|Default|GetShielded)
        (if (Variables|Default|GetChooseAttack)
          (Utilities|FlowControl|Delay 1e+01)
          (CallFunction|ThunderDiscShower)
          (Variables|Default|SetChooseAttack false)
          (else
            (Utilities|FlowControl|Delay 1e+01)
            (CallFunction|Thunder)
            (Variables|Default|SetChooseAttack true)))))
    (:then_1
      (if (Variables|Default|GetShielded)
        (Rendering|SetVisibility (Variables|Default|GetShield) true false)
        (else
          (Rendering|SetVisibility (Variables|Default|GetShield) false false)
          (Sprite|SetFlipbook (Variables|Default|GetSprite) "/Game/SetchOnLegs/Sprites/Creator/Character/Resting/A_Resting.A_Resting"))))
    (:then_2
      (if (Math|Float|InRange(Float) (Variables|Default|GetCurrentHealth) 0.0 7.5e+03)
        (Utilities|FlowControl|Delay 2.0)
        (Game|SpawnActorfromClass "/Game/SetchOnLegs/Blueprint/Creator/BP_Cross.BP_Cross_C" (Math|Transform|MakeTransform (Math|Vector|MakeVector 3932.0 0.0 -2292.0) "0, 0, 0" "1,1,1") "Undefined" 0 0)
        (Game|SpawnActorfromClass "/Game/SetchOnLegs/Blueprint/Creator/BP_Cross.BP_Cross_C" (Math|Transform|MakeTransform (Math|Vector|MakeVector 4347.0 0.0 -2292.0) "0, 0, 0" "1,1,1") "Undefined" 0 0)))
    (:then_3
      (if (Math|Float|InRange(Float) (Variables|Default|GetCurrentHealth) 0.0 5e+03)
        _))))

(fn ConstructionScript)
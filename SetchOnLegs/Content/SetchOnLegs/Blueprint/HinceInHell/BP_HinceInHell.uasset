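; Flying flipbook boss Hince in Hell, which follows the player at a positional offset and periodically fires spin blades aimed through screen-space projection.
; Bullet and charged-bullet overlaps lower its health with a blink effect.
; On phase-one death it swaps health-bar widgets and spawns two copies of itself using little-head settings.
; Damage totalled on BP_Spike across heads triggers the level end, spawning steps and flagging the defeat in the GameInstance.
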(event OnComponentBeginOverlap(HeadCollision)
  (params (OverlappedComponent :type Primitive%20Component%20Object%20Reference) (OtherActor :type Actor%20Object%20Reference) (OtherComp :type Primitive%20Component%20Object%20Reference) (OtherBodyIndex :type Integer) (bFromSweep :type Boolean) (SweepResult :type Hit%20Result%20Structure%20%28by%20ref%29))
  ;[1 1 1] Bullet Collision
  (Utilities|FlowControl|Sequence
    (:then_0
      (bind _asbp_bullet (Utilities|Casting|CastToBP_Bullet OtherActor))
      (Actor|DestroyActor _asbp_bullet)
      (if (not (Variables|Default|GetIsDead))
        (CallFunction|DamageSytsem (Variables|Default|GetBulletDamage))
        (bind _asbp_spike (Utilities|Casting|CastToBP_Spike (Game|GetPlayerCharacter 0)))
        (Variables|/Game/SetchOnLegs/Blueprint/Spike/BP_Spike.BP_Spike_C|SetHinceInHellDamage _asbp_spike (+ (Variables|/Game/SetchOnLegs/Blueprint/Spike/BP_Spike.BP_Spike_C|GetHinceInHellDamage _asbp_spike) (Variables|Default|GetBulletDamage)))))
    (:then_1
      (bind _asbp_charged_bullet (Utilities|Casting|CastToBP_ChargedBullet OtherActor))
      (Actor|DestroyActor _asbp_charged_bullet)
      (if (not (Variables|Default|GetIsDead))
        (bind _asbp_spike_2 (Utilities|Casting|CastToBP_Spike (Game|GetPlayerCharacter 0)))
        (if (> (Variables|Default|GetCurrentHealth) (Variables|Default|GetChargedBulletDamage))
          (Variables|/Game/SetchOnLegs/Blueprint/Spike/BP_Spike.BP_Spike_C|SetHinceInHellDamage _asbp_spike_2 (+ (Variables|/Game/SetchOnLegs/Blueprint/Spike/BP_Spike.BP_Spike_C|GetHinceInHellDamage _asbp_spike_2) (Variables|Default|GetChargedBulletDamage)))
          (CallFunction|DamageSytsem (Variables|Default|GetChargedBulletDamage))
          (else
            (Variables|/Game/SetchOnLegs/Blueprint/Spike/BP_Spike.BP_Spike_C|SetHinceInHellDamage _asbp_spike_2 (+ (Variables|/Game/SetchOnLegs/Blueprint/Spike/BP_Spike.BP_Spike_C|GetHinceInHellDamage _asbp_spike_2) (Variables|Default|GetCurrentHealth)))
            (CallFunction|DamageSytsem (Variables|Default|GetChargedBulletDamage))))))))

(event Custom|Blink
  (bind _sprite (Variables|Default|GetSprite))
  ;[1 1 1] Damage & Death System
  (Development|SetHiddeninGame _sprite (not (Variables|/Script/Engine.SceneComponent|GetbHiddenInGame _sprite)) false))

(event Custom|Damage%20Sytsem
  (params (DamageIn :type Float%20%28single-precision%29))
  ;[1 1 1] Damage & Death System
  (bind _output_get (Variables|Default|SetCurrentHealth (- (Variables|Default|GetCurrentHealth) DamageIn)))
  (if (<= _output_get 0.0)
    (Utilities|FlowControl|Sequence
      (:then_0
        (Variables|Default|SetState "NewEnumerator2")
        (Variables|Default|SetIsDead true)
        (CallFunction|UpdateAnimation)
        (Utilities|FlowControl|Delay 2.2)
        (Actor|DestroyActor))
      (:then_1
        (if (Variables|Default|GetPhase1)
          (Widget|RemovefromParent (stale EventBeginPlay _returnvalue))
          (CallFunction|Respawn)
          (Variables|Default|SetPhase1 false)
          (Variables|Default|SetPhase2 true)
          (if (Variables|Default|GetPhase2)
            (bind _returnvalue (UserInterface|CreateWidget "/Game/SetchOnLegs/Blueprint/HinceInHell/Widget_HinceInHellPhase2.Widget_HinceInHellPhase2_C"))
            (bind _output_get_2 (Variables|Default|SetHealthBar1 _returnvalue))
            (bind _output_get_3 (Variables|Default|SetHealthBar2 _output_get_2))
            (UserInterface|Viewport|AddtoViewport _output_get_3 0)))))
    (else
      (Utilities|Time|SetTimerbyFunctionName 0 "Blink" 0.05 true)
      (Utilities|FlowControl|Delay 0.2)
      (Utilities|Time|ClearTimerbyFunctionName 0 "Blink")
      (Development|SetHiddeninGame (Variables|Default|GetSprite) false false))))

(event Custom|UpdateAnimation
  ;[1 1 1] Handle Animation
  (switch Utilities|FlowControl|Switch|SwitchonHinceInHellState (Variables|Default|GetState)
    (:NewEnumerator0
      (Sprite|SetFlipbook (Variables|Default|GetSprite) "/Game/SetchOnLegs/Sprites/HinceInHell/HinceInHellCharacter/A_Moving.A_Moving"))
    (:NewEnumerator1
      (Sprite|SetFlipbook (Variables|Default|GetSprite) "/Game/SetchOnLegs/Sprites/HinceInHell/HinceInHellCharacter/A_Attacking.A_Attacking"))
    (:NewEnumerator2
      (Sprite|SetFlipbook (Variables|Default|GetSprite) "/Game/SetchOnLegs/Sprites/HinceInHell/HinceInHellCharacter/A_dead.A_Dead"))))

(event Custom|Respawn
  (bind _returnvalue (Game|GetPlayerCharacter 0))
  (bind _littleheadscale (Variables|Default|GetLittleHeadScale))
  (bind _returnvalue_2 (Transformation|GetActorLocation _returnvalue))
  (bind _returnvalue_3 (- (.x _returnvalue_2) 2e+02))
  (bind _returnvalue_4 (+ (.z _returnvalue_2) 1e+03))
  (bind _returnvalue_5 (Math|Transform|MakeTransform (Math|Vector|MakeVector _returnvalue_3 0.0 _returnvalue_4) "0, 0, 0" _littleheadscale))
  ;[1 1 1] Respawn System
  (Utilities|FlowControl|Delay 1.0)
  (Utilities|FlowControl|Sequence
    (:then_0
      (Game|SpawnActorfromClass "BP_HinceInHell_C" _returnvalue_5 "Undefined" 0 (Variables|Default|GetLittleHeadHealth) 3.0 "-400.000000,0.000000,400.000000" (Variables|Default|GetLittleHeadBladeScale) false true 0)
      (Game|SpawnActorfromClass "BP_HinceInHell_C" _returnvalue_5 "Undefined" 0 (Variables|Default|GetLittleHeadHealth) 3.0 "400.000000,0.000000,400.000000" (Variables|Default|GetLittleHeadBladeScale) false true 0))))

(event Custom|Shoot
  (bind _returnvalue (Transformation|GetActorLocation))
  (bind _returnvalue_2 (Game|GetPlayerController 0))
  (bind _returnvalue_3 (Game|GetPlayerController 0))
  (bind _returnvalue_4 (Transformation|GetActorLocation))
  (bind _arrow1 (Variables|Default|GetArrow1))
  (bind _returnvalue_5 (Transformation|GetWorldLocation _arrow1))
  (bind _returnvalue_6 (Pawn|GetControlledPawn _returnvalue_2))
  (bind _screenlocation (Class|PlayerController|ProjectWorldLocationtoScreen _returnvalue_3 _returnvalue_4 false))
  (bind (_x _y _z) (Math|Vector|BreakVector _returnvalue))
  (bind _returnvalue_7 (Transformation|GetActorLocation _returnvalue_6))
  (bind (_x_2 _y_2) (Math|Vector2D|BreakVector2D _screenlocation))
  (bind _screenlocation_2 (Class|PlayerController|ProjectWorldLocationtoScreen _returnvalue_2 _returnvalue_7 false))
  (bind (_x_3 _y_3) (Math|Vector2D|BreakVector2D _screenlocation_2))
  ;[1 1 1] Handle Shoot
  (if (Utilities|Enum|NotEqual(Enum) (Variables|Default|GetState) "NewEnumerator2")
    (Variables|Default|SetState "NewEnumerator1")
    (CallFunction|UpdateAnimation)
    (Game|SpawnActorfromClass "/Game/SetchOnLegs/Blueprint/HinceInHell/BP_HinceInHellSpinBlade.BP_HinceInHellSpinBlade_C" (Math|Transform|MakeTransform (Math|Vector|MakeVector (.x _returnvalue_5) 5.0 (.z _returnvalue_5)) (Math|Rotator|FindLookatRotation _returnvalue (Math|Vector|MakeVector (+ _x (- _x_3 _x_2)) 0.0 (+ _z (- _y_2 _y_3)))) (Variables|Default|GetBladeScale)) "AlwaysSpawn" 0 0)
    (Utilities|FlowControl|Delay 1.0)
    (Variables|Default|SetState "NewEnumerator0")
    (CallFunction|UpdateAnimation)))

(event EventBeginPlay
  ;[1 1 1] Initialise
  (Utilities|FlowControl|Sequence
    (:then_0
      (Variables|Default|SetState "NewEnumerator0")
      (Pawn|Components|CharacterMovement|SetMovementMode (Variables|Character|GetCharacterMovement) "MOVE_Flying" 0))
    (:then_1
      (bind _asbp_game_instance (Utilities|Casting|CastToBP_GameInstance (Game|GetGameInstance)))
      (if (Variables|/Game/SetchOnLegs/Blueprint/Misc/BP_GameInstance.BP_GameInstance_C|GetMegaCannon _asbp_game_instance)
        (Variables|Default|SetBulletDamage 4.0)))
    (:then_2
      (if (Variables|Default|GetPhase1)
        (bind _returnvalue (UserInterface|CreateWidget "/Game/SetchOnLegs/Blueprint/HinceInHell/Widget_HinceInHellPhase1.Widget_HinceInHellPhase1_C"))
        (bind _output_get (Variables|Default|SetHealthBar _returnvalue))
        (UserInterface|Viewport|AddtoViewport _output_get 0)))))

(event EventTick
  (params (DeltaSeconds :type Float%20%28single-precision%29))
  ;[1 1 1] Tick
  (Utilities|FlowControl|Sequence
    (:then_0
      (Utilities|FlowControl|Delay 0.1)
      (Variables|Default|SetOurPosition (- (Transformation|GetActorLocation) (Variables|Default|GetMoveToPos)))
      (Variables|Default|SetPlayerPosition (Transformation|GetActorLocation (Pawn|GetControlledPawn (Game|GetPlayerController 0))))
      (Pawn|Input|AddMovementInput (- (Variables|Default|GetPlayerPosition) (Variables|Default|GetOurPosition)) 1.0 false))
    (:then_1
      (if (not (Variables|Default|GetIsDead))
        (Utilities|FlowControl|Delay (Variables|Default|GetAttackLag))
        (CallFunction|Shoot)))
    (:then_2
      (CallFunction|UpdateAnimation))
    (:then_3
      (if (not (Variables|Default|GetEndLevel))
        (bind _asbp_spike (Utilities|Casting|CastToBP_Spike (Game|GetPlayerCharacter 0)))
        (if (>= (Variables|/Game/SetchOnLegs/Blueprint/Spike/BP_Spike.BP_Spike_C|GetHinceInHellDamage _asbp_spike) 2.5e+02)
          (Game|SpawnActorfromClass "/Game/SetchOnLegs/Blueprint/HinceInHell/BP_Step.BP_Step_C" (Math|Transform|MakeTransform "-362.000000, 0,225.000000" "0, 0, 0" "1,1,1") "Undefined" 0 0)
          (Game|SpawnActorfromClass "/Game/SetchOnLegs/Blueprint/HinceInHell/BP_Step.BP_Step_C" (Math|Transform|MakeTransform "338.000000, 0,225.000000" "0, 0, 0" "1,1,1") "Undefined" 0 0)
          (Game|SpawnActorfromClass "/Game/SetchOnLegs/Blueprint/HinceInHell/BP_Step.BP_Step_C" (Math|Transform|MakeTransform "618.000000, 0,225.000000" "0, 0, 0" "1,1,1") "Undefined" 0 0)
          (Game|SpawnActorfromClass "/Game/SetchOnLegs/Blueprint/HinceInHell/BP_Step.BP_Step_C" (Math|Transform|MakeTransform "1322.000000, 0,225.000000" "0, 0, 0" "1,1,1") "Undefined" 0 0)
          (Variables|Default|SetEndLevel true)
          (bind _asbp_game_instance (Utilities|Casting|CastToBP_GameInstance (Game|GetGameInstance)))
          (Variables|/Game/SetchOnLegs/Blueprint/Misc/BP_GameInstance.BP_GameInstance_C|SetHinceInHellDefeated _asbp_game_instance true))))))

(fn ConstructionScript)
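; BP_Bat is a flying enemy that homes in on the BP_Spike player and damages it on contact, except in one player state.
; Projectile movement drives the chase, starting at BeginPlay, while a wake sphere resumes homing on entry and halts it on exit.
; Tick flips the bat and its light to face the player.
; Bullets hitting the hit sphere reduce health, triggering a timer-driven visibility blink or destroying the bat at zero.
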(event OnComponentBeginOverlap(WakeSphere)
  (params (OverlappedComponent :type Primitive%20Component%20Object%20Reference) (OtherActor :type Actor%20Object%20Reference) (OtherComp :type Primitive%20Component%20Object%20Reference) (OtherBodyIndex :type Integer) (bFromSweep :type Boolean) (SweepResult :type Hit%20Result%20Structure%20%28by%20ref%29))
  ;[1 1 1] Wake Sphere Logic
  (Utilities|Casting|CastToBP_Spike OtherActor)
  (Variables|/Script/Engine.ProjectileMovementComponent|SetbIsHomingProjectile (Variables|Default|GetProjectileMovement) true))

(event OnComponentBeginOverlap(HitSphere)
  (params (OverlappedComponent :type Primitive%20Component%20Object%20Reference) (OtherActor :type Actor%20Object%20Reference) (OtherComp :type Primitive%20Component%20Object%20Reference) (OtherBodyIndex :type Integer) (bFromSweep :type Boolean) (SweepResult :type Hit%20Result%20Structure%20%28by%20ref%29))
  ;[1 1 1] Collision Logic
  (Utilities|FlowControl|Sequence
    (:then_0
      (bind _asbp_bullet (Utilities|Casting|CastToBP_Bullet OtherActor))
      (Actor|DestroyActor _asbp_bullet)
      (if (not (Variables|Default|GetIsDead))
        (CallFunction|DamageSytsem (Variables|/Game/SetchOnLegs/00Blueprint/07Spike/BP_Spike.BP_Spike_C|GetBulletDamage (Variables|Default|GetPlayer)))
        (Audio|PlaySound2D "/Game/SetchOnLegs/03Audio/07Spike/EnemyHit.EnemyHit" 1.0 1.0 0.0 0 0)))
    (:then_1
      (bind _asbp_spike (Utilities|Casting|CastToBP_Spike OtherActor))
      (if (Utilities|Enum|NotEqual(Enum) (Variables|/Game/SetchOnLegs/00Blueprint/07Spike/BP_Spike.BP_Spike_C|GetState _asbp_spike) "NewEnumerator5")
        (Default|DamageSystem _asbp_spike 1)))))

(event OnComponentEndOverlap(WakeSphere)
  (params (OverlappedComponent :type Primitive%20Component%20Object%20Reference) (OtherActor :type Actor%20Object%20Reference) (OtherComp :type Primitive%20Component%20Object%20Reference) (OtherBodyIndex :type Integer))
  ;[1 1 1] Wake Sphere Logic
  (Utilities|Casting|CastToBP_Spike OtherActor)
  (Variables|/Script/Engine.ProjectileMovementComponent|SetbIsHomingProjectile (Variables|Default|GetProjectileMovement) false)
  (Components|Movement|StopMovementImmediately (Variables|Default|GetProjectileMovement)))

(event Custom|Blink
  (bind _bat (Variables|Default|GetBat))
  ;[1 1 1] Damage & Death System
  (Development|SetHiddeninGame _bat (not (Variables|/Script/Engine.SceneComponent|GetbHiddenInGame _bat)) false))

(event Custom|Damage%20Sytsem
  (params (DamageIn :type Float%20%28single-precision%29))
  ;[1 1 1] Damage & Death System
  (bind _output_get (Variables|Default|SetCurrentHealth (- (Variables|Default|GetCurrentHealth) DamageIn)))
  (if (<= _output_get 0.0)
    (Variables|Default|SetIsDead true)
    (Actor|DestroyActor)
    (else
      (Utilities|Time|SetTimerbyFunctionName 0 "Blink" 0.05 true)
      (Utilities|FlowControl|Delay 0.2)
      (Utilities|Time|ClearTimerbyFunctionName 0 "Blink")
      (Development|SetHiddeninGame (Variables|Default|GetBat) false false))))

(event EventBeginPlay
  ;[1 1 1] Move towards Spike
  (bind _asbp_spike (Utilities|Casting|CastToBP_Spike (Game|GetPlayerCharacter 0)))
  (bind _output_get (Variables|Default|SetPlayer _asbp_spike))
  (Variables|/Script/Engine.ProjectileMovementComponent|SetbIsHomingProjectile (Variables|Default|GetProjectileMovement) true)
  (Variables|/Script/Engine.ProjectileMovementComponent|SetHomingTargetComponent (Variables|Default|GetProjectileMovement) (Variables|/Script/Engine.Character|GetCapsuleComponent _output_get))
  (Variables|/Script/Engine.ProjectileMovementComponent|SetHomingAccelerationMagnitude (Variables|Default|GetProjectileMovement) 7.5e+02)
  (Variables|/Script/Engine.ProjectileMovementComponent|SetMaxSpeed (Variables|Default|GetProjectileMovement) 2.5e+02))

(event EventTick
  (params (DeltaSeconds :type Float%20%28single-precision%29))
  (bind _pointlight (Variables|Default|GetPointLight))
  ;[1 1 1] Rotate according to position
  (bind _asbp_spike (Utilities|Casting|CastToBP_Spike (Game|GetPlayerCharacter 0)))
  (if (> (.x (Transformation|GetActorLocation _asbp_spike)) (.x (Transformation|GetActorLocation)))
    (Transformation|SetActorRotation "0,180.000000, 0")
    (Transformation|SetRelativeLocation _pointlight "0,-80.000000, 0" false false)
    (else
      (Transformation|SetActorRotation "0, 0, 0")
      (Transformation|SetRelativeLocation _pointlight "0.000000,80.000000, 0" false false))))

(fn ConstructionScript)
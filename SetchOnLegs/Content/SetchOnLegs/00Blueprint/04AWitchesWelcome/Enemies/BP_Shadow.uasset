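; BP_Shadow is a flipbook-sprite enemy that rises, switches to a chasing state and dies when its health system reports death.
; A State enum selects the rise, chase or death animation, with chasing set one second after BeginPlay.
; It extends parent damage logic, disabling its HitBox on death, and calls SetRotation every tick.
; HitBox overlaps trigger bullet-hit handling or deal damage to BP_Spike actors, each with a sound.
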(event OnComponentBeginOverlap(HitBox)
  (params (OverlappedComponent :type Primitive%20Component%20Object%20Reference) (OtherActor :type Actor%20Object%20Reference) (OtherComp :type Primitive%20Component%20Object%20Reference) (OtherBodyIndex :type Integer) (bFromSweep :type Boolean) (SweepResult :type Hit%20Result%20Structure%20%28by%20ref%29))
  ;[1 1 1] Bullet Collision
  (Utilities|FlowControl|Sequence
    (:then_0
      (Utilities|Casting|CastToBP_Bullet OtherActor)
      (CallFunction|BulletCollision)
      (Audio|PlaySound2D "/Game/SetchOnLegs/03Audio/07Spike/EnemyHit.EnemyHit" 1.0 1.0 0.0 0 0))
    (:then_1
      (bind _asbp_spike (Utilities|Casting|CastToBP_Spike OtherActor))
      (Default|DamageSystem _asbp_spike 1)
      (Audio|PlaySound2D "/Game/SetchOnLegs/03Audio/08Misc/Fire.Fire" 1.0 1.0 0.0 0 0))))

(event Custom|UpdateAnimation
  (bind _sprite (Variables|Default|GetSprite))
  ;[1 1 1] Update Animation
  (switch Utilities|FlowControl|Switch|SwitchonShadowState (Variables|Default|GetState)
    (:NewEnumerator0
      (Sprite|SetFlipbook (Variables|Default|GetSprite) "/Game/SetchOnLegs/01Sprites/04AWitchesWelcome/Shadow/A_ShadowRise.A_ShadowRise"))
    (:NewEnumerator1
      (Sprite|SetFlipbook _sprite "/Game/SetchOnLegs/01Sprites/04AWitchesWelcome/Shadow/A_ShadowChase.A_ShadowChase"))
    (:NewEnumerator2
      (Sprite|SetFlipbook _sprite "/Game/SetchOnLegs/01Sprites/04AWitchesWelcome/Shadow/A_ShadowDeath.A_ShadowDeath"))))

(event EventTick
  (params (DeltaSeconds :type Float%20%28single-precision%29))
  ;[1 1 1] Movement Logic
  (CallFunction|SetRotation))

(event EventBeginPlay
  ;[1 1 1] Movement Logic
  (|CallParentFunction)
  (Variables|Default|SetActive true)
  (Variables|/Script/Engine.CharacterMovementComponent|SetMaxWalkSpeed (Variables|Character|GetCharacterMovement) (Variables|Default|GetWalkSpeed))
  (Utilities|FlowControl|Delay 1.0)
  (Variables|Default|SetState "NewEnumerator1")
  (CallFunction|UpdateAnimation))

(event EventDamageSystem
  (params (DamageIn :type Float%20%28single-precision%29))
  ;[1 1 1] Damage & Death System
  (|CallParentFunction DamageIn)
  (if (Variables|Default|GetIsDead)
    (Variables|Default|SetState "NewEnumerator2")
    (CallFunction|UpdateAnimation)
    (Collision|SetCollisionEnabled (Variables|Default|GetHitBox) "NoCollision")))

(fn ConstructionScript)
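; Wicked Witch boss: a flipbook-animated flying character that fights the player (BP_Spike) with spell orbs and fireballs.
; StartFight adds the HUD and begins a delay-driven loop alternating SpellAttack and FireballAttack.
; Tick updates facing and launch vectors, triggers two health-based phases that quicken attacks and activate bat spawners, then minions, and clears spawned hazards on death.
; Head and body hits deal damage; the shield blocks non-piercing bullets and knocks back the player.
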(event OnComponentBeginOverlap(BodyBox)
  (params (OverlappedComponent :type Primitive%20Component%20Object%20Reference) (OtherActor :type Actor%20Object%20Reference) (OtherComp :type Primitive%20Component%20Object%20Reference) (OtherBodyIndex :type Integer) (bFromSweep :type Boolean) (SweepResult :type Hit%20Result%20Structure%20%28by%20ref%29))
  ;[1 1 1] Collision Logic
  (bind _asbp_bullet (Utilities|Casting|CastToBP_Bullet OtherActor))
  (Actor|DestroyActor _asbp_bullet)
  (if (not (Variables|Default|GetIsDead))
    (CallFunction|DamageSytsem (Variables|/Game/SetchOnLegs/00Blueprint/07Spike/BP_Spike.BP_Spike_C|GetBulletDamage (Variables|Default|GetPlayer)))))

(event OnComponentBeginOverlap(HeadSphere)
  (params (OverlappedComponent :type Primitive%20Component%20Object%20Reference) (OtherActor :type Actor%20Object%20Reference) (OtherComp :type Primitive%20Component%20Object%20Reference) (OtherBodyIndex :type Integer) (bFromSweep :type Boolean) (SweepResult :type Hit%20Result%20Structure%20%28by%20ref%29))
  ;[1 1 1] Collision Logic
  (bind _asbp_bullet (Utilities|Casting|CastToBP_Bullet OtherActor))
  (Actor|DestroyActor _asbp_bullet)
  (if (not (Variables|Default|GetIsDead))
    (CallFunction|DamageSytsem (Variables|/Game/SetchOnLegs/00Blueprint/07Spike/BP_Spike.BP_Spike_C|GetBulletDamage (Variables|Default|GetPlayer)))))

(event OnComponentBeginOverlap(ShieldSphere)
  (params (OverlappedComponent :type Primitive%20Component%20Object%20Reference) (OtherActor :type Actor%20Object%20Reference) (OtherComp :type Primitive%20Component%20Object%20Reference) (OtherBodyIndex :type Integer) (bFromSweep :type Boolean) (SweepResult :type Hit%20Result%20Structure%20%28by%20ref%29))
  ;[1 1 1] Collision Logic
  (Utilities|FlowControl|Sequence
    (:then_0
      (bind _asbp_bullet (Utilities|Casting|CastToBP_Bullet OtherActor))
      (if (Variables|Default|GetShielded)
        (if (not (Variables|/Game/SetchOnLegs/00Blueprint/07Spike/BP_Spike.BP_Spike_C|GetShieldPiercing (Variables|Default|GetPlayer)))
          (Actor|DestroyActor _asbp_bullet))))
    (:then_1
      (bind _asbp_spike (Utilities|Casting|CastToBP_Spike OtherActor))
      (if (Variables|/Game/SetchOnLegs/00Blueprint/07Spike/BP_Spike.BP_Spike_C|GetBossFight _asbp_spike)
        (if (Variables|Default|GetShielded)
          (Character|LaunchCharacter (Variables|Default|GetPlayer) (Variables|Default|GetShieldLaunchVelocity) true true)
          (Default|DamageSystem (Variables|Default|GetPlayer) 1))))))

(event Custom|Blink
  (bind _sprite (Variables|Default|GetSprite))
  ;[1 1 1] Damage & Death System
  (Development|SetHiddeninGame _sprite (not (Variables|/Script/Engine.SceneComponent|GetbHiddenInGame _sprite)) false))

(event Custom|Damage%20Sytsem
  (params (DamageIn :type Float%20%28single-precision%29))
  ;[1 1 1] Damage & Death System
  (bind _output_get (Variables|Default|SetCurrentHealth (- (Variables|Default|GetCurrentHealth) DamageIn)))
  (if (<= _output_get 0.0)
    (Variables|Default|SetState "NewEnumerator3")
    (Variables|Default|SetIsDead true)
    (Widget|RemovefromParent (Variables|Default|GetHUD))
    (Transformation|SetRelativeScale3D (Variables|Default|GetSprite) "3.000000,3.000000,3.000000")
    (CallFunction|UpdateAnimation)
    (Audio|PlaySound2D "/Game/SetchOnLegs/03Audio/04AWitchesWelcome/WickedWitchDeath.WickedWitchDeath" 1.0 1.0 0.0 0 0)
    (Variables|/Script/Engine.MovementComponent|SetVelocity (Variables|Character|GetCharacterMovement) "0, 0, 0")
    (Components|Movement|StopMovementImmediately (Variables|Character|GetCharacterMovement))
    (Rendering|SetVisibility (Variables|Default|GetShield) false false)
    (Utilities|FlowControl|Delay 6.0)
    (Actor|DestroyActor)
    (else
      (Utilities|Time|SetTimerbyFunctionName 0 "Blink" 0.05 true)
      (Utilities|FlowControl|Delay 0.2)
      (Utilities|Time|ClearTimerbyFunctionName 0 "Blink")
      (Development|SetHiddeninGame (Variables|Default|GetSprite) false false))))

(event Custom|UpdateAnimation
  ;[1 1 1] Handle Animation
  (switch Utilities|FlowControl|Switch|SwitchonEnum_WickedWitchState (Variables|Default|GetState)
    (:NewEnumerator0
      (Sprite|SetFlipbook (Variables|Default|GetSprite) "/Game/SetchOnLegs/01Sprites/04AWitchesWelcome/Character/Animations/A_WickedWitchFlying.A_WickedWitchFlying"))
    (:NewEnumerator1
      (Sprite|SetFlipbook (Variables|Default|GetSprite) "/Game/SetchOnLegs/01Sprites/04AWitchesWelcome/Character/Animations/A_WickedWitchThrowing.A_WickedWitchThrowing"))
    (:NewEnumerator3
      (Sprite|SetFlipbook (Variables|Default|GetSprite) "/Game/SetchOnLegs/01Sprites/04AWitchesWelcome/Character/Death/A_WickedWitchDeath.A_WickedWitchDeath"))))

(event Custom|StartFight
  (bind _returnvalue (UserInterface|CreateWidget "/Game/SetchOnLegs/00Blueprint/04AWitchesWelcome/Boss/Widget_WickedWitch.Widget_WickedWitch_C"))
  (bind _output_get (Variables|Default|SetHUD _returnvalue))
  (UserInterface|Viewport|AddtoViewport _output_get 0)
  (Utilities|FlowControl|Delay (Variables|Default|GetAttackDelay))
  (CallFunction|SpellAttack))

(event Custom|FireballAttack
  ;[1 1 1] Fireball Attack
  (if (not (Variables|Default|GetIsDead))
    (Utilities|FlowControl|Delay 0.5)
    (Audio|PlaySound2D "/Game/SetchOnLegs/03Audio/04AWitchesWelcome/Cackle.Cackle" 1.0 1.0 0.0 0 0)
    (Utilities|ForLoopwithDelay 0 (- (Variables|Default|GetFireballCount) 1) :!label _label
      (:Loop%20Body
        (Game|SpawnActorfromClass "/Game/SetchOnLegs/00Blueprint/04AWitchesWelcome/Boss/BP_Flameball.BP_Flameball_C" (Math|Transform|MakeTransform (Transformation|GetWorldLocation (Variables|Default|GetFireballSpawn)) "0, 0, 0" "1,1,1") "Undefined" 0 0))
      (:Completed
        (Utilities|FlowControl|Delay (Variables|Default|GetAttackDelay))
        (CallFunction|SpellAttack))
      (:Delay%20Out
        (Utilities|FlowControl|Delay 0.25)
        (goto _label Delay%20In)))))

(event Custom|SpellAttack
  ;[1 1 1] Spell Attack
  (if (not (Variables|Default|GetIsDead))
    (Variables|Default|SetState "NewEnumerator1")
    (CallFunction|UpdateAnimation)
    (Utilities|FlowControl|Delay 0.45)
    (Game|SpawnActorfromClass "/Game/SetchOnLegs/00Blueprint/04AWitchesWelcome/Boss/BP_SpellOrb.BP_SpellOrb_C" (Transformation|GetWorldTransform (Variables|Default|GetSpellSpawn)) "Undefined" 0 (Variables|Default|GetOrbLaunchVelocity) 0)
    (Audio|PlaySound2D "/Game/SetchOnLegs/03Audio/04AWitchesWelcome/Cackle.Cackle" 1.0 1.0 0.0 0 0)
    (Variables|Default|SetState "NewEnumerator0")
    (CallFunction|UpdateAnimation)
    (Utilities|FlowControl|Delay (Variables|Default|GetAttackDelay))
    (CallFunction|FireballAttack)))

(event Custom|SetCharacterRotation
  (bind _spellspawn (Variables|Default|GetSpellSpawn))
  (bind _fireballspawn (Variables|Default|GetFireballSpawn))
  ;[1 1 1] Set Character Rotation
  (if (>= (.x (Variables|/Script/Engine.MovementComponent|GetVelocity (Variables|Character|GetCharacterMovement))) 0.0)
    (Transformation|SetActorRotation "0, 0, 0")
    (Transformation|SetRelativeLocation _spellspawn "58.000000,0.100000,-96.000000" false false)
    (Transformation|SetRelativeLocation _fireballspawn "12.000000,-0.100000,-96.000000" false false)
    (else
      (Transformation|SetActorRotation "0,180.000000, 0")
      (Transformation|SetRelativeLocation _spellspawn "58.000000,-0.100000,-96.000000" false false)
      (Transformation|SetRelativeLocation _fireballspawn "12.000000,0.100000,-96.000000" false false))))

(event Custom|SetShieldLaunchVelocity
  ;[1 1 1] Set Shield Launch Velocity
  (Utilities|FlowControl|Sequence
    (:then_0
      (if (> (.x (Transformation|GetActorLocation (Variables|Default|GetPlayer))) (.x (Transformation|GetActorLocation)))
        (Variables|Default|SetShieldLaunchVelocity (Math|Vector|MakeVector (Variables|Default|GetShieldLaunchPower) 0.0 (.z (Variables|Default|GetShieldLaunchVelocity))))
        (else
          (Variables|Default|SetShieldLaunchVelocity (Math|Vector|MakeVector (* (Variables|Default|GetShieldLaunchPower) -1.0) 0.0 (.z (Variables|Default|GetShieldLaunchVelocity)))))))
    (:then_1
      (if (> (.z (Transformation|GetActorLocation (Variables|Default|GetPlayer))) (.z (Transformation|GetActorLocation)))
        (Variables|Default|SetShieldLaunchVelocity (Math|Vector|MakeVector (.x (Variables|Default|GetShieldLaunchVelocity)) 0.0 (Variables|Default|GetShieldLaunchPower)))
        (else
          (Variables|Default|SetShieldLaunchVelocity (Math|Vector|MakeVector (.x (Variables|Default|GetShieldLaunchVelocity)) 0.0 (* (Variables|Default|GetShieldLaunchPower) -1.0))))))))

(event Custom|SetOrbLaunchVelocity
  ;[1 1 1] Set Orb Launch Velocity
  (if (Math|Rotator|Equal(Rotator) (Transformation|GetActorRotation) "0, 0, 0" 0.0001)
    (Variables|Default|SetOrbLaunchVelocity "500.000000,0.000000,-500.000000")
    (else
      (Variables|Default|SetOrbLaunchVelocity "-500.000000,0.000000,-500.000000"))))

(event EventBeginPlay
  ;[1 1 1] Initialise
  (Variables|Default|SetState "NewEnumerator0")
  (CallFunction|UpdateAnimation)
  (bind _asbp_spike (Utilities|Casting|CastToBP_Spike (Game|GetPlayerCharacter 0)))
  (Variables|Default|SetPlayer _asbp_spike))

(event EventTick
  (params (DeltaSeconds :type Float%20%28single-precision%29))
  ;[1 1 1] Tick
  (Utilities|FlowControl|Sequence
    (:then_0
      (CallFunction|SetCharacterRotation)
      (CallFunction|SetShieldLaunchVelocity)
      (CallFunction|SetOrbLaunchVelocity))
    (:then_1
      (if (Math|Float|InRange(Float) (Variables|Default|GetCurrentHealth) 101.0 2e+02)
        (Utilities|FlowControl|DoOnce false
          (:Completed
            (Variables|Default|SetAttackDelay 2.75)
            (Variables|Default|SetFireballCount 4)
            (bind _outactors (Actor|GetAllActorsOfClass "/Game/SetchOnLegs/00Blueprint/04AWitchesWelcome/BP_BatSpawner.BP_BatSpawner_C"))
            (for _array_element _outactors
              (Variables|/Game/SetchOnLegs/00Blueprint/04AWitchesWelcome/BP_BatSpawner.BP_BatSpawner_C|SetActive _array_element true))))))
    (:then_2
      (if (Math|Float|InRange(Float) (Variables|Default|GetCurrentHealth) 1.0 1e+02)
        (Utilities|FlowControl|DoOnce false
          (:Completed
            (Variables|Default|SetAttackDelay 2.5)
            (Variables|Default|SetFireballCount 5)
            (bind _outactors_2 (Actor|GetAllActorsOfClass "/Game/SetchOnLegs/00Blueprint/04AWitchesWelcome/Enemies/BP_Minion.BP_Minion_C"))
            (for _array_element_2 _outactors_2
              (Variables|/Game/SetchOnLegs/00Blueprint/04AWitchesWelcome/Enemies/BP_Minion.BP_Minion_C|SetActive _array_element_2 true))))))
    (:then_3
      (if (Variables|Default|GetIsDead)
        (Utilities|FlowControl|DoOnce false
          (:Completed
            (bind _outactors_3 (Actor|GetAllActorsOfClass "/Game/SetchOnLegs/00Blueprint/04AWitchesWelcome/Enemies/BP_Minion.BP_Minion_C"))
            (Actor|DestroyActor _outactors_3)
            (bind _outactors_4 (Actor|GetAllActorsOfClass "/Game/SetchOnLegs/00Blueprint/04AWitchesWelcome/Boss/BP_Flameball.BP_Flameball_C"))
            (Actor|DestroyActor _outactors_4)
            (bind _outactors_5 (Actor|GetAllActorsOfClass "/Game/SetchOnLegs/00Blueprint/04AWitchesWelcome/BP_Orb.BP_Orb_C"))
            (Actor|DestroyActor _outactors_5)
            (bind _outactors_6 (Actor|GetAllActorsOfClass "/Game/SetchOnLegs/00Blueprint/04AWitchesWelcome/BP_BatSpawner.BP_BatSpawner_C"))
            (Actor|DestroyActor _outactors_6)
            (bind _outactors_7 (Actor|GetAllActorsOfClass "/Game/SetchOnLegs/00Blueprint/04AWitchesWelcome/Enemies/BP_Bat.BP_Bat_C"))
            (Actor|DestroyActor _outactors_7)
            (bind _outactors_8 (Actor|GetAllActorsOfClass "/Game/SetchOnLegs/00Blueprint/04AWitchesWelcome/Boss/BP_SpellOrb.BP_SpellOrb_C"))
            (Actor|DestroyActor _outactors_8)))))))

(fn ConstructionScript)

(fn SetSpeed
  (params (XSpeed :type Float%20%28single-precision%29) (ZSpeed :type Float%20%28single-precision%29))
  (Variables|/Script/Engine.MovementComponent|SetVelocity (Variables|Character|GetCharacterMovement) (Math|Vector|MakeVector XSpeed 0.0 ZSpeed)))
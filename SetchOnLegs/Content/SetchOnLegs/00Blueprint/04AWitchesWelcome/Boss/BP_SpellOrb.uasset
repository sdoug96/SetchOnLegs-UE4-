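; BP_SpellOrb is a boss-fight projectile that inflicts a random spell effect on BP_Spike, the player.
; On spawn it picks slow, reversed movement, poison or damage, tints its sprite to match and starts a 30-second self-destruct timer.
; Overlapping a BP_MapBoundary bounces it by flipping X or Z velocity according to the boundary type.
; Overlapping the player calls the matching effect function and destroys the orb.
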(event OnComponentBeginOverlap(SpriteHitSphere)
  (params (OverlappedComponent :type Primitive%20Component%20Object%20Reference) (OtherActor :type Actor%20Object%20Reference) (OtherComp :type Primitive%20Component%20Object%20Reference) (OtherBodyIndex :type Integer) (bFromSweep :type Boolean) (SweepResult :type Hit%20Result%20Structure%20%28by%20ref%29))
  (bind _projectilemovement (Variables|Default|GetProjectileMovement))
  ;[1 1 1] Collision Logic
  (Utilities|FlowControl|Sequence
    (:then_0
      (bind _asbp_map_boundary (Utilities|Casting|CastToBP_MapBoundary OtherActor))
      (switch Utilities|FlowControl|Switch|SwitchonBoundaryType (Variables|/Game/SetchOnLegs/00Blueprint/12Misc/Core/BP_MapBoundary.BP_MapBoundary_C|GetBoundaryType _asbp_map_boundary)
        (:NewEnumerator0
          (Variables|/Script/Engine.MovementComponent|SetVelocity _projectilemovement (Math|Vector|MakeVector (.x (Variables|/Script/Engine.MovementComponent|GetVelocity (Variables|Default|GetProjectileMovement))) 0.0 (* (.z (Variables|/Script/Engine.MovementComponent|GetVelocity (Variables|Default|GetProjectileMovement))) -1.0))))
        (:NewEnumerator1
          (Variables|/Script/Engine.MovementComponent|SetVelocity _projectilemovement (Math|Vector|MakeVector (* (.x (Variables|/Script/Engine.MovementComponent|GetVelocity (Variables|Default|GetProjectileMovement))) -1.0) 0.0 (.z (Variables|/Script/Engine.MovementComponent|GetVelocity (Variables|Default|GetProjectileMovement))))))))
    (:then_1
      (bind _asbp_spike (Utilities|Casting|CastToBP_Spike OtherActor))
      (Variables|Default|SetPlayer _asbp_spike)
      (switch Utilities|FlowControl|Switch|SwitchonEnum_SpellType (Variables|Default|GetSpellType)
        (:NewEnumerator0
          (Default|SlowMovement (Variables|Default|GetPlayer)))
        (:NewEnumerator1
          (Default|ReverseMovement (Variables|Default|GetPlayer)))
        (:NewEnumerator2
          (Default|Poison (Variables|Default|GetPlayer)))
        (:NewEnumerator3
          (Default|DamageSystem (Variables|Default|GetPlayer) 1)))
      (Actor|DestroyActor))))

(event EventBeginPlay
  (bind _sprite (Variables|Default|GetSprite))
  ;[1 1 1] Set Spell Type & Colour
  (Utilities|FlowControl|Sequence
    (:then_0
      (Utilities|FlowControl|Delay 3e+01)
      (Actor|DestroyActor))
    (:then_1
      (switch int (Math|Random|RandomIntegerinRange 0 3)
        (:0
          (Variables|Default|SetSpellType "NewEnumerator0")
          (Sprite|SetSpriteColor (Variables|Default|GetSprite) "(R=0.000000,G=1.000000,B=0.000000,A=1.000000)"))
        (:1
          (Variables|Default|SetSpellType "NewEnumerator1")
          (Sprite|SetSpriteColor _sprite "(R=0.000000,G=0.000000,B=1.000000,A=1.000000)"))
        (:2
          (Variables|Default|SetSpellType "NewEnumerator2")
          (Sprite|SetSpriteColor _sprite "(R=0.750000,G=0.000000,B=1.000000,A=1.000000)"))
        (:3
          (Variables|Default|SetSpellType "NewEnumerator3")
          (Sprite|SetSpriteColor (Variables|Default|GetSprite) "(R=1.000000,G=0.000000,B=0.000000,A=1.000000)"))))))

(fn ConstructionScript)
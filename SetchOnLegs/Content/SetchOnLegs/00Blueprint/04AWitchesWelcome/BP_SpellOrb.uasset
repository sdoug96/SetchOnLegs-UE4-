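; BP_SpellOrb is a bouncing spell projectile that picks one of four colour-coded effects at spawn: slow, reversed movement, poison or damage.
; Overlapping BP_MapBoundary flips the X or Z component of OrbVelocity, which Tick reapplies to ProjectileMovement while spinning the orb.
; Overlapping BP_Spike, the player, calls the matching effect function and destroys the orb, which otherwise expires after a fixed delay.
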(event OnComponentBeginOverlap(HitSphere)
  (params (OverlappedComponent :type Primitive%20Component%20Object%20Reference) (OtherActor :type Actor%20Object%20Reference) (OtherComp :type Primitive%20Component%20Object%20Reference) (OtherBodyIndex :type Integer) (bFromSweep :type Boolean) (SweepResult :type Hit%20Result%20Structure%20%28by%20ref%29))
  (bind _projectilemovement (Variables|Default|GetProjectileMovement))
  (bind _projectilemovement_2 (Variables|Default|GetProjectileMovement))
  (bind _velocity (Variables|/Script/Engine.MovementComponent|GetVelocity _projectilemovement_2))
  (bind _velocity_2 (Variables|/Script/Engine.MovementComponent|GetVelocity _projectilemovement))
  (Utilities|FlowControl|Sequence
    (:then_0
      (bind _asbp_map_boundary (Utilities|Casting|CastToBP_MapBoundary OtherActor))
      (switch Utilities|FlowControl|Switch|SwitchonBoundaryType (Variables|/Game/SetchOnLegs/00Blueprint/12Misc/BP_MapBoundary.BP_MapBoundary_C|GetBoundaryType _asbp_map_boundary)
        (:NewEnumerator0
          (Variables|Default|SetOrbVelocity (Math|Vector|MakeVector (.x _velocity) 0.0 (* (.z _velocity) -1.0))))
        (:NewEnumerator1
          (Variables|Default|SetOrbVelocity (Math|Vector|MakeVector (* (.x _velocity_2) -1.0) 0.0 (.z _velocity_2))))))
    (:then_1
      (bind _asbp_spike (Utilities|Casting|CastToBP_Spike OtherActor))
      (Variables|Default|SetPlayer _asbp_spike)
      (switch Utilities|FlowControl|Switch|SwitchonEnum_SpellType (Variables|Default|GetSpellType)
        (:NewEnumerator0
          (Default|SlowMovement (Variables|Default|GetPlayer)))
        (:NewEnumerator1
          (Default|ReverseMovement (Variables|Default|GetPlayer)))
        (:NewEnumerator2
          (Default|PoisonSpike (Variables|Default|GetPlayer)))
        (:NewEnumerator3
          (Default|DamageSytsem (Variables|Default|GetPlayer) 1)))
      (Actor|DestroyActor))))

(event EventTick
  (params (DeltaSeconds :type Float%20%28single-precision%29))
  ;[1 1 1] Set Velocity & Rotation
  (Utilities|FlowControl|Sequence
    (:then_0
      (Variables|/Script/Engine.MovementComponent|SetVelocity (Variables|Default|GetProjectileMovement) (Variables|Default|GetOrbVelocity)))
    (:then_1
      (Variables|Default|SetTimer (+ DeltaSeconds (Variables|Default|GetTimer)))
      (Transformation|SetActorRotation (Math|Rotator|MakeRotator 0.0 (* (Variables|Default|GetTimer) (Variables|Default|GetRotation)) 0.0)))))

(event EventBeginPlay
  (bind _orb (Variables|Default|GetOrb))
  (Utilities|FlowControl|Sequence
    (:then_0
      (Utilities|FlowControl|Delay 3e+01)
      (Actor|DestroyActor))
    (:then_1
      (switch int (Math|Random|RandomIntegerinRange 0 3)
        (:0
          (Variables|Default|SetSpellType "NewEnumerator0")
          (Sprite|SetSpriteColor (Variables|Default|GetOrb) "(R=0.000000,G=1.000000,B=0.000000,A=1.000000)"))
        (:1
          (Variables|Default|SetSpellType "NewEnumerator1")
          (Sprite|SetSpriteColor _orb "(R=0.000000,G=0.000000,B=1.000000,A=1.000000)"))
        (:2
          (Variables|Default|SetSpellType "NewEnumerator2")
          (Sprite|SetSpriteColor _orb "(R=0.750000,G=0.000000,B=1.000000,A=1.000000)"))
        (:3
          (Variables|Default|SetSpellType "NewEnumerator3")
          (Sprite|SetSpriteColor (Variables|Default|GetOrb) "(R=1.000000,G=0.000000,B=0.000000,A=1.000000)"))))))

(fn ConstructionScript)
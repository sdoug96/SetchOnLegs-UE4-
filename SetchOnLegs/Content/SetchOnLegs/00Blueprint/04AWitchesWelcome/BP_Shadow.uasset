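; BP_Shadow is a flipbook-animated enemy that plays a rise animation, switches to walking, and chases BP_Spike along the X axis, turning to face the player.
; Its hitbox consumes normal and charged bullets, taking damage amounts read from the player.
; Hits make the sprite blink via a looping timer, while death plays the rise flipbook backwards before destruction.
; Touching Spike outside one exempt state damages the player and destroys the shadow.
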(event OnComponentBeginOverlap(HitBox)
  (params (OverlappedComponent :type Primitive%20Component%20Object%20Reference) (OtherActor :type Actor%20Object%20Reference) (OtherComp :type Primitive%20Component%20Object%20Reference) (OtherBodyIndex :type Integer) (bFromSweep :type Boolean) (SweepResult :type Hit%20Result%20Structure%20%28by%20ref%29))
  ;[1 1 1] Hitbox logic
  (Utilities|FlowControl|Sequence
    (:then_0
      (bind _asbp_bullet (Utilities|Casting|CastToBP_Bullet OtherActor))
      (Actor|DestroyActor _asbp_bullet)
      (if (not (Variables|Default|GetIsDead))
        (bind _asbp_spike (Utilities|Casting|CastToBP_Spike (Game|GetPlayerCharacter 0)))
        (CallFunction|DamageSytsem (Variables|/Game/SetchOnLegs/00Blueprint/07Spike/BP_Spike.BP_Spike_C|GetBulletDamage _asbp_spike))))
    (:then_1
      (bind _asbp_charged_bullet (Utilities|Casting|CastToBP_ChargedBullet OtherActor))
      (Actor|DestroyActor _asbp_charged_bullet)
      (if (not (Variables|Default|GetIsDead))
        (bind _asbp_spike_2 (Utilities|Casting|CastToBP_Spike (Game|GetPlayerCharacter 0)))
        (CallFunction|DamageSytsem (Variables|/Game/SetchOnLegs/00Blueprint/07Spike/BP_Spike.BP_Spike_C|GetChargedShotDamage _asbp_spike_2))))
    (:then_2
      (bind _asbp_spike_3 (Utilities|Casting|CastToBP_Spike OtherActor))
      (if (Utilities|Enum|NotEqual(Enum) (Variables|/Game/SetchOnLegs/00Blueprint/07Spike/BP_Spike.BP_Spike_C|GetState _asbp_spike_3) "NewEnumerator5")
        (Default|DamageSytsem _asbp_spike_3 1)
        (Actor|DestroyActor)))))

(event Custom|Blink
  (bind _sprite (Variables|Default|GetSprite))
  ;[1 1 1] Damage & Death System
  (Development|SetHiddeninGame _sprite (not (Variables|/Script/Engine.SceneComponent|GetbHiddenInGame _sprite)) false))

(event Custom|Damage%20Sytsem
  (params (DamageIn :type Float%20%28single-precision%29))
  ;[1 1 1] Damage & Death System
  (bind _output_get (Variables|Default|SetCurrentHealth (- (Variables|Default|GetCurrentHealth) DamageIn)))
  (if (<= _output_get 0.0)
    (Variables|Default|SetIsDead true)
    (Sprite|SetFlipbook (Variables|Default|GetSprite) "/Game/SetchOnLegs/01Sprites/04AWitchesWelcome/Shadow/A_Rise.A_Rise")
    (Components|Timeline|SetPlayRate (Variables|Default|GetSprite) -1.0)
    (Utilities|FlowControl|Delay 0.4)
    (Actor|DestroyActor)
    (else
      (Utilities|Time|SetTimerbyFunctionName 0 "Blink" 0.05 true)
      (Utilities|FlowControl|Delay 0.2)
      (Utilities|Time|ClearTimerbyFunctionName 0 "Blink")
      (Development|SetHiddeninGame (Variables|Default|GetSprite) false false))))

(event EventBeginPlay
  ;[1 1 1] Initialise
  (Sprite|SetFlipbook (Variables|Default|GetSprite) "/Game/SetchOnLegs/01Sprites/04AWitchesWelcome/Shadow/A_Rise.A_Rise")
  (Utilities|FlowControl|Delay 1.0)
  (Sprite|SetFlipbook (Variables|Default|GetSprite) "/Game/SetchOnLegs/01Sprites/04AWitchesWelcome/Shadow/A_Chase.A_Chase")
  (Pawn|Components|CharacterMovement|SetMovementMode (Variables|Character|GetCharacterMovement) "MOVE_Walking" 0))

(event EventTick
  (params (DeltaSeconds :type Float%20%28single-precision%29))
  ;[1 1 1] Tick
  (bind _asbp_spike (Utilities|Casting|CastToBP_Spike (Game|GetPlayerCharacter 0)))
  (if (> (.x (Transformation|GetActorLocation)) (.x (Transformation|GetActorLocation _asbp_spike)))
    (Transformation|SetActorRotation "0, 0, 0")
    (Pawn|Input|AddMovementInput "-1.000000, 0, 0" 1.0 false)
    (else
      (Transformation|SetActorRotation "0,180.000000, 0")
      (Pawn|Input|AddMovementInput "1.000000, 0, 0" 1.0 false))))

(fn ConstructionScript)
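; BP_Minion is an orb shooter that spawns a BP_Orb at its OrbSpawn component on a repeating timer.
; BeginPlay caches the player as BP_Spike and, only if that cast succeeds, starts a looping FireOrb timer at FireDelay intervals.
; Each FireOrb tick spawns only while Active is set, with an optional 2D sound gated by the Sound flag.
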(event Custom|FireOrb
  ;[1 1 1] Spawn orb every 2 seconds
  (if (Variables|Default|GetActive)
    (Game|SpawnActorfromClass "/Game/SetchOnLegs/00Blueprint/04AWitchesWelcome/BP_Orb.BP_Orb_C" (Transformation|GetWorldTransform (Variables|Default|GetOrbSpawn)) "Undefined" 0 0)
    (if (Variables|Default|GetSound)
      (Audio|PlaySound2D "/Game/SetchOnLegs/03Audio/04AWitchesWelcome/Orb.Orb" 1.0 1.0 0.0 0 0))))

(event EventBeginPlay
  (bind _asbp_spike (Utilities|Casting|CastToBP_Spike (Game|GetPlayerCharacter 0)))
  (Variables|Default|SetPlayer _asbp_spike)
  (Utilities|Time|SetTimerbyFunctionName 0 "FireOrb" (Variables|Default|GetFireDelay) true))

(fn ConstructionScript)
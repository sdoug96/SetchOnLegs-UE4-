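; BP_WickedWitch is a flying boss that fights the BP_Spike player.
; StartFight shows its health HUD, activates minions and starts a self-repeating fireball volley, whose count becomes four within a health band.
; Player bullets deal damage with a timer-driven blink; death swaps the flipbook and destroys the witch after a delay.
; Tick clears spawned hazards on death and queues LevelSelect behind a delay longer than the witch's remaining lifetime.
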(event OnComponentBeginOverlap(BodyBox)
  (params (OverlappedComponent :type Primitive%20Component%20Object%20Reference) (OtherActor :type Actor%20Object%20Reference) (OtherComp :type Primitive%20Component%20Object%20Reference) (OtherBodyIndex :type Integer) (bFromSweep :type Boolean) (SweepResult :type Hit%20Result%20Structure%20%28by%20ref%29))
  ;[1 1 1] Bullet Collision
  (bind _asbp_bullet (Utilities|Casting|CastToBP_Bullet OtherActor))
  (Actor|DestroyActor _asbp_bullet)
  (if (not (Variables|Default|GetIsDead))
    (CallFunction|DamageSytsem (Variables|/Game/SetchOnLegs/00Blueprint/07Spike/BP_Spike.BP_Spike_C|GetBulletDamage (Variables|Default|GetPlayer)))))

(event Custom|Blink
  (bind _sprite (Variables|Default|GetSprite))
  ;[1 1 1] Damage & Death System
  (Development|SetHiddeninGame _sprite (not (Variables|/Script/Engine.SceneComponent|GetbHiddenInGame _sprite)) false))

(event Custom|Damage%20Sytsem
  (params (DamageIn :type Float%20%28single-precision%29))
  ;[1 1 1] Damage & Death System
  (bind _output_get (Variables|Default|SetCurrentHealth (- (Variables|Default|GetCurrentHealth) DamageIn)))
  (if (<= _output_get 0.0)
    (Variables|Default|SetState "NewEnumerator3")
    (Variables|Default|SetIsDead true)
    (Widget|RemovefromParent (Variables|Default|GetHUD))
    (Transformation|SetRelativeScale3D (Variables|Default|GetSprite) "3.000000,3.000000,3.000000")
    (CallFunction|UpdateAnimation)
    (Audio|PlaySound2D "/Game/SetchOnLegs/03Audio/04AWitchesWelcome/WickedWitchDeath.WickedWitchDeath" 1.0 1.0 0.0 0 0)
    (Utilities|FlowControl|Delay 6.0)
    (Actor|DestroyActor)
    (else
      (Utilities|Time|SetTimerbyFunctionName 0 "Blink" 0.05 true)
      (Utilities|FlowControl|Delay 0.2)
      (Utilities|Time|ClearTimerbyFunctionName 0 "Blink")
      (Development|SetHiddeninGame (Variables|Default|GetSprite) false false))))

(event Custom|UpdateAnimation
  ;[1 1 1] Handle Animation
  (switch Utilities|FlowControl|Switch|SwitchonEnum_WickedWitchState (Variables|Default|GetState)
    (:NewEnumerator0
      (Sprite|SetFlipbook (Variables|Default|GetSprite) "/Game/SetchOnLegs/01Sprites/04AWitchesWelcome/Character/Animations/A_WickedWitchFlying.A_WickedWitchFlying"))
    (:NewEnumerator3
      (Sprite|SetFlipbook (Variables|Default|GetSprite) "/Game/SetchOnLegs/01Sprites/04AWitchesWelcome/Character/Death/A_WickedWitchDeath.A_WickedWitchDeath"))))

(event Custom|StartFight
  (bind _returnvalue (UserInterface|CreateWidget "/Game/SetchOnLegs/00Blueprint/04AWitchesWelcome/Widget_WickedWitch.Widget_WickedWitch_C"))
  (bind _output_get (Variables|Default|SetHUD _returnvalue))
  (UserInterface|Viewport|AddtoViewport _output_get 0)
  (Utilities|FlowControl|Delay (Variables|Default|GetAttackDelay))
  (CallFunction|FireballAttack)
  (bind _outactors (Actor|GetAllActorsOfClass "/Game/SetchOnLegs/00Blueprint/04AWitchesWelcome/BP_Minion.BP_Minion_C"))
  (for _array_element _outactors
    (Variables|/Game/SetchOnLegs/00Blueprint/04AWitchesWelcome/BP_Minion.BP_Minion_C|SetActive _array_element true)))

(event Custom|FireballAttack
  ;[1 1 1] Fireball Attack
  (Utilities|ForLoopwithDelay 0 (- (Variables|Default|GetFireballCount) 1) :!label _label
    (:Loop%20Body
      (Game|SpawnActorfromClass "/Game/SetchOnLegs/00Blueprint/04AWitchesWelcome/BP_Flameball.BP_Flameball_C" (Math|Transform|MakeTransform (Transformation|GetWorldLocation (Variables|Default|GetFireballSpawn)) "0, 0, 0" "0.750000,0.750000,0.750000") "Undefined" 0 0))
    (:Completed
      (Utilities|FlowControl|Delay (Variables|Default|GetAttackDelay))
      (CallFunction|FireballAttack))
    (:Delay%20Out
      (Utilities|FlowControl|Delay 0.2)
      (goto _label Delay%20In))))

(event Custom|OrbAttack)

(event EventBeginPlay
  ;[1 1 1] Initialise
  (Variables|Default|SetState "NewEnumerator0")
  (CallFunction|UpdateAnimation)
  (bind _asbp_spike (Utilities|Casting|CastToBP_Spike (Game|GetPlayerCharacter 0)))
  (Variables|Default|SetPlayer _asbp_spike))

(event EventTick
  (params (DeltaSeconds :type Float%20%28single-precision%29))
  ;[1 1 1] Tick
  (Utilities|FlowControl|Sequence
    (:then_0
      (if (Math|Float|InRange(Float) (Variables|Default|GetCurrentHealth) 201.0 4e+02)
        (Variables|Default|SetFireballCount 4)))
    (:then_3
      (if (Variables|Default|GetIsDead)
        (bind _outactors (Actor|GetAllActorsOfClass "/Game/SetchOnLegs/00Blueprint/04AWitchesWelcome/BP_Minion.BP_Minion_C"))
        (Actor|DestroyActor _outactors)
        (bind _outactors_2 (Actor|GetAllActorsOfClass "/Game/SetchOnLegs/00Blueprint/04AWitchesWelcome/BP_Flameball.BP_Flameball_C"))
        (Actor|DestroyActor _outactors_2)
        (bind _outactors_3 (Actor|GetAllActorsOfClass "/Game/SetchOnLegs/00Blueprint/04AWitchesWelcome/BP_Shadow.BP_Shadow_C"))
        (Actor|DestroyActor _outactors_3)
        (bind _outactors_4 (Actor|GetAllActorsOfClass "/Game/SetchOnLegs/00Blueprint/04AWitchesWelcome/BP_Orb.BP_Orb_C"))
        (Actor|DestroyActor _outactors_4)
        (Utilities|FlowControl|Delay 7.0)
        (Game|OpenLevel(byName) "LevelSelect")))))

(fn ConstructionScript)

(fn SetSpeed
  (params (XSpeed :type Float%20%28single-precision%29) (ZSpeed :type Float%20%28single-precision%29))
  (Variables|/Script/Engine.MovementComponent|SetVelocity (Variables|Character|GetCharacterMovement) (Math|Vector|MakeVector XSpeed 0.0 ZSpeed)))
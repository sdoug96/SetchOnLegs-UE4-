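; BP_Flameball is a falling fireball hazard that damages the player character, BP_Spike.
; Each Tick forces its ProjectileMovement velocity straight down at a constant speed.
; A Box overlap with BP_Spike calls its DamageSytsem and destroys the flameball, unless Spike is in one exempt state.
; Otherwise the flameball destroys itself after a short fixed lifetime started on BeginPlay.
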(event OnComponentBeginOverlap(Box)
  (params (OverlappedComponent :type Primitive%20Component%20Object%20Reference) (OtherActor :type Actor%20Object%20Reference) (OtherComp :type Primitive%20Component%20Object%20Reference) (OtherBodyIndex :type Integer) (bFromSweep :type Boolean) (SweepResult :type Hit%20Result%20Structure%20%28by%20ref%29))
  ;[1 1 1] Hit Player
  (bind _asbp_spike (Utilities|Casting|CastToBP_Spike OtherActor))
  (if (Utilities|Enum|NotEqual(Enum) (Variables|/Game/SetchOnLegs/00Blueprint/07Spike/BP_Spike.BP_Spike_C|GetState _asbp_spike) "NewEnumerator5")
    (Default|DamageSytsem _asbp_spike 1)
    (Actor|DestroyActor)))

(event EventBeginPlay
  ;[1 1 1] Kill flame ball after 4 seconds
  (Utilities|FlowControl|Delay 4.0)
  (Actor|DestroyActor))

(event EventTick
  (params (DeltaSeconds :type Float%20%28single-precision%29))
  ;[1 1 1] Set Velocity
  (Variables|/Script/Engine.MovementComponent|SetVelocity (Variables|Default|GetProjectileMovement) "0, 0,-750.000000"))

(fn ConstructionScript)
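; BP_FireballBoy is a giggling moving hazard that damages BP_Spike on contact and destroys itself after six seconds.
; Every tick it sets its ProjectileMovement velocity to MoveSpeed, and on spawn it rotates the FireballBoy component 180 degrees when that speed's X is negative.
; HitSphere overlaps with BP_Spike call its DamageSystem and play a fire sound, without destroying the fireball.
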(event OnComponentBeginOverlap(HitSphere)
  (params (OverlappedComponent :type Primitive%20Component%20Object%20Reference) (OtherActor :type Actor%20Object%20Reference) (OtherComp :type Primitive%20Component%20Object%20Reference) (OtherBodyIndex :type Integer) (bFromSweep :type Boolean) (SweepResult :type Hit%20Result%20Structure%20%28by%20ref%29))
  (bind _asbp_spike (Utilities|Casting|CastToBP_Spike OtherActor))
  (Default|DamageSystem _asbp_spike 1)
  (Audio|PlaySound2D "/Game/SetchOnLegs/03Audio/00Menus/Fire.Fire" 1.0 1.0 0.0 0 0))

(event EventBeginPlay
  (Audio|PlaySound2D "/Game/SetchOnLegs/03Audio/01HinceInHell/Giggle.Giggle" 1.0 1.0 0.0 0 0)
  (Utilities|FlowControl|Sequence
    (:then_0
      (if (< (.x (Variables|Default|GetMoveSpeed)) 0.0)
        (Transformation|SetRelativeRotation (Variables|Default|GetFireballBoy) "0,180.000000, 0" false false)))
    (:then_1
      (Utilities|FlowControl|Delay 6.0)
      (Actor|DestroyActor))))

(event EventTick
  (params (DeltaSeconds :type Float%20%28single-precision%29))
  (Variables|/Script/Engine.MovementComponent|SetVelocity (Variables|Default|GetProjectileMovement) (Variables|Default|GetMoveSpeed)))

(fn ConstructionScript)
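; Flying 2D mini Hince In Hell enemy that chases the BP_Spike player at an offset and shoots fireballs.
; Tick steers it, updates state-driven flipbooks and fires, using a Delay as the attack cooldown.
; Fireballs are aimed in the XZ plane from projected screen positions of enemy and player.
; Bullets hitting either sphere deal the player's damage with a timer-driven blink; death increments the player's kill count, then destroys the actor.
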(event OnComponentBeginOverlap(HitSphere2)
  (params (OverlappedComponent :type Primitive%20Component%20Object%20Reference) (OtherActor :type Actor%20Object%20Reference) (OtherComp :type Primitive%20Component%20Object%20Reference) (OtherBodyIndex :type Integer) (bFromSweep :type Boolean) (SweepResult :type Hit%20Result%20Structure%20%28by%20ref%29))
  ;[1 1 1] Bullet Collision
  (bind _asbp_bullet (Utilities|Casting|CastToBP_Bullet OtherActor))
  (Actor|DestroyActor _asbp_bullet)
  (if (not (Variables|Default|GetIsDead))
    (CallFunction|DamageSytsem (Variables|/Game/SetchOnLegs/00Blueprint/07Spike/BP_Spike.BP_Spike_C|GetBulletDamage (Variables|Default|GetPlayer)))))

(event OnComponentBeginOverlap(HitSphere1)
  (params (OverlappedComponent :type Primitive%20Component%20Object%20Reference) (OtherActor :type Actor%20Object%20Reference) (OtherComp :type Primitive%20Component%20Object%20Reference) (OtherBodyIndex :type Integer) (bFromSweep :type Boolean) (SweepResult :type Hit%20Result%20Structure%20%28by%20ref%29))
  ;[1 1 1] Bullet Collision
  (bind _asbp_bullet (Utilities|Casting|CastToBP_Bullet OtherActor))
  (Actor|DestroyActor _asbp_bullet)
  (if (not (Variables|Default|GetIsDead))
    (CallFunction|DamageSytsem (Variables|/Game/SetchOnLegs/00Blueprint/07Spike/BP_Spike.BP_Spike_C|GetBulletDamage (Variables|Default|GetPlayer)))))

(event Custom|Blink
  (bind _sprite (Variables|Default|GetSprite))
  ;[1 1 1] Damage & Death System
  (Development|SetHiddeninGame _sprite (not (Variables|/Script/Engine.SceneComponent|GetbHiddenInGame _sprite)) false))

(event Custom|Damage%20Sytsem
  (params (DamageIn :type Float%20%28single-precision%29))
  (bind _player (Variables|Default|GetPlayer))
  ;[1 1 1] Damage & Death System
  (bind _output_get (Variables|Default|SetCurrentHealth (- (Variables|Default|GetCurrentHealth) DamageIn)))
  (if (<= _output_get 0.0)
    (Variables|Default|SetState "NewEnumerator2")
    (CallFunction|UpdateAnimation)
    (Variables|Default|SetIsDead true)
    (Variables|/Game/SetchOnLegs/00Blueprint/07Spike/BP_Spike.BP_Spike_C|SetHinceInHellKillCount _player (+ (Variables|/Game/SetchOnLegs/00Blueprint/07Spike/BP_Spike.BP_Spike_C|GetHinceInHellKillCount _player) 1))
    (Utilities|FlowControl|Delay 2.2)
    (Actor|DestroyActor)
    (else
      (Utilities|Time|SetTimerbyFunctionName 0 "Blink" 0.05 true)
      (Utilities|FlowControl|Delay 0.2)
      (Utilities|Time|ClearTimerbyFunctionName 0 "Blink")
      (Development|SetHiddeninGame (Variables|Default|GetSprite) false false))))

(event Custom|UpdateAnimation
  (bind _sprite (Variables|Default|GetSprite))
  ;[1 1 1] Handle Animation
  (switch Utilities|FlowControl|Switch|SwitchonHinceInHellState (Variables|Default|GetState)
    (:NewEnumerator0
      (Sprite|SetFlipbook _sprite "/Game/SetchOnLegs/01Sprites/01HinceInHell/Character/A_HinceInHellMoving.A_HinceInHellMoving"))
    (:NewEnumerator1
      (Sprite|SetFlipbook _sprite "/Game/SetchOnLegs/01Sprites/01HinceInHell/Character/A_HinceInHellAttacking.A_HinceInHellAttacking"))
    (:NewEnumerator2
      (Sprite|SetFlipbook _sprite "/Game/SetchOnLegs/01Sprites/01HinceInHell/Character/A_HinceInHellDead.A_HinceInHellDead"))))

(event Custom|HandleMovement
  ;[1 1 1] Handle Movement
  (Utilities|FlowControl|Delay 0.1)
  (Variables|Default|SetOurPosition (- (Transformation|GetActorLocation) (Variables|Default|GetMoveToPos)))
  (Variables|Default|SetPlayerPosition (Transformation|GetActorLocation (Pawn|GetControlledPawn (Game|GetPlayerController 0))))
  (Pawn|Input|AddMovementInput (- (Variables|Default|GetPlayerPosition) (Variables|Default|GetOurPosition)) 1.0 false))

(event Custom|Shoot
  (bind _fireballspawn (Variables|Default|GetFireballSpawn))
  (bind _returnvalue (Transformation|GetWorldLocation _fireballspawn))
  ;[1 1 1] Shoot Logic
  ;;[1 1 1] Handle Shoot
  (if (not (Variables|Default|GetIsDead))
    (Variables|Default|SetState "NewEnumerator1")
    (CallFunction|UpdateAnimation)
    (Game|SpawnActorfromClass "/Game/SetchOnLegs/00Blueprint/01HinceInHell/Boss/BP_HinceInHellFireball.BP_HinceInHellFireball_C" (Math|Transform|MakeTransform (Math|Vector|MakeVector (.x _returnvalue) 5.0 (.z _returnvalue)) (Variables|Default|GetFireRotation) (Variables|Default|GetBladeScale)) "AlwaysSpawn" 0 0)
    (Audio|PlaySound2D "/Game/SetchOnLegs/03Audio/00Menus/Fire.Fire" 1.0 1.0 0.0 0 0)
    (Utilities|FlowControl|Delay 1.0)
    (if (not (Variables|Default|GetIsDead))
      (Variables|Default|SetState "NewEnumerator0")
      (CallFunction|UpdateAnimation))))

(event Custom|GetFireRotation
  (bind _returnvalue (Game|GetPlayerController 0))
  (bind _returnvalue_2 (Game|GetPlayerController 0))
  (bind _returnvalue_3 (Transformation|GetActorLocation))
  (bind _fireballspawn (Variables|Default|GetFireballSpawn))
  (bind _returnvalue_4 (Pawn|GetControlledPawn _returnvalue))
  (bind _screenlocation (Class|PlayerController|ProjectWorldLocationtoScreen _returnvalue_2 _returnvalue_3 false))
  (bind _returnvalue_5 (Transformation|GetWorldLocation _fireballspawn))
  (bind _returnvalue_6 (Transformation|GetActorLocation _returnvalue_4))
  (bind (_x _y) (Math|Vector2D|BreakVector2D _screenlocation))
  (bind (_x_2 _y_2 _z) (Math|Vector|BreakVector _returnvalue_5))
  (bind _screenlocation_2 (Class|PlayerController|ProjectWorldLocationtoScreen _returnvalue _returnvalue_6 false))
  (bind (_x_3 _y_3) (Math|Vector2D|BreakVector2D _screenlocation_2))
  ;[1 1 1] Shoot Logic
  ;;[1 1 1] Get fire rotation
  (Variables|Default|SetFireRotation (Math|Rotator|FindLookatRotation _returnvalue_5 (Math|Vector|MakeVector (+ _x_2 (- _x_3 _x)) 0.0 (+ _z (- _y _y_3))))))

(event EventBeginPlay
  ;[1 1 1] Initialise
  (Variables|Default|SetState "NewEnumerator0")
  (Pawn|Components|CharacterMovement|SetMovementMode (Variables|Character|GetCharacterMovement) "MOVE_Flying" 0)
  (bind _asbp_spike (Utilities|Casting|CastToBP_Spike (Game|GetPlayerCharacter 0)))
  (Variables|Default|SetPlayer _asbp_spike))

(event EventTick
  (params (DeltaSeconds :type Float%20%28single-precision%29))
  ;[1 1 1] Tick
  (Utilities|FlowControl|Sequence
    (:then_0
      (CallFunction|GetFireRotation))
    (:then_1
      (CallFunction|HandleMovement))
    (:then_2
      (if (not (Variables|Default|GetIsDead))
        (Utilities|FlowControl|Delay (Variables|Default|GetAttackLag))
        (CallFunction|Shoot)))
    (:then_3
      (CallFunction|UpdateAnimation))))

(fn ConstructionScript)
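; Flying God Mode Hince in Hell boss, opening with a cutscene that locks player input before combat.
; Tick follows the player at an offset and aims via screen-space projection for a self-repeating disc attack loop.
; Low health latches phase two, adding falling discs with alternating sideways velocity.
; Bullet overlaps on two hit spheres cause damage blinking; death increments the player's kill count and spawns two mini versions.
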(event OnComponentBeginOverlap(HitSphere2)
  (params (OverlappedComponent :type Primitive%20Component%20Object%20Reference) (OtherActor :type Actor%20Object%20Reference) (OtherComp :type Primitive%20Component%20Object%20Reference) (OtherBodyIndex :type Integer) (bFromSweep :type Boolean) (SweepResult :type Hit%20Result%20Structure%20%28by%20ref%29))
  ;[1 1 1] Bullet Collision
  (bind _asbp_bullet (Utilities|Casting|CastToBP_Bullet OtherActor))
  (Actor|DestroyActor _asbp_bullet)
  (if (not (Variables|Default|GetIsDead))
    (CallFunction|DamageSytsem (Variables|/Game/SetchOnLegs/00Blueprint/07Spike/BP_Spike.BP_Spike_C|GetBulletDamage (Variables|Default|GetPlayer)))))

(event OnComponentBeginOverlap(HitSphere1)
  (params (OverlappedComponent :type Primitive%20Component%20Object%20Reference) (OtherActor :type Actor%20Object%20Reference) (OtherComp :type Primitive%20Component%20Object%20Reference) (OtherBodyIndex :type Integer) (bFromSweep :type Boolean) (SweepResult :type Hit%20Result%20Structure%20%28by%20ref%29))
  ;[1 1 1] Bullet Collision
  (bind _asbp_bullet (Utilities|Casting|CastToBP_Bullet OtherActor))
  (Actor|DestroyActor _asbp_bullet)
  (if (not (Variables|Default|GetIsDead))
    (CallFunction|DamageSytsem (Variables|/Game/SetchOnLegs/00Blueprint/07Spike/BP_Spike.BP_Spike_C|GetBulletDamage (Variables|Default|GetPlayer)))))

(event Custom|Blink
  (bind _sprite (Variables|Default|GetSprite))
  ;[1 1 1] Damage & Death System
  (Development|SetHiddeninGame _sprite (not (Variables|/Script/Engine.SceneComponent|GetbHiddenInGame _sprite)) false))

(event Custom|Damage%20Sytsem
  (params (DamageIn :type Float%20%28single-precision%29))
  (bind _player (Variables|Default|GetPlayer))
  ;[1 1 1] Damage & Death System
  (bind _output_get (Variables|Default|SetCurrentHealth (- (Variables|Default|GetCurrentHealth) DamageIn)))
  (if (<= _output_get 0.0)
    (Variables|Default|SetState "NewEnumerator2")
    (CallFunction|UpdateAnimation)
    (Variables|Default|SetIsDead true)
    (Variables|/Game/SetchOnLegs/00Blueprint/07Spike/BP_Spike.BP_Spike_C|SetHinceInHellKillCount _player (+ (Variables|/Game/SetchOnLegs/00Blueprint/07Spike/BP_Spike.BP_Spike_C|GetHinceInHellKillCount _player) 1))
    (Utilities|FlowControl|Delay 2.2)
    (CallFunction|Respawn)
    (Actor|DestroyActor)
    (else
      (Utilities|Time|SetTimerbyFunctionName 0 "Blink" 0.05 true)
      (Utilities|FlowControl|Delay 0.2)
      (Utilities|Time|ClearTimerbyFunctionName 0 "Blink")
      (Development|SetHiddeninGame (Variables|Default|GetSprite) false false))))

(event Custom|UpdateAnimation
  (bind _sprite (Variables|Default|GetSprite))
  ;[1 1 1] Handle Animation
  (switch Utilities|FlowControl|Switch|SwitchonHinceInHellState (Variables|Default|GetState)
    (:NewEnumerator0
      (Sprite|SetFlipbook _sprite "/Game/SetchOnLegs/01Sprites/01HinceInHell/Character/A_HinceInHellMoving.A_HinceInHellMoving"))
    (:NewEnumerator1
      (Sprite|SetFlipbook _sprite "/Game/SetchOnLegs/01Sprites/01HinceInHell/Character/A_HinceInHellAttacking.A_HinceInHellAttacking"))
    (:NewEnumerator2
      (Sprite|SetFlipbook _sprite "/Game/SetchOnLegs/01Sprites/01HinceInHell/Character/A_HinceInHellDead.A_HinceInHellDead"))))

(event Custom|Respawn
  (bind _returnvalue (Game|GetPlayerCharacter 0))
  (bind _returnvalue_2 (Game|GetPlayerCharacter 0))
  (bind _returnvalue_3 (Transformation|GetActorLocation _returnvalue))
  (bind _returnvalue_4 (Transformation|GetActorLocation _returnvalue_2))
  ;[1 1 1] Respawn System
  (Game|SpawnActorfromClass "/Game/SetchOnLegs/00Blueprint/01HinceInHell/GodMode/BP_MiniHinceInHellGodMode.BP_MiniHinceInHellGodMode_C" (Math|Transform|MakeTransform (Math|Vector|MakeVector (- (.x _returnvalue_3) 4e+02) 0.0 (+ (.z _returnvalue_3) 1e+03)) "0, 0, 0" "0.500000,0.500000,0.500000") "Undefined" 0 "-400.000000,0.000000,500.000000" 0)
  (Game|SpawnActorfromClass "/Game/SetchOnLegs/00Blueprint/01HinceInHell/GodMode/BP_MiniHinceInHellGodMode.BP_MiniHinceInHellGodMode_C" (Math|Transform|MakeTransform (Math|Vector|MakeVector (+ (.x _returnvalue_4) 4e+02) 0.0 (+ (.z _returnvalue_4) 1e+03)) "0, 0, 0" "0.500000,0.500000,0.500000") "Undefined" 0 "400.000000,0.000000,500.000000" 0))

(event Custom|HandleMovement
  ;[1 1 1] Handle Movement
  (Utilities|FlowControl|Delay 0.1)
  (Variables|Default|SetOurPosition (- (Transformation|GetActorLocation) (Variables|Default|GetMoveToPos)))
  (Variables|Default|SetPlayerPosition (Transformation|GetActorLocation (Pawn|GetControlledPawn (Game|GetPlayerController 0))))
  (Pawn|Input|AddMovementInput (- (Variables|Default|GetPlayerPosition) (Variables|Default|GetOurPosition)) 1.0 false))

(event Custom|Shoot
  (bind _fireballspawn (Variables|Default|GetFireballSpawn))
  (bind _returnvalue (Transformation|GetWorldLocation _fireballspawn))
  ;[1 1 1] Shoot Logic
  ;;[1 1 1] Handle Shoot
  (if (not (Variables|Default|GetIsDead))
    (Variables|Default|SetState "NewEnumerator1")
    (CallFunction|UpdateAnimation)
    (Game|SpawnActorfromClass "/Game/SetchOnLegs/00Blueprint/01HinceInHell/GodMode/BP_HinceInHellGodDisc.BP_HinceInHellGodDisc_C" (Math|Transform|MakeTransform (Math|Vector|MakeVector (.x _returnvalue) -0.1 (.z _returnvalue)) (Variables|Default|GetFireRotation) (Variables|Default|GetFireballScale)) "AlwaysSpawn" 0 2 0)
    (Utilities|FlowControl|Delay 1.1)
    (if (not (Variables|Default|GetIsDead))
      (Variables|Default|SetState "NewEnumerator0")
      (CallFunction|UpdateAnimation)
      (Utilities|FlowControl|Delay (Variables|Default|GetAttackDelay))
      (CallFunction|Shoot))))

(event Custom|GetFireRotation
  (bind _returnvalue (Game|GetPlayerController 0))
  (bind _returnvalue_2 (Game|GetPlayerController 0))
  (bind _fireballspawn (Variables|Default|GetFireballSpawn))
  (bind _returnvalue_3 (Pawn|GetControlledPawn _returnvalue))
  (bind _returnvalue_4 (Transformation|GetWorldLocation _fireballspawn))
  (bind _returnvalue_5 (Transformation|GetActorLocation _returnvalue_3))
  (bind _screenlocation (Class|PlayerController|ProjectWorldLocationtoScreen _returnvalue_2 _returnvalue_4 false))
  (bind (_x _y _z) (Math|Vector|BreakVector _returnvalue_4))
  (bind (_x_2 _y_2) (Math|Vector2D|BreakVector2D _screenlocation))
  (bind _screenlocation_2 (Class|PlayerController|ProjectWorldLocationtoScreen _returnvalue _returnvalue_5 false))
  (bind (_x_3 _y_3) (Math|Vector2D|BreakVector2D _screenlocation_2))
  ;[1 1 1] Shoot Logic
  ;;[1 1 1] Get fire rotation
  (Variables|Default|SetFireRotation (Math|Rotator|FindLookatRotation _returnvalue_4 (Math|Vector|MakeVector (+ _x (- _x_3 _x_2)) 0.0 (+ _z (- _y_2 _y_3))))))

(event Custom|IntroCutscene
  ;[1 1 1] Intro Cutscene
  (bind _asbp_spike (Utilities|Casting|CastToBP_Spike (Game|GetPlayerCharacter 0)))
  (bind _output_get (Variables|Default|SetPlayer _asbp_spike))
  (Input|DisableInput _output_get 0)
  (Pawn|Components|CharacterMovement|SetMovementMode (Variables|Character|GetCharacterMovement) "MOVE_Flying" 0)
  (Utilities|FlowControl|Delay 2.0)
  (Audio|PlaySound2D "/Game/SetchOnLegs/03Audio/01HinceInHell/Unused/GodScream.GodScream" 1.0 1.0 0.0 0 0)
  (Camera|PlayWorldCameraShake "/Game/SetchOnLegs/00Blueprint/01HinceInHell/Boss/CameraShakes/BP_IntroShake.BP_IntroShake_C" (Transformation|GetWorldLocation (Variables|/Game/SetchOnLegs/00Blueprint/07Spike/BP_Spike.BP_Spike_C|GetSideViewCameraComponent (Variables|Default|GetPlayer))) 0.0 5e+02)
  (Sprite|SetFlipbook (Variables|Default|GetSprite) "/Game/SetchOnLegs/01Sprites/01HinceInHell/Character/A_HinceInHellAttacking.A_HinceInHellAttacking")
  (Utilities|FlowControl|Delay 3.0)
  (bind _returnvalue (UserInterface|CreateWidget "/Game/SetchOnLegs/00Blueprint/01HinceInHell/GodMode/Widget_HinceInHellGodModeIntro.Widget_HinceInHellGodModeIntro_C"))
  (UserInterface|Viewport|AddtoViewport _returnvalue 0)
  (Utilities|FlowControl|Delay 1.5)
  (Variables|Default|SetState "NewEnumerator0")
  (CallFunction|UpdateAnimation)
  (Input|EnableInput (Variables|Default|GetPlayer) 0)
  (Variables|Default|SetIntro false)
  (bind _returnvalue_2 (UserInterface|CreateWidget "/Game/SetchOnLegs/00Blueprint/01HinceInHell/GodMode/Widget_HinceInHellGodMode.Widget_HinceInHellGodMode_C"))
  (UserInterface|Viewport|AddtoViewport _returnvalue_2 0)
  (Utilities|FlowControl|Delay 2.5)
  (CallFunction|Shoot))

(event EventBeginPlay
  ;[1 1 1] Initialise
  (CallFunction|IntroCutscene))

(event EventTick
  (params (DeltaSeconds :type Float%20%28single-precision%29))
  ;[1 1 1] Tick
  (Utilities|FlowControl|Sequence
    (:then_0
      (if (Math|Float|InRange(Float) (Variables|Default|GetCurrentHealth) 1.0 4e+02)
        (Utilities|FlowControl|DoOnce false
          (:Completed
            (Variables|Default|SetPhase2 true)))))
    (:then_1
      (CallFunction|GetFireRotation)
      (if (not (Variables|Default|GetIntro))
        (CallFunction|HandleMovement)
        (CallFunction|UpdateAnimation)
        (if (Variables|Default|GetPhase2)
          (Utilities|FlowControl|Delay 0.5)
          (if (not (Variables|Default|GetIsDead))
            (Game|SpawnActorfromClass "/Game/SetchOnLegs/00Blueprint/01HinceInHell/GodMode/BP_HinceInHellFallingGodDisc.BP_HinceInHellFallingGodDisc_C" (Math|Transform|MakeTransform (Transformation|GetWorldLocation (Variables|Default|GetFallingFireballSpawn)) "0, 0, 0" (Variables|Default|GetFireballScale)) "Undefined" 0 (Variables|Default|GetFallingXVelocity) 0)
            (Variables|Default|SetFallingXVelocity (* (Variables|Default|GetFallingXVelocity) -1.0))))))))

(fn ConstructionScript)
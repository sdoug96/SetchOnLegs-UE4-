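; BP_HinceInHellFallingGodDisc is a spinning disc projectile in the HinceInHell god mode that damages the player, BP_Spike.
; On BeginPlay it plays a fire sound and launches through ProjectileMovement with a variable X speed and a fixed upward kick.
; Tick drives pitch spin from an accumulated timer.
; HitSphere overlap applies damage and destroys the disc, unless Spike is in one exempt state.
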(event OnComponentBeginOverlap(HitSphere)
  (params (OverlappedComponent :type Primitive%20Component%20Object%20Reference) (OtherActor :type Actor%20Object%20Reference) (OtherComp :type Primitive%20Component%20Object%20Reference) (OtherBodyIndex :type Integer) (bFromSweep :type Boolean) (SweepResult :type Hit%20Result%20Structure%20%28by%20ref%29))
  ;[1 1 1] Player Collision
  (bind _asbp_spike (Utilities|Casting|CastToBP_Spike OtherActor))
  (if (Utilities|Enum|NotEqual(Enum) (Variables|/Game/SetchOnLegs/00Blueprint/07Spike/BP_Spike.BP_Spike_C|GetState _asbp_spike) "NewEnumerator5")
    (Default|DamageSystem _asbp_spike 2)
    (Actor|DestroyActor)))

(event EventBeginPlay
  ;[1 1 1] Set Velocity
  (Audio|PlaySound2D "/Game/SetchOnLegs/03Audio/08Misc/Fire.Fire" 1.0 1.0 0.0 0 0)
  (Variables|/Script/Engine.MovementComponent|SetVelocity (Variables|Default|GetProjectileMovement) (Math|Vector|MakeVector (Variables|Default|GetXVelocity) 0.0 7.5e+02)))

(event EventTick
  (params (DeltaSeconds :type Float%20%28single-precision%29))
  ;[1 1 1] Rotate
  (Variables|Default|SetTimer (+ DeltaSeconds (Variables|Default|GetTimer)))
  (Transformation|SetActorRotation (Math|Rotator|MakeRotator 0.0 (* (Variables|Default|GetTimer) (Variables|Default|GetRotation)) 0.0)))

(fn ConstructionScript)
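; The Butcher, a flipbook boss in the Slaughterhouse, hurt by bullets and spikes.
; StartFight shows its HUD, moves it left and throws cleavers on a looping timer.
; Health thresholds in Tick first start a self-chaining attack, alternating falling buzz saw rows with two random gaps and side-switching horizontal waves, then retune its timing and speed.
; Death swaps the sprite, removes the HUD and clears saws, cleavers and drag pads.
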(event OnComponentBeginOverlap(HitBox)
  (params (OverlappedComponent :type Primitive%20Component%20Object%20Reference) (OtherActor :type Actor%20Object%20Reference) (OtherComp :type Primitive%20Component%20Object%20Reference) (OtherBodyIndex :type Integer) (bFromSweep :type Boolean) (SweepResult :type Hit%20Result%20Structure%20%28by%20ref%29))
  ;[1 1 1] Collision Logic
  (Utilities|FlowControl|Sequence
    (:then_0
      (Utilities|Casting|CastToBP_Bullet OtherActor)
      (CallFunction|BulletCollision)
      (Audio|PlaySound2D "/Game/SetchOnLegs/03Audio/07Spike/EnemyHit.EnemyHit" 1.0 1.0 0.0 0 0))
    (:then_1
      (Utilities|Casting|CastToBP_Spike OtherActor)
      (CallFunction|DamageSpike))))

(event Custom|UpdateAnimation
  ;[1 1 1] Update Animation
  (switch Utilities|FlowControl|Switch|SwitchonButcherState (Variables|Core|GetState)
    (:NewEnumerator0
      (Sprite|SetFlipbook (Variables|Default|GetSprite) "/Game/SetchOnLegs/01Sprites/03TheButcher/Character/A_ButcherIdle.A_ButcherIdle"))
    (:NewEnumerator1
      (Sprite|SetFlipbook (Variables|Default|GetSprite) "/Game/SetchOnLegs/01Sprites/03TheButcher/Character/A_ButcherAttack.A_ButcherAttack"))
    (:NewEnumerator2
      (Sprite|SetFlipbook (Variables|Default|GetSprite) "/Game/SetchOnLegs/01Sprites/07Spike/Character/A_Dead.A_Dead")
      (Transformation|SetWorldScale3D (Variables|Default|GetSprite) "1.500000,1.500000,1.500000")
      (Transformation|SetRelativeLocation (Variables|Default|GetSprite) "-48.000000,0.000000,-350.000000" false false))))

(event Custom|SetBladesToSpawn
  ;[1 1 1] Drop Blade Logic
  (Variables|RoofBlades|SetRandomBlade1 (Math|Random|RandomIntegerinRange 0 6))
  (Variables|RoofBlades|SetRandomBlade2 (Math|Random|RandomIntegerinRange 0 6))
  (while (== (Variables|RoofBlades|GetRandomBlade1) (Variables|RoofBlades|GetRandomBlade2))
    (Variables|RoofBlades|SetRandomBlade2 (Math|Random|RandomIntegerinRange 0 6))))

(event Custom|StartFight
  ;[1 1 1] Start Fight
  (bind _returnvalue (UserInterface|CreateWidget "/Game/SetchOnLegs/00Blueprint/03TheSlaughterhouse/Boss/Widget_TheButcher.Widget_TheButcher_C"))
  (bind _output_get (Variables|Core|SetHUD _returnvalue))
  (UserInterface|Viewport|AddtoViewport _output_get 0)
  (Sprite|SetFlipbook (Variables|Default|GetSprite) "/Game/SetchOnLegs/01Sprites/03TheButcher/Character/A_ButcherAttack.A_ButcherAttack")
  (Variables|/Script/Engine.MovementComponent|SetVelocity (Variables|Character|GetCharacterMovement) "-200.000000, 0, 0")
  (Utilities|Time|SetTimerbyFunctionName 0 "SpawnCleaver" (Variables|Cleavers|GetCleaverDelay) true)
  (Variables|Default|SetActive true))

(event Custom|DropBlades
  ;[1 1 1] Drop Blade Logic
  (Audio|PlaySound2D "/Game/SetchOnLegs/03Audio/03TheButcher/SawBlade.SawBlade" 1.0 1.0 0.0 0 0)
  (for _index (range 0 (- (Variables|RoofBlades|GetBladesToDrop) 1))
    (if (== _index (Variables|RoofBlades|GetRandomBlade1))
      _
      (elif (== _index (Variables|RoofBlades|GetRandomBlade2))
        _
        (else
          (Game|SpawnActorfromClass "/Game/SetchOnLegs/00Blueprint/03TheSlaughterhouse/Hazards/BP_BuzzSaw.BP_BuzzSaw_C" (Math|Transform|MakeTransform (Math|Vector|MakeVector (Variables|RoofBlades|GetBladeXPos) -0.1 2.4e+02) "0, 0, 0" "0.120000,0.120000,0.120000") "Undefined" 0 false 0.0 0.0 0.0 (Variables|RoofBlades|GetBladeDropSpeed) 1 0.0 true -6e+02 0.0 false 0))))
    (Variables|RoofBlades|SetBladeXPos (+ (Variables|RoofBlades|GetBladeXPos) 1.8e+02)))
  (Variables|RoofBlades|SetBladeXPos 6e+01)
  (CallFunction|SetBladestoSpawn)
  (Utilities|FlowControl|Delay (Variables|Core|GetAttackDelay))
  (CallFunction|SideBlades))

(event Custom|SpawnCleaver
  ;[1 1 1] Cleaver Logic
  (if (not (Variables|Default|GetIsDead))
    (Game|SpawnActorfromClass "/Game/SetchOnLegs/00Blueprint/03TheSlaughterhouse/Boss/BP_Cleaver.BP_Cleaver_C" (Transformation|GetWorldTransform (Variables|Default|GetCleaverSpawn)) "Undefined" 0 0)
    (Audio|PlaySound2D "/Game/SetchOnLegs/03Audio/03TheButcher/Knife.Knife" 1.0 1.0 0.0 0 0)))

(event Custom|SideBlades
  ;[1 1 1] Blade Logic
  (if (Variables|SideBlades|GetSideBladeRight)
    (if (not (Variables|Default|GetIsDead))
      (Utilities|ForLoopwithDelay 0 (- (Variables|SideBlades|GetSideBladesToSpawn) 1) :!label _label
        (:Loop%20Body
          (Game|SpawnActorfromClass "/Game/SetchOnLegs/00Blueprint/03TheSlaughterhouse/Hazards/BP_BuzzSaw.BP_BuzzSaw_C" (Math|Transform|MakeTransform "1640.000000,-0.100000,-690.000000" "0, 0, 0" "0.150000,0.150000,0.150000") "Undefined" 0 false 0.0 0.0 (* (Variables|SideBlades|GetSideBladeSpeed) -1.0) 0.0 1 0.0 true -6e+02 0.0 false 0)
          (Audio|PlaySound2D "/Game/SetchOnLegs/03Audio/03TheButcher/SawBladeShort.SawBladeShort" 1.0 1.0 0.0 0 0))
        (:Completed
          (Utilities|FlowControl|Delay (Variables|Core|GetAttackDelay))
          (CallFunction|DropBlades)
          (Variables|SideBlades|SetSideBladeRight false))
        (:Delay%20Out
          (Utilities|FlowControl|Delay (Variables|SideBlades|GetSideBladeDelay))
          (goto _label Delay%20In))))
    (elif (not (Variables|Default|GetIsDead))
      (Utilities|ForLoopwithDelay 0 (- (Variables|SideBlades|GetSideBladesToSpawn) 1) :!label _label_2
        (:Loop%20Body
          (Game|SpawnActorfromClass "/Game/SetchOnLegs/00Blueprint/03TheSlaughterhouse/Hazards/BP_BuzzSaw.BP_BuzzSaw_C" (Math|Transform|MakeTransform "-440.000000,-0.100000,-690.000000" "0, 0, 0" "0.150000,0.150000,0.150000") "Undefined" 0 false 0.0 0.0 (Variables|SideBlades|GetSideBladeSpeed) 0.0 1 0.0 true -6e+02 0.0 false 0)
          (Audio|PlaySound2D "/Game/SetchOnLegs/03Audio/03TheButcher/SawBladeShort.SawBladeShort" 1.0 1.0 0.0 0 0))
        (:Completed
          (Utilities|FlowControl|Delay (Variables|Core|GetAttackDelay))
          (CallFunction|DropBlades)
          (Variables|SideBlades|SetSideBladeRight true))
        (:Delay%20Out
          (Utilities|FlowControl|Delay (Variables|SideBlades|GetSideBladeDelay))
          (goto _label_2 Delay%20In))))))

(event EventDamageSystem
  (params (DamageIn :type Float%20%28single-precision%29))
  ;[1 1 1] Damage & Death System
  (|CallParentFunction DamageIn)
  (if (Variables|Default|GetIsDead)
    (Variables|Core|SetState "NewEnumerator2")
    (CallFunction|UpdateAnimation)
    (Widget|RemovefromParent (Variables|Core|GetHUD))
    (Utilities|Time|ClearTimerbyFunctionName 0 "SpawnCleaver")
    (Utilities|Time|ClearTimerbyFunctionName 0 "SpawnBlades")
    (Variables|/Script/Engine.MovementComponent|SetVelocity (Variables|Character|GetCharacterMovement) "0, 0, 0")
    (Audio|PlaySound2D "/Game/SetchOnLegs/03Audio/08Misc/Splat.Splat" 1.0 1.0 0.0 0 0)))

(event EventTick
  (params (DeltaSeconds :type Float%20%28single-precision%29))
  (bind _currenthealth (Variables|Default|GetCurrentHealth))
  ;[1 1 1] Tick Attack and Death Logic
  (Utilities|FlowControl|Sequence
    (:then_0
      (if (< _currenthealth 3.2e+02)
        (Utilities|FlowControl|DoOnce false
          (:Completed
            (CallFunction|DropBlades)))))
    (:then_1
      (if (< _currenthealth 1.6e+02)
        (Utilities|FlowControl|DoOnce false
          (:Completed
            (Variables|Core|SetAttackDelay 3.5)
            (Variables|SideBlades|SetSideBladeDelay 0.75)
            (Variables|SideBlades|SetSideBladeSpeed 7.5e+02)))))
    (:then_2
      (if (Variables|Default|GetIsDead)
        (bind _outactors (Actor|GetAllActorsOfClass "/Game/SetchOnLegs/00Blueprint/03TheSlaughterhouse/Hazards/BP_BuzzSaw.BP_BuzzSaw_C"))
        (Actor|DestroyActor _outactors)
        (bind _outactors_2 (Actor|GetAllActorsOfClass "/Game/SetchOnLegs/00Blueprint/03TheSlaughterhouse/Hazards/BP_DragPad.BP_DragPad_C"))
        (Actor|DestroyActor _outactors_2)
        (bind _outactors_3 (Actor|GetAllActorsOfClass "/Game/SetchOnLegs/00Blueprint/03TheSlaughterhouse/Boss/BP_Cleaver.BP_Cleaver_C"))
        (Actor|DestroyActor _outactors_3)))))

(fn ConstructionScript)
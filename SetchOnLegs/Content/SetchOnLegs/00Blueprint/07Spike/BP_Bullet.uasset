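; BP_Bullet is a projectile that takes its behavior from the BP_Spike player character's shooting stats.
; On BeginPlay it casts the player character to BP_Spike and copies BulletSpeed to the ProjectileMovement initial and max speeds.
; It raises gravity scale for the cannon shooter type, giving an arced shot.
; BulletRange acts as a lifetime, destroying the bullet after that delay.
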(event Custom|CannonBulletLogic
  ;[1 1 1] Cannon bullet logic
  (if (Utilities|Enum|Equal(Enum) (Variables|/Game/SetchOnLegs/00Blueprint/07Spike/BP_Spike.BP_Spike_C|GetShooter (Variables|Default|GetPlayer)) "NewEnumerator4")
    (Variables|/Script/Engine.ProjectileMovementComponent|SetProjectileGravityScale (Variables|Default|GetProjectileMovement) 1.5)))

(event Custom|KillBullet
  ;[1 1 1] Set Bullet Range
  (Utilities|FlowControl|Delay (Variables|/Game/SetchOnLegs/00Blueprint/07Spike/BP_Spike.BP_Spike_C|GetBulletRange (Variables|Default|GetPlayer)))
  (Actor|DestroyActor))

(event Custom|SetBulletSpeed
  (bind _player (Variables|Default|GetPlayer))
  (bind _bulletspeed (Variables|/Game/SetchOnLegs/00Blueprint/07Spike/BP_Spike.BP_Spike_C|GetBulletSpeed _player))
  ;[1 1 1] Set Bullet Speed
  (Variables|/Script/Engine.ProjectileMovementComponent|SetInitialSpeed (Variables|Default|GetProjectileMovement) _bulletspeed)
  (Variables|/Script/Engine.ProjectileMovementComponent|SetMaxSpeed (Variables|Default|GetProjectileMovement) _bulletspeed))

(event EventBeginPlay
  ;[1 1 1] Initialise
  (bind _asbp_spike (Utilities|Casting|CastToBP_Spike (Game|GetPlayerCharacter 0)))
  (Variables|Default|SetPlayer _asbp_spike)
  (Utilities|FlowControl|Sequence
    (:then_0
      (CallFunction|SetBulletSpeed))
    (:then_1
      (CallFunction|CannonBulletLogic))
    (:then_2
      (CallFunction|KillBullet))))

(fn ConstructionScript)
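; Mike the Mystical, an NPC who talks to the player, then opens the fast travel menu.
; On BeginPlay it caches the DialogueList rows matching its NPCID.
; Hitbox overlap toggles a listen prompt and Spike's CutScene flag, while each Interact, ignored if Spike is falling, advances a text box by ConversationID and line number.
; Without exactly one matching line, dialogue closes and resets, the menu appears, and conversation 1 switches to 2.
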(event OnComponentBeginOverlap(Hitbox)
  (params (OverlappedComponent :type Primitive%20Component%20Object%20Reference) (OtherActor :type Actor%20Object%20Reference) (OtherComp :type Primitive%20Component%20Object%20Reference) (OtherBodyIndex :type Integer) (bFromSweep :type Boolean) (SweepResult :type Hit%20Result%20Structure%20%28by%20ref%29))
  (Utilities|Casting|CastToBP_Spike OtherActor)
  (bind _returnvalue (UserInterface|CreateWidget "/Game/SetchOnLegs/00Blueprint/12Misc/Widgets/Widget_Listen.Widget_Listen_C"))
  (bind _output_get (Variables|Default|SetListenPrompt _returnvalue))
  (UserInterface|Viewport|AddtoViewport _output_get 0)
  (Variables|/Game/SetchOnLegs/00Blueprint/07Spike/BP_Spike.BP_Spike_C|SetCutScene (Variables|Default|GetPlayer) true))

(event OnComponentEndOverlap(Hitbox)
  (params (OverlappedComponent :type Primitive%20Component%20Object%20Reference) (OtherActor :type Actor%20Object%20Reference) (OtherComp :type Primitive%20Component%20Object%20Reference) (OtherBodyIndex :type Integer))
  (Utilities|Casting|CastToBP_Spike OtherActor)
  (Widget|RemovefromParent (Variables|Default|GetListenPrompt))
  (Variables|/Game/SetchOnLegs/00Blueprint/07Spike/BP_Spike.BP_Spike_C|SetCutScene (Variables|Default|GetPlayer) false))

(event EventInteract
  (if (not (AI|Components|NavMovement|IsFalling (Variables|/Script/Engine.Character|GetCharacterMovement (Variables|Default|GetPlayer))))
    (Math|Integer|IncrementInt (Variables|Default|GetLineCurrent)
      (:%20%20
        (CallFunction|DialogueCreate)
        (Audio|PlaySound2D "/Game/SetchOnLegs/03Audio/00Menus/click.click" 1.0 1.0 0.0 0 0)
        (Widget|RemovefromParent (Variables|Default|GetListenPrompt))))))

(event EventBeginPlay
  (bind _asbp_spike (Utilities|Casting|CastToBP_Spike (Game|GetPlayerCharacter 0)))
  (Variables|Default|SetPlayer _asbp_spike)
  (bind _outrownames (DataTable|GetDataTableRowNames "/Game/SetchOnLegs/00Blueprint/12Misc/DialogueList.DialogueList"))
  (for _array_element _outrownames
    (bind _returnvalue (Utilities|GetDataTableRow "/Game/SetchOnLegs/00Blueprint/12Misc/DialogueList.DialogueList" _array_element)
      (:then
        (if (== (.NPC_ID (Utilities|Struct|BreakDialogueStructure _returnvalue)) (Variables|Default|GetNPC_ID))
          (Utilities|Array|Add (Variables|Default|GetMyDialogue) _array_element))))))

(fn ConstructionScript)

(fn DialogueCreate
  (Utilities|IsValid (Variables|Default|GetDialogueWidget)
    (:Is%20Valid
      (bind _returnedline (CallFunction|DialogueGetLine))
      (if (Utilities|Enum|NotEqual(Enum) (Variables|Default|GetEmptyText) _returnedline)
        (Variables|/Game/SetchOnLegs/00Blueprint/12Misc/Widgets/Widget_TextBox.Widget_TextBox_C|SetDialogueText (Variables|Default|GetDialogueWidget) _returnedline)))
    (:Is%20Not%20Valid
      (bind _returnvalue (UserInterface|CreateWidget "/Game/SetchOnLegs/00Blueprint/12Misc/Widgets/Widget_TextBox.Widget_TextBox_C"))
      (bind _output_get (Variables|Default|SetDialogueWidget _returnvalue))
      (UserInterface|Viewport|AddtoViewport _output_get 0)
      (bind _returnedline_2 (CallFunction|DialogueGetLine))
      (Variables|/Game/SetchOnLegs/00Blueprint/12Misc/Widgets/Widget_TextBox.Widget_TextBox_C|SetDialogueText (Variables|Default|GetDialogueWidget) _returnedline_2))))

(fn DialogueGetLine
  (for _array_element (Variables|Default|GetMyDialogue)
    (bind _returnvalue (Utilities|GetDataTableRow "/Game/SetchOnLegs/00Blueprint/12Misc/DialogueList.DialogueList" _array_element)
      (:then
        (if (and (== (.Conversation_ID (Utilities|Struct|BreakDialogueStructure _returnvalue)) (Variables|Default|GetConversation_ID)) (== (.Line_ID (Utilities|Struct|BreakDialogueStructure _returnvalue)) (Variables|Default|GetLineCurrent)))
          (Utilities|Array|Add (LocalVariables|GetReturnedLines) (.Dialogue (Utilities|Struct|BreakDialogueStructure _returnvalue)))))))
  (if (== (Utilities|Array|Length (LocalVariables|GetReturnedLines)) 1)
    (return (Utilities|Array|Get(acopy) (LocalVariables|GetReturnedLines)))
    (else
      (Widget|RemovefromParent (Variables|Default|GetDialogueWidget))
      (Variables|Default|SetDialogueWidget 0)
      (Variables|Default|SetLineCurrent 0)
      (bind _returnvalue_2 (UserInterface|CreateWidget "/Game/SetchOnLegs/00Blueprint/08NPCs/02MikeTheMystical/Widget_FastTravelMenu.Widget_FastTravelMenu_C"))
      (UserInterface|Viewport|AddtoViewport _returnvalue_2 0)
      (if (== (Variables|Default|GetConversation_ID) 1)
        (Variables|Default|SetConversation_ID 2)))))
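; Spinning blade hazard that damages the player (BP_Spike) on sphere overlap.
; With Lerp on, a Timeline ping-pongs it between its start and an X/Z offset; otherwise Tick drives ProjectileMovement at a constant Z velocity.
; Tick also spins its pitch from accumulated time.
; Overlap skips one player state, then deals lethal damage if IsKiller, or armor-reduced damage followed by a short damage cooldown.
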(event OnComponentBeginOverlap(Sphere)
  (params (OverlappedComponent :type Primitive%20Component%20Object%20Reference) (OtherActor :type Actor%20Object%20Reference) (OtherComp :type Primitive%20Component%20Object%20Reference) (OtherBodyIndex :type Integer) (bFromSweep :type Boolean) (SweepResult :type Hit%20Result%20Structure%20%28by%20ref%29))
  (bind _damage (Variables|Default|GetDamage))
  ;[1 1 1] Player Collision
  (if (Variables|Default|GetCanDamage)
    (bind _asbp_spike (Utilities|Casting|CastToBP_Spike OtherActor))
    (if (Utilities|Enum|NotEqual(Enum) (Variables|/Game/SetchOnLegs/00Blueprint/07Spike/BP_Spike.BP_Spike_C|GetState _asbp_spike) "NewEnumerator5")
      (if (Variables|Default|GetIsKiller)
        (Default|DamageSytsem _asbp_spike (Variables|/Game/SetchOnLegs/00Blueprint/07Spike/BP_Spike.BP_Spike_C|GetMaxHealth _asbp_spike) 0.0)
        (else
          (switch int (Variables|/Game/SetchOnLegs/00Blueprint/07Spike/BP_Spike.BP_Spike_C|GetArmorLevel _asbp_spike)
            (:0
              (Default|DamageSytsem _asbp_spike _damage 0.0))
            (:1
              (Default|DamageSytsem _asbp_spike (* _damage 0.9) 0.0))
            (:2
              (Default|DamageSytsem _asbp_spike (* _damage 0.8) 0.0))
            (:3
              (Default|DamageSytsem _asbp_spike (* _damage 0.7) 0.0))
            (:4
              (Default|DamageSytsem _asbp_spike (* _damage 0.6) 0.0))
            (:5
              (Default|DamageSytsem _asbp_spike (* _damage 0.5) 0.0)))
          (Variables|Default|SetCanDamage false)
          (Utilities|FlowControl|Delay 1.0)
          (Variables|Default|SetCanDamage true))))))

(event EventBeginPlay
  ;[1 1 1] Movement
  (if (Variables|Default|GetLerp)
    (bind _output_get (Variables|Default|SetInitialLocation (Transformation|GetActorLocation)))
    (Variables|Default|SetEndLocation (+ _output_get (Math|Vector|MakeVector (Variables|Default|GetPosDiffX) 0.0 (Variables|Default|GetPosDiffZ))))
    (bind _newtrack_0 (Timeline|Timeline_0 Play)
      (:Update
        (Transformation|SetActorLocation (Math|Vector|Lerp(Vector) (Variables|Default|GetInitialLocation) (Variables|Default|GetEndLocation) _newtrack_0) false false))
      (:Finished
        (if (Variables|Default|GetTimeFactor)
          (Variables|Default|SetTimeFactor false)
          (Timeline|Timeline_0 ReverseFromEnd)
          (else
            (Variables|Default|SetTimeFactor true)
            (Timeline|Timeline_0 PlayFromStart)))))))

(event EventTick
  (params (DeltaSeconds :type Float%20%28single-precision%29))
  ;[1 1 1] Rotate
  (Variables|Default|SetTimer (+ DeltaSeconds (Variables|Default|GetTimer)))
  (Transformation|SetActorRotation (Math|Rotator|MakeRotator 0.0 (* (Variables|Default|GetTimer) (Variables|Default|GetRotation)) 0.0))
  (if (not (Variables|Default|GetLerp))
    (Variables|/Script/Engine.MovementComponent|SetVelocity (Variables|Default|GetProjectileMovement) (Math|Vector|MakeVector 0.0 0.0 (Variables|Default|GetZVelocity)))))

(fn ConstructionScript)
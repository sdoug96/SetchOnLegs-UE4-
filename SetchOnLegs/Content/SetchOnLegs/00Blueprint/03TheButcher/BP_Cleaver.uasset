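; BP_Cleaver is a physics projectile from The Butcher that damages the player character, BP_Spike.
; On spawn it launches by impulse, scaling the X gap between the Butcher's spawn point and the player, with fixed upward lift.
; Burst cleavers skip that calculation and use their existing Impulse value.
; Hitbox overlap deals damage unless Spike is in one exempt state; the cleaver destroys itself on damage, any hit, or timeout.
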(event OnComponentBeginOverlap(HitBox)
  (params (OverlappedComponent :type Primitive%20Component%20Object%20Reference) (OtherActor :type Actor%20Object%20Reference) (OtherComp :type Primitive%20Component%20Object%20Reference) (OtherBodyIndex :type Integer) (bFromSweep :type Boolean) (SweepResult :type Hit%20Result%20Structure%20%28by%20ref%29))
  ;[1 1 1] Player Collision
  (bind _asbp_spike (Utilities|Casting|CastToBP_Spike OtherActor))
  (if (Utilities|Enum|NotEqual(Enum) (Variables|/Game/SetchOnLegs/00Blueprint/07Spike/BP_Spike.BP_Spike_C|GetState _asbp_spike) "NewEnumerator5")
    (Default|DamageSytsem _asbp_spike 1)
    (Actor|DestroyActor)))

(event OnComponentHit(Cleaver)
  (params (HitComponent :type Primitive%20Component%20Object%20Reference) (OtherActor :type Actor%20Object%20Reference) (OtherComp :type Primitive%20Component%20Object%20Reference) (NormalImpulse :type Vector :default "0, 0, 0") (Hit :type Hit%20Result%20Structure%20%28by%20ref%29))
  ;[1 1 1] Destroy actor if it hits anything
  (Actor|DestroyActor))

(event Custom|CalculateImpulse
  ;[1 1 1] Calculate impulse function
  (bind _outactors (Actor|GetAllActorsOfClass "/Game/SetchOnLegs/00Blueprint/03TheButcher/BP_TheButcher.BP_TheButcher_C"))
  (Variables|Default|SetImpulse (Math|Vector|MakeVector (/ (- (.x (Transformation|GetWorldLocation (Variables|/Script/Engine.Character|GetCapsuleComponent (Variables|Default|GetPlayer)))) (.x (Transformation|GetWorldLocation (Variables|/Game/SetchOnLegs/00Blueprint/03TheButcher/BP_TheButcher.BP_TheButcher_C|GetCleaverSpawn (Utilities|Array|Get(acopy) _outactors))))) 18.0) 0.0 5e+01)))

(event EventBeginPlay
  ;[1 1 1] Initialise
  (bind _asbp_spike (Utilities|Casting|CastToBP_Spike (Game|GetPlayerCharacter 0)))
  (Variables|Default|SetPlayer _asbp_spike)
  (Utilities|FlowControl|Sequence
    (:then_0
      (if (not (Variables|Default|GetBurstCleaver))
        (CallFunction|CalculateImpulse)))
    (:then_1
      (Physics|AddImpulse (Variables|Default|GetCleaver) (Variables|Default|GetImpulse) "None" false)
      (Utilities|FlowControl|Delay 5.0)
      (Actor|DestroyActor))))

(fn ConstructionScript)
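; BP_Spikes is a spike trap that cycles between two positions and damages the player character, BP_Spike.
; A WakeBox, detached at BeginPlay so it stays put, activates the trap while the player overlaps it.
; A self-calling Delay loop teleports the actor between StartPos and EndPos with sound, arming damage at EndPos.
; Tick applies damage every frame the player overlaps HitBox while armed.
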(event OnComponentBeginOverlap(WakeBox)
  (params (OverlappedComponent :type Primitive%20Component%20Object%20Reference) (OtherActor :type Actor%20Object%20Reference) (OtherComp :type Primitive%20Component%20Object%20Reference) (OtherBodyIndex :type Integer) (bFromSweep :type Boolean) (SweepResult :type Hit%20Result%20Structure%20%28by%20ref%29))
  (Utilities|Casting|CastToBP_Spike OtherActor)
  (Variables|Default|SetActive true)
  (CallFunction|SpikesStart))

(event OnComponentEndOverlap(WakeBox)
  (params (OverlappedComponent :type Primitive%20Component%20Object%20Reference) (OtherActor :type Actor%20Object%20Reference) (OtherComp :type Primitive%20Component%20Object%20Reference) (OtherBodyIndex :type Integer))
  (Utilities|Casting|CastToBP_Spike OtherActor)
  (Variables|Default|SetActive false)
  (Variables|Default|SetHitPlayer false)
  (if (Math|Vector|Equal(Vector) (Transformation|GetActorLocation) (Variables|Default|GetEndPos) 0.0001)
    (Transformation|SetActorLocation (Variables|Default|GetStartPos) false false)
    (Audio|PlaySound2D "/Game/SetchOnLegs/03Audio/06Rosemarkie/SpikesUp.SpikesUp" 1.0 1.0 0.0 0 0)))

(event Custom|SpikesStart
  (if (Variables|Default|GetActive)
    (Transformation|SetActorLocation (Variables|Default|GetEndPos) false false)
    (Audio|PlaySound2D "/Game/SetchOnLegs/03Audio/06Rosemarkie/SpikesUp.SpikesUp" 1.0 1.0 0.0 0 0)
    (Variables|Default|SetHitPlayer true)
    (Utilities|FlowControl|Delay (Variables|Default|GetSwitchDelay))
    (Transformation|SetActorLocation (Variables|Default|GetStartPos) false false)
    (Audio|PlaySound2D "/Game/SetchOnLegs/03Audio/06Rosemarkie/SpikesUp.SpikesUp" 1.0 1.0 0.0 0 0)
    (Variables|Default|SetHitPlayer false)
    (Utilities|FlowControl|Delay (Variables|Default|GetSwitchDelay))
    (CallFunction|SpikesStart)))

(event EventBeginPlay
  (Transformation|SetActorLocation (Variables|Default|GetStartPos) false false)
  (Transformation|DetachFromComponent (Variables|Default|GetWakeBox) "KeepWorld" "KeepWorld" "KeepWorld" true)
  (bind _asbp_spike (Utilities|Casting|CastToBP_Spike (Game|GetPlayerCharacter 0)))
  (Variables|Default|SetPlayer _asbp_spike))

(event EventTick
  (params (DeltaSeconds :type Float%20%28single-precision%29))
  (if (Variables|Default|GetActive)
    (if (Collision|IsOverlappingActor (Variables|Default|GetHitBox) (Variables|Default|GetPlayer) :!class /Script/Engine.PrimitiveComponent)
      (if (Variables|Default|GetHitPlayer)
        (Default|DamageSystem (Variables|Default|GetPlayer) 1)))))

(fn ConstructionScript)
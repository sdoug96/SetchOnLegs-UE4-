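; BP_SpinBlade is a hazard that spins in pitch on Tick and damages the BP_Spike player character.
; With Lerp set, a timeline ping-pongs it between its start and an X/Z offset; otherwise ProjectileMovement velocity drives it.
; Sphere overlap deals damage unless the player is in one excluded state, optionally launching them along X with briefly raised falling lateral friction.
; The delayed self-destroy branch for projectile mode is unconnected.
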(event OnComponentBeginOverlap(Sphere)
  (params (OverlappedComponent :type Primitive%20Component%20Object%20Reference) (OtherActor :type Actor%20Object%20Reference) (OtherComp :type Primitive%20Component%20Object%20Reference) (OtherBodyIndex :type Integer) (bFromSweep :type Boolean) (SweepResult :type Hit%20Result%20Structure%20%28by%20ref%29))
  ;[1 1 1] Player Collision
  (bind _asbp_spike (Utilities|Casting|CastToBP_Spike OtherActor))
  (if (Utilities|Enum|NotEqual(Enum) (Variables|/Game/SetchOnLegs/00Blueprint/07Spike/BP_Spike.BP_Spike_C|GetState _asbp_spike) "NewEnumerator5")
    (Default|DamageSytsem _asbp_spike 1)
    (if (Variables|Default|GetLaunch)
      (Character|LaunchCharacter (Variables|Default|GetPlayer) (Math|Vector|MakeVector (Variables|Default|GetLaunchForce) 0.0 0.0) false false)
      (Variables|/Script/Engine.CharacterMovementComponent|SetFallingLateralFriction (Variables|/Script/Engine.Character|GetCharacterMovement (Variables|Default|GetPlayer)) 8.0)
      (Utilities|FlowControl|Delay 0.4)
      (Variables|/Script/Engine.CharacterMovementComponent|SetFallingLateralFriction (Variables|/Script/Engine.Character|GetCharacterMovement (Variables|Default|GetPlayer)) 0.0))))

(event EventBeginPlay
  ;[1 1 1] Movement
  (bind _asbp_spike (Utilities|Casting|CastToBP_Spike (Game|GetPlayerCharacter 0)))
  (Variables|Default|SetPlayer _asbp_spike)
  (if (Variables|Default|GetLerp)
    (bind _output_get (Variables|Default|SetInitialLocation (Transformation|GetActorLocation)))
    (Variables|Default|SetEndLocation (+ _output_get (Math|Vector|MakeVector (Variables|Default|GetPosDiffX) 0.0 (Variables|Default|GetPosDiffZ))))
    (bind _newtrack_0 (Timeline|LerpTimeline Play)
      (:Update
        (Transformation|SetActorLocation (Math|Vector|Lerp(Vector) (Variables|Default|GetInitialLocation) (Variables|Default|GetEndLocation) _newtrack_0) false false))
      (:Finished
        (if (Variables|Default|GetTimeFactor)
          (Variables|Default|SetTimeFactor false)
          (Timeline|LerpTimeline ReverseFromEnd)
          (else
            (Variables|Default|SetTimeFactor true)
            (Timeline|LerpTimeline PlayFromStart)))))))

(event EventTick
  (params (DeltaSeconds :type Float%20%28single-precision%29))
  ;[1 1 1] Rotate or move
  (Variables|Default|SetTimer (+ DeltaSeconds (Variables|Default|GetTimer)))
  (Transformation|SetActorRotation (Math|Rotator|MakeRotator 0.0 (* (Variables|Default|GetTimer) (Variables|Default|GetRotation)) 0.0))
  (if (not (Variables|Default|GetLerp))
    (Variables|/Script/Engine.MovementComponent|SetVelocity (Variables|Default|GetProjectileMovement) (Math|Vector|MakeVector (Variables|Default|GetXVelocity) 0.0 (Variables|Default|GetZVelocity)))))

(fn ConstructionScript)
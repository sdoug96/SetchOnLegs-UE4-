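; The Butcher boss: StartFight shows its HUD, sets it moving and starts timed cleaver throws.
; Tick uses one-shot health thresholds to begin a self-chaining blade cycle, then retune its timing and speed.
; The cycle alternates drop rows with two random gaps and delayed-loop volleys from alternating sides.
; Player bullets deal damage with a timer-driven blink; death stops attacks, clears hazards and shows a death flipbook before destroying the boss.
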(event OnComponentBeginOverlap(BulletBox)
  (params (OverlappedComponent :type Primitive%20Component%20Object%20Reference) (OtherActor :type Actor%20Object%20Reference) (OtherComp :type Primitive%20Component%20Object%20Reference) (OtherBodyIndex :type Integer) (bFromSweep :type Boolean) (SweepResult :type Hit%20Result%20Structure%20%28by%20ref%29))
  ;[1 1 1] Bullet Collision
  (bind _asbp_bullet (Utilities|Casting|CastToBP_Bullet OtherActor))
  (Actor|DestroyActor _asbp_bullet)
  (if (not (Variables|Default|GetIsDead))
    (CallFunction|DamageSytsem (Variables|/Game/SetchOnLegs/00Blueprint/07Spike/BP_Spike.BP_Spike_C|GetBulletDamage (Variables|Default|GetPlayer)))))

(event Custom|Blink
  (bind _sprite (Variables|Default|GetSprite))
  ;[1 1 1] Damage & Death System
  (Development|SetHiddeninGame _sprite (not (Variables|/Script/Engine.SceneComponent|GetbHiddenInGame _sprite)) false))

(event Custom|Damage%20Sytsem
  (params (DamageIn :type Float%20%28single-precision%29))
  ;[1 1 1] Damage & Death System
  (bind _output_get (Variables|Default|SetCurrentHealth (- (Variables|Default|GetCurrentHealth) DamageIn)))
  (if (<= _output_get 0.0)
    (Variables|Default|SetIsDead true)
    (Widget|RemovefromParent (Variables|Default|GetHUD))
    (Utilities|Time|ClearTimerbyFunctionName 0 "SpawnCleaver")
    (Utilities|Time|ClearTimerbyFunctionName 0 "SpawnBlades")
    (Variables|/Script/Engine.MovementComponent|SetVelocity (Variables|Character|GetCharacterMovement) "0, 0, 0")
    (Sprite|SetFlipbook (Variables|Default|GetSprite) "/Game/SetchOnLegs/01Sprites/07Spike/Character/A_Dead.A_Dead")
    (Transformation|SetWorldScale3D (Variables|Default|GetSprite) "1.500000,1.500000,1.500000")
    (Transformation|SetRelativeLocation (Variables|Default|GetSprite) "-48.000000,0.000000,-350.000000" false false)
    (Audio|PlaySound2D "/Game/SetchOnLegs/03Audio/00Menus/Splat.Splat" 1.0 1.0 0.0 0 0)
    (Utilities|FlowControl|Delay 2.0)
    (Actor|DestroyActor)
    (else
      (Utilities|Time|SetTimerbyFunctionName 0 "Blink" 0.05 true)
      (Utilities|FlowControl|Delay 0.2)
      (Utilities|Time|ClearTimerbyFunctionName 0 "Blink")
      (Development|SetHiddeninGame (Variables|Default|GetSprite) false false))))

(event Custom|SetBladesToSpawn
  ;[1 1 1] Drop Blade Logic
  (Variables|Default|SetRandomBlade1 (Math|Random|RandomIntegerinRange 0 6))
  (Variables|Default|SetRandomBlade2 (Math|Random|RandomIntegerinRange 0 6))
  (while (== (Variables|Default|GetRandomBlade1) (Variables|Default|GetRandomBlade2))
    (Variables|Default|SetRandomBlade2 (Math|Random|RandomIntegerinRange 0 6))))

(event Custom|StartFight
  ;[1 1 1] Start Fight Function
  (bind _returnvalue (UserInterface|CreateWidget "/Game/SetchOnLegs/00Blueprint/03TheButcher/Boss/Widget_TheButcher.Widget_TheButcher_C"))
  (bind _output_get (Variables|Default|SetHUD _returnvalue))
  (UserInterface|Viewport|AddtoViewport _output_get 0)
  (Sprite|SetFlipbook (Variables|Default|GetSprite) "/Game/SetchOnLegs/01Sprites/03TheButcher/Character/A_ButcherAttack.A_ButcherAttack")
  (Variables|/Script/Engine.MovementComponent|SetVelocity (Variables|Character|GetCharacterMovement) "-200.000000, 0, 0")
  (Utilities|Time|SetTimerbyFunctionName 0 "SpawnCleaver" (Variables|Default|GetCleaverDelay) true))

(event Custom|DropBlades
  ;[1 1 1] Drop Blade Logic
  (Audio|PlaySound2D "/Game/SetchOnLegs/03Audio/03TheButcher/SawBlade.SawBlade" 1.0 1.0 0.0 0 0)
  (for _index (range 0 (- (Variables|Default|GetBladesToDrop) 1))
    (if (== _index (Variables|Default|GetRandomBlade1))
      _
      (elif (== _index (Variables|Default|GetRandomBlade2))
        _
        (else
          (Game|SpawnActorfromClass "/Game/SetchOnLegs/00Blueprint/03TheButcher/BP_SpinBlade.BP_SpinBlade_C" (Math|Transform|MakeTransform (Math|Vector|MakeVector (Variables|Default|GetBladeXPos) -0.1 2.4e+02) "0, 0, 0" "0.187500,0.187500,0.187500") "Undefined" 0 false 0.0 0.0 0.0 (Variables|Default|GetBladeDropSpeed) 0))))
    (Variables|Default|SetBladeXPos (+ (Variables|Default|GetBladeXPos) 1.8e+02)))
  (Variables|Default|SetBladeXPos 6e+01)
  (CallFunction|SetBladestoSpawn)
  (Utilities|FlowControl|Delay (Variables|Default|GetAttackDelay))
  (CallFunction|SideBlades))

(event Custom|SpawnCleaver
  ;[1 1 1] Cleaver Logic
  (if (not (Variables|Default|GetIsDead))
    (Game|SpawnActorfromClass "/Game/SetchOnLegs/00Blueprint/03TheButcher/Boss/BP_Cleaver.BP_Cleaver_C" (Transformation|GetWorldTransform (Variables|Default|GetCleaverSpawn)) "Undefined" 0 0)
    (Audio|PlaySound2D "/Game/SetchOnLegs/03Audio/03TheButcher/Knife.Knife" 1.0 1.0 0.0 0 0)))

(event Custom|SideBlades
  ;[1 1 1] Blade Logic
  (if (Variables|Default|GetSideBladeRight)
    (if (not (Variables|Default|GetIsDead))
      (Utilities|ForLoopwithDelay 0 (- (Variables|Default|GetSideBladesToSpawn) 1) :!label _label
        (:Loop%20Body
          (Game|SpawnActorfromClass "/Game/SetchOnLegs/00Blueprint/03TheButcher/BP_SpinBlade.BP_SpinBlade_C" (Math|Transform|MakeTransform "1640.000000,-0.100000,-690.000000" "0, 0, 0" "0.187500,0.187500,0.187500") "Undefined" 0 false 0.0 0.0 (* (Variables|Default|GetSideBladeSpeed) -1.0) 0.0 0)
          (Audio|PlaySound2D "/Game/SetchOnLegs/03Audio/03TheButcher/SawBladeShort.SawBladeShort" 1.0 1.0 0.0 0 0))
        (:Completed
          (Utilities|FlowControl|Delay (Variables|Default|GetAttackDelay))
          (CallFunction|DropBlades)
          (Variables|Default|SetSideBladeRight false))
        (:Delay%20Out
          (Utilities|FlowControl|Delay (Variables|Default|GetSideBladeDelay))
          (goto _label Delay%20In))))
    (elif (not (Variables|Default|GetIsDead))
      (Utilities|ForLoopwithDelay 0 (- (Variables|Default|GetSideBladesToSpawn) 1) :!label _label_2
        (:Loop%20Body
          (Game|SpawnActorfromClass "/Game/SetchOnLegs/00Blueprint/03TheButcher/BP_SpinBlade.BP_SpinBlade_C" (Math|Transform|MakeTransform "-440.000000,-0.100000,-690.000000" "0, 0, 0" "0.187500,0.187500,0.187500") "Undefined" 0 false 0.0 0.0 (Variables|Default|GetSideBladeSpeed) 0.0 0)
          (Audio|PlaySound2D "/Game/SetchOnLegs/03Audio/03TheButcher/SawBladeShort.SawBladeShort" 1.0 1.0 0.0 0 0))
        (:Completed
          (Utilities|FlowControl|Delay (Variables|Default|GetAttackDelay))
          (CallFunction|DropBlades)
          (Variables|Default|SetSideBladeRight true))
        (:Delay%20Out
          (Utilities|FlowControl|Delay (Variables|Default|GetSideBladeDelay))
          (goto _label_2 Delay%20In))))))

(event EventBeginPlay
  ;[1 1 1] Initialise
  (bind _asbp_spike (Utilities|Casting|CastToBP_Spike (Game|GetPlayerCharacter 0)))
  (Variables|Default|SetPlayer _asbp_spike))

(event EventTick
  (params (DeltaSeconds :type Float%20%28single-precision%29))
  (bind _currenthealth (Variables|Default|GetCurrentHealth))
  ;[1 1 1] Tick Attack and Death Logic
  (Utilities|FlowControl|Sequence
    (:then_0
      (if (< _currenthealth 3.2e+02)
        (Utilities|FlowControl|DoOnce false
          (:Completed
            (CallFunction|DropBlades)))))
    (:then_1
      (if (< _currenthealth 1.6e+02)
        (Utilities|FlowControl|DoOnce false
          (:Completed
            (Variables|Default|SetAttackDelay 3.5)
            (Variables|Default|SetSideBladeDelay 0.75)
            (Variables|Default|SetSideBladeSpeed 7.5e+02)))))
    (:then_2
      (if (Variables|Default|GetIsDead)
        (bind _outactors (Actor|GetAllActorsOfClass "/Game/SetchOnLegs/00Blueprint/03TheButcher/BP_SpinBlade.BP_SpinBlade_C"))
        (Actor|DestroyActor _outactors)
        (bind _outactors_2 (Actor|GetAllActorsOfClass "/Game/SetchOnLegs/00Blueprint/03TheButcher/BP_DragPad.BP_DragPad_C"))
        (Actor|DestroyActor _outactors_2)
        (bind _outactors_3 (Actor|GetAllActorsOfClass "/Game/SetchOnLegs/00Blueprint/03TheButcher/Boss/BP_Cleaver.BP_Cleaver_C"))
        (Actor|DestroyActor _outactors_3)))))

(fn ConstructionScript)
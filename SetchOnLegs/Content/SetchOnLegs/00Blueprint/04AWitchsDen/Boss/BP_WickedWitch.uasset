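; Flying Wicked Witch boss with flipbook animation states, a health-phased fight and a HUD added on fight start.
; StartFight begins an alternating loop of spell orb throws and delayed fireball volleys.
; Tick updates facing and launch vectors; health thresholds retune attacks and activate bat spawners, then minions, while death destroys spawned hazards and helpers.
; Bullets damage head and body; the shield knocks back and damages the player.
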(event OnComponentBeginOverlap(BodyBox)
  (params (OverlappedComponent :type Primitive%20Component%20Object%20Reference) (OtherActor :type Actor%20Object%20Reference) (OtherComp :type Primitive%20Component%20Object%20Reference) (OtherBodyIndex :type Integer) (bFromSweep :type Boolean) (SweepResult :type Hit%20Result%20Structure%20%28by%20ref%29))
  ;[1 1 1] Collision Logic
  (Utilities|Casting|CastToBP_Bullet OtherActor)
  (CallFunction|BulletCollision)
  (Audio|PlaySound2D "/Game/SetchOnLegs/03Audio/07Spike/EnemyHit.EnemyHit" 1.0 1.0 0.0 0 0))

(event OnComponentBeginOverlap(HeadSphere)
  (params (OverlappedComponent :type Primitive%20Component%20Object%20Reference) (OtherActor :type Actor%20Object%20Reference) (OtherComp :type Primitive%20Component%20Object%20Reference) (OtherBodyIndex :type Integer) (bFromSweep :type Boolean) (SweepResult :type Hit%20Result%20Structure%20%28by%20ref%29))
  ;[1 1 1] Collision Logic
  (Utilities|Casting|CastToBP_Bullet OtherActor)
  (CallFunction|BulletCollision)
  (Audio|PlaySound2D "/Game/SetchOnLegs/03Audio/07Spike/EnemyHit.EnemyHit" 1.0 1.0 0.0 0 0))

(event OnComponentBeginOverlap(ShieldSphere)
  (params (OverlappedComponent :type Primitive%20Component%20Object%20Reference) (OtherActor :type Actor%20Object%20Reference) (OtherComp :type Primitive%20Component%20Object%20Reference) (OtherBodyIndex :type Integer) (bFromSweep :type Boolean) (SweepResult :type Hit%20Result%20Structure%20%28by%20ref%29))
  ;[1 1 1] Collision Logic
  (Utilities|Casting|CastToBP_Spike OtherActor)
  (if (Variables|Default|GetActive)
    (Character|LaunchCharacter (Variables|Default|GetPlayer) (Variables|Default|GetShieldLaunchVelocity) true true)
    (Default|DamageSystem (Variables|Default|GetPlayer) 1)))

(event Custom|UpdateAnimation
  ;[1 1 1] Handle Animation
  (switch Utilities|FlowControl|Switch|SwitchonEnum_WickedWitchState (Variables|Default|GetState)
    (:NewEnumerator0
      (Sprite|SetFlipbook (Variables|Default|GetSprite) "/Game/SetchOnLegs/01Sprites/04AWitchesWelcome/Character/Animations/A_WickedWitchFlying.A_WickedWitchFlying"))
    (:NewEnumerator1
      (Sprite|SetFlipbook (Variables|Default|GetSprite) "/Game/SetchOnLegs/01Sprites/04AWitchesWelcome/Character/Animations/A_WickedWitchThrowing.A_WickedWitchThrowing"))
    (:NewEnumerator3
      (Sprite|SetFlipbook (Variables|Default|GetSprite) "/Game/SetchOnLegs/01Sprites/04AWitchesWelcome/Character/Death/A_WickedWitchDeath.A_WickedWitchDeath")
      (Transformation|SetRelativeScale3D (Variables|Default|GetSprite) "3.000000,3.000000,3.000000"))))

(event Custom|StartFight
  ;[1 1 1] Start Fight
  (bind _returnvalue (UserInterface|CreateWidget "/Game/SetchOnLegs/00Blueprint/04AWitchsDen/Boss/Widget_WickedWitch.Widget_WickedWitch_C"))
  (bind _output_get (Variables|Default|SetHUD _returnvalue))
  (UserInterface|Viewport|AddtoViewport _output_get 0)
  (Variables|Default|SetActive true)
  (Utilities|FlowControl|Delay (Variables|Default|GetAttackDelay))
  (CallFunction|SpellAttack))

(event Custom|FireballAttack
  ;[1 1 1] Fireball Attack
  (if (not (Variables|Default|GetIsDead))
    (Utilities|FlowControl|Delay 0.5)
    (Audio|PlaySound2D "/Game/SetchOnLegs/03Audio/04AWitchesWelcome/Cackle.Cackle" 1.0 1.0 0.0 0 0)
    (Utilities|ForLoopwithDelay 0 (- (Variables|Default|GetFireballCount) 1) :!label _label
      (:Loop%20Body
        (Game|SpawnActorfromClass "/Game/SetchOnLegs/00Blueprint/04AWitchsDen/Boss/BP_Flameball.BP_Flameball_C" (Math|Transform|MakeTransform (Transformation|GetWorldLocation (Variables|Default|GetFireballSpawn)) "0, 0, 0" "1,1,1") "Undefined" 0 1 5.0 false 0.0 0.0 true 0))
      (:Completed
        (Utilities|FlowControl|Delay (Variables|Default|GetAttackDelay))
        (CallFunction|SpellAttack))
      (:Delay%20Out
        (Utilities|FlowControl|Delay 0.25)
        (goto _label Delay%20In)))))

(event Custom|SpellAttack
  ;[1 1 1] Spell Attack
  (if (not (Variables|Default|GetIsDead))
    (Variables|Default|SetState "NewEnumerator1")
    (CallFunction|UpdateAnimation)
    (Utilities|FlowControl|Delay 0.45)
    (Game|SpawnActorfromClass "/Game/SetchOnLegs/00Blueprint/04AWitchsDen/Boss/BP_SpellOrb.BP_SpellOrb_C" (Transformation|GetWorldTransform (Variables|Default|GetSpellSpawn)) "Undefined" 0 1 3e+01 true 6e+02 0.0 true 0)
    (Audio|PlaySound2D "/Game/SetchOnLegs/03Audio/04AWitchesWelcome/Cackle.Cackle" 1.0 1.0 0.0 0 0)
    (Variables|Default|SetState "NewEnumerator0")
    (CallFunction|UpdateAnimation)
    (Utilities|FlowControl|Delay (Variables|Default|GetAttackDelay))
    (CallFunction|FireballAttack)))

(event Custom|SetCharacterRotation
  (bind _spellspawn (Variables|Default|GetSpellSpawn))
  (bind _fireballspawn (Variables|Default|GetFireballSpawn))
  ;[1 1 1] Set Character Rotation
  (if (>= (.x (Variables|/Script/Engine.MovementComponent|GetVelocity (Variables|Character|GetCharacterMovement))) 0.0)
    (Transformation|SetActorRotation "0, 0, 0")
    (Transformation|SetRelativeLocation _spellspawn "58.000000,0.100000,-96.000000" false false)
    (Transformation|SetRelativeLocation _fireballspawn "12.000000,-0.100000,-96.000000" false false)
    (else
      (Transformation|SetActorRotation "0,180.000000, 0")
      (Transformation|SetRelativeLocation _spellspawn "58.000000,-0.100000,-96.000000" false false)
      (Transformation|SetRelativeLocation _fireballspawn "12.000000,0.100000,-96.000000" false false))))

(event Custom|SetShieldLaunchVelocity
  ;[1 1 1] Set Shield Launch Velocity
  (Utilities|FlowControl|Sequence
    (:then_0
      (if (> (.x (Transformation|GetActorLocation (Variables|Default|GetPlayer))) (.x (Transformation|GetActorLocation)))
        (Variables|Default|SetShieldLaunchVelocity (Math|Vector|MakeVector (Variables|Default|GetShieldLaunchPower) 0.0 (.z (Variables|Default|GetShieldLaunchVelocity))))
        (else
          (Variables|Default|SetShieldLaunchVelocity (Math|Vector|MakeVector (* (Variables|Default|GetShieldLaunchPower) -1.0) 0.0 (.z (Variables|Default|GetShieldLaunchVelocity)))))))
    (:then_1
      (if (> (.z (Transformation|GetActorLocation (Variables|Default|GetPlayer))) (.z (Transformation|GetActorLocation)))
        (Variables|Default|SetShieldLaunchVelocity (Math|Vector|MakeVector (.x (Variables|Default|GetShieldLaunchVelocity)) 0.0 (Variables|Default|GetShieldLaunchPower)))
        (else
          (Variables|Default|SetShieldLaunchVelocity (Math|Vector|MakeVector (.x (Variables|Default|GetShieldLaunchVelocity)) 0.0 (* (Variables|Default|GetShieldLaunchPower) -1.0))))))))

(event Custom|SetOrbLaunchVelocity
  ;[1 1 1] Set Orb Launch Velocity
  (if (Math|Rotator|Equal(Rotator) (Transformation|GetActorRotation) "0, 0, 0" 0.0001)
    (Variables|Default|SetOrbLaunchVelocity "500.000000,0.000000,-500.000000")
    (else
      (Variables|Default|SetOrbLaunchVelocity "-500.000000,0.000000,-500.000000"))))

(event EventDamageSystem
  (params (DamageIn :type Float%20%28single-precision%29))
  ;[1 1 1] Damage & Death System
  (|CallParentFunction DamageIn)
  (if (Variables|Default|GetIsDead)
    (Variables|Default|SetState "NewEnumerator3")
    (CallFunction|UpdateAnimation)
    (Widget|RemovefromParent (Variables|Default|GetHUD))
    (Audio|PlaySound2D "/Game/SetchOnLegs/03Audio/04AWitchesWelcome/WickedWitchDeath.WickedWitchDeath" 1.0 1.0 0.0 0 0)
    (Rendering|SetVisibility (Variables|Default|GetShield) false false)
    (Collision|SetCollisionEnabled (Variables|Default|GetHeadSphere) "NoCollision")))

(event EventBeginPlay
  ;[1 1 1] Begin Play
  (|CallParentFunction)
  (Variables|Default|SetState "NewEnumerator0")
  (CallFunction|UpdateAnimation))

(event EventTick
  (params (DeltaSeconds :type Float%20%28single-precision%29))
  ;[1 1 1] Tick
  (Utilities|FlowControl|Sequence
    (:then_0
      (CallFunction|SetCharacterRotation)
      (CallFunction|SetShieldLaunchVelocity)
      (CallFunction|SetOrbLaunchVelocity))
    (:then_1
      (if (Math|Float|InRange(Float) (Variables|Default|GetCurrentHealth) 76.0 1.5e+02)
        (Utilities|FlowControl|DoOnce false
          (:Completed
            (Variables|Default|SetAttackDelay 2.75)
            (Variables|Default|SetFireballCount 4)
            (bind _outactors (Actor|GetAllActorsOfClass "/Game/SetchOnLegs/00Blueprint/04AWitchsDen/Hazards/BP_BatSpawner.BP_BatSpawner_C"))
            (for _array_element _outactors
              (Variables|/Game/SetchOnLegs/00Blueprint/04AWitchsDen/Hazards/BP_BatSpawner.BP_BatSpawner_C|SetActive _array_element true))))))
    (:then_2
      (if (Math|Float|InRange(Float) (Variables|Default|GetCurrentHealth) 1.0 75.0)
        (Utilities|FlowControl|DoOnce false
          (:Completed
            (Variables|Default|SetAttackDelay 2.5)
            (Variables|Default|SetFireballCount 5)
            (bind _outactors_2 (Actor|GetAllActorsOfClass "/Game/SetchOnLegs/00Blueprint/04AWitchsDen/Enemies/BP_Minion.BP_Minion_C"))
            (for _array_element_2 _outactors_2
              (Variables|/Game/SetchOnLegs/00Blueprint/04AWitchsDen/Enemies/BP_Minion.BP_Minion_C|SetActive _array_element_2 true))))))
    (:then_3
      (if (Variables|Default|GetIsDead)
        (Utilities|FlowControl|DoOnce false
          (:Completed
            (bind _outactors_3 (Actor|GetAllActorsOfClass "/Game/SetchOnLegs/00Blueprint/04AWitchsDen/Enemies/BP_Minion.BP_Minion_C"))
            (Actor|DestroyActor _outactors_3)
            (bind _outactors_4 (Actor|GetAllActorsOfClass "/Game/SetchOnLegs/00Blueprint/04AWitchsDen/Boss/BP_Flameball.BP_Flameball_C"))
            (Actor|DestroyActor _outactors_4)
            (bind _outactors_5 (Actor|GetAllActorsOfClass "/Game/SetchOnLegs/00Blueprint/04AWitchsDen/Hazards/BP_Orb.BP_Orb_C"))
            (Actor|DestroyActor _outactors_5)
            (bind _outactors_6 (Actor|GetAllActorsOfClass "/Game/SetchOnLegs/00Blueprint/04AWitchsDen/Hazards/BP_BatSpawner.BP_BatSpawner_C"))
            (Actor|DestroyActor _outactors_6)
            (bind _outactors_7 (Actor|GetAllActorsOfClass "/Game/SetchOnLegs/00Blueprint/04AWitchsDen/Enemies/BP_Bat.BP_Bat_C"))
            (Actor|DestroyActor _outactors_7)
            (bind _outactors_8 (Actor|GetAllActorsOfClass "/Game/SetchOnLegs/00Blueprint/04AWitchsDen/Boss/BP_SpellOrb.BP_SpellOrb_C"))
            (Actor|DestroyActor _outactors_8)))))))

(fn ConstructionScript)

(fn SetSpeed
  (params (XSpeed :type Float%20%28single-precision%29) (ZSpeed :type Float%20%28single-precision%29))
  (Variables|/Script/Engine.MovementComponent|SetVelocity (Variables|Character|GetCharacterMovement) (Math|Vector|MakeVector XSpeed 0.0 ZSpeed)))
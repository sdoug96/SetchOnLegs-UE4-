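; Flying bat enemy that homes toward the player, takes bullet hits and damages BP_Spike on contact.
; Homing projectile movement targets the player's capsule from BeginPlay, while BP_Spike entering or leaving the wake sphere starts or stops the chase.
; Idle, Chasing and Dead states drive the flipbook, and death disables hit collision on top of parent damage logic.
; Tick updates rotation and shifts the point light according to the player's side.
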(event OnComponentBeginOverlap(WakeSphere)
  (params (OverlappedComponent :type Primitive%20Component%20Object%20Reference) (OtherActor :type Actor%20Object%20Reference) (OtherComp :type Primitive%20Component%20Object%20Reference) (OtherBodyIndex :type Integer) (bFromSweep :type Boolean) (SweepResult :type Hit%20Result%20Structure%20%28by%20ref%29))
  ;[1 1 1] Wake Sphere Logic
  (Utilities|Casting|CastToBP_Spike OtherActor)
  (Variables|/Script/Engine.ProjectileMovementComponent|SetbIsHomingProjectile (Variables|Default|GetProjectileMovement) true)
  (Variables|Default|SetActive true)
  (Variables|Default|SetState "NewEnumerator1")
  (CallFunction|UpdateAnimation))

(event OnComponentBeginOverlap(HitSphere)
  (params (OverlappedComponent :type Primitive%20Component%20Object%20Reference) (OtherActor :type Actor%20Object%20Reference) (OtherComp :type Primitive%20Component%20Object%20Reference) (OtherBodyIndex :type Integer) (bFromSweep :type Boolean) (SweepResult :type Hit%20Result%20Structure%20%28by%20ref%29))
  ;[1 1 1] Collision Logic
  (Utilities|FlowControl|Sequence
    (:then_0
      (Utilities|Casting|CastToBP_Bullet OtherActor)
      (CallFunction|BulletCollision)
      (Audio|PlaySound2D "/Game/SetchOnLegs/03Audio/07Spike/EnemyHit.EnemyHit" 1.0 1.0 0.0 0 0))
    (:then_1
      (bind _asbp_spike (Utilities|Casting|CastToBP_Spike OtherActor))
      (Default|DamageSystem _asbp_spike 1))))

(event OnComponentEndOverlap(WakeSphere)
  (params (OverlappedComponent :type Primitive%20Component%20Object%20Reference) (OtherActor :type Actor%20Object%20Reference) (OtherComp :type Primitive%20Component%20Object%20Reference) (OtherBodyIndex :type Integer))
  ;[1 1 1] Wake Sphere Logic
  (Utilities|Casting|CastToBP_Spike OtherActor)
  (Variables|/Script/Engine.ProjectileMovementComponent|SetbIsHomingProjectile (Variables|Default|GetProjectileMovement) false)
  (Components|Movement|StopMovementImmediately (Variables|Default|GetProjectileMovement))
  (Variables|Default|SetActive false)
  (Variables|Default|SetState "NewEnumerator0")
  (CallFunction|UpdateAnimation))

(event Custom|UpdateAnimation
  (bind _sprite (Variables|Default|GetSprite))
  ;[1 1 1] Update Animation
  (switch Utilities|FlowControl|Switch|SwitchonBatState (Variables|Default|GetState)
    (:NewEnumerator0
      (Sprite|SetFlipbook (Variables|Default|GetSprite) "/Game/SetchOnLegs/01Sprites/04AWitchesWelcome/Bat/A_Bat.A_Bat"))
    (:NewEnumerator1
      (Sprite|SetFlipbook _sprite "/Game/SetchOnLegs/01Sprites/04AWitchesWelcome/Bat/A_Bat.A_Bat"))
    (:NewEnumerator2
      (Sprite|SetFlipbook _sprite))))

(event EventBeginPlay
  ;[1 1 1] Homing Projectile Logic
  (|CallParentFunction)
  (Variables|/Script/Engine.ProjectileMovementComponent|SetbIsHomingProjectile (Variables|Default|GetProjectileMovement) true)
  (Variables|/Script/Engine.ProjectileMovementComponent|SetHomingTargetComponent (Variables|Default|GetProjectileMovement) (Variables|/Script/Engine.Character|GetCapsuleComponent (Variables|Default|GetPlayer)))
  (Variables|/Script/Engine.ProjectileMovementComponent|SetHomingAccelerationMagnitude (Variables|Default|GetProjectileMovement) 7.5e+02)
  (Variables|/Script/Engine.ProjectileMovementComponent|SetMaxSpeed (Variables|Default|GetProjectileMovement) 2.5e+02))

(event EventTick
  (params (DeltaSeconds :type Float%20%28single-precision%29))
  (bind _pointlight (Variables|Default|GetPointLight))
  ;[1 1 1] Rotate Actor & Light
  (CallFunction|SetRotation)
  (if (Variables|Default|GetIsRightOfPlayer)
    (Transformation|SetRelativeLocation _pointlight "0,-80.000000, 0" false false)
    (else
      (Transformation|SetRelativeLocation _pointlight "0.000000,80.000000, 0" false false))))

(event EventDamageSystem
  (params (DamageIn :type Float%20%28single-precision%29))
  ;[1 1 1] Damage & Death System
  (|CallParentFunction DamageIn)
  (if (Variables|Default|GetIsDead)
    (Variables|Default|SetState "NewEnumerator2")
    (CallFunction|UpdateAnimation)
    (Collision|SetCollisionEnabled (Variables|Default|GetHitSphere) "NoCollision")))

(fn ConstructionScript)
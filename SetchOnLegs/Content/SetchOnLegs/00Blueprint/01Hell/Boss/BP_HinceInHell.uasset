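; Flying Hince boss for the Hell level, with a rising intro cutscene that creates its HUD before combat.
; It follows the player with a position offset and loops delayed fireball attacks, aimed using screen-projected positions.
; Two hit spheres handle bullet and spike damage, with random pain sounds for bullets.
; On death it increments the player's kill count and, if respawning is enabled, spawns two mini bosses for phase two.
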(event OnComponentBeginOverlap(HitSphereTop)
  (params (OverlappedComponent :type Primitive%20Component%20Object%20Reference) (OtherActor :type Actor%20Object%20Reference) (OtherComp :type Primitive%20Component%20Object%20Reference) (OtherBodyIndex :type Integer) (bFromSweep :type Boolean) (SweepResult :type Hit%20Result%20Structure%20%28by%20ref%29))
  ;[1 1 1] Collision Logic
  (Utilities|FlowControl|Sequence
    (:then_0
      (Utilities|Casting|CastToBP_Bullet OtherActor)
      (CallFunction|BulletCollision)
      (switch int (Math|Random|RandomIntegerinRange 0 2)
        (:Default
          (Audio|PlaySound2D "/Game/SetchOnLegs/03Audio/07Spike/EnemyHit.EnemyHit" 1.0 1.0 0.0 0 0 :!label _label))
        (:0
          (switch int (Math|Random|RandomIntegerinRange 0 3)
            (:Default
              (Audio|PlaySound2D "/Game/SetchOnLegs/03Audio/01HinceInHell/SamOuch1.SamOuch1" 1.0 1.0 0.0 0 0 :!label _label_2))
            (:0
              (goto _label_2))
            (:1
              (Audio|PlaySound2D "/Game/SetchOnLegs/03Audio/01HinceInHell/SamOuch2.SamOuch2" 1.0 1.0 0.0 0 0))
            (:2
              (Audio|PlaySound2D "/Game/SetchOnLegs/03Audio/01HinceInHell/SamOuch3.SamOuch3" 1.0 1.0 0.0 0 0))
            (:3
              (Audio|PlaySound2D "/Game/SetchOnLegs/03Audio/01HinceInHell/SamOuch4.SamOuch4" 1.0 1.0 0.0 0 0))))
        (:1
          (goto _label))
        (:2
          (goto _label))))
    (:then_1
      (Utilities|Casting|CastToBP_Spike OtherActor)
      (CallFunction|DamageSpike))))

(event OnComponentBeginOverlap(HitSphereBottom)
  (params (OverlappedComponent :type Primitive%20Component%20Object%20Reference) (OtherActor :type Actor%20Object%20Reference) (OtherComp :type Primitive%20Component%20Object%20Reference) (OtherBodyIndex :type Integer) (bFromSweep :type Boolean) (SweepResult :type Hit%20Result%20Structure%20%28by%20ref%29))
  ;[1 1 1] Collision Logic
  (Utilities|FlowControl|Sequence
    (:then_0
      (Utilities|Casting|CastToBP_Bullet OtherActor)
      (CallFunction|BulletCollision)
      (switch int (Math|Random|RandomIntegerinRange 0 2)
        (:Default
          (Audio|PlaySound2D "/Game/SetchOnLegs/03Audio/07Spike/EnemyHit.EnemyHit" 1.0 1.0 0.0 0 0 :!label _label))
        (:0
          (switch int (Math|Random|RandomIntegerinRange 0 3)
            (:Default
              (Audio|PlaySound2D "/Game/SetchOnLegs/03Audio/01HinceInHell/SamOuch1.SamOuch1" 1.0 1.0 0.0 0 0 :!label _label_2))
            (:0
              (goto _label_2))
            (:1
              (Audio|PlaySound2D "/Game/SetchOnLegs/03Audio/01HinceInHell/SamOuch2.SamOuch2" 1.0 1.0 0.0 0 0))
            (:2
              (Audio|PlaySound2D "/Game/SetchOnLegs/03Audio/01HinceInHell/SamOuch3.SamOuch3" 1.0 1.0 0.0 0 0))
            (:3
              (Audio|PlaySound2D "/Game/SetchOnLegs/03Audio/01HinceInHell/SamOuch4.SamOuch4" 1.0 1.0 0.0 0 0))))
        (:1
          (goto _label))
        (:2
          (goto _label))))
    (:then_1
      (Utilities|Casting|CastToBP_Spike OtherActor)
      (CallFunction|DamageSpike))))

(event Custom|UpdateAnimation
  (bind _sprite (Variables|Default|GetSprite))
  ;[1 1 1] Handle Animation
  (switch Utilities|FlowControl|Switch|SwitchonHinceInHellState (Variables|Default|GetState)
    (:NewEnumerator0
      (Sprite|SetFlipbook _sprite "/Game/SetchOnLegs/01Sprites/01HinceInHell/Character/A_HinceInHellMoving.A_HinceInHellMoving"))
    (:NewEnumerator1
      (Sprite|SetFlipbook _sprite "/Game/SetchOnLegs/01Sprites/01HinceInHell/Character/A_HinceInHellAttacking.A_HinceInHellAttacking"))
    (:NewEnumerator2
      (Sprite|SetFlipbook _sprite "/Game/SetchOnLegs/01Sprites/01HinceInHell/Character/A_HinceInHellDead.A_HinceInHellDead"))))

(event Custom|Phase2Spawn
  (bind _returnvalue (Game|GetPlayerCharacter 0))
  (bind _returnvalue_2 (Game|GetPlayerCharacter 0))
  (bind _returnvalue_3 (Transformation|GetActorLocation _returnvalue))
  (bind _returnvalue_4 (Transformation|GetActorLocation _returnvalue_2))
  ;[1 1 1] Respawn System
  (Game|SpawnActorfromClass "/Game/SetchOnLegs/00Blueprint/01Hell/Boss/BP_MiniHinceInHell.BP_MiniHinceInHell_C" (Math|Transform|MakeTransform (Math|Vector|MakeVector (- (.x _returnvalue_3) 4e+02) 0.0 (+ (.z _returnvalue_3) 1.5e+03)) "0, 0, 0" "0.500000,0.500000,0.500000") "Undefined" 0 3.0 "-400.000000,0.000000,400.000000" 4e+01 0 0 false 0.05 0.35 2.2 0)
  (Game|SpawnActorfromClass "/Game/SetchOnLegs/00Blueprint/01Hell/Boss/BP_MiniHinceInHell.BP_MiniHinceInHell_C" (Math|Transform|MakeTransform (Math|Vector|MakeVector (+ (.x _returnvalue_4) 4e+02) 0.0 (+ (.z _returnvalue_4) 1.5e+03)) "0, 0, 0" "0.500000,0.500000,0.500000") "Undefined" 0 3.5 "400.000000,0.000000,400.000000" 4e+01 0 0 false 0.05 0.35 2.2 0))

(event Custom|HandleMovement
  ;[1 1 1] Handle Movement
  (Utilities|FlowControl|Delay 0.1)
  (Variables|Default|SetOurPosition (- (Transformation|GetActorLocation) (Variables|Default|GetMoveToPos)))
  (Variables|Default|SetPlayerPosition (Transformation|GetActorLocation (Pawn|GetControlledPawn (Game|GetPlayerController 0))))
  (Pawn|Input|AddMovementInput (- (Variables|Default|GetPlayerPosition) (Variables|Default|GetOurPosition)) 1.0 false))

(event Custom|Shoot
  (bind _fireballspawn (Variables|Default|GetFireballSpawn))
  (bind _returnvalue (Transformation|GetWorldLocation _fireballspawn))
  ;[1 1 1] Shoot Logic
  ;;[1 1 1] Handle Shoot
  (if (not (Variables|Default|GetIsDead))
    (Variables|Default|SetState "NewEnumerator1")
    (CallFunction|UpdateAnimation)
    (Game|SpawnActorfromClass "/Game/SetchOnLegs/00Blueprint/01Hell/Boss/BP_HinceInHellFireball.BP_HinceInHellFireball_C" (Math|Transform|MakeTransform (Math|Vector|MakeVector (.x _returnvalue) 5.0 (.z _returnvalue)) (Variables|Default|GetFireRotation) (Variables|Default|GetFireballScale)) "AlwaysSpawn" 0 1 5.0 true 5e+02 4e+02 true 0)
    (Audio|PlaySound2D "/Game/SetchOnLegs/03Audio/08Misc/Fire.Fire" 1.0 1.0 0.0 0 0)
    (Audio|PlaySound2D "/Game/SetchOnLegs/03Audio/01HinceInHell/SamYeahBaby.SamYeahBaby" 1.0 1.0 0.0 0 0)
    (Utilities|FlowControl|Delay 1.1)
    (if (not (Variables|Default|GetIsDead))
      (Variables|Default|SetState "NewEnumerator0")
      (CallFunction|UpdateAnimation)
      (Utilities|FlowControl|Delay (Variables|Default|GetAttackDelay))
      (CallFunction|Shoot))))

(event Custom|GetFireRotation
  (bind _returnvalue (Game|GetPlayerController 0))
  (bind _returnvalue_2 (Game|GetPlayerController 0))
  (bind _fireballspawn (Variables|Default|GetFireballSpawn))
  (bind _returnvalue_3 (Pawn|GetControlledPawn _returnvalue))
  (bind _returnvalue_4 (Transformation|GetWorldLocation _fireballspawn))
  (bind _returnvalue_5 (Transformation|GetActorLocation _returnvalue_3))
  (bind _screenlocation (Class|PlayerController|ProjectWorldLocationtoScreen _returnvalue_2 _returnvalue_4 false))
  (bind (_x _y _z) (Math|Vector|BreakVector _returnvalue_4))
  (bind (_x_2 _y_2) (Math|Vector2D|BreakVector2D _screenlocation))
  (bind _screenlocation_2 (Class|PlayerController|ProjectWorldLocationtoScreen _returnvalue _returnvalue_5 false))
  (bind (_x_3 _y_3) (Math|Vector2D|BreakVector2D _screenlocation_2))
  ;[1 1 1] Shoot Logic
  ;;[1 1 1] Get fire rotation
  (Variables|Default|SetFireRotation (Math|Rotator|FindLookatRotation _returnvalue_4 (Math|Vector|MakeVector (+ _x (- _x_3 _x_2)) 0.0 (+ _z (- _y_2 _y_3))))))

(event Custom|IntroCutscene
  ;[1 1 1] Intro Cutscene
  (Variables|/Script/Engine.MovementComponent|SetVelocity (Variables|Character|GetCharacterMovement) "0.000000,0.000000,1000.000000")
  (Utilities|FlowControl|Delay 1.25)
  (Variables|/Script/Engine.MovementComponent|SetVelocity (Variables|Character|GetCharacterMovement) "0, 0, 0")
  (Utilities|FlowControl|Delay 0.5)
  (Audio|PlaySound2D "/Game/SetchOnLegs/03Audio/01HinceInHell/SamIntro.SamIntro" 1.0 1.0 0.0 0 0)
  (Camera|PlayWorldCameraShake "/Game/SetchOnLegs/00Blueprint/01Hell/Boss/CameraShakes/BP_IntroShake.BP_IntroShake_C" (Transformation|GetWorldLocation (Variables|/Game/SetchOnLegs/00Blueprint/07Spike/BP_Spike.BP_Spike_C|GetSideViewCameraComponent (Variables|Default|GetPlayer))) 0.0 5e+02)
  (Sprite|SetFlipbook (Variables|Default|GetSprite) "/Game/SetchOnLegs/01Sprites/01HinceInHell/Character/A_HinceInHellAttacking.A_HinceInHellAttacking")
  (Utilities|FlowControl|Delay 2.0)
  (Variables|Default|SetState "NewEnumerator0")
  (CallFunction|UpdateAnimation)
  (Variables|Default|SetIntro false)
  (bind _returnvalue (UserInterface|CreateWidget "/Game/SetchOnLegs/00Blueprint/01Hell/Boss/Widget_HinceInHell.Widget_HinceInHell_C"))
  (bind _output_get (Variables|Default|SetHUD _returnvalue))
  (UserInterface|Viewport|AddtoViewport _output_get 0)
  (Variables|Default|SetActive true)
  (Utilities|FlowControl|Delay (Variables|Default|GetAttackDelay))
  (CallFunction|Shoot))

(event EventBeginPlay
  ;[1 1 1] Begin Play
  (|CallParentFunction)
  (Pawn|Components|CharacterMovement|SetMovementMode (Variables|Character|GetCharacterMovement) "MOVE_Flying" 0)
  (CallFunction|IntroCutscene))

(event EventDamageSystem
  (params (DamageIn :type Float%20%28single-precision%29))
  ;[1 1 1] Damage & Death System
  (|CallParentFunction DamageIn)
  (if (Variables|Default|GetIsDead)
    (Variables|Default|SetState "NewEnumerator2")
    (CallFunction|UpdateAnimation)
    (Collision|SetCollisionEnabled (Variables|Default|GetHitSphereTop) "NoCollision")
    (Variables|/Game/SetchOnLegs/00Blueprint/07Spike/BP_Spike.BP_Spike_C|SetHinceInHellKillCount (Variables|Default|GetPlayer) (+ (Variables|/Game/SetchOnLegs/00Blueprint/07Spike/BP_Spike.BP_Spike_C|GetHinceInHellKillCount (Variables|Default|GetPlayer)) 1))
    (if (Variables|Default|GetRespawn)
      (Variables|/Game/SetchOnLegs/00Blueprint/01Hell/Boss/Widget_HinceInHell.Widget_HinceInHell_C|SetPhase (Variables|Default|GetHUD) "NewEnumerator1")
      (CallFunction|Phase2Spawn))))

(event EventTick
  (params (DeltaSeconds :type Float%20%28single-precision%29))
  ;[1 1 1] Tick
  (CallFunction|GetFireRotation)
  (if (not (Variables|Default|GetIntro))
    (CallFunction|HandleMovement)))

(fn ConstructionScript)
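; Fireball Boy enemy that giggles on spawn and walks continuously along its MoveDirection.
; BeginPlay runs the parent setup, applies walk speed and rotates the sprite if it starts to the right of the player; Tick feeds the movement input.
; HitSphere overlaps run BulletCollision with a hit sound for bullets, and deal damage to BP_Spike with a fire sound.
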(event OnComponentBeginOverlap(HitSphere)
  (params (OverlappedComponent :type Primitive%20Component%20Object%20Reference) (OtherActor :type Actor%20Object%20Reference) (OtherComp :type Primitive%20Component%20Object%20Reference) (OtherBodyIndex :type Integer) (bFromSweep :type Boolean) (SweepResult :type Hit%20Result%20Structure%20%28by%20ref%29))
  ;[1 1 1] Collision Logic
  (Utilities|FlowControl|Sequence
    (:then_0
      (Utilities|Casting|CastToBP_Bullet OtherActor)
      (CallFunction|BulletCollision)
      (Audio|PlaySound2D "/Game/SetchOnLegs/03Audio/07Spike/EnemyHit.EnemyHit" 1.0 1.0 0.0 0 0))
    (:then_1
      (bind _asbp_spike (Utilities|Casting|CastToBP_Spike OtherActor))
      (Default|DamageSystem _asbp_spike 1)
      (Audio|PlaySound2D "/Game/SetchOnLegs/03Audio/08Misc/Fire.Fire" 1.0 1.0 0.0 0 0))))

(event EventBeginPlay
  ;[1 1 1] Movement Logic
  (|CallParentFunction)
  (Audio|PlaySound2D "/Game/SetchOnLegs/03Audio/01HinceInHell/FlameboyGiggle.FlameboyGiggle" 1.0 1.0 0.0 0 0)
  (Variables|Default|SetActive true)
  (Variables|/Script/Engine.CharacterMovementComponent|SetMaxWalkSpeed (Variables|Character|GetCharacterMovement) (Variables|Default|GetWalkSpeed))
  (if (> (.x (Transformation|GetWorldLocation (Variables|Default|GetSprite))) (.x (Transformation|GetActorLocation (Variables|Default|GetPlayer))))
    (Transformation|SetRelativeRotation (Variables|Default|GetSprite) "0,180.000000, 0" false false)))

(event EventTick
  (params (DeltaSeconds :type Float%20%28single-precision%29))
  ;[1 1 1] Movement Logic
  (Pawn|Input|AddMovementInput (Variables|Default|GetMoveDirection) 1.0 false))

(fn ConstructionScript)
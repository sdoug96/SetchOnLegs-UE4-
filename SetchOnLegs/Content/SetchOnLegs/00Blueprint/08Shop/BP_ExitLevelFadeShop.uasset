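; Shop exit trigger that sends the player (BP_Spike) to the HinceinHell level with a fade-out.
; Box overlap disables input, sets the walking flipbook and shows a quick fade widget, while Tick auto-walks the player along +X.
; Player stats, currency, upgrades and checkpoints are copied into BP_GameInstance to persist, then the level opens after a short delay.
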(event OnComponentBeginOverlap(Box)
  (params (OverlappedComponent :type Primitive%20Component%20Object%20Reference) (OtherActor :type Actor%20Object%20Reference) (OtherComp :type Primitive%20Component%20Object%20Reference) (OtherBodyIndex :type Integer) (bFromSweep :type Boolean) (SweepResult :type Hit%20Result%20Structure%20%28by%20ref%29))
  ;[1 1 1] Exit Level Logic
  (bind _asbp_spike (Utilities|Casting|CastToBP_Spike OtherActor))
  (Variables|Default|SetHit true)
  (Input|DisableInput _asbp_spike 0)
  (Sprite|SetFlipbook (Variables|/Script/Paper2D.PaperCharacter|GetSprite _asbp_spike) "/Game/SetchOnLegs/01Sprites/07Spike/Character/A_SpikeWalking.A_SpikeWalking")
  (Components|Timeline|SetPlayRate (Variables|/Script/Paper2D.PaperCharacter|GetSprite _asbp_spike) 1.0)
  (bind _returnvalue (UserInterface|CreateWidget "/Game/SetchOnLegs/00Blueprint/11Misc/Fades/Widget_QuickFadeOut.Widget_QuickFadeOut_C"))
  (UserInterface|Viewport|AddtoViewport _returnvalue 0)
  (Utilities|FlowControl|Sequence
    (:then_0
      (bind _asbp_game_instance (Utilities|Casting|CastToBP_GameInstance (Game|GetGameInstance)))
      (Utilities|FlowControl|Sequence
        (:then_0
          (Variables|/Game/SetchOnLegs/00Blueprint/11Misc/BP_GameInstance.BP_GameInstance_C|SetHealth _asbp_game_instance (Variables|/Game/SetchOnLegs/00Blueprint/07Spike/BP_Spike.BP_Spike_C|GetCurrentHealth _asbp_spike)))
        (:then_1
          (Variables|/Game/SetchOnLegs/00Blueprint/11Misc/BP_GameInstance.BP_GameInstance_C|SetCurrency _asbp_game_instance (Variables|/Game/SetchOnLegs/00Blueprint/07Spike/BP_Spike.BP_Spike_C|GetMasterBalls _asbp_spike)))
        (:then_2
          (Variables|/Game/SetchOnLegs/00Blueprint/11Misc/BP_GameInstance.BP_GameInstance_C|SetDeathCount _asbp_game_instance (Variables|/Game/SetchOnLegs/00Blueprint/07Spike/BP_Spike.BP_Spike_C|GetDeathCount _asbp_spike)))
        (:then_3
          (Variables|/Game/SetchOnLegs/00Blueprint/11Misc/BP_GameInstance.BP_GameInstance_C|SetChargedShot _asbp_game_instance (Variables|/Game/SetchOnLegs/00Blueprint/07Spike/BP_Spike.BP_Spike_C|GetChargedShot _asbp_spike)))
        (:then_4
          (Variables|/Game/SetchOnLegs/00Blueprint/11Misc/BP_GameInstance.BP_GameInstance_C|Set3BulletSpread _asbp_game_instance (Variables|/Game/SetchOnLegs/00Blueprint/07Spike/BP_Spike.BP_Spike_C|Get3Bullet _asbp_spike)))
        (:then_5
          (Variables|/Game/SetchOnLegs/00Blueprint/11Misc/BP_GameInstance.BP_GameInstance_C|Set5BulletSpread _asbp_game_instance (Variables|/Game/SetchOnLegs/00Blueprint/07Spike/BP_Spike.BP_Spike_C|Get5Bullet _asbp_spike)))
        (:then_6
          (Variables|/Game/SetchOnLegs/00Blueprint/11Misc/BP_GameInstance.BP_GameInstance_C|SetMaxHealth _asbp_game_instance (Variables|/Game/SetchOnLegs/00Blueprint/07Spike/BP_Spike.BP_Spike_C|GetMaxHealth _asbp_spike)))
        (:then_7
          (Variables|/Game/SetchOnLegs/00Blueprint/11Misc/BP_GameInstance.BP_GameInstance_C|SetHealthLevel _asbp_game_instance (Variables|/Game/SetchOnLegs/00Blueprint/07Spike/BP_Spike.BP_Spike_C|GetHealthLevel _asbp_spike)))
        (:then_8
          (Variables|/Game/SetchOnLegs/00Blueprint/11Misc/BP_GameInstance.BP_GameInstance_C|SetCheckpoints _asbp_game_instance (Variables|/Game/SetchOnLegs/00Blueprint/07Spike/BP_Spike.BP_Spike_C|GetCheckpoints _asbp_spike)))
        (:then_9
          (Variables|/Game/SetchOnLegs/00Blueprint/11Misc/BP_GameInstance.BP_GameInstance_C|SetArmorLevel _asbp_game_instance (Variables|/Game/SetchOnLegs/00Blueprint/07Spike/BP_Spike.BP_Spike_C|GetArmorLevel _asbp_spike)))
        (:then_10
          (Variables|/Game/SetchOnLegs/00Blueprint/11Misc/BP_GameInstance.BP_GameInstance_C|SetBulletDamage _asbp_game_instance (Variables|/Game/SetchOnLegs/00Blueprint/07Spike/BP_Spike.BP_Spike_C|GetBulletDamage _asbp_spike)))
        (:then_11
          (Variables|/Game/SetchOnLegs/00Blueprint/11Misc/BP_GameInstance.BP_GameInstance_C|SetChargedBulletCooldown _asbp_game_instance (Variables|/Game/SetchOnLegs/00Blueprint/07Spike/BP_Spike.BP_Spike_C|GetMaxChargedShotCooldown _asbp_spike)))
        (:then_12
          (Variables|/Game/SetchOnLegs/00Blueprint/11Misc/BP_GameInstance.BP_GameInstance_C|SetChargedBulletDamage _asbp_game_instance (Variables|/Game/SetchOnLegs/00Blueprint/07Spike/BP_Spike.BP_Spike_C|GetChargedShotDamage _asbp_spike)))
        (:then_13
          (Variables|/Game/SetchOnLegs/00Blueprint/11Misc/BP_GameInstance.BP_GameInstance_C|SetShields _asbp_game_instance (Variables|/Game/SetchOnLegs/00Blueprint/07Spike/BP_Spike.BP_Spike_C|GetShields _asbp_spike)))))
    (:then_1
      (Utilities|FlowControl|Delay 2.0)
      (Game|OpenLevel(byName) "HinceinHell"))))

(event EventTick
  (params (DeltaSeconds :type Float%20%28single-precision%29))
  ;[1 1 1] Exit Level Logic
  (if (Variables|Default|GetHit)
    (bind _asbp_spike (Utilities|Casting|CastToBP_Spike (Game|GetPlayerCharacter 0)))
    (Pawn|Input|AddMovementInput _asbp_spike "1.000000, 0, 0" 1.0 false)))

(fn ConstructionScript)
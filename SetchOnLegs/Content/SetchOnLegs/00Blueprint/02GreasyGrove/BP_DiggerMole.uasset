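; BP_DiggerMole is an enemy mole that wakes when BP_Spike enters its trigger and goes back to sleep when Spike leaves.
; While active, it plays flipbook animations and throws BP_Rock on a looping timer with randomized X force.
; Two bullet spheres apply the player's bullet damage only while awake, blinking the sprite via a timer.
; On death, it launches a few BP_MasterBall pickups and destroys itself.
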(event OnComponentBeginOverlap(WakeTrigger)
  (params (OverlappedComponent :type Primitive%20Component%20Object%20Reference) (OtherActor :type Actor%20Object%20Reference) (OtherComp :type Primitive%20Component%20Object%20Reference) (OtherBodyIndex :type Integer) (bFromSweep :type Boolean) (SweepResult :type Hit%20Result%20Structure%20%28by%20ref%29))
  ;[1 1 1] Wake up and throw rocks
  (Utilities|Casting|CastToBP_Spike OtherActor)
  (Variables|Default|SetActive true)
  (Sprite|SetFlipbook (Variables|Default|GetDiggerMole) "/Game/SetchOnLegs/01Sprites/02GreasyGrove/DiggerMole/Animations/A_DiggerMoleWake.A_DiggerMoleWake")
  (Utilities|FlowControl|Delay 0.7)
  (if (Variables|Default|GetActive)
    (Sprite|SetFlipbook (Variables|Default|GetDiggerMole) "/Game/SetchOnLegs/01Sprites/02GreasyGrove/DiggerMole/Animations/A_DiggerMoleAttack.A_DiggerMoleAttack")
    (Utilities|FlowControl|Delay (Variables|Default|GetInitialThrowDelay))
    (if (Variables|Default|GetActive)
      (CallFunction|ThrowRock)
      (Utilities|Time|SetTimerbyFunctionName 0 "ThrowRock" (Variables|Default|GetThrowDelay) true))))

(event OnComponentEndOverlap(WakeTrigger)
  (params (OverlappedComponent :type Primitive%20Component%20Object%20Reference) (OtherActor :type Actor%20Object%20Reference) (OtherComp :type Primitive%20Component%20Object%20Reference) (OtherBodyIndex :type Integer))
  ;[1 1 1] Wake up and throw rocks
  (Utilities|Casting|CastToBP_Spike OtherActor)
  (Variables|Default|SetActive false)
  (Sprite|SetFlipbook (Variables|Default|GetDiggerMole) "/Game/SetchOnLegs/01Sprites/02GreasyGrove/DiggerMole/Animations/A_DiggerMoleSleep.A_DiggerMoleSleep")
  (Utilities|Time|ClearTimerbyFunctionName 0 "ThrowRock")
  (Utilities|FlowControl|Delay 0.5)
  (Sprite|SetFlipbook (Variables|Default|GetDiggerMole)))

(event OnComponentBeginOverlap(BulletSphere1)
  (params (OverlappedComponent :type Primitive%20Component%20Object%20Reference) (OtherActor :type Actor%20Object%20Reference) (OtherComp :type Primitive%20Component%20Object%20Reference) (OtherBodyIndex :type Integer) (bFromSweep :type Boolean) (SweepResult :type Hit%20Result%20Structure%20%28by%20ref%29))
  ;[1 1 1] Bullet Collision
  (bind _asbp_bullet (Utilities|Casting|CastToBP_Bullet OtherActor))
  (if (Variables|Default|GetActive)
    (Actor|DestroyActor _asbp_bullet)
    (if (not (Variables|Default|GetIsDead))
      (CallFunction|DamageSytsem (Variables|/Game/SetchOnLegs/00Blueprint/07Spike/BP_Spike.BP_Spike_C|GetBulletDamage (Variables|Default|GetPlayer))))))

(event OnComponentBeginOverlap(BulletSphere2)
  (params (OverlappedComponent :type Primitive%20Component%20Object%20Reference) (OtherActor :type Actor%20Object%20Reference) (OtherComp :type Primitive%20Component%20Object%20Reference) (OtherBodyIndex :type Integer) (bFromSweep :type Boolean) (SweepResult :type Hit%20Result%20Structure%20%28by%20ref%29))
  ;[1 1 1] Bullet Collision
  (bind _asbp_bullet (Utilities|Casting|CastToBP_Bullet OtherActor))
  (if (Variables|Default|GetActive)
    (Actor|DestroyActor _asbp_bullet)
    (if (not (Variables|Default|GetIsDead))
      (CallFunction|DamageSytsem (Variables|/Game/SetchOnLegs/00Blueprint/07Spike/BP_Spike.BP_Spike_C|GetBulletDamage (Variables|Default|GetPlayer))))))

(event Custom|SpawnPickups
  ;[1 1 1] Spawn pickups function
  (Utilities|ForLoopwithDelay 0 (Math|Random|RandomIntegerinRange 2 4) :!label _label
    (:Loop%20Body
      (Game|SpawnActorfromClass "/Game/SetchOnLegs/00Blueprint/12Misc/BP_MasterBall.BP_MasterBall_C" (Math|Transform|MakeTransform (Transformation|GetWorldLocation (Variables|Default|GetDiggerMole)) "0, 0, 0" "1,1,1") "Undefined" 0 0)
      (Audio|PlaySound2D "/Game/SetchOnLegs/03Audio/08Misc/PickupLaunch.PickupLaunch" 1.0 1.0 0.0 0 0))
    (:Delay%20Out
      (Utilities|FlowControl|Delay 0.2)
      (goto _label Delay%20In))))

(event Custom|Damage%20Sytsem
  (params (DamageIn :type Float%20%28single-precision%29))
  ;[1 1 1] Damage & Death System
  (if (Variables|Default|GetCanBeDamaged)
    (bind _output_get (Variables|Default|SetCurrentHealth (- (Variables|Default|GetCurrentHealth) DamageIn)))
    (if (<= _output_get 0.0)
      (Variables|Default|SetIsDead true)
      (Sprite|SetFlipbook (Variables|Default|GetDiggerMole) "/Game/SetchOnLegs/01Sprites/02GreasyGrove/DiggerMole/Animations/A_DiggerMoleSleep.A_DiggerMoleSleep")
      (CallFunction|SpawnPickups)
      (Utilities|FlowControl|Delay 0.5)
      (Actor|DestroyActor)
      (else
        (Utilities|Time|SetTimerbyFunctionName 0 "Blink" 0.05 true)
        (Utilities|FlowControl|Delay 0.2)
        (Utilities|Time|ClearTimerbyFunctionName 0 "Blink")
        (Development|SetHiddeninGame (Variables|Default|GetDiggerMole) false false)))))

(event Custom|ThrowRock
  ;[1 1 1] Throw rock function
  (Variables|Default|SetThrowForce (Math|Vector|MakeVector (Math|Random|RandomFloatinRange (Variables|Default|GetMinXForce) (Variables|Default|GetMaxXForce)) 0.0 (Variables|Default|GetZForce)))
  (if (Variables|Default|GetActive)
    (Game|SpawnActorfromClass "/Game/SetchOnLegs/00Blueprint/02GreasyGrove/BP_Rock.BP_Rock_C" (Math|Transform|MakeTransform (Transformation|GetWorldLocation (Variables|Default|GetRockSpawn)) "0, 0, 0" "0.187500,0.187500,0.187500") "Undefined" 0 (Variables|Default|GetThrowForce) 0)
    (Audio|PlaySound2D "/Game/SetchOnLegs/03Audio/02GreasyGrove/Dir.Dir" 1.0 1.0 0.0 0 0)))

(event Custom|Blink
  (bind _diggermole (Variables|Default|GetDiggerMole))
  ;[1 1 1] Damage & Death System
  (Development|SetHiddeninGame _diggermole (not (Variables|/Script/Engine.SceneComponent|GetbHiddenInGame _diggermole)) false))

(event EventBeginPlay
  (bind _asbp_spike (Utilities|Casting|CastToBP_Spike (Game|GetPlayerCharacter 0)))
  (Variables|Default|SetPlayer _asbp_spike))

(fn ConstructionScript)
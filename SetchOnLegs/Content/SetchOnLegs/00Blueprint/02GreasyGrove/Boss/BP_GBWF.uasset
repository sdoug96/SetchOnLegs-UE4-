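; GBWF boss for a 2D side-view level, a flipbook character that chases the player during the boss fight.
; BeginPlay runs a timed fall, idle, howl and run intro with camera shakes and sounds, then adds its HUD.
; Tick moves it toward the player while a state enum selects flipbooks.
; Overlapping bullets and rocks are destroyed; bullets deal damage, triggering a timer-driven blink or death.
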(event OnComponentBeginOverlap(BulletBox)
  (params (OverlappedComponent :type Primitive%20Component%20Object%20Reference) (OtherActor :type Actor%20Object%20Reference) (OtherComp :type Primitive%20Component%20Object%20Reference) (OtherBodyIndex :type Integer) (bFromSweep :type Boolean) (SweepResult :type Hit%20Result%20Structure%20%28by%20ref%29))
  ;[1 1 1] Bullet Collision
  (Utilities|FlowControl|Sequence
    (:then_0
      (bind _asbp_bullet (Utilities|Casting|CastToBP_Bullet OtherActor))
      (Actor|DestroyActor _asbp_bullet)
      (if (not (Variables|Default|GetIsDead))
        (bind _asbp_spike (Utilities|Casting|CastToBP_Spike (Game|GetPlayerCharacter 0)))
        (CallFunction|DamageSytsem (Variables|/Game/SetchOnLegs/00Blueprint/07Spike/BP_Spike.BP_Spike_C|GetBulletDamage _asbp_spike))))
    (:then_1
      (bind _asbp_rock (Utilities|Casting|CastToBP_Rock OtherActor))
      (Actor|DestroyActor _asbp_rock))))

(event Custom|Blink
  (bind _sprite (Variables|Default|GetSprite))
  ;[1 1 1] Damage & Death System
  (Development|SetHiddeninGame _sprite (not (Variables|/Script/Engine.SceneComponent|GetbHiddenInGame _sprite)) false))

(event Custom|Damage%20Sytsem
  (params (DamageIn :type Float%20%28single-precision%29))
  ;[1 1 1] Damage & Death System
  (bind _output_get (Variables|Default|SetCurrentHealth (- (Variables|Default|GetCurrentHealth) DamageIn)))
  (if (<= _output_get 0.0)
    (Variables|Default|SetState "NewEnumerator3")
    (Variables|Default|SetIsDead true)
    (Widget|RemovefromParent (Variables|Default|GetHUD))
    (CallFunction|UpdateAnimation)
    (Utilities|FlowControl|Delay 5.0)
    (Components|Timeline|SetPlayRate (Variables|Default|GetSprite) 0.0)
    (else
      (Utilities|Time|SetTimerbyFunctionName 0 "Blink" 0.05 true)
      (Utilities|FlowControl|Delay 0.2)
      (Utilities|Time|ClearTimerbyFunctionName 0 "Blink")
      (Development|SetHiddeninGame (Variables|Default|GetSprite) false false))))

(event Custom|UpdateAnimation
  (bind _sprite (Variables|Default|GetSprite))
  ;[1 1 1] Handle Animation
  (switch Utilities|FlowControl|Switch|SwitchonGBWF_State (Variables|Default|GetState)
    (:NewEnumerator0
      (Sprite|SetFlipbook _sprite "/Game/SetchOnLegs/01Sprites/02GreasyGrove/Character/Animations/A_GBWFFalling.A_GBWFFalling"))
    (:NewEnumerator1
      (Sprite|SetFlipbook _sprite "/Game/SetchOnLegs/01Sprites/02GreasyGrove/Character/Animations/A_GBWFSwipe.A_GBWFSwipe"))
    (:NewEnumerator2
      (Sprite|SetFlipbook _sprite "/Game/SetchOnLegs/01Sprites/02GreasyGrove/Character/Animations/A_GBWFRun.A_GBWFRun"))
    (:NewEnumerator3
      (Sprite|SetFlipbook _sprite "/Game/SetchOnLegs/01Sprites/02GreasyGrove/Character/Animations/A_GBWFDead.A_GBWFDead"))
    (:NewEnumerator4
      (Sprite|SetFlipbook _sprite "/Game/SetchOnLegs/01Sprites/02GreasyGrove/Character/Animations/A_GBWFHowl.A_GBWFHowl"))
    (:NewEnumerator5
      (Sprite|SetFlipbook _sprite "/Game/SetchOnLegs/01Sprites/02GreasyGrove/Character/Animations/A_GBWFIdle.A_GBWFIdle"))))

(event Custom|Movement
  ;[1 1 1] Movement
  (if (Variables|/Game/SetchOnLegs/00Blueprint/07Spike/BP_Spike.BP_Spike_C|GetBossFight (Variables|Default|GetPlayer))
    (if (> (.x (Transformation|GetActorLocation)) (.x (Transformation|GetActorLocation (Variables|Default|GetPlayer))))
      (Pawn|Input|AddMovementInput "-1.000000, 0, 0" 1.0 false)
      (Transformation|SetActorRotation "0,180.000000, 0")
      (else
        (Pawn|Input|AddMovementInput "1.000000, 0, 0" 1.0 false)
        (Transformation|SetActorRotation "0, 0, 0")))))

(event EventBeginPlay
  ;[1 1 1] Initialise
  (bind _asbp_spike (Utilities|Casting|CastToBP_Spike (Game|GetPlayerCharacter 0)))
  (Variables|Default|SetPlayer _asbp_spike)
  (Variables|Default|SetState "NewEnumerator0")
  (CallFunction|UpdateAnimation)
  (Utilities|FlowControl|Delay 0.6)
  (Audio|PlaySound2D "/Game/SetchOnLegs/03Audio/02GreasyGrove/Boom.Boom" 1.0 1.0 0.0 0 0)
  (Camera|PlayWorldCameraShake "/Game/SetchOnLegs/00Blueprint/02GreasyGrove/Boss/BP_GBWFDropShake.BP_GBWFDropShake_C" (Transformation|GetWorldLocation (Variables|/Game/SetchOnLegs/00Blueprint/07Spike/BP_Spike.BP_Spike_C|GetSideViewCameraComponent (Variables|Default|GetPlayer))) 0.0 5e+02)
  (Variables|Default|SetState "NewEnumerator5")
  (CallFunction|UpdateAnimation)
  (Utilities|FlowControl|Delay 1.5)
  (Variables|Default|SetState "NewEnumerator4")
  (CallFunction|UpdateAnimation)
  (Utilities|FlowControl|Delay 0.75)
  (Camera|PlayWorldCameraShake "/Game/SetchOnLegs/00Blueprint/02GreasyGrove/Boss/BP_GBWFHowlShake.BP_GBWFHowlShake_C" (Transformation|GetWorldLocation (Variables|/Game/SetchOnLegs/00Blueprint/07Spike/BP_Spike.BP_Spike_C|GetSideViewCameraComponent (Variables|Default|GetPlayer))) 0.0 5e+02)
  (Audio|PlaySound2D "/Game/SetchOnLegs/03Audio/02GreasyGrove/Howl.Howl" 1.0 1.0 0.0 0 0)
  (Utilities|FlowControl|Delay 2.0)
  (Variables|Default|SetState "NewEnumerator2")
  (CallFunction|UpdateAnimation)
  (bind _returnvalue (UserInterface|CreateWidget "/Game/SetchOnLegs/00Blueprint/02GreasyGrove/Boss/Widget_GBWF.Widget_GBWF_C"))
  (bind _output_get (Variables|Default|SetHUD _returnvalue))
  (UserInterface|Viewport|AddtoViewport _output_get 0))

(event EventTick
  (params (DeltaSeconds :type Float%20%28single-precision%29))
  ;[1 1 1] Tick
  (if (not (Variables|Default|GetIsDead))
    (CallFunction|Movement)))

(fn ConstructionScript)
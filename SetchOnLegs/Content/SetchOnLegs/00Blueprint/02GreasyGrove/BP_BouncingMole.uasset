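; BP_BouncingMole is a 2D flipbook enemy that wakes when Spike approaches, then repeatedly bounces toward the player.
; A state variable drives animation, while landing either schedules the next launch or returns the mole underground at its spawn point.
; Detached wake and active triggers bound its behaviour unless InstaWake is set.
; Hit spheres handle bullet and contact damage, with blink feedback, random pickups and a kill count on death.
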(event OnComponentBeginOverlap(WakeTrigger)
  (params (OverlappedComponent :type Primitive%20Component%20Object%20Reference) (OtherActor :type Actor%20Object%20Reference) (OtherComp :type Primitive%20Component%20Object%20Reference) (OtherBodyIndex :type Integer) (bFromSweep :type Boolean) (SweepResult :type Hit%20Result%20Structure%20%28by%20ref%29))
  ;[1 1 1] Wake up and bounce
  (Utilities|Casting|CastToBP_Spike OtherActor)
  (if (not (Variables|Default|GetActive))
    (Variables|Default|SetState "NewEnumerator5")
    (CallFunction|UpdateAnimation)
    (Utilities|FlowControl|Delay 0.7)
    (Variables|Default|SetState "NewEnumerator1")
    (CallFunction|UpdateAnimation)
    (Variables|Default|SetActive true)
    (Utilities|FlowControl|Delay (Variables|Default|GetBounceDelay))
    (CallFunction|Bounce)))

(event OnComponentBeginOverlap(HitSphereBody)
  (params (OverlappedComponent :type Primitive%20Component%20Object%20Reference) (OtherActor :type Actor%20Object%20Reference) (OtherComp :type Primitive%20Component%20Object%20Reference) (OtherBodyIndex :type Integer) (bFromSweep :type Boolean) (SweepResult :type Hit%20Result%20Structure%20%28by%20ref%29))
  ;[1 1 1] Collision
  (Utilities|FlowControl|Sequence
    (:then_0
      (bind _asbp_bullet (Utilities|Casting|CastToBP_Bullet OtherActor))
      (CallFunction|BulletCollision _asbp_bullet))
    (:then_1
      (Utilities|Casting|CastToBP_Spike OtherActor)
      (CallFunction|DamageSpike))))

(event OnComponentEndOverlap(ActiveTrigger)
  (params (OverlappedComponent :type Primitive%20Component%20Object%20Reference) (OtherActor :type Actor%20Object%20Reference) (OtherComp :type Primitive%20Component%20Object%20Reference) (OtherBodyIndex :type Integer))
  ;[1 1 1] Wake up and bounce
  (Utilities|Casting|CastToBP_Spike OtherActor)
  (if (not (Variables|Default|GetInstaWake))
    (if (Variables|Default|GetActive)
      (Variables|Default|SetActive false)
      (if (not (AI|Components|NavMovement|IsFalling (Variables|Character|GetCharacterMovement)))
        (Variables|Default|SetState "NewEnumerator0")
        (CallFunction|UpdateAnimation)
        (Utilities|FlowControl|Delay 0.5)
        (Variables|Default|SetState "NewEnumerator4")
        (CallFunction|UpdateAnimation)
        (Components|Movement|StopMovementImmediately (Variables|Character|GetCharacterMovement))
        (Transformation|SetActorLocation (Variables|Default|GetBaseLocation) false false)
        (Variables|Default|SetActive false)))))

(event OnComponentBeginOverlap(HitSphereHead)
  (params (OverlappedComponent :type Primitive%20Component%20Object%20Reference) (OtherActor :type Actor%20Object%20Reference) (OtherComp :type Primitive%20Component%20Object%20Reference) (OtherBodyIndex :type Integer) (bFromSweep :type Boolean) (SweepResult :type Hit%20Result%20Structure%20%28by%20ref%29))
  ;[1 1 1] Collision
  (Utilities|FlowControl|Sequence
    (:then_0
      (bind _asbp_bullet (Utilities|Casting|CastToBP_Bullet OtherActor))
      (CallFunction|BulletCollision _asbp_bullet))
    (:then_1
      (Utilities|Casting|CastToBP_Spike OtherActor)
      (CallFunction|DamageSpike))))

(event Custom|SpawnPickups
  (bind _sprite (Variables|Default|GetSprite))
  (bind _returnvalue (Transformation|GetWorldLocation _sprite))
  ;[1 1 1] Spawn pickups function
  (Utilities|ForLoopwithDelay 0 (Math|Random|RandomIntegerinRange 0 1) :!label _label
    (:Loop%20Body
      (Game|SpawnActorfromClass "/Game/SetchOnLegs/00Blueprint/12Misc/GameObjects/BP_MasterBall.BP_MasterBall_C" (Math|Transform|MakeTransform (Math|Vector|MakeVector (.x _returnvalue) 0.1 (.z _returnvalue)) "0, 0, 0" "1,1,1") "Undefined" 0 0)
      (Audio|PlaySound2D "/Game/SetchOnLegs/03Audio/08Misc/PickupLaunch.PickupLaunch" 1.0 1.0 0.0 0 0))
    (:Delay%20Out
      (Utilities|FlowControl|Delay 0.2)
      (goto _label Delay%20In))))

(event Custom|Damage%20Sytsem
  (params (DamageIn :type Float%20%28single-precision%29))
  ;[1 1 1] Damage & Death System
  (bind _output_get (Variables|Default|SetCurrentHealth (- (Variables|Default|GetCurrentHealth) DamageIn)))
  (if (<= _output_get 0.0)
    (Variables|Default|SetIsDead true)
    (Components|Movement|StopMovementImmediately (Variables|Character|GetCharacterMovement))
    (Variables|Default|SetState "NewEnumerator3")
    (CallFunction|UpdateAnimation)
    (CallFunction|SpawnPickups)
    (bind _asbp_game_instance (Utilities|Casting|CastToBP_GameInstance (Game|GetGameInstance)))
    (Variables|/Game/SetchOnLegs/00Blueprint/12Misc/Core/BP_GameInstance.BP_GameInstance_C|SetEnemiesKilled _asbp_game_instance (+ (Variables|/Game/SetchOnLegs/00Blueprint/12Misc/Core/BP_GameInstance.BP_GameInstance_C|GetEnemiesKilled _asbp_game_instance) 1))
    (Utilities|FlowControl|Delay 1.0)
    (Actor|DestroyActor)
    (else
      (Utilities|Time|SetTimerbyFunctionName 0 "Blink" 0.05 true)
      (Utilities|FlowControl|Delay 0.2)
      (Utilities|Time|ClearTimerbyFunctionName 0 "Blink")
      (Development|SetHiddeninGame (Variables|Default|GetSprite) false false))))

(event Custom|Blink
  (bind _sprite (Variables|Default|GetSprite))
  ;[1 1 1] Damage & Death System
  (Development|SetHiddeninGame _sprite (not (Variables|/Script/Engine.SceneComponent|GetbHiddenInGame _sprite)) false))

(event Custom|SetRotation
  ;[1 1 1] Set rotation
  (if true
    (if (> (.x (Transformation|GetWorldLocation (Variables|Default|GetSprite))) (.x (Transformation|GetActorLocation (Variables|Default|GetPlayer))))
      (Transformation|SetWorldRotation (Variables|Default|GetSprite) "0, 0, 0" false false)
      (Transformation|SetRelativeLocation (Variables|Default|GetHitSphereHead) "-25.000000,0.000000,100.000000" false false)
      (Variables|Default|SetBounceDirection -1)
      (else
        (Transformation|SetWorldRotation (Variables|Default|GetSprite) "0,180.000000, 0" false false)
        (Transformation|SetRelativeLocation (Variables|Default|GetHitSphereHead) "30.000000,0.000000,100.000000" false false)
        (Variables|Default|SetBounceDirection 1)))))

(event Custom|Bounce
  (bind _bounceforce (Variables|Default|GetBounceForce))
  ;[1 1 1] Bounce
  (if (Variables|Default|GetActive)
    (if (not (Variables|Default|GetIsDead))
      (Audio|PlaySound2D "/Game/SetchOnLegs/03Audio/02GreasyGrove/Dir.Dir" 1.0 1.0 0.0 0 0)
      (Character|LaunchCharacter (Math|Vector|MakeVector (* (Variables|Default|GetBounceDirection) (.x _bounceforce)) 0.0 (.z _bounceforce)) true true)
      (Variables|Default|SetState "NewEnumerator2")
      (CallFunction|UpdateAnimation))))

(event Custom|BulletCollision
  (params (Bullet :type BP%20Bullet%20Object%20Reference))
  ;[1 1 1] Collision
  (if (Variables|Default|GetActive)
    (Actor|DestroyActor Bullet)
    (if (not (Variables|Default|GetIsDead))
      (CallFunction|DamageSytsem (Variables|/Game/SetchOnLegs/00Blueprint/07Spike/BP_Spike.BP_Spike_C|GetBulletDamage (Variables|Default|GetPlayer)))
      (switch int (Math|Random|RandomIntegerinRange 0 2)
        (:Default
          (Audio|PlaySound2D "/Game/SetchOnLegs/03Audio/07Spike/EnemyHit.EnemyHit" 1.0 1.0 0.0 0 0 :!label _label))
        (:0
          (Audio|PlaySound2D "/Game/SetchOnLegs/03Audio/02GreasyGrove/JohnOuch.JohnOuch" 1.0 1.0 0.0 0 0))
        (:1
          (goto _label))
        (:2
          (goto _label))))))

(event Custom|DamageSpike
  ;[1 1 1] Collision
  (if (Variables|Default|GetActive)
    (if (not (Variables|Default|GetIsDead))
      (Default|DamageSystem (Variables|Default|GetPlayer) 1))))

(event Custom|UpdateAnimation
  (bind _isdead (Variables|Default|GetIsDead))
  ;[1 1 1] Handle Animation
  (switch Utilities|FlowControl|Switch|SwitchonBouncingMoleState (Variables|Default|GetState)
    (:NewEnumerator4
      (if (not _isdead)
        (Sprite|SetFlipbook (Variables|Default|GetSprite))))
    (:NewEnumerator5
      (if (not _isdead)
        (Sprite|SetFlipbook (Variables|Default|GetSprite) "/Game/SetchOnLegs/01Sprites/02GreasyGrove/BouncingMole/Animations/A_BouncingMoleWake.A_BouncingMoleWake")))
    (:NewEnumerator1
      (if (not _isdead)
        (Sprite|SetFlipbook (Variables|Default|GetSprite) "/Game/SetchOnLegs/01Sprites/02GreasyGrove/BouncingMole/Animations/A_BouncingMoleIdle.A_BouncingMoleIdle")))
    (:NewEnumerator2
      (if (not _isdead)
        (Sprite|SetFlipbook (Variables|Default|GetSprite) "/Game/SetchOnLegs/01Sprites/02GreasyGrove/BouncingMole/Animations/A_BouncingMoleBounce.A_BouncingMoleBounce")))
    (:NewEnumerator0
      (if (not _isdead)
        (Sprite|SetFlipbook (Variables|Default|GetSprite) "/Game/SetchOnLegs/01Sprites/02GreasyGrove/BouncingMole/Animations/A_BouncingMoleSleep.A_BouncingMoleSleep")))
    (:NewEnumerator3
      (Sprite|SetFlipbook (Variables|Default|GetSprite) "/Game/SetchOnLegs/01Sprites/02GreasyGrove/BouncingMole/Animations/A_BouncingMoleDeath.A_BouncingMoleDeath"))))

(event EventBeginPlay
  ;[1 1 1] Begin Play
  (bind _asbp_spike (Utilities|Casting|CastToBP_Spike (Game|GetPlayerCharacter 0)))
  (Variables|Default|SetPlayer _asbp_spike)
  (Variables|Default|SetBaseLocation (Transformation|GetActorLocation))
  (Transformation|DetachFromComponent (Variables|Default|GetWakeTrigger) "KeepWorld" "KeepWorld" "KeepWorld" true)
  (Transformation|DetachFromComponent (Variables|Default|GetActiveTrigger) "KeepWorld" "KeepWorld" "KeepWorld" true)
  (Pawn|SpawnDefaultController)
  (CallFunction|UpdateAnimation)
  (if (Variables|Default|GetInstaWake)
    (if (not (Variables|Default|GetActive))
      (Variables|Default|SetState "NewEnumerator5")
      (CallFunction|UpdateAnimation)
      (Utilities|FlowControl|Delay 0.7)
      (Variables|Default|SetState "NewEnumerator1")
      (CallFunction|UpdateAnimation)
      (Variables|Default|SetActive true)
      (Utilities|FlowControl|Delay (Variables|Default|GetBounceDelay))
      (CallFunction|Bounce))))

(event EventTick
  (params (DeltaSeconds :type Float%20%28single-precision%29))
  ;[1 1 1] Set rotation
  (CallFunction|SetRotation))

(event EventOnLanded
  (params (Hit :type Hit%20Result%20Structure%20%28by%20ref%29))
  ;[1 1 1] Landed Logic
  (if (Collision|IsOverlappingActor (Variables|Default|GetActiveTrigger) (Variables|Default|GetPlayer) :!class /Script/Engine.PrimitiveComponent)
    (Variables|Default|SetState "NewEnumerator1" :!label _label)
    (CallFunction|UpdateAnimation)
    (Utilities|FlowControl|Delay (Variables|Default|GetBounceDelay))
    (if (Variables|Default|GetActive)
      (CallFunction|Bounce))
    (elif (Variables|Default|GetInstaWake)
      (if (Variables|Default|GetActive)
        (goto _label))
      (else
        (Components|Movement|StopMovementImmediately (Variables|Character|GetCharacterMovement))
        (Variables|Default|SetState "NewEnumerator0")
        (CallFunction|UpdateAnimation)
        (Utilities|FlowControl|Delay 0.5)
        (Variables|Default|SetState "NewEnumerator4")
        (CallFunction|UpdateAnimation)
        (Transformation|SetActorLocation (Variables|Default|GetBaseLocation) false false)
        (Variables|Default|SetActive false)))))

(fn ConstructionScript)
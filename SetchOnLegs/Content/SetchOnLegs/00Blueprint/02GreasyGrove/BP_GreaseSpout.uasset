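; BP_GreaseSpout is a spout that spawns grease blobs while BP_Spike is inside its WakeBox.
; Entering the box fires one blob immediately, then starts a looping timer using either DropDelay or, with RandomDropTime, an interval randomized once on entry.
; Each shot spawns a small BP_GreaseBlob at GreaseBlobSpawn and plays a 2D sound.
; Leaving the box clears the timer.
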(event OnComponentBeginOverlap(WakeBox)
  (params (OverlappedComponent :type Primitive%20Component%20Object%20Reference) (OtherActor :type Actor%20Object%20Reference) (OtherComp :type Primitive%20Component%20Object%20Reference) (OtherBodyIndex :type Integer) (bFromSweep :type Boolean) (SweepResult :type Hit%20Result%20Structure%20%28by%20ref%29))
  (Utilities|Casting|CastToBP_Spike OtherActor)
  (CallFunction|FireGreaseBlob)
  (if (Variables|Default|GetRandomDropTime)
    (Utilities|Time|SetTimerbyFunctionName 0 "FireGreaseBlob" (Math|Random|RandomFloatinRange 1.75 3.0) true)
    (else
      (Utilities|Time|SetTimerbyFunctionName 0 "FireGreaseBlob" (Variables|Default|GetDropDelay) true))))

(event OnComponentEndOverlap(WakeBox)
  (params (OverlappedComponent :type Primitive%20Component%20Object%20Reference) (OtherActor :type Actor%20Object%20Reference) (OtherComp :type Primitive%20Component%20Object%20Reference) (OtherBodyIndex :type Integer))
  (Utilities|Casting|CastToBP_Spike OtherActor)
  (Utilities|Time|ClearTimerbyFunctionName 0 "FireGreaseBlob"))

(event Custom|FireGreaseBlob
  (bind _greaseblobspawn (Variables|Default|GetGreaseBlobSpawn))
  (bind _returnvalue (Transformation|GetWorldTransform _greaseblobspawn))
  (Game|SpawnActorfromClass "/Game/SetchOnLegs/00Blueprint/02GreasyGrove/BP_GreaseBlob.BP_GreaseBlob_C" (Math|Transform|MakeTransform (.location _returnvalue) (.rotation _returnvalue) "0.030000,0.030000,0.030000") "Undefined" 0 0)
  (Audio|PlaySound2D "/Game/SetchOnLegs/03Audio/02GreasyGrove/GreaseBlob.GreaseBlob" 1.0 1.0 0.0 0 0))

(fn ConstructionScript)
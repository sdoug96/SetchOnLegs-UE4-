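; BP_DiggerMole is a Paper2D enemy that wakes when BP_Spike enters its trigger and throws rocks.
; Timed states drive flipbook changes and hit-sphere collision, while a looping timer spawns BP_Rock with randomized X force.
; When Spike leaves, it sleeps, stops throwing and returns underground.
; Its hit spheres handle bullet hits and damage Spike on contact, and death through the parent damage system disables them.
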(event OnComponentBeginOverlap(WakeTrigger)
  (params (OverlappedComponent :type Primitive%20Component%20Object%20Reference) (OtherActor :type Actor%20Object%20Reference) (OtherComp :type Primitive%20Component%20Object%20Reference) (OtherBodyIndex :type Integer) (bFromSweep :type Boolean) (SweepResult :type Hit%20Result%20Structure%20%28by%20ref%29))
  ;[1 1 1] Wake up and throw rocks
  (Utilities|Casting|CastToBP_Spike OtherActor)
  (Variables|Default|SetActive true)
  (Variables|Default|SetState "NewEnumerator1")
  (CallFunction|UpdateAnimation)
  (Utilities|FlowControl|Delay 0.7)
  (Collision|SetCollisionEnabled (Variables|Default|GetHitSphereBottom) "QueryOnly")
  (if (Variables|Default|GetActive)
    (Variables|Default|SetState "NewEnumerator3")
    (CallFunction|UpdateAnimation)
    (Utilities|FlowControl|Delay (Variables|Default|GetInitialThrowDelay))
    (if (Variables|Default|GetActive)
      (CallFunction|ThrowRock)
      (Utilities|Time|SetTimerbyFunctionName 0 "ThrowRock" (Variables|Default|GetThrowDelay) true))))

(event OnComponentEndOverlap(WakeTrigger)
  (params (OverlappedComponent :type Primitive%20Component%20Object%20Reference) (OtherActor :type Actor%20Object%20Reference) (OtherComp :type Primitive%20Component%20Object%20Reference) (OtherBodyIndex :type Integer))
  ;[1 1 1] Wake up and throw rocks
  (Utilities|Casting|CastToBP_Spike OtherActor)
  (Variables|Default|SetActive false)
  (Variables|Default|SetState "NewEnumerator6")
  (CallFunction|UpdateAnimation)
  (Utilities|Time|ClearTimerbyFunctionName 0 "ThrowRock")
  (Collision|SetCollisionEnabled (Variables|Default|GetHitSphereBottom) "NoCollision")
  (Utilities|FlowControl|Delay 0.5)
  (Variables|Default|SetState "NewEnumerator0")
  (CallFunction|UpdateAnimation))

(event OnComponentBeginOverlap(HitSphereTop)
  (params (OverlappedComponent :type Primitive%20Component%20Object%20Reference) (OtherActor :type Actor%20Object%20Reference) (OtherComp :type Primitive%20Component%20Object%20Reference) (OtherBodyIndex :type Integer) (bFromSweep :type Boolean) (SweepResult :type Hit%20Result%20Structure%20%28by%20ref%29))
  ;[1 1 1] Collision Logic
  (Utilities|FlowControl|Sequence
    (:then_0
      (Utilities|Casting|CastToBP_Bullet OtherActor)
      (CallFunction|BulletCollision)
      (switch int (Math|Random|RandomIntegerinRange 0 2)
        (:Default
          (Audio|PlaySound2D "/Game/SetchOnLegs/03Audio/07Spike/EnemyHit.EnemyHit" 1.0 1.0 0.0 0 0 :!label _label))
        (:0
          (Audio|PlaySound2D "/Game/SetchOnLegs/03Audio/02GreasyGrove/JohnOuch.JohnOuch" 1.0 1.0 0.0 0 0))
        (:1
          (goto _label))
        (:2
          (goto _label))))
    (:then_1
      (Utilities|Casting|CastToBP_Spike OtherActor)
      (CallFunction|DamageSpike))))

(event OnComponentBeginOverlap(HitSphereBottom)
  (params (OverlappedComponent :type Primitive%20Component%20Object%20Reference) (OtherActor :type Actor%20Object%20Reference) (OtherComp :type Primitive%20Component%20Object%20Reference) (OtherBodyIndex :type Integer) (bFromSweep :type Boolean) (SweepResult :type Hit%20Result%20Structure%20%28by%20ref%29))
  ;[1 1 1] Collision Logic
  (Utilities|FlowControl|Sequence
    (:then_0
      (Utilities|Casting|CastToBP_Bullet OtherActor)
      (CallFunction|BulletCollision)
      (switch int (Math|Random|RandomIntegerinRange 0 2)
        (:Default
          (Audio|PlaySound2D "/Game/SetchOnLegs/03Audio/07Spike/EnemyHit.EnemyHit" 1.0 1.0 0.0 0 0 :!label _label))
        (:0
          (Audio|PlaySound2D "/Game/SetchOnLegs/03Audio/02GreasyGrove/JohnOuch.JohnOuch" 1.0 1.0 0.0 0 0))
        (:1
          (goto _label))
        (:2
          (goto _label))))
    (:then_1
      (Utilities|Casting|CastToBP_Spike OtherActor)
      (CallFunction|DamageSpike))))

(event Custom|UpdateAnimation
  (bind _isdead (Variables|Default|GetIsDead))
  ;[1 1 1] Update Animation
  (switch Utilities|FlowControl|Switch|SwitchonDiggerMoleState (Variables|Default|GetState)
    (:NewEnumerator0
      (if (not _isdead)
        (Sprite|SetFlipbook (Variables|Default|GetSprite))))
    (:NewEnumerator1
      (if (not _isdead)
        (Sprite|SetFlipbook (Variables|Default|GetSprite) "/Game/SetchOnLegs/01Sprites/02GreasyGrove/DiggerMole/Animations/A_DiggerMoleWake.A_DiggerMoleWake")))
    (:NewEnumerator2
      (if (not _isdead)
        (Sprite|SetFlipbook (Variables|Default|GetSprite) "/Game/SetchOnLegs/01Sprites/02GreasyGrove/DiggerMole/Animations/A_DiggerMoleIdle.A_DiggerMoleIdle")))
    (:NewEnumerator3
      (if (not _isdead)
        (Sprite|SetFlipbook (Variables|Default|GetSprite) "/Game/SetchOnLegs/01Sprites/02GreasyGrove/DiggerMole/Animations/A_DiggerMoleAttack.A_DiggerMoleAttack")))
    (:NewEnumerator6
      (if (not _isdead)
        (Sprite|SetFlipbook (Variables|Default|GetSprite) "/Game/SetchOnLegs/01Sprites/02GreasyGrove/DiggerMole/Animations/A_DiggerMoleSleep.A_DiggerMoleSleep")))
    (:NewEnumerator5
      (Sprite|SetFlipbook (Variables|Default|GetSprite) "/Game/SetchOnLegs/01Sprites/02GreasyGrove/DiggerMole/Animations/A_DiggerMoleSleep.A_DiggerMoleSleep"))))

(event Custom|ThrowRock
  ;[1 1 1] Throw rock function
  (Variables|Default|SetThrowForce (Math|Vector|MakeVector (Math|Random|RandomFloatinRange (Variables|Default|GetMinXForce) (Variables|Default|GetMaxXForce)) 0.0 (Variables|Default|GetZForce)))
  (if (Variables|Default|GetActive)
    (if (not (Variables|Default|GetIsDead))
      (Game|SpawnActorfromClass "/Game/SetchOnLegs/00Blueprint/02GreasyGrove/Enemies/BP_Rock.BP_Rock_C" (Math|Transform|MakeTransform (Transformation|GetWorldLocation (Variables|Default|GetRockSpawn)) "0, 0, 0" "0.187500,0.187500,0.187500") "Undefined" 0 (Variables|Default|GetThrowForce) 1 2.0 false 0.0 0.0 true 0)
      (Audio|PlaySound2D "/Game/SetchOnLegs/03Audio/02GreasyGrove/Dir.Dir" 1.0 1.0 0.0 0 0))))

(event EventDamageSystem
  (params (DamageIn :type Float%20%28single-precision%29))
  ;[1 1 1] Damage & Death System
  (|CallParentFunction DamageIn)
  (if (Variables|Default|GetIsDead)
    (Variables|Default|SetState "NewEnumerator5")
    (CallFunction|UpdateAnimation)
    (Collision|SetCollisionEnabled (Variables|Default|GetHitSphereTop) "NoCollision")))

(fn ConstructionScript)
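; Bouncing mole enemy with flipbook animation that wakes when BP_Spike enters its wake trigger, then repeatedly hops toward the player.
; A state enum drives the sprite, and each landing schedules the next delayed launch.
; Leaving the detached active trigger puts it to sleep and resets it to its spawn point, except in boss fights, where it wakes on BeginPlay.
; Body and head spheres take bullet hits and damage Spike on contact.
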(event OnComponentBeginOverlap(WakeTrigger)
  (params (OverlappedComponent :type Primitive%20Component%20Object%20Reference) (OtherActor :type Actor%20Object%20Reference) (OtherComp :type Primitive%20Component%20Object%20Reference) (OtherBodyIndex :type Integer) (bFromSweep :type Boolean) (SweepResult :type Hit%20Result%20Structure%20%28by%20ref%29))
  ;[1 1 1] Player Detection and Resulting Logic
  (Utilities|Casting|CastToBP_Spike OtherActor)
  (CallFunction|WakeUp))

(event OnComponentBeginOverlap(HitSphereBody)
  (params (OverlappedComponent :type Primitive%20Component%20Object%20Reference) (OtherActor :type Actor%20Object%20Reference) (OtherComp :type Primitive%20Component%20Object%20Reference) (OtherBodyIndex :type Integer) (bFromSweep :type Boolean) (SweepResult :type Hit%20Result%20Structure%20%28by%20ref%29))
  ;[1 1 1] Collision
  (Utilities|FlowControl|Sequence
    (:then_0
      (Utilities|Casting|CastToBP_Bullet OtherActor)
      (CallFunction|BulletCollision)
      (switch int (Math|Random|RandomIntegerinRange 0 2)
        (:Default
          (Audio|PlaySound2D "/Game/SetchOnLegs/03Audio/07Spike/EnemyHit.EnemyHit" 1.0 1.0 0.0 0 0 :!label _label))
        (:0
          (Audio|PlaySound2D "/Game/SetchOnLegs/03Audio/02GreasyGrove/JohnOuch.JohnOuch" 1.0 1.0 0.0 0 0))
        (:1
          (goto _label))
        (:2
          (goto _label))))
    (:then_1
      (Utilities|Casting|CastToBP_Spike OtherActor)
      (CallFunction|DamageSpike))))

(event OnComponentEndOverlap(ActiveTrigger)
  (params (OverlappedComponent :type Primitive%20Component%20Object%20Reference) (OtherActor :type Actor%20Object%20Reference) (OtherComp :type Primitive%20Component%20Object%20Reference) (OtherBodyIndex :type Integer))
  ;[1 1 1] Player Detection and Resulting Logic
  (Utilities|Casting|CastToBP_Spike OtherActor)
  (if (not (Variables|Default|GetIsBossFight))
    (if (Variables|Default|GetActive)
      (Variables|Default|SetActive false)
      (if (not (AI|Components|NavMovement|IsFalling (Variables|Character|GetCharacterMovement)))
        (Variables|Default|SetState "NewEnumerator0")
        (CallFunction|UpdateAnimation)
        (Utilities|FlowControl|Delay 0.5)
        (Variables|Default|SetState "NewEnumerator4")
        (CallFunction|UpdateAnimation)
        (Collision|SetCollisionEnabled (Variables|Default|GetHitSphereBody) "NoCollision")
        (Components|Movement|StopMovementImmediately (Variables|Character|GetCharacterMovement))
        (Transformation|SetActorLocation (Variables|Default|GetBaseLocation) false false)
        (Variables|Default|SetActive false)))))

(event OnComponentBeginOverlap(HitSphereHead)
  (params (OverlappedComponent :type Primitive%20Component%20Object%20Reference) (OtherActor :type Actor%20Object%20Reference) (OtherComp :type Primitive%20Component%20Object%20Reference) (OtherBodyIndex :type Integer) (bFromSweep :type Boolean) (SweepResult :type Hit%20Result%20Structure%20%28by%20ref%29))
  ;[1 1 1] Collision
  (Utilities|FlowControl|Sequence
    (:then_0
      (Utilities|Casting|CastToBP_Bullet OtherActor)
      (CallFunction|BulletCollision)
      (switch int (Math|Random|RandomIntegerinRange 0 2)
        (:Default
          (Audio|PlaySound2D "/Game/SetchOnLegs/03Audio/07Spike/EnemyHit.EnemyHit" 1.0 1.0 0.0 0 0 :!label _label))
        (:0
          (Audio|PlaySound2D "/Game/SetchOnLegs/03Audio/02GreasyGrove/JohnOuch.JohnOuch" 1.0 1.0 0.0 0 0))
        (:1
          (goto _label))
        (:2
          (goto _label))))
    (:then_1
      (Utilities|Casting|CastToBP_Spike OtherActor)
      (CallFunction|DamageSpike))))

(event Custom|Bounce
  (bind _bounceforce (Variables|Default|GetBounceForce))
  ;[1 1 1] Bounce
  (if (Variables|Default|GetActive)
    (if (not (Variables|Default|GetIsDead))
      (Audio|PlaySound2D "/Game/SetchOnLegs/03Audio/02GreasyGrove/Dir.Dir" 1.0 1.0 0.0 0 0)
      (Character|LaunchCharacter (Math|Vector|MakeVector (* (Variables|Default|GetBounceDirection) (.x _bounceforce)) 0.0 (.z _bounceforce)) true true)
      (Variables|Default|SetState "NewEnumerator2")
      (CallFunction|UpdateAnimation))))

(event Custom|UpdateAnimation
  (bind _isdead (Variables|Default|GetIsDead))
  ;[1 1 1] Handle Animation
  (switch Utilities|FlowControl|Switch|SwitchonBouncingMoleState (Variables|Default|GetState)
    (:NewEnumerator4
      (if (not _isdead)
        (Sprite|SetFlipbook (Variables|Default|GetSprite))))
    (:NewEnumerator5
      (if (not _isdead)
        (Sprite|SetFlipbook (Variables|Default|GetSprite) "/Game/SetchOnLegs/01Sprites/02GreasyGrove/BouncingMole/Animations/A_BouncingMoleWake.A_BouncingMoleWake")))
    (:NewEnumerator1
      (if (not _isdead)
        (Sprite|SetFlipbook (Variables|Default|GetSprite) "/Game/SetchOnLegs/01Sprites/02GreasyGrove/BouncingMole/Animations/A_BouncingMoleIdle.A_BouncingMoleIdle")))
    (:NewEnumerator2
      (if (not _isdead)
        (Sprite|SetFlipbook (Variables|Default|GetSprite) "/Game/SetchOnLegs/01Sprites/02GreasyGrove/BouncingMole/Animations/A_BouncingMoleBounce.A_BouncingMoleBounce")))
    (:NewEnumerator0
      (if (not _isdead)
        (Sprite|SetFlipbook (Variables|Default|GetSprite) "/Game/SetchOnLegs/01Sprites/02GreasyGrove/BouncingMole/Animations/A_BouncingMoleSleep.A_BouncingMoleSleep")))
    (:NewEnumerator3
      (Sprite|SetFlipbook (Variables|Default|GetSprite) "/Game/SetchOnLegs/01Sprites/02GreasyGrove/BouncingMole/Animations/A_BouncingMoleDeath.A_BouncingMoleDeath"))))

(event Custom|WakeUp
  ;[1 1 1] Wake Up
  (if (not (Variables|Default|GetActive))
    (Variables|Default|SetState "NewEnumerator5")
    (CallFunction|UpdateAnimation)
    (Utilities|FlowControl|Delay 0.7)
    (Variables|Default|SetState "NewEnumerator1")
    (CallFunction|UpdateAnimation)
    (Variables|Default|SetActive true)
    (Collision|SetCollisionEnabled (Variables|Default|GetHitSphereBody) "QueryOnly")
    (Utilities|FlowControl|Delay (Variables|Default|GetBounceDelay))
    (CallFunction|Bounce)))

(event EventBeginPlay
  ;[1 1 1] Begin Play
  (|CallParentFunction)
  (Variables|Default|SetBaseLocation (Transformation|GetActorLocation))
  (Transformation|DetachFromComponent (Variables|Default|GetWakeTrigger) "KeepWorld" "KeepWorld" "KeepWorld" true)
  (Transformation|DetachFromComponent (Variables|Default|GetActiveTrigger) "KeepWorld" "KeepWorld" "KeepWorld" true)
  (Pawn|SpawnDefaultController)
  (CallFunction|UpdateAnimation)
  (if (Variables|Default|GetIsBossFight)
    (CallFunction|WakeUp)))

(event EventSetRotation
  ;[1 1 1] Set rotation
  (|CallParentFunction)
  (if (Variables|Default|GetIsRightOfPlayer)
    (Variables|Default|SetBounceDirection -1)
    (else
      (Variables|Default|SetBounceDirection 1))))

(event EventOnLanded
  (params (Hit :type Hit%20Result%20Structure%20%28by%20ref%29))
  ;[1 1 1] Landed Logic
  (if (Collision|IsOverlappingActor (Variables|Default|GetActiveTrigger) (Variables|Default|GetPlayer) :!class /Script/Engine.PrimitiveComponent)
    (Variables|Default|SetState "NewEnumerator1" :!label _label)
    (CallFunction|UpdateAnimation)
    (Utilities|FlowControl|Delay (Variables|Default|GetBounceDelay))
    (if (Variables|Default|GetActive)
      (CallFunction|Bounce))
    (elif (Variables|Default|GetIsBossFight)
      (if (Variables|Default|GetActive)
        (goto _label))
      (else
        (Components|Movement|StopMovementImmediately (Variables|Character|GetCharacterMovement))
        (Variables|Default|SetState "NewEnumerator0")
        (CallFunction|UpdateAnimation)
        (Utilities|FlowControl|Delay 0.5)
        (Variables|Default|SetState "NewEnumerator4")
        (CallFunction|UpdateAnimation)
        (Transformation|SetActorLocation (Variables|Default|GetBaseLocation) false false)
        (Variables|Default|SetActive false)))))

(event EventDamageSystem
  (params (DamageIn :type Float%20%28single-precision%29))
  ;[1 1 1] Damage & Death System
  (|CallParentFunction DamageIn)
  (if (Variables|Default|GetIsDead)
    (Variables|Default|SetState "NewEnumerator3")
    (CallFunction|UpdateAnimation)
    (Collision|SetCollisionEnabled (Variables|Default|GetHitSphereHead) "NoCollision")))

(event EventTick
  (params (DeltaSeconds :type Float%20%28single-precision%29))
  ;[1 1 1] Set rotation
  (if (Variables|Default|GetActive)
    (CallFunction|SetRotation)))

(fn ConstructionScript)
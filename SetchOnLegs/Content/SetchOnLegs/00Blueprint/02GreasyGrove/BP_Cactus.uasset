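; BP_Cactus is a hazard actor that damages the player's BP_Spike character when it overlaps the HitBox.
; Damage is skipped during cutscenes or while the character is in one particular state.
; A custom Lerp event, not called within this graph, starts timeline-driven movement between the actor's location and an X/Z offset.
; The timeline alternates forward and reverse on each finish via TimeFactor, producing continuous back-and-forth motion without sweep.
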(event OnComponentBeginOverlap(HitBox)
  (params (OverlappedComponent :type Primitive%20Component%20Object%20Reference) (OtherActor :type Actor%20Object%20Reference) (OtherComp :type Primitive%20Component%20Object%20Reference) (OtherBodyIndex :type Integer) (bFromSweep :type Boolean) (SweepResult :type Hit%20Result%20Structure%20%28by%20ref%29))
  ;[1 1 1] Player Collision
  (bind _asbp_spike (Utilities|Casting|CastToBP_Spike OtherActor))
  (if (Utilities|Enum|NotEqual(Enum) (Variables|/Game/SetchOnLegs/00Blueprint/07Spike/BP_Spike.BP_Spike_C|GetState _asbp_spike) "NewEnumerator5")
    (if (not (Variables|/Game/SetchOnLegs/00Blueprint/07Spike/BP_Spike.BP_Spike_C|GetCutScene (Variables|Default|GetPlayer)))
      (Default|DamageSytsem _asbp_spike 1))))

(event Custom|Lerp
  ;[1 1 1] Lerp Movement
  (bind _output_get (Variables|Default|SetInitialLocation (Transformation|GetActorLocation)))
  (Variables|Default|SetEndLocation (+ _output_get (Math|Vector|MakeVector (Variables|Default|GetPosDiffX) 0.0 (Variables|Default|GetPosDiffZ))))
  (bind _newtrack_0 (Timeline|LerpTimeline Play)
    (:Update
      (Transformation|SetActorLocation (Math|Vector|Lerp(Vector) (Variables|Default|GetInitialLocation) (Variables|Default|GetEndLocation) _newtrack_0) false false))
    (:Finished
      (if (Variables|Default|GetTimeFactor)
        (Variables|Default|SetTimeFactor false)
        (Timeline|LerpTimeline ReverseFromEnd)
        (else
          (Variables|Default|SetTimeFactor true)
          (Timeline|LerpTimeline PlayFromStart))))))

(event EventBeginPlay
  ;[1 1 1] Begin Play
  (bind _asbp_spike (Utilities|Casting|CastToBP_Spike (Game|GetPlayerCharacter 0)))
  (Variables|Default|SetPlayer _asbp_spike))

(fn ConstructionScript)
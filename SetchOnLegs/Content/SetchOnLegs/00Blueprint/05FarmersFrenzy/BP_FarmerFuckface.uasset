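; Farmer boss for Farmer's Frenzy, a flipbook character with a health HUD that fights the player Spike.
; It alternates timed horizontal runs with stops, reversing direction and spawning pitchforks at shuffled points for delayed launch.
; A parallel self-calling delay loop throws rotten parsnips continuously.
; Player bullets reduce health and make the sprite blink, while health-range phases checked on Tick raise the pitchfork count until death.
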(event OnComponentBeginOverlap(BulletBox)
  (params (OverlappedComponent :type Primitive%20Component%20Object%20Reference) (OtherActor :type Actor%20Object%20Reference) (OtherComp :type Primitive%20Component%20Object%20Reference) (OtherBodyIndex :type Integer) (bFromSweep :type Boolean) (SweepResult :type Hit%20Result%20Structure%20%28by%20ref%29))
  ;[1 1 1] Bullet Collision
  (Utilities|FlowControl|Sequence
    (:then_0
      (bind _asbp_bullet (Utilities|Casting|CastToBP_Bullet OtherActor))
      (Actor|DestroyActor _asbp_bullet)
      (if (not (Variables|Default|GetIsDead))
        (CallFunction|DamageSytsem (Variables|/Game/SetchOnLegs/00Blueprint/07Spike/BP_Spike.BP_Spike_C|GetBulletDamage (Variables|Default|GetPlayer)))))))

(event Custom|Blink
  (bind _sprite (Variables|Default|GetSprite))
  ;[1 1 1] Damage & Death System
  ;;[1 1 1] Blink when damaged
  (Development|SetHiddeninGame _sprite (not (Variables|/Script/Engine.SceneComponent|GetbHiddenInGame _sprite)) false))

(event Custom|Damage%20Sytsem
  (params (DamageIn :type Float%20%28single-precision%29))
  ;[1 1 1] Damage & Death System
  (bind _output_get (Variables|Default|SetCurrentHealth (- (Variables|Default|GetCurrentHealth) DamageIn)))
  (if (<= _output_get 0.0)
    (Variables|Default|SetIsDead true)
    (Widget|RemovefromParent (Variables|Default|GetHUD))
    (Utilities|FlowControl|Delay 5.0)
    (Actor|DestroyActor)
    (else
      (Utilities|Time|SetTimerbyFunctionName 0 "Blink" 0.05 true)
      (Utilities|FlowControl|Delay 0.2)
      (Utilities|Time|ClearTimerbyFunctionName 0 "Blink")
      (Development|SetHiddeninGame (Variables|Default|GetSprite) false false))))

(event Custom|Move
  (bind _returnvalue (Transformation|GetActorRotation))
  ;[1 1 1] Move
  (Variables|Default|SetCanMove true)
  (Audio|PlaySound2D 0 1.0 1.0 0.0 0 0)
  (Utilities|FlowControl|Delay 14.5)
  (if (== (Variables|Default|GetMoveSpeed) 1.5e+02)
    (Transformation|SetActorRotation (Math|Rotator|MakeRotator (.roll _returnvalue) (.pitch _returnvalue) 1.8e+02))
    (else
      (Transformation|SetActorRotation (Math|Rotator|MakeRotator (.roll _returnvalue) (.pitch _returnvalue) 0.0))))
  (Variables|Default|SetMoveSpeed (* (Variables|Default|GetMoveSpeed) -1.0))
  (Variables|Default|SetCanMove false)
  (CallFunction|SpawnPitchforks)
  (Utilities|FlowControl|Delay (Variables|Default|GetMoveAgainDelay))
  (CallFunction|Move))

(event Custom|SpawnPitchforks
  ;[1 1 1] Pitchforks
  (Audio|PlaySound2D 0 1.0 1.0 0.0 0 0)
  (Utilities|Array|Shuffle (Variables|Default|GetPitchforkSpawns))
  (for _index (range 0 (- (Variables|Default|GetPitchforks) 1))
    (Game|SpawnActorfromClass "/Game/SetchOnLegs/00Blueprint/05FarmersFrenzy/BP_Pitchfork.BP_Pitchfork_C" (Math|Transform|MakeTransform (Utilities|Array|Get(acopy) (Variables|Default|GetPitchforkSpawns) (Variables|Default|GetPitchforkIndex)) "0, 0, 0" "1,1,1") "Undefined" 0 5e+03 (Variables|Default|GetPitchforkLaunchDelay) 0)
    (Variables|Default|SetPitchforkIndex (+ (Variables|Default|GetPitchforkIndex) 1)))
  (Variables|Default|SetPitchforkIndex 0)
  (Utilities|FlowControl|Delay (Variables|Default|GetPitchforkLaunchDelay))
  (Audio|PlaySound2D 0 1.0 1.0 0.0 0 0))

(event Custom|SetMovement
  ;[1 1 1] Set Movement on Tick
  (if (Variables|Default|GetCanMove)
    (Variables|/Script/Engine.MovementComponent|SetVelocity (Variables|Character|GetCharacterMovement) (Math|Vector|MakeVector (Variables|Default|GetMoveSpeed) 0.0 0.0))
    (Sprite|SetFlipbook (Variables|Default|GetSprite))
    (else
      (Variables|/Script/Engine.MovementComponent|SetVelocity (Variables|Character|GetCharacterMovement) "0, 0, 0")
      (Sprite|SetFlipbook (Variables|Default|GetSprite)))))

(event Custom|SetPhase
  ;[1 1 1] Set phase
  (if (Math|Float|InRange(Float) (Variables|Default|GetCurrentHealth) 2e+04 39999.0)
    (Variables|Default|SetPhase1 false)
    (Variables|Default|SetPhase2 true)
    (Variables|Default|SetPitchforks 2)
    (elif (Math|Float|InRange(Float) (Variables|Default|GetCurrentHealth) 1.0 19999.0)
      (Variables|Default|SetPhase2 false)
      (Variables|Default|SetPhase3 true)
      (Variables|Default|SetPitchforks 3))))

(event Custom|ThrowRottenFood
  (Game|SpawnActorfromClass "/Game/SetchOnLegs/00Blueprint/05FarmersFrenzy/BP_RottenParsnip.BP_RottenParsnip_C" (Transformation|GetWorldTransform (Variables|Default|GetProjectileSpawn)) "Undefined" 0 0)
  (Utilities|FlowControl|Delay 1.5)
  (CallFunction|ThrowRottenFood))

(event EventBeginPlay
  ;[1 1 1] Initialise
  (bind _returnvalue (UserInterface|CreateWidget "/Game/SetchOnLegs/00Blueprint/05FarmersFrenzy/Widget_FarmerFuckface.Widget_FarmerFuckface_C"))
  (bind _output_get (Variables|Default|SetHUD _returnvalue))
  (UserInterface|Viewport|AddtoViewport _output_get 0)
  (bind _asbp_spike (Utilities|Casting|CastToBP_Spike (Game|GetPlayerCharacter 0)))
  (Variables|Default|SetPlayer _asbp_spike)
  (Utilities|FlowControl|Delay 1.0)
  (CallFunction|Move)
  (CallFunction|ThrowRottenFood))

(event EventTick
  (params (DeltaSeconds :type Float%20%28single-precision%29))
  ;[1 1 1] Tick
  (Utilities|FlowControl|Sequence
    (:then_0
      (CallFunction|SetPhase))
    (:then_1
      (CallFunction|SetMovement))))

(fn ConstructionScript)
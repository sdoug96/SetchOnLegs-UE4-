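; BP_ExitLevelFade is a level-exit trigger that sends Spike to another level behind a travelling widget.
; On overlap it disables input, shows the widget and copies health, currency, deaths, shop upgrades and double jump into BP_GameInstance.
; It also stores the next spawn location, then opens the target level after a random delay of several seconds.
; Meanwhile, if movement is enabled, Tick auto-walks Spike left or right, or climbs him upward.
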(event OnComponentBeginOverlap(Box)
  (params (OverlappedComponent :type Primitive%20Component%20Object%20Reference) (OtherActor :type Actor%20Object%20Reference) (OtherComp :type Primitive%20Component%20Object%20Reference) (OtherBodyIndex :type Integer) (bFromSweep :type Boolean) (SweepResult :type Hit%20Result%20Structure%20%28by%20ref%29))
  ;[1 1 1] Exit Level Logic
  (bind _asbp_spike (Utilities|Casting|CastToBP_Spike OtherActor))
  (Variables|Default|SetPlayer _asbp_spike)
  (bind _asbp_game_instance (Utilities|Casting|CastToBP_GameInstance (Game|GetGameInstance)))
  (Variables|Default|SetGameInstance _asbp_game_instance)
  (Variables|Default|SetHit true)
  (Input|DisableInput (Variables|Default|GetPlayer) 0)
  (Sprite|SetFlipbook (Variables|/Script/Paper2D.PaperCharacter|GetSprite (Variables|Default|GetPlayer)) "/Game/SetchOnLegs/01Sprites/07Spike/Character/A_SpikeWalking.A_SpikeWalking")
  (Components|Timeline|SetPlayRate (Variables|/Script/Paper2D.PaperCharacter|GetSprite (Variables|Default|GetPlayer)) 1.0)
  (bind _returnvalue (UserInterface|CreateWidget "/Game/SetchOnLegs/00Blueprint/11Misc/Widget_Travelling.Widget_Travelling_C"))
  (UserInterface|Viewport|AddtoViewport _returnvalue 0)
  (Utilities|FlowControl|Sequence
    (:then_0
      (CallFunction|SetGameInstanceValues))
    (:then_1
      (Variables|/Game/SetchOnLegs/00Blueprint/11Misc/BP_GameInstance.BP_GameInstance_C|SetSpawnLocation (Variables|Default|GetGameInstance) (Variables|Default|GetNewSpawn)))
    (:then_2
      (Utilities|FlowControl|Delay (Math|Random|RandomFloatinRange 5.0 7.0))
      (Game|OpenLevel(byName) (Variables|Default|GetLevelToOpen)))))

(event Custom|SetGameInstanceValues
  ;[1 1 1] Set game instance values to players values
  (Utilities|FlowControl|Sequence
    (:then_0
      (CallFunction|SetMainValues))
    (:then_1
      (CallFunction|SetShopValues))
    (:then_2
      (CallFunction|SetAbilityValues))))

(event Custom|SetMainValues
  (bind _player (Variables|Default|GetPlayer))
  (bind _gameinstance (Variables|Default|GetGameInstance))
  ;[1 1 1] Set main values
  (Utilities|FlowControl|Sequence
    (:then_0
      (Variables|/Game/SetchOnLegs/00Blueprint/11Misc/BP_GameInstance.BP_GameInstance_C|SetHealth _gameinstance (Variables|/Game/SetchOnLegs/00Blueprint/07Spike/BP_Spike.BP_Spike_C|GetCurrentHealth _player)))
    (:then_1
      (Variables|/Game/SetchOnLegs/00Blueprint/11Misc/BP_GameInstance.BP_GameInstance_C|SetMaxHealth _gameinstance (Variables|/Game/SetchOnLegs/00Blueprint/07Spike/BP_Spike.BP_Spike_C|GetMaxHealth _player)))
    (:then_2
      (Variables|/Game/SetchOnLegs/00Blueprint/11Misc/BP_GameInstance.BP_GameInstance_C|SetCurrency _gameinstance (Variables|/Game/SetchOnLegs/00Blueprint/07Spike/BP_Spike.BP_Spike_C|GetMasterBalls _player)))
    (:then_3
      (Variables|/Game/SetchOnLegs/00Blueprint/11Misc/BP_GameInstance.BP_GameInstance_C|SetDeathCount _gameinstance (Variables|/Game/SetchOnLegs/00Blueprint/07Spike/BP_Spike.BP_Spike_C|GetDeathCount _player)))))

(event Custom|SetShopValues
  (bind _player (Variables|Default|GetPlayer))
  (bind _gameinstance (Variables|Default|GetGameInstance))
  ;[1 1 1] Set shop values
  (Utilities|FlowControl|Sequence
    (:then_0
      (Variables|/Game/SetchOnLegs/00Blueprint/11Misc/BP_GameInstance.BP_GameInstance_C|SetChargedShot _gameinstance (Variables|/Game/SetchOnLegs/00Blueprint/07Spike/BP_Spike.BP_Spike_C|GetChargedShot _player)))
    (:then_1
      (Variables|/Game/SetchOnLegs/00Blueprint/11Misc/BP_GameInstance.BP_GameInstance_C|Set3BulletSpread _gameinstance (Variables|/Game/SetchOnLegs/00Blueprint/07Spike/BP_Spike.BP_Spike_C|Get3Bullet _player)))
    (:then_2
      (Variables|/Game/SetchOnLegs/00Blueprint/11Misc/BP_GameInstance.BP_GameInstance_C|Set5BulletSpread _gameinstance (Variables|/Game/SetchOnLegs/00Blueprint/07Spike/BP_Spike.BP_Spike_C|Get5Bullet _player)))
    (:then_3
      (Variables|/Game/SetchOnLegs/00Blueprint/11Misc/BP_GameInstance.BP_GameInstance_C|SetCheckpoints _gameinstance (Variables|/Game/SetchOnLegs/00Blueprint/07Spike/BP_Spike.BP_Spike_C|GetCheckpoints _player)))
    (:then_4
      (Variables|/Game/SetchOnLegs/00Blueprint/11Misc/BP_GameInstance.BP_GameInstance_C|SetShields _gameinstance (Variables|/Game/SetchOnLegs/00Blueprint/07Spike/BP_Spike.BP_Spike_C|GetShields _player)))
    (:then_5
      (Variables|/Game/SetchOnLegs/00Blueprint/11Misc/BP_GameInstance.BP_GameInstance_C|SetBulletDamage _gameinstance (Variables|/Game/SetchOnLegs/00Blueprint/07Spike/BP_Spike.BP_Spike_C|GetBulletDamage _player)))
    (:then_6
      (Variables|/Game/SetchOnLegs/00Blueprint/11Misc/BP_GameInstance.BP_GameInstance_C|SetChargedBulletCooldown _gameinstance (Variables|/Game/SetchOnLegs/00Blueprint/07Spike/BP_Spike.BP_Spike_C|GetMaxChargedShotCooldown _player)))
    (:then_7
      (Variables|/Game/SetchOnLegs/00Blueprint/11Misc/BP_GameInstance.BP_GameInstance_C|SetChargedBulletDamage _gameinstance (Variables|/Game/SetchOnLegs/00Blueprint/07Spike/BP_Spike.BP_Spike_C|GetChargedShotDamage _player)))))

(event Custom|SetAbilityValues
  ;[1 1 1] Set ability values
  (Utilities|FlowControl|Sequence
    (:then_0
      (Variables|/Game/SetchOnLegs/00Blueprint/11Misc/BP_GameInstance.BP_GameInstance_C|SetDoubleJump (Variables|Default|GetGameInstance) (Variables|/Game/SetchOnLegs/00Blueprint/07Spike/BP_Spike.BP_Spike_C|GetDoubleJump (Variables|Default|GetPlayer))))))

(event EventTick
  (params (DeltaSeconds :type Float%20%28single-precision%29))
  (bind _player (Variables|Default|GetPlayer))
  ;[1 1 1] Exit Level Logic
  ;;[1 1 1] Move Spike
  (if (Variables|Default|GetMove)
    (if (Variables|Default|GetHit)
      (if (Variables|Default|GetClimb)
        (Variables|/Game/SetchOnLegs/00Blueprint/07Spike/BP_Spike.BP_Spike_C|SetState _player "NewEnumerator7")
        (Default|UpdateAnimation _player)
        (Pawn|Input|AddMovementInput _player (Math|Vector|MakeVector 0.0 0.0 0.5) 1.0 false)
        (elif (Variables|Default|GetLeft)
          (Pawn|Input|AddMovementInput (Variables|Default|GetPlayer) (Math|Vector|MakeVector -1.0 0.0 0.0) 1.0 false)
          (else
            (Pawn|Input|AddMovementInput (Variables|Default|GetPlayer) (Math|Vector|MakeVector 1.0 0.0 0.0) 1.0 false)))))))

(fn ConstructionScript)
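; Checkpoint actor that lets the BP_Spike player heal to full, save the game and set a respawn point.
; Overlapping the hit box shows a save prompt, and Interact activates the checkpoint unless a saving widget is already up.
; Activation lights only this checkpoint, switching off all others.
; It writes player stats, level name and an offset spawn location to a new save slot object, also updating the GameInstance spawn location.
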(event OnComponentBeginOverlap(HitBox)
  (params (OverlappedComponent :type Primitive%20Component%20Object%20Reference) (OtherActor :type Actor%20Object%20Reference) (OtherComp :type Primitive%20Component%20Object%20Reference) (OtherBodyIndex :type Integer) (bFromSweep :type Boolean) (SweepResult :type Hit%20Result%20Structure%20%28by%20ref%29))
  ;[1 1 1] Show and hide save game
  (Utilities|Casting|CastToBP_Spike OtherActor)
  (bind _foundwidgets (Widget|GetAllWidgetsOfClass "/Game/SetchOnLegs/00Blueprint/11Misc/Widget_Saving.Widget_Saving_C" true))
  (Utilities|IsValid (Utilities|Array|Get(acopy) _foundwidgets)
    (:Is%20Not%20Valid
      (bind _returnvalue (UserInterface|CreateWidget "/Game/SetchOnLegs/00Blueprint/11Misc/Widget_SavePrompt.Widget_SavePrompt_C"))
      (bind _output_get (Variables|Default|SetSavePrompt _returnvalue))
      (UserInterface|Viewport|AddtoViewport _output_get 0))))

(event OnComponentEndOverlap(HitBox)
  (params (OverlappedComponent :type Primitive%20Component%20Object%20Reference) (OtherActor :type Actor%20Object%20Reference) (OtherComp :type Primitive%20Component%20Object%20Reference) (OtherBodyIndex :type Integer))
  ;[1 1 1] Show and hide save game
  (Utilities|Casting|CastToBP_Spike OtherActor)
  (Widget|RemovefromParent (Variables|Default|GetSavePrompt)))

(event Custom|Activate
  ;[1 1 1] Activate this checkpoint
  (if (Utilities|IsValid (Variables|Default|GetSavePrompt))
    (if (Variables|/Script/Engine.SceneComponent|GetbVisible (Variables|Default|GetPointLight))
      _
      (else
        (bind _outactors (Actor|GetAllActorsOfClass "BP_Checkpoint_C"))
        (for _array_element _outactors
          (Rendering|SetVisibility (Variables|BP_Checkpoint_C|GetPointLight _array_element) false false))
        (Rendering|ToggleVisibility (Variables|Default|GetPointLight) false)))
    (Widget|RemovefromParent (Variables|Default|GetSavePrompt))
    (Audio|PlaySound2D "/Game/SetchOnLegs/03Audio/08Misc/Checkpoint.Checkpoint" 1.0 1.0 0.0 0 0)
    (bind _asbp_spike (Utilities|Casting|CastToBP_Spike (Game|GetPlayerCharacter 0)))
    (bind _output_get (Variables|Default|SetPlayer _asbp_spike))
    (Variables|/Game/SetchOnLegs/00Blueprint/07Spike/BP_Spike.BP_Spike_C|SetCurrentHealth _output_get (Variables|/Game/SetchOnLegs/00Blueprint/07Spike/BP_Spike.BP_Spike_C|GetMaxHealth _output_get))
    (CallFunction|SaveGame)
    (bind _returnvalue (UserInterface|CreateWidget "/Game/SetchOnLegs/00Blueprint/11Misc/Widget_Saving.Widget_Saving_C"))
    (UserInterface|Viewport|AddtoViewport _returnvalue 0)))

(event Custom|SaveGame
  ;[1 1 1] Save Game
  (bind _returnvalue (SaveGame|CreateSaveGameObject "/Game/SetchOnLegs/00Blueprint/11Misc/BP_SaveInfo.BP_SaveInfo_C"))
  (Variables|Default|SetSaveInfo _returnvalue)
  (CallFunction|SetSaveLocation)
  (CallFunction|SetSaveValues)
  (SaveGame|SaveGametoSlot (Variables|Default|GetSaveInfo) "SaveInfo"))

(event Custom|SetSaveLocation
  (bind _returnvalue (Transformation|GetActorLocation))
  (bind _returnvalue_2 (- (.z _returnvalue) 1.4e+02))
  (bind _returnvalue_3 (+ (.x _returnvalue) 75.0))
  ;[1 1 1] Set spawn location
  (Variables|/Game/SetchOnLegs/00Blueprint/11Misc/BP_SaveInfo.BP_SaveInfo_C|SetCheckLocation (Variables|Default|GetSaveInfo) (Math|Vector|MakeVector _returnvalue_3 0.0 _returnvalue_2))
  (bind _asbp_game_instance (Utilities|Casting|CastToBP_GameInstance (Game|GetGameInstance)))
  (Variables|/Game/SetchOnLegs/00Blueprint/11Misc/BP_GameInstance.BP_GameInstance_C|SetSpawnLocation _asbp_game_instance (Math|Vector|MakeVector _returnvalue_3 0.0 _returnvalue_2)))

(event Custom|SetSaveValues
  (bind _player (Variables|Default|GetPlayer))
  (bind _saveinfo (Variables|Default|GetSaveInfo))
  ;[1 1 1] Set Save Values
  (Utilities|FlowControl|Sequence
    (:then_0
      (Variables|/Game/SetchOnLegs/00Blueprint/11Misc/BP_SaveInfo.BP_SaveInfo_C|SetMasterBalls _saveinfo (Variables|/Game/SetchOnLegs/00Blueprint/07Spike/BP_Spike.BP_Spike_C|GetMasterBalls _player)))
    (:then_1
      (Variables|/Game/SetchOnLegs/00Blueprint/11Misc/BP_SaveInfo.BP_SaveInfo_C|SetDeaths _saveinfo (Variables|/Game/SetchOnLegs/00Blueprint/07Spike/BP_Spike.BP_Spike_C|GetDeathCount _player)))
    (:then_4
      (Variables|/Game/SetchOnLegs/00Blueprint/11Misc/BP_SaveInfo.BP_SaveInfo_C|SetCheckpoints _saveinfo (Variables|/Game/SetchOnLegs/00Blueprint/07Spike/BP_Spike.BP_Spike_C|GetCheckpoints _player)))
    (:then_5
      (Variables|/Game/SetchOnLegs/00Blueprint/11Misc/BP_SaveInfo.BP_SaveInfo_C|SetChargedShot _saveinfo (Variables|/Game/SetchOnLegs/00Blueprint/07Spike/BP_Spike.BP_Spike_C|GetChargedShot _player)))
    (:then_6
      (Variables|/Game/SetchOnLegs/00Blueprint/11Misc/BP_SaveInfo.BP_SaveInfo_C|Set3Bullet _saveinfo (Variables|/Game/SetchOnLegs/00Blueprint/07Spike/BP_Spike.BP_Spike_C|Get3Bullet _player)))
    (:then_7
      (Variables|/Game/SetchOnLegs/00Blueprint/11Misc/BP_SaveInfo.BP_SaveInfo_C|Set5Bullet _saveinfo (Variables|/Game/SetchOnLegs/00Blueprint/07Spike/BP_Spike.BP_Spike_C|Get5Bullet _player)))
    (:then_8
      (Variables|/Game/SetchOnLegs/00Blueprint/11Misc/BP_SaveInfo.BP_SaveInfo_C|SetMaxHealth _saveinfo (Variables|/Game/SetchOnLegs/00Blueprint/07Spike/BP_Spike.BP_Spike_C|GetMaxHealth _player)))
    (:then_9
      (Variables|/Game/SetchOnLegs/00Blueprint/11Misc/BP_SaveInfo.BP_SaveInfo_C|SetBulletDamage _saveinfo (Variables|/Game/SetchOnLegs/00Blueprint/07Spike/BP_Spike.BP_Spike_C|GetBulletDamage _player)))
    (:then_10
      (Variables|/Game/SetchOnLegs/00Blueprint/11Misc/BP_SaveInfo.BP_SaveInfo_C|SetChargedBulletDamage _saveinfo (Variables|/Game/SetchOnLegs/00Blueprint/07Spike/BP_Spike.BP_Spike_C|GetChargedShotDamage _player)))
    (:then_11
      (Variables|/Game/SetchOnLegs/00Blueprint/11Misc/BP_SaveInfo.BP_SaveInfo_C|SetChargedBulletCooldown _saveinfo (Variables|/Game/SetchOnLegs/00Blueprint/07Spike/BP_Spike.BP_Spike_C|GetChargedShotCooldown _player)))
    (:then_12
      (Variables|/Game/SetchOnLegs/00Blueprint/11Misc/BP_SaveInfo.BP_SaveInfo_C|SetCurrentHealth _saveinfo (Variables|/Game/SetchOnLegs/00Blueprint/07Spike/BP_Spike.BP_Spike_C|GetCurrentHealth _player)))
    (:then_14
      (bind _returnvalue (Game|GetCurrentLevelName true))
      (Variables|/Game/SetchOnLegs/00Blueprint/11Misc/BP_SaveInfo.BP_SaveInfo_C|SetLevelName (Variables|Default|GetSaveInfo) (Utilities|String|StringToName _returnvalue)))))

(event EventInteract
  ;[1 1 1] Interact to activate
  (bind _foundwidgets (Widget|GetAllWidgetsOfClass "/Game/SetchOnLegs/00Blueprint/11Misc/Widget_Saving.Widget_Saving_C" true))
  (Utilities|IsValid (Utilities|Array|Get(acopy) _foundwidgets)
    (:Is%20Not%20Valid
      (CallFunction|Activate))))

(fn ConstructionScript)
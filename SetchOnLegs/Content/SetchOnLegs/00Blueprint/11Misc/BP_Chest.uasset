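; BP_Chest is a shootable chest that opens when its randomized health runs out and launches a stream of pickups.
; Bullet overlaps subtract the player's bullet damage, and Tick fires a one-time open that swaps the sprite and runs a delayed spawn loop.
; Regular chests save their opened state by ID in the GameInstance and load inactive if already opened.
; Boss chests skip saving and spawn a typed ability after the pickups.
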(event OnComponentBeginOverlap(HitBox)
  (params (OverlappedComponent :type Primitive%20Component%20Object%20Reference) (OtherActor :type Actor%20Object%20Reference) (OtherComp :type Primitive%20Component%20Object%20Reference) (OtherBodyIndex :type Integer) (bFromSweep :type Boolean) (SweepResult :type Hit%20Result%20Structure%20%28by%20ref%29))
  ;[1 1 1] Bullet Collision
  (bind _asbp_bullet (Utilities|Casting|CastToBP_Bullet OtherActor))
  (Actor|DestroyActor _asbp_bullet)
  (Audio|PlaySound2D "/Game/SetchOnLegs/03Audio/08Misc/ChestHit.ChestHit" 1.0 1.0 0.0 0 0)
  (if (Variables|Default|GetActive)
    (bind _asbp_spike (Utilities|Casting|CastToBP_Spike (Game|GetPlayerCharacter 0)))
    (Variables|Default|SetCurrentHealth (- (Variables|Default|GetCurrentHealth) (Variables|/Game/SetchOnLegs/00Blueprint/07Spike/BP_Spike.BP_Spike_C|GetBulletDamage _asbp_spike)))))

(event Custom|SpawnPickups
  ;[1 1 1] Spawn pickups function
  (Utilities|ForLoopwithDelay 0 (- (Variables|Default|GetValue) 1) :!label _label
    (:Loop%20Body
      (Game|SpawnActorfromClass "/Game/SetchOnLegs/00Blueprint/11Misc/BP_MasterBall.BP_MasterBall_C" (Math|Transform|MakeTransform (Transformation|GetWorldLocation (Variables|Default|GetPickupSpawn)) "0, 0, 0" "1,1,1") "Undefined" 0 0)
      (Audio|PlaySound2D "/Game/SetchOnLegs/03Audio/08Misc/PickupLaunch.PickupLaunch" 1.0 1.0 0.0 0 0))
    (:Completed
      (if (Variables|Default|GetBossChest)
        (Utilities|FlowControl|Delay 1.0)
        (bind _returnvalue (Game|SpawnActorfromClass "/Game/SetchOnLegs/00Blueprint/11Misc/BP_Ability.BP_Ability_C" (Transformation|GetWorldTransform (Variables|Default|GetPickupSpawn)) "Undefined" 0 0))
        (Variables|/Game/SetchOnLegs/00Blueprint/11Misc/BP_Ability.BP_Ability_C|SetType _returnvalue (Variables|Default|GetAbilityType))))
    (:Delay%20Out
      (Utilities|FlowControl|Delay (Variables|Default|GetSpawnDelay))
      (goto _label Delay%20In))))

(event EventBeginPlay
  ;[1 1 1] Set chest health
  (Variables|Default|SetCurrentHealth (Math|Random|RandomFloatinRange (Variables|Default|GetHealthMin) (Variables|Default|GetHealthMax)))
  (bind _asbp_game_instance (Utilities|Casting|CastToBP_GameInstance (Game|GetGameInstance)))
  (bind _output_get (Variables|Default|SetGameInstance _asbp_game_instance))
  (for (_array_element _array_index) (Variables|/Game/SetchOnLegs/00Blueprint/11Misc/BP_GameInstance.BP_GameInstance_C|GetChestsOpened _output_get)
    (if (== _array_index (Variables|Default|GetID))
      (if _array_element
        (Rendering|Components|Sprite|SetSprite (Variables|Default|GetChest) "/Game/SetchOnLegs/01Sprites/10Misc/Chests/SilverChestOpen.SilverChestOpen")
        (Variables|Default|SetActive false)))))

(event EventTick
  (params (DeltaSeconds :type Float%20%28single-precision%29))
  ;[1 1 1] Open chest and spawn pickups
  (if (<= (Variables|Default|GetCurrentHealth) 0.0)
    (Utilities|FlowControl|DoOnce false
      (:Completed
        (Rendering|Components|Sprite|SetSprite (Variables|Default|GetChest) "/Game/SetchOnLegs/01Sprites/10Misc/Chests/SilverChestOpen.SilverChestOpen")
        (Audio|PlaySound2D "/Game/SetchOnLegs/03Audio/08Misc/ChestOpen.ChestOpen" 1.0 1.0 0.0 0 0)
        (CallFunction|SpawnPickups)
        (if (not (Variables|Default|GetBossChest))
          (Utilities|Array|SetArrayElem (Variables|/Game/SetchOnLegs/00Blueprint/11Misc/BP_GameInstance.BP_GameInstance_C|GetChestsOpened (Variables|Default|GetGameInstance)) (Variables|Default|GetID) true true))))))

(fn ConstructionScript)
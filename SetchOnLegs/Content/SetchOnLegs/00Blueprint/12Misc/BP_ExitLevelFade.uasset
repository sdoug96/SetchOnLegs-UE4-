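; Level exit trigger that takes over BP_Spike on overlap and sends the game to a configured level.
; Overlap disables input, shows the travelling widget, copies player stats, abilities and items plus the new spawn point into BP_GameInstance, then opens the level after a random delay.
; Meanwhile, if Move is set, Tick keeps Spike walking left or right, or climbing upward, according to the Left and Climb flags.
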(event OnComponentBeginOverlap(Box)
  (params (OverlappedComponent :type Primitive%20Component%20Object%20Reference) (OtherActor :type Actor%20Object%20Reference) (OtherComp :type Primitive%20Component%20Object%20Reference) (OtherBodyIndex :type Integer) (bFromSweep :type Boolean) (SweepResult :type Hit%20Result%20Structure%20%28by%20ref%29))
  ;[1 1 1] Exit Level Logic
  (bind _asbp_spike (Utilities|Casting|CastToBP_Spike OtherActor))
  (Variables|Default|SetPlayer _asbp_spike)
  (bind _asbp_game_instance (Utilities|Casting|CastToBP_GameInstance (Game|GetGameInstance)))
  (Variables|Default|SetGameInstance _asbp_game_instance)
  (Variables|Default|SetHit true)
  (Input|DisableInput (Variables|Default|GetPlayer) 0)
  (Sprite|SetFlipbook (Variables|/Script/Paper2D.PaperCharacter|GetSprite (Variables|Default|GetPlayer)) "/Game/SetchOnLegs/01Sprites/07Spike/Character/A_SpikeWalking.A_SpikeWalking")
  (Components|Timeline|SetPlayRate (Variables|/Script/Paper2D.PaperCharacter|GetSprite (Variables|Default|GetPlayer)) 1.0)
  (bind _returnvalue (UserInterface|CreateWidget "/Game/SetchOnLegs/00Blueprint/12Misc/Widget_Travelling.Widget_Travelling_C"))
  (UserInterface|Viewport|AddtoViewport _returnvalue 0)
  (Utilities|FlowControl|Sequence
    (:then_0
      (CallFunction|SetGameInstanceValues))
    (:then_1
      (Variables|/Game/SetchOnLegs/00Blueprint/12Misc/BP_GameInstance.BP_GameInstance_C|SetSpawnLocation (Variables|Default|GetGameInstance) (Variables|Default|GetNewSpawn)))
    (:then_2
      (Utilities|FlowControl|Delay (Math|Random|RandomFloatinRange 5.0 7.0))
      (Game|OpenLevel(byName) (Variables|Default|GetLevelToOpen)))))

(event Custom|SetGameInstanceValues
  ;[1 1 1] Set game instance values to players values
  (Utilities|FlowControl|Sequence
    (:then_0
      (CallFunction|SetMain))
    (:then_1
      (CallFunction|SetAbilities))
    (:then_2
      (CallFunction|SetMisc))))

(event Custom|SetMain
  (bind _player (Variables|Default|GetPlayer))
  (bind _gameinstance (Variables|Default|GetGameInstance))
  ;[1 1 1] Set Main Values
  (Utilities|FlowControl|Sequence
    (:then_0
      (Variables|/Game/SetchOnLegs/00Blueprint/12Misc/BP_GameInstance.BP_GameInstance_C|SetBadges _gameinstance (Variables|/Game/SetchOnLegs/00Blueprint/07Spike/BP_Spike.BP_Spike_C|GetBadges _player)))
    (:then_1
      (Variables|/Game/SetchOnLegs/00Blueprint/12Misc/BP_GameInstance.BP_GameInstance_C|SetMaxBadges _gameinstance (Variables|/Game/SetchOnLegs/00Blueprint/07Spike/BP_Spike.BP_Spike_C|GetMaxBadges _player)))
    (:then_2
      (Variables|/Game/SetchOnLegs/00Blueprint/12Misc/BP_GameInstance.BP_GameInstance_C|SetCurrency _gameinstance (Variables|/Game/SetchOnLegs/00Blueprint/07Spike/BP_Spike.BP_Spike_C|GetMasterBalls _player)))
    (:then_3
      (Variables|/Game/SetchOnLegs/00Blueprint/12Misc/BP_GameInstance.BP_GameInstance_C|SetDeathCount _gameinstance (Variables|/Game/SetchOnLegs/00Blueprint/07Spike/BP_Spike.BP_Spike_C|GetDeathCount _player)))))

(event Custom|SetMisc
  (bind _player (Variables|Default|GetPlayer))
  (bind _gameinstance (Variables|Default|GetGameInstance))
  ;[1 1 1] Set Misc
  (Utilities|FlowControl|Sequence
    (:then_0
      (Variables|/Game/SetchOnLegs/00Blueprint/12Misc/BP_GameInstance.BP_GameInstance_C|SetHasShooter _gameinstance (Variables|/Game/SetchOnLegs/00Blueprint/07Spike/BP_Spike.BP_Spike_C|GetHasShooter _player)))
    (:then_1
      (Variables|/Game/SetchOnLegs/00Blueprint/12Misc/BP_GameInstance.BP_GameInstance_C|SetShooter _gameinstance (Variables|/Game/SetchOnLegs/00Blueprint/07Spike/BP_Spike.BP_Spike_C|GetShooter _player)))
    (:then_2
      (Variables|/Game/SetchOnLegs/00Blueprint/12Misc/BP_GameInstance.BP_GameInstance_C|SetRelic _gameinstance (Variables|/Game/SetchOnLegs/00Blueprint/07Spike/BP_Spike.BP_Spike_C|GetRelic _player)))
    (:then_3
      (Variables|/Game/SetchOnLegs/00Blueprint/12Misc/BP_GameInstance.BP_GameInstance_C|SetShields _gameinstance (Variables|/Game/SetchOnLegs/00Blueprint/07Spike/BP_Spike.BP_Spike_C|GetShields _player)))
    (:then_4
      (Variables|/Game/SetchOnLegs/00Blueprint/12Misc/BP_GameInstance.BP_GameInstance_C|SetAntidotes _gameinstance (Variables|/Game/SetchOnLegs/00Blueprint/07Spike/BP_Spike.BP_Spike_C|GetAntidotes _player)))
    (:then_5
      (Variables|/Game/SetchOnLegs/00Blueprint/12Misc/BP_GameInstance.BP_GameInstance_C|SetPastorsSeal _gameinstance (Variables|/Game/SetchOnLegs/00Blueprint/07Spike/BP_Spike.BP_Spike_C|GetPastorsSeal _player)))
    (:then_6
      (Variables|/Game/SetchOnLegs/00Blueprint/12Misc/BP_GameInstance.BP_GameInstance_C|SetNightmareShards _gameinstance (Variables|/Game/SetchOnLegs/00Blueprint/07Spike/BP_Spike.BP_Spike_C|GetNightmareShards _player)))))

(event Custom|SetAbilities
  (bind _player (Variables|Default|GetPlayer))
  (bind _gameinstance (Variables|Default|GetGameInstance))
  ;[1 1 1] Set Abilities
  (Utilities|FlowControl|Sequence
    (:then_0
      (Variables|/Game/SetchOnLegs/00Blueprint/12Misc/BP_GameInstance.BP_GameInstance_C|SetDoubleJump _gameinstance (Variables|/Game/SetchOnLegs/00Blueprint/07Spike/BP_Spike.BP_Spike_C|GetDoubleJump _player)))
    (:then_1
      (Variables|/Game/SetchOnLegs/00Blueprint/12Misc/BP_GameInstance.BP_GameInstance_C|SetIllumination _gameinstance (Variables|/Game/SetchOnLegs/00Blueprint/07Spike/BP_Spike.BP_Spike_C|GetIllumination _player)))
    (:then_2
      (Variables|/Game/SetchOnLegs/00Blueprint/12Misc/BP_GameInstance.BP_GameInstance_C|SetDash _gameinstance (Variables|/Game/SetchOnLegs/00Blueprint/07Spike/BP_Spike.BP_Spike_C|GetDash _player)))
    (:then_3
      (Variables|/Game/SetchOnLegs/00Blueprint/12Misc/BP_GameInstance.BP_GameInstance_C|SetShadowDash _gameinstance (Variables|/Game/SetchOnLegs/00Blueprint/07Spike/BP_Spike.BP_Spike_C|GetShadowDash _player)))))

(event EventTick
  (params (DeltaSeconds :type Float%20%28single-precision%29))
  (bind _player (Variables|Default|GetPlayer))
  ;[1 1 1] Exit Level Logic
  ;;[1 1 1] Move Spike
  (if (Variables|Default|GetMove)
    (if (Variables|Default|GetHit)
      (if (Variables|Default|GetClimb)
        (Variables|/Game/SetchOnLegs/00Blueprint/07Spike/BP_Spike.BP_Spike_C|SetState _player "NewEnumerator7")
        (Default|UpdateAnimation _player)
        (Pawn|Input|AddMovementInput _player (Math|Vector|MakeVector 0.0 0.0 0.5) 1.0 false)
        (elif (Variables|Default|GetLeft)
          (Pawn|Input|AddMovementInput (Variables|Default|GetPlayer) (Math|Vector|MakeVector -1.0 0.0 0.0) 1.0 false)
          (else
            (Pawn|Input|AddMovementInput (Variables|Default|GetPlayer) (Math|Vector|MakeVector 1.0 0.0 0.0) 1.0 false)))))))

(fn ConstructionScript)
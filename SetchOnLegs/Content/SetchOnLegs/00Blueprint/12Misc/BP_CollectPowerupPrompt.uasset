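; BP_CollectPowerupPrompt is a trigger volume that shows a collect-powerup prompt widget when the player's BP_Spike enters it without the associated ability.
; An ID selects which ability it tracks: double jump, illumination or dash.
; Tick copies that flag from the player reference cached at BeginPlay into AbilityGained, which gates the Box overlap.
; Each qualifying overlap creates a new widget, and this Blueprint never removes it.
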(event OnComponentBeginOverlap(Box)
  (params (OverlappedComponent :type Primitive%20Component%20Object%20Reference) (OtherActor :type Actor%20Object%20Reference) (OtherComp :type Primitive%20Component%20Object%20Reference) (OtherBodyIndex :type Integer) (bFromSweep :type Boolean) (SweepResult :type Hit%20Result%20Structure%20%28by%20ref%29))
  (Utilities|Casting|CastToBP_Spike OtherActor)
  (if (not (Variables|Default|GetAbilityGained))
    (bind _returnvalue (UserInterface|CreateWidget "/Game/SetchOnLegs/00Blueprint/12Misc/Widgets/Widget_CollectPowerupPrompt.Widget_CollectPowerupPrompt_C"))
    (UserInterface|Viewport|AddtoViewport _returnvalue 0)))

(event EventBeginPlay
  (bind _asbp_spike (Utilities|Casting|CastToBP_Spike (Game|GetPlayerCharacter 0)))
  (Variables|Default|SetPlayer _asbp_spike))

(event EventTick
  (params (DeltaSeconds :type Float%20%28single-precision%29))
  (switch int (Variables|Default|GetID)
    (:0
      (Variables|Default|SetAbilityGained (Variables|/Game/SetchOnLegs/00Blueprint/07Spike/BP_Spike.BP_Spike_C|GetDoubleJump (Variables|Default|GetPlayer))))
    (:1
      (Variables|Default|SetAbilityGained (Variables|/Game/SetchOnLegs/00Blueprint/07Spike/BP_Spike.BP_Spike_C|GetIllumination (Variables|Default|GetPlayer))))
    (:2
      (Variables|Default|SetAbilityGained (Variables|/Game/SetchOnLegs/00Blueprint/07Spike/BP_Spike.BP_Spike_C|GetDash (Variables|Default|GetPlayer))))))

(fn ConstructionScript)
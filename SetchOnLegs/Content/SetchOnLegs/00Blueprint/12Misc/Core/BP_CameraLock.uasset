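; BP_CameraLock is a volume that locks the player camera along one axis while BP_Spike is inside it.
; Entering its box detaches Spike's camera boom, keeping its world transform.
; Each tick, lock type X follows only the player's height, while type Z follows only the player's X position.
; Leaving reattaches the boom to Spike's capsule and zeroes its relative location.
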(event OnComponentBeginOverlap(Box)
  (params (OverlappedComponent :type Primitive%20Component%20Object%20Reference) (OtherActor :type Actor%20Object%20Reference) (OtherComp :type Primitive%20Component%20Object%20Reference) (OtherBodyIndex :type Integer) (bFromSweep :type Boolean) (SweepResult :type Hit%20Result%20Structure%20%28by%20ref%29))
  (Utilities|Casting|CastToBP_Spike OtherActor)
  (if (Utilities|IsValid (Variables|Default|GetCamBoom))
    (Transformation|DetachFromComponent (Variables|Default|GetCamBoom) "KeepWorld" "KeepWorld" "KeepWorld" true)
    (Variables|Default|SetActive true)))

(event OnComponentEndOverlap(Box)
  (params (OverlappedComponent :type Primitive%20Component%20Object%20Reference) (OtherActor :type Actor%20Object%20Reference) (OtherComp :type Primitive%20Component%20Object%20Reference) (OtherBodyIndex :type Integer))
  (bind _asbp_spike (Utilities|Casting|CastToBP_Spike OtherActor))
  (Transformation|AttachComponentToComponent (Variables|Default|GetCamBoom) (Variables|/Script/Engine.Character|GetCapsuleComponent _asbp_spike) "None" "KeepWorld" "KeepWorld" "KeepWorld" true)
  (Transformation|SetRelativeLocation (Variables|Default|GetCamBoom) "0, 0, 0" false false)
  (Variables|Default|SetActive false))

(event EventBeginPlay
  (bind _asbp_spike (Utilities|Casting|CastToBP_Spike (Game|GetPlayerCharacter 0)))
  (bind _output_get (Variables|Default|SetPlayer _asbp_spike))
  (Variables|Default|SetCamBoom (Variables|/Game/SetchOnLegs/00Blueprint/07Spike/BP_Spike.BP_Spike_C|GetCameraBoom _output_get)))

(event EventTick
  (params (DeltaSeconds :type Float%20%28single-precision%29))
  (bind _camboom (Variables|Default|GetCamBoom))
  (bind _camboom_2 (Variables|Default|GetCamBoom))
  (bind _returnvalue (Transformation|GetWorldLocation _camboom))
  (bind _returnvalue_2 (Transformation|GetWorldLocation _camboom_2))
  (bind (_x _y _z) (Math|Vector|BreakVector _returnvalue))
  (bind (_x_2 _y_2) (Math|Vector|BreakVector _returnvalue_2))
  ;[1 1 1] Fix camera movement based on lock type
  (if (Variables|Default|GetActive)
    (switch Utilities|FlowControl|Switch|SwitchonCamLockType (Variables|Default|GetCamLockType)
      (:NewEnumerator0
        (Transformation|SetWorldLocation (Variables|Default|GetCamBoom) (Math|Vector|MakeVector _x_2 _y_2 (.Z (Math|Vector|BreakVector (Transformation|GetActorLocation (Variables|Default|GetPlayer))))) false false))
      (:NewEnumerator1
        (Transformation|SetWorldLocation (Variables|Default|GetCamBoom) (Math|Vector|MakeVector (.X (Math|Vector|BreakVector (Transformation|GetActorLocation (Variables|Default|GetPlayer)))) _y _z) false false)))))

(fn ConstructionScript)
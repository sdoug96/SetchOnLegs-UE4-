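; BP_BossGates is a movable gate actor, by its name for boss encounters, that slides between a start and an end position.
; On BeginPlay it snaps to the start position and caches the BP_Spike player character.
; CloseGates and OpenGates each play a timeline that lerps its location in opposite directions.
; Both events also play a rumble sound and a camera shake centred on the player's side-view camera.
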(event Custom|CloseGates
  (Camera|PlayWorldCameraShake "/Game/SetchOnLegs/00Blueprint/12Misc/Gate/BP_GateShake.BP_GateShake_C" (Transformation|GetWorldLocation (Variables|/Game/SetchOnLegs/00Blueprint/07Spike/BP_Spike.BP_Spike_C|GetSideViewCameraComponent (Variables|Default|GetPlayer))) 0.0 2e+02)
  (Audio|PlaySound2D "/Game/SetchOnLegs/03Audio/08Misc/GateRumble.GateRumble" 1.0 1.0 0.0 0 0)
  (bind _defaulttrack (Timeline|GateTimeline PlayFromStart)
    (:Update
      (Transformation|SetActorLocation (Math|Vector|Lerp(Vector) (Variables|Default|GetGatesStartPos) (Variables|Default|GetGatesEndPos) _defaulttrack) false false))))

(event Custom|OpenGates
  (Camera|PlayWorldCameraShake "/Game/SetchOnLegs/00Blueprint/12Misc/Gate/BP_GateShake.BP_GateShake_C" (Transformation|GetWorldLocation (Variables|/Game/SetchOnLegs/00Blueprint/07Spike/BP_Spike.BP_Spike_C|GetSideViewCameraComponent (Variables|Default|GetPlayer))) 0.0 2e+02)
  (Audio|PlaySound2D "/Game/SetchOnLegs/03Audio/08Misc/GateRumble.GateRumble" 1.0 1.0 0.0 0 0)
  (bind _defaulttrack (Timeline|Timeline_0 PlayFromStart)
    (:Update
      (Transformation|SetActorLocation (Math|Vector|Lerp(Vector) (Variables|Default|GetGatesEndPos) (Variables|Default|GetGatesStartPos) _defaulttrack) false false))))

(event EventBeginPlay
  (Transformation|SetActorLocation (Variables|Default|GetGatesStartPos) false false)
  (bind _asbp_spike (Utilities|Casting|CastToBP_Spike (Game|GetPlayerCharacter 0)))
  (Variables|Default|SetPlayer _asbp_spike))

(fn ConstructionScript)
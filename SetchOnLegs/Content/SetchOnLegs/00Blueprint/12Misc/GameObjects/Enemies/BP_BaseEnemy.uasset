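; Base enemy for a 2D side-view game, handling facing, player following, damage and death against the BP_Spike player.
; Exposed events turn the enemy toward Spike, optionally walk after him, exchange damage while active and alive, and flash the sprite red via a looping timer.
; Death stops movement, launches a random number of MasterBall pickups through a delayed loop, increments the GameInstance kill count, and optionally destroys the actor after a delay.
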(event Custom|FlashRed
  (bind _sprite (Variables|Default|GetSprite))
  ;[1 1 1] Damage & Death Logic
  (if (== (.g (Variables|/Script/Paper2D.PaperFlipbookComponent|GetSpriteColor (Variables|Default|GetSprite))) 1.0)
    (Sprite|SetSpriteColor _sprite "(R=1.000000,G=0.000000,B=0.000000,A=1.000000)")
    (else
      (Sprite|SetSpriteColor _sprite "(R=1.000000,G=1.000000,B=1.000000,A=1.000000)"))))

(event Custom|Death
  ;[1 1 1] Damage & Death Logic
  (Variables|Default|SetActive false)
  (Variables|Default|SetIsDead true)
  (Components|Movement|StopMovementImmediately (Variables|Character|GetCharacterMovement))
  (Variables|/Script/Engine.MovementComponent|SetVelocity (Variables|Character|GetCharacterMovement) "0, 0, 0")
  (CallFunction|SpawnMasterBalls)
  (Variables|/Game/SetchOnLegs/00Blueprint/12Misc/Core/BP_GameInstance.BP_GameInstance_C|SetEnemiesKilled (Variables|Default|GetGameInstance) (+ (Variables|/Game/SetchOnLegs/00Blueprint/12Misc/Core/BP_GameInstance.BP_GameInstance_C|GetEnemiesKilled (Variables|Default|GetGameInstance)) 1))
  (Utilities|FlowControl|Delay (Variables|Default|GetKillDelay))
  (if (Variables|Default|GetDestroyOnDeath)
    (Actor|DestroyActor)))

(event Custom|SetRotation
  ;[1 1 1] Set Enemy Rotation & Follow Movement
  (Variables|Default|SetIsRightOfPlayer (> (.x (Transformation|GetWorldLocation (Variables|Default|GetSprite))) (.x (Transformation|GetActorLocation (Variables|Default|GetPlayer)))))
  (Utilities|FlowControl|Sequence
    (:then_0
      (if (Variables|Default|GetIsRightOfPlayer)
        (Transformation|SetActorRotation "0,180.000000, 0")
        (else
          (Transformation|SetActorRotation "0, 0, 0"))))
    (:then_1
      (if (Variables|Default|GetFollowPlayer)
        (if (Variables|Default|GetIsRightOfPlayer)
          (Pawn|Input|AddMovementInput "-1.000000, 0, 0" 1.0 false)
          (else
            (Pawn|Input|AddMovementInput "1.000000, 0, 0" 1.0 false)))))))

(event Custom|PlayFlash
  ;[1 1 1] Damage & Death Logic
  (Utilities|Time|SetTimerbyFunctionName 0 "FlashRed" (Variables|Default|GetHitFlashSpeed) true)
  (Utilities|FlowControl|Delay (Variables|Default|GetHitFlashDuration))
  (Utilities|Time|ClearTimerbyFunctionName 0 "FlashRed")
  (Sprite|SetSpriteColor (Variables|Default|GetSprite) "(R=1.000000,G=1.000000,B=1.000000,A=1.000000)"))

(event Custom|SpawnMasterBalls
  (bind _sprite (Variables|Default|GetSprite))
  (bind _returnvalue (Transformation|GetWorldLocation _sprite))
  ;[1 1 1] Spawn pickups function
  (Utilities|ForLoopwithDelay 0 (Math|Random|RandomIntegerinRange (- (Variables|Default|GetMinMasterBallsToSpawn) 1) (- (Variables|Default|GetMaxMasterBallsToSpawn) 1)) :!label _label
    (:Loop%20Body
      (Game|SpawnActorfromClass "/Game/SetchOnLegs/00Blueprint/12Misc/GameObjects/Pickups/BP_MasterBall.BP_MasterBall_C" (Math|Transform|MakeTransform (Math|Vector|MakeVector (.x _returnvalue) 0.1 (.z _returnvalue)) "0, 0, 0" "1,1,1") "Undefined" 0 0)
      (Audio|PlaySound2D "/Game/SetchOnLegs/03Audio/08Misc/PickupLaunch.PickupLaunch" 1.0 1.0 0.0 0 0))
    (:Delay%20Out
      (Utilities|FlowControl|Delay 0.2)
      (goto _label Delay%20In))))

(event Custom|DamageSpike
  ;[1 1 1] Collision Logic
  (if (not (Variables|Default|GetIsDead))
    (if (Variables|Default|GetActive)
      (Default|DamageSystem (Variables|Default|GetPlayer) 1))))

(event Custom|DamageSystem
  (params (DamageIn :type Float%20%28single-precision%29))
  ;[1 1 1] Damage & Death Logic
  (bind _output_get (Variables|Default|SetCurrentHealth (- (Variables|Default|GetCurrentHealth) DamageIn)))
  (if (<= _output_get 0.0)
    (CallFunction|Death)
    (else
      (CallFunction|PlayFlash))))

(event Custom|BulletCollision
  ;[1 1 1] Collision Logic
  (if (not (Variables|Default|GetIsDead))
    (if (Variables|Default|GetActive)
      (CallFunction|DamageSystem (Variables|/Game/SetchOnLegs/00Blueprint/07Spike/BP_Spike.BP_Spike_C|GetBulletDamage (Variables|Default|GetPlayer))))))

(event EventBeginPlay
  ;[1 1 1] Find Player & Game Instance
  (bind _asbp_spike (Utilities|Casting|CastToBP_Spike (Game|GetPlayerCharacter 0)))
  (Variables|Default|SetPlayer _asbp_spike)
  (bind _asbp_game_instance (Utilities|Casting|CastToBP_GameInstance (Game|GetGameInstance)))
  (Variables|Default|SetGameInstance _asbp_game_instance))

(fn ConstructionScript)
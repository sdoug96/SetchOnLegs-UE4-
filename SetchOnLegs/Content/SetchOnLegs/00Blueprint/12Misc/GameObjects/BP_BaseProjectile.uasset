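; Base projectile actor that damages the player (BP_Spike) on contact and destroys itself after a set lifetime.
; Overlaps on either the sprite or flipbook hit sphere call DamagePlayer, which skips two player states, applies damage through DamageSystem and optionally destroys the projectile.
; The construction script sets initial and max movement speed from ProjectileSpeed, and Tick optionally spins the actor in pitch.
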(event OnComponentBeginOverlap(SpriteHitSphere)
  (params (OverlappedComponent :type Primitive%20Component%20Object%20Reference) (OtherActor :type Actor%20Object%20Reference) (OtherComp :type Primitive%20Component%20Object%20Reference) (OtherBodyIndex :type Integer) (bFromSweep :type Boolean) (SweepResult :type Hit%20Result%20Structure%20%28by%20ref%29))
  ;[1 1 1] Collision Logic
  (bind _asbp_spike (Utilities|Casting|CastToBP_Spike OtherActor))
  (CallFunction|DamagePlayer _asbp_spike))

(event OnComponentBeginOverlap(FlipbookHitSphere)
  (params (OverlappedComponent :type Primitive%20Component%20Object%20Reference) (OtherActor :type Actor%20Object%20Reference) (OtherComp :type Primitive%20Component%20Object%20Reference) (OtherBodyIndex :type Integer) (bFromSweep :type Boolean) (SweepResult :type Hit%20Result%20Structure%20%28by%20ref%29))
  ;[1 1 1] Collision Logic
  (bind _asbp_spike (Utilities|Casting|CastToBP_Spike OtherActor))
  (CallFunction|DamagePlayer _asbp_spike))

(event Custom|DamagePlayer
  (params (Player :type BP%20Spike%20Object%20Reference))
  ;[1 1 1] Damage Player
  (bind _output_get (Variables|Default|SetPlayer Player))
  (if (and (Utilities|Enum|NotEqual(Enum) (Variables|/Game/SetchOnLegs/00Blueprint/07Spike/BP_Spike.BP_Spike_C|GetState (Variables|Default|GetPlayer)) "NewEnumerator5") (Utilities|Enum|NotEqual(Enum) (Variables|/Game/SetchOnLegs/00Blueprint/07Spike/BP_Spike.BP_Spike_C|GetState (Variables|Default|GetPlayer)) "NewEnumerator14"))
    (Default|DamageSystem _output_get (Variables|Default|GetProjectileDamage))
    (if (Variables|Default|GetDestroyOnHit)
      (Actor|DestroyActor))))

(event EventBeginPlay
  ;[1 1 1] Destroy Self Logic
  (Utilities|FlowControl|Delay (Variables|Default|GetKillDelay))
  (Actor|DestroyActor))

(event EventTick
  (params (DeltaSeconds :type Float%20%28single-precision%29))
  ;[1 1 1] Rotation Logic
  (if (Variables|Default|GetRotate)
    (Variables|Default|SetTimer (+ DeltaSeconds (Variables|Default|GetTimer)))
    (Transformation|SetActorRotation (Math|Rotator|MakeRotator 0.0 (* (Variables|Default|GetTimer) (Variables|Default|GetRotationSpeed)) 0.0))))

(fn ConstructionScript
  (bind _output_get (Variables|/Script/Engine.ProjectileMovementComponent|SetInitialSpeed (Variables|Default|GetProjectileMovement) (Variables|Default|GetProjectileSpeed)))
  (Variables|/Script/Engine.ProjectileMovementComponent|SetMaxSpeed (Variables|Default|GetProjectileMovement) _output_get))
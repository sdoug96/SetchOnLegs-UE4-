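; BP_Ability is an ability pickup that grants Double Jump, Illumination, Dash or Shadow Dash, selected by its Type.
; On BeginPlay it plays a spawn sound, sets its sprite and popup widget from Type, and clears Move after a second to stop any upward drift driven in Tick.
; When BP_Spike overlaps outside one excluded state, it sets the player's ability flag, shows the widget, freezes the player's sprite animation and calls CollisionLogic.
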(event OnComponentBeginOverlap(SpriteHitSphere)
  (params (OverlappedComponent :type Primitive%20Component%20Object%20Reference) (OtherActor :type Actor%20Object%20Reference) (OtherComp :type Primitive%20Component%20Object%20Reference) (OtherBodyIndex :type Integer) (bFromSweep :type Boolean) (SweepResult :type Hit%20Result%20Structure%20%28by%20ref%29))
  ;[1 1 1] Collision Logic
  (bind _asbp_spike (Utilities|Casting|CastToBP_Spike OtherActor))
  (if (Utilities|Enum|NotEqual(Enum) (Variables|/Game/SetchOnLegs/00Blueprint/07Spike/BP_Spike.BP_Spike_C|GetState _asbp_spike) "NewEnumerator5")
    (CallFunction|AbilityLogic)
    (bind _returnvalue (UserInterface|CreateWidget (Variables|Default|GetWidgetToSpawn)))
    (UserInterface|Viewport|AddtoViewport _returnvalue 0)
    (Components|Timeline|SetPlayRate (Variables|/Script/Paper2D.PaperCharacter|GetSprite (Variables|Default|GetPlayer)) 0.0)
    (CallFunction|CollisionLogic)))

(event Custom|AbilityLogic
  ;[1 1 1] Logic based on ability type
  (switch Utilities|FlowControl|Switch|SwitchonAbilityType (Variables|Default|GetType)
    (:NewEnumerator2
      (Variables|/Game/SetchOnLegs/00Blueprint/07Spike/BP_Spike.BP_Spike_C|SetDoubleJump (Variables|Default|GetPlayer) true)
      (Variables|/Script/Engine.Character|SetJumpMaxCount (Variables|Default|GetPlayer) 2))
    (:NewEnumerator3
      (Variables|/Game/SetchOnLegs/00Blueprint/07Spike/BP_Spike.BP_Spike_C|SetIllumination (Variables|Default|GetPlayer) true))
    (:NewEnumerator4
      (Variables|/Game/SetchOnLegs/00Blueprint/07Spike/BP_Spike.BP_Spike_C|SetDash (Variables|Default|GetPlayer) true))
    (:NewEnumerator5
      (Variables|/Game/SetchOnLegs/00Blueprint/07Spike/BP_Spike.BP_Spike_C|SetShadowDash (Variables|Default|GetPlayer) true))))

(event Custom|DisplayAbilityWidget
  ;[1 1 1] Display Ability Widget & Sprite
  (switch Utilities|FlowControl|Switch|SwitchonAbilityType (Variables|Default|GetType)
    (:NewEnumerator2
      (Variables|Default|SetWidgetToSpawn "/Game/SetchOnLegs/00Blueprint/11Prompts/01Abilities/Widget_DoubleJump.Widget_DoubleJump_C")
      (Rendering|Components|Sprite|SetSprite (Variables|Default|GetSprite) "/Game/SetchOnLegs/01Sprites/11Misc/QuestItems/FlameOfTheUnderworld.FlameOfTheUnderworld"))
    (:NewEnumerator3
      (Variables|Default|SetWidgetToSpawn "/Game/SetchOnLegs/00Blueprint/11Prompts/01Abilities/Widget_Illumination.Widget_Illumination_C")
      (Rendering|Components|Sprite|SetSprite (Variables|Default|GetSprite) "/Game/SetchOnLegs/01Sprites/11Misc/QuestItems/JarOfGrease.JarOfGrease")
      (Transformation|SetRelativeScale3D (Variables|Default|GetSprite) "0.175000,0.175000,0.175000"))
    (:NewEnumerator4
      (Variables|Default|SetWidgetToSpawn "/Game/SetchOnLegs/00Blueprint/11Prompts/01Abilities/Widget_Dash.Widget_Dash_C")
      (Rendering|Components|Sprite|SetSprite (Variables|Default|GetSprite) "/Game/SetchOnLegs/01Sprites/11Misc/QuestItems/ButchersBloodVessel.ButchersBloodVessel")
      (Transformation|SetRelativeScale3D (Variables|Default|GetSprite) "0.600000,0.600000,0.600000"))
    (:NewEnumerator5
      (Variables|Default|SetWidgetToSpawn "/Game/SetchOnLegs/00Blueprint/11Prompts/01Abilities/Widget_ShadowDash.Widget_ShadowDash_C")
      (Rendering|Components|Sprite|SetSprite (Variables|Default|GetSprite) "/Game/SetchOnLegs/01Sprites/11Misc/QuestItems/PinkFedora.PinkFedora"))))

(event EventBeginPlay
  ;[1 1 1] Begin Play
  (|CallParentFunction)
  (Audio|PlaySound2D "/Game/SetchOnLegs/03Audio/08Misc/AbilitySpawn.AbilitySpawn" 1.0 1.0 0.0 0 0)
  (CallFunction|DisplayAbilityWidget)
  (Variables|Default|SetPickupSound "/Game/SetchOnLegs/03Audio/08Misc/AbilitySpawn.AbilitySpawn")
  (Utilities|FlowControl|Delay 1.0)
  (Variables|Default|SetMove false))

(event EventTick
  (params (DeltaSeconds :type Float%20%28single-precision%29))
  (bind _projectilemovement (Variables|Default|GetProjectileMovement))
  ;[1 1 1] Set velocity
  (if (Variables|Default|GetMove)
    (Variables|/Script/Engine.MovementComponent|SetVelocity _projectilemovement "0, 0,200.000000")
    (else
      (Variables|/Script/Engine.MovementComponent|SetVelocity _projectilemovement "0, 0, 0"))))

(fn ConstructionScript)
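; BP_Collectible is a sprite pickup that a BP_Spike collects on overlap, unless that actor is in one particular excluded state.
; Collection destroys the pickup, plays a sound, increments the game instance's collectible count and flags the current level's slot in its Collectibles array, chosen by GameState.
; The construction script sets the sprite, and BeginPlay shows or hides the point light based on IsLit.
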(event OnComponentBeginOverlap(HitSphere)
  (params (OverlappedComponent :type Primitive%20Component%20Object%20Reference) (OtherActor :type Actor%20Object%20Reference) (OtherComp :type Primitive%20Component%20Object%20Reference) (OtherBodyIndex :type Integer) (bFromSweep :type Boolean) (SweepResult :type Hit%20Result%20Structure%20%28by%20ref%29))
  ;[1 1 1] When hit
  (bind _asbp_spike (Utilities|Casting|CastToBP_Spike OtherActor))
  (if (Utilities|Enum|NotEqual(Enum) (Variables|/Game/SetchOnLegs/00Blueprint/07Spike/BP_Spike.BP_Spike_C|GetState _asbp_spike) "NewEnumerator5")
    (Actor|DestroyActor)
    (Audio|PlaySound2D (Variables|Default|GetPickupSound) 1.0 1.0 0.0 0 0)
    (CallFunction|SetCollectibles)))

(event Custom|SetCollectibles
  ;[1 1 1] Set collectibles for individual levels
  (bind _asbp_game_instance (Utilities|Casting|CastToBP_GameInstance (Game|GetGameInstance)))
  (Variables|/Game/SetchOnLegs/00Blueprint/12Misc/Core/BP_GameInstance.BP_GameInstance_C|SetCollectibleCount _asbp_game_instance (+ (Variables|/Game/SetchOnLegs/00Blueprint/12Misc/Core/BP_GameInstance.BP_GameInstance_C|GetCollectibleCount _asbp_game_instance) 1))
  (switch Utilities|FlowControl|Switch|SwitchonGameState (Variables|/Game/SetchOnLegs/00Blueprint/12Misc/Core/BP_GameInstance.BP_GameInstance_C|GetGameState _asbp_game_instance)
    (:NewEnumerator2
      (Utilities|Array|SetArrayElem (Variables|/Game/SetchOnLegs/00Blueprint/12Misc/Core/BP_GameInstance.BP_GameInstance_C|GetCollectibles _asbp_game_instance) 0 true true))
    (:NewEnumerator3
      (Utilities|Array|SetArrayElem (Variables|/Game/SetchOnLegs/00Blueprint/12Misc/Core/BP_GameInstance.BP_GameInstance_C|GetCollectibles _asbp_game_instance) 1 true true))
    (:NewEnumerator4
      (Utilities|Array|SetArrayElem (Variables|/Game/SetchOnLegs/00Blueprint/12Misc/Core/BP_GameInstance.BP_GameInstance_C|GetCollectibles _asbp_game_instance) 2 true true))
    (:NewEnumerator5
      (Utilities|Array|SetArrayElem (Variables|/Game/SetchOnLegs/00Blueprint/12Misc/Core/BP_GameInstance.BP_GameInstance_C|GetCollectibles _asbp_game_instance) 3 true true))
    (:NewEnumerator8
      (Utilities|Array|SetArrayElem (Variables|/Game/SetchOnLegs/00Blueprint/12Misc/Core/BP_GameInstance.BP_GameInstance_C|GetCollectibles _asbp_game_instance) 4 true true))
    (:NewEnumerator6
      (Utilities|Array|SetArrayElem (Variables|/Game/SetchOnLegs/00Blueprint/12Misc/Core/BP_GameInstance.BP_GameInstance_C|GetCollectibles _asbp_game_instance) 5 true true))))

(event EventBeginPlay
  ;[1 1 1] Set Light
  (Rendering|SetVisibility (Variables|Default|GetPointLight) (Variables|Default|GetIsLit) false))

(fn ConstructionScript
  (Rendering|Components|Sprite|SetSprite (Variables|Default|GetPickup) (Variables|Default|GetNewSprite)))
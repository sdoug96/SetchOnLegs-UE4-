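; Checkpoint actor that saves progress and refills the player's health when BP_Spike overlaps its hit box.
; Activation switches off every checkpoint's lights, lights its own, plays a sound and shows a saving widget, whose visibility blocks re-triggering.
; Each save writes a new BP_SaveInfo to one slot, copying player stats, abilities, items and level name.
; An offset spawn point at Y=0 goes to both the save and BP_GameInstance.
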(event OnComponentBeginOverlap(HitBox)
  (params (OverlappedComponent :type Primitive%20Component%20Object%20Reference) (OtherActor :type Actor%20Object%20Reference) (OtherComp :type Primitive%20Component%20Object%20Reference) (OtherBodyIndex :type Integer) (bFromSweep :type Boolean) (SweepResult :type Hit%20Result%20Structure%20%28by%20ref%29))
  ;[1 1 1] Show and hide save game
  (bind _asbp_spike (Utilities|Casting|CastToBP_Spike OtherActor))
  (Variables|Default|SetPlayer _asbp_spike)
  (bind _asbp_game_instance (Utilities|Casting|CastToBP_GameInstance (Game|GetGameInstance)))
  (Variables|Default|SetGameInstance _asbp_game_instance)
  (CallFunction|Activate))

(event Custom|SetMain
  (bind _player (Variables|Default|GetPlayer))
  (bind _saveinfo (Variables|Default|GetSaveInfo))
  ;[1 1 1] Set Main Values
  (Utilities|FlowControl|Sequence
    (:then_0
      (Variables|/Game/SetchOnLegs/00Blueprint/12Misc/Core/BP_SaveInfo.BP_SaveInfo_C|SetBadges _saveinfo (Variables|/Game/SetchOnLegs/00Blueprint/07Spike/BP_Spike.BP_Spike_C|GetBadges _player)))
    (:then_1
      (Variables|/Game/SetchOnLegs/00Blueprint/12Misc/Core/BP_SaveInfo.BP_SaveInfo_C|SetMaxBadges _saveinfo (Variables|/Game/SetchOnLegs/00Blueprint/07Spike/BP_Spike.BP_Spike_C|GetMaxBadges _player)))
    (:then_2
      (Variables|/Game/SetchOnLegs/00Blueprint/12Misc/Core/BP_SaveInfo.BP_SaveInfo_C|SetMasterBalls _saveinfo (Variables|/Game/SetchOnLegs/00Blueprint/07Spike/BP_Spike.BP_Spike_C|GetMasterBalls _player)))
    (:then_3
      (Variables|/Game/SetchOnLegs/00Blueprint/12Misc/Core/BP_SaveInfo.BP_SaveInfo_C|SetDeaths _saveinfo (Variables|/Game/SetchOnLegs/00Blueprint/07Spike/BP_Spike.BP_Spike_C|GetDeathCount _player)))))

(event Custom|Activate
  ;[1 1 1] Activate this checkpoint
  (Utilities|IsValid (Variables|Default|GetSavingWidget)
    (:Is%20Valid
      (if (not (Widget|IsVisible (Variables|Default|GetSavingWidget)))
        (if (Variables|/Script/Engine.SceneComponent|GetbVisible (Variables|Default|GetMiddleLight))
          _
          (else
            (bind _outactors (Actor|GetAllActorsOfClass "BP_Checkpoint_C" :!label _label))
            (for _array_element _outactors
              (Rendering|SetVisibility (Variables|BP_Checkpoint_C|GetMiddleLight _array_element) false false))
            (Rendering|ToggleVisibility (Variables|Default|GetMiddleLight) false)))
        (Audio|PlaySound2D "/Game/SetchOnLegs/03Audio/08Misc/Checkpoint.Checkpoint" 1.0 1.0 0.0 0 0)
        (Default|RefillHealth (Variables|Default|GetPlayer))
        (Default|ResetHealthSound (Variables|Default|GetPlayer))
        (CallFunction|SaveGame)
        (bind _returnvalue (UserInterface|CreateWidget "/Game/SetchOnLegs/00Blueprint/12Misc/Widgets/Widget_Saving.Widget_Saving_C"))
        (bind _output_get (Variables|Default|SetSavingWidget _returnvalue))
        (UserInterface|Viewport|AddtoViewport _output_get 0)))
    (:Is%20Not%20Valid
      (goto _label))))

(event Custom|SetMisc
  (bind _player (Variables|Default|GetPlayer))
  (bind _saveinfo (Variables|Default|GetSaveInfo))
  ;[1 1 1] Set Misc
  (Utilities|FlowControl|Sequence
    (:then_0
      (Variables|/Game/SetchOnLegs/00Blueprint/12Misc/Core/BP_SaveInfo.BP_SaveInfo_C|SetHasShooter _saveinfo (Variables|/Game/SetchOnLegs/00Blueprint/07Spike/BP_Spike.BP_Spike_C|GetHasShooter _player)))
    (:then_1
      (Variables|/Game/SetchOnLegs/00Blueprint/12Misc/Core/BP_SaveInfo.BP_SaveInfo_C|SetKeys _saveinfo (Variables|/Game/SetchOnLegs/00Blueprint/07Spike/BP_Spike.BP_Spike_C|GetKeys _player)))
    (:then_2
      (Variables|/Game/SetchOnLegs/00Blueprint/12Misc/Core/BP_SaveInfo.BP_SaveInfo_C|SetShields _saveinfo (Variables|/Game/SetchOnLegs/00Blueprint/07Spike/BP_Spike.BP_Spike_C|GetShields _player)))
    (:then_3
      (Variables|/Game/SetchOnLegs/00Blueprint/12Misc/Core/BP_SaveInfo.BP_SaveInfo_C|SetAntidotes _saveinfo (Variables|/Game/SetchOnLegs/00Blueprint/07Spike/BP_Spike.BP_Spike_C|GetAntidotes _player)))
    (:then_4
      (Variables|/Game/SetchOnLegs/00Blueprint/12Misc/Core/BP_SaveInfo.BP_SaveInfo_C|SetSuperSpike _saveinfo (Variables|/Game/SetchOnLegs/00Blueprint/07Spike/BP_Spike.BP_Spike_C|GetSuperSpike _player)))
    (:then_5
      (Variables|/Game/SetchOnLegs/00Blueprint/12Misc/Core/BP_SaveInfo.BP_SaveInfo_C|SetPastorsSeal _saveinfo (Variables|/Game/SetchOnLegs/00Blueprint/07Spike/BP_Spike.BP_Spike_C|GetPastorsSeal _player)))
    (:then_6
      (Variables|/Game/SetchOnLegs/00Blueprint/12Misc/Core/BP_SaveInfo.BP_SaveInfo_C|SetSecondBossItems _saveinfo (Variables|/Game/SetchOnLegs/00Blueprint/07Spike/BP_Spike.BP_Spike_C|GetSecondBossItems _player)))))

(event Custom|SetAbilities
  (bind _player (Variables|Default|GetPlayer))
  (bind _saveinfo (Variables|Default|GetSaveInfo))
  ;[1 1 1] Set Abilities
  (Utilities|FlowControl|Sequence
    (:then_0
      (Variables|/Game/SetchOnLegs/00Blueprint/12Misc/Core/BP_SaveInfo.BP_SaveInfo_C|SetDoubleJump _saveinfo (Variables|/Game/SetchOnLegs/00Blueprint/07Spike/BP_Spike.BP_Spike_C|GetDoubleJump _player)))
    (:then_1
      (Variables|/Game/SetchOnLegs/00Blueprint/12Misc/Core/BP_SaveInfo.BP_SaveInfo_C|SetIllumination _saveinfo (Variables|/Game/SetchOnLegs/00Blueprint/07Spike/BP_Spike.BP_Spike_C|GetIllumination _player)))
    (:then_2
      (Variables|/Game/SetchOnLegs/00Blueprint/12Misc/Core/BP_SaveInfo.BP_SaveInfo_C|SetDash _saveinfo (Variables|/Game/SetchOnLegs/00Blueprint/07Spike/BP_Spike.BP_Spike_C|GetDash _player)))
    (:then_3
      (Variables|/Game/SetchOnLegs/00Blueprint/12Misc/Core/BP_SaveInfo.BP_SaveInfo_C|SetShadowDash _saveinfo (Variables|/Game/SetchOnLegs/00Blueprint/07Spike/BP_Spike.BP_Spike_C|GetShadowDash _player)))
    (:then_4
      (Variables|/Game/SetchOnLegs/00Blueprint/12Misc/Core/BP_SaveInfo.BP_SaveInfo_C|SetMegaJump _saveinfo (Variables|/Game/SetchOnLegs/00Blueprint/07Spike/BP_Spike.BP_Spike_C|GetMegaJump _player)))))

(event Custom|SetSaveLocation
  (bind _returnvalue (Transformation|GetActorLocation))
  (bind _returnvalue_2 (- (.z _returnvalue) 1.4e+02))
  (bind _returnvalue_3 (+ (.x _returnvalue) 75.0))
  ;[1 1 1] Set spawn location
  (Variables|/Game/SetchOnLegs/00Blueprint/12Misc/Core/BP_SaveInfo.BP_SaveInfo_C|SetSpawnLocation (Variables|Default|GetSaveInfo) (Math|Vector|MakeVector _returnvalue_3 0.0 _returnvalue_2))
  (Variables|/Game/SetchOnLegs/00Blueprint/12Misc/Core/BP_GameInstance.BP_GameInstance_C|SetSpawnLocation (Variables|Default|GetGameInstance) (Math|Vector|MakeVector _returnvalue_3 0.0 _returnvalue_2)))

(event Custom|SaveGame
  ;[1 1 1] Save Game
  (bind _returnvalue (SaveGame|CreateSaveGameObject "/Game/SetchOnLegs/00Blueprint/12Misc/Core/BP_SaveInfo.BP_SaveInfo_C"))
  (Variables|Default|SetSaveInfo _returnvalue)
  (CallFunction|SetSaveLocation)
  (CallFunction|SetSaveValues)
  (SaveGame|SaveGametoSlot (Variables|Default|GetSaveInfo) "SaveInfo"))

(event Custom|SetSaveValues
  ;[1 1 1] Set Save Values
  (Utilities|FlowControl|Sequence
    (:then_0
      (CallFunction|SetMain))
    (:then_1
      (CallFunction|SetShooter))
    (:then_2
      (CallFunction|SetAbilities))
    (:then_3
      (CallFunction|SetMisc))
    (:then_4
      (bind _returnvalue (Game|GetCurrentLevelName true))
      (Variables|/Game/SetchOnLegs/00Blueprint/12Misc/Core/BP_SaveInfo.BP_SaveInfo_C|SetCurrentLevelName (Variables|Default|GetSaveInfo) (Utilities|String|StringToName _returnvalue)))))

(event Custom|SetShooter
  (bind _player (Variables|Default|GetPlayer))
  (bind _saveinfo (Variables|Default|GetSaveInfo))
  ;[1 1 1] Set shooter values
  (Utilities|FlowControl|Sequence
    (:then_0
      (Variables|/Game/SetchOnLegs/00Blueprint/12Misc/Core/BP_SaveInfo.BP_SaveInfo_C|SetBulletDamage _saveinfo (Variables|/Game/SetchOnLegs/00Blueprint/07Spike/BP_Spike.BP_Spike_C|GetBulletDamage _player)))
    (:then_1
      (Variables|/Game/SetchOnLegs/00Blueprint/12Misc/Core/BP_SaveInfo.BP_SaveInfo_C|SetBulletSpeed _saveinfo (Variables|/Game/SetchOnLegs/00Blueprint/07Spike/BP_Spike.BP_Spike_C|GetBulletSpeed _player)))
    (:then_2
      (Variables|/Game/SetchOnLegs/00Blueprint/12Misc/Core/BP_SaveInfo.BP_SaveInfo_C|SetRateOfFire _saveinfo (Variables|/Game/SetchOnLegs/00Blueprint/07Spike/BP_Spike.BP_Spike_C|GetRateOfFire _player)))
    (:then_3
      (Variables|/Game/SetchOnLegs/00Blueprint/12Misc/Core/BP_SaveInfo.BP_SaveInfo_C|SetBulletRange _saveinfo (Variables|/Game/SetchOnLegs/00Blueprint/07Spike/BP_Spike.BP_Spike_C|GetBulletRange _player)))))

(fn ConstructionScript)
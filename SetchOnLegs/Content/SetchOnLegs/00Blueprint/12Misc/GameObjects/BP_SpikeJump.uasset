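; BP_SpikeJump is a bounce pad that launches a falling BP_Spike player and then raises its spikes as a trap.
; BeginPlay caches the player and sets the point light's visibility from IsLit.
; A box overlap, skipped in one player state, overrides velocity with LaunchSpeed, plays a sound, and sets jump count, state and sprite animation.
; After a short delay, SetSpikeTrap moves the middle spikes with a sound, with no reset.
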(event OnComponentBeginOverlap(Box)
  (params (OverlappedComponent :type Primitive%20Component%20Object%20Reference) (OtherActor :type Actor%20Object%20Reference) (OtherComp :type Primitive%20Component%20Object%20Reference) (OtherBodyIndex :type Integer) (bFromSweep :type Boolean) (SweepResult :type Hit%20Result%20Structure%20%28by%20ref%29))
  (bind _player (Variables|Default|GetPlayer))
  (bind _asbp_spike (Utilities|Casting|CastToBP_Spike OtherActor))
  (if (Utilities|Enum|NotEqual(Enum) (Variables|/Game/SetchOnLegs/00Blueprint/07Spike/BP_Spike.BP_Spike_C|GetState _asbp_spike) "NewEnumerator5")
    (if (AI|Components|NavMovement|IsFalling (Variables|/Script/Engine.Character|GetCharacterMovement (Variables|Default|GetPlayer)))
      (Character|LaunchCharacter (Variables|Default|GetPlayer) (Variables|Default|GetLaunchSpeed) true true)
      (Audio|PlaySound2D "/Game/SetchOnLegs/03Audio/08Misc/OneBouncepad.OneBouncepad" 1.0 1.0 0.0 0 0)
      (Variables|/Game/SetchOnLegs/00Blueprint/07Spike/BP_Spike.BP_Spike_C|SetJumpCount (Variables|Default|GetPlayer) 1)
      (Variables|/Game/SetchOnLegs/00Blueprint/07Spike/BP_Spike.BP_Spike_C|SetState _player "NewEnumerator13")
      (Components|Timeline|SetPlaybackPosition (Variables|/Script/Paper2D.PaperCharacter|GetSprite _player) 0.0 false)
      (Default|UpdateAnimation (Variables|Default|GetPlayer))
      (Utilities|FlowControl|Delay 0.5)
      (CallFunction|SetSpikeTrap))))

(event Custom|SetSpikeTrap
  (Transformation|SetRelativeLocation (Variables|Default|GetSpikesMiddle) "1.000000,-0.100000,19.000000" false false)
  (Audio|PlaySound2D "/Game/SetchOnLegs/03Audio/06Rosemarkie/SpikesUp.SpikesUp" 1.0 1.0 0.0 0 0))

(event EventBeginPlay
  (bind _pointlight (Variables|Default|GetPointLight))
  (bind _asbp_spike (Utilities|Casting|CastToBP_Spike (Game|GetPlayerCharacter 0)))
  (Variables|Default|SetPlayer _asbp_spike)
  (if (Variables|Default|GetIsLit)
    (Rendering|SetVisibility _pointlight true false)
    (else
      (Rendering|SetVisibility _pointlight false false))))

(fn ConstructionScript)
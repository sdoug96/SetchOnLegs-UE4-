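; BP_FallTrap is a fall hazard that damages the BP_Spike player and returns them to a respawn point.
; On box overlap, it applies one point of damage unless the player is in one exempt state.
; A surviving player gets a fade widget and frozen movement, then after a short delay teleports to SpawnLocation.
; Walking, state, animation and jump count are then reset.
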(event OnComponentBeginOverlap(Box)
  (params (OverlappedComponent :type Primitive%20Component%20Object%20Reference) (OtherActor :type Actor%20Object%20Reference) (OtherComp :type Primitive%20Component%20Object%20Reference) (OtherBodyIndex :type Integer) (bFromSweep :type Boolean) (SweepResult :type Hit%20Result%20Structure%20%28by%20ref%29))
  (bind _asbp_spike (Utilities|Casting|CastToBP_Spike OtherActor))
  (bind _output_get (Variables|Default|SetPlayer _asbp_spike))
  (if (Utilities|Enum|NotEqual(Enum) (Variables|/Game/SetchOnLegs/00Blueprint/07Spike/BP_Spike.BP_Spike_C|GetState _output_get) "NewEnumerator5")
    (Default|DamageSystem (Variables|Default|GetPlayer) 1)
    (if (not (Variables|/Game/SetchOnLegs/00Blueprint/07Spike/BP_Spike.BP_Spike_C|GetIsDead (Variables|Default|GetPlayer)))
      (bind _returnvalue (UserInterface|CreateWidget "/Game/SetchOnLegs/00Blueprint/12Misc/Fades/Widget_FallTrapFade.Widget_FallTrapFade_C"))
      (UserInterface|Viewport|AddtoViewport _returnvalue 0)
      (Pawn|Components|CharacterMovement|DisableMovement (Variables|/Script/Engine.Character|GetCharacterMovement (Variables|Default|GetPlayer)))
      (Utilities|FlowControl|Delay 1.0)
      (Transformation|SetActorLocation (Variables|Default|GetPlayer) (Variables|Default|GetSpawnLocation) false false)
      (Pawn|Components|CharacterMovement|SetMovementMode (Variables|/Script/Engine.Character|GetCharacterMovement (Variables|Default|GetPlayer)) "MOVE_Walking" 0)
      (Variables|/Game/SetchOnLegs/00Blueprint/07Spike/BP_Spike.BP_Spike_C|SetState (Variables|Default|GetPlayer) "NewEnumerator0")
      (Default|UpdateAnimation (Variables|Default|GetPlayer))
      (Variables|/Game/SetchOnLegs/00Blueprint/07Spike/BP_Spike.BP_Spike_C|SetJumpCount (Variables|Default|GetPlayer) 0))))

(fn ConstructionScript)
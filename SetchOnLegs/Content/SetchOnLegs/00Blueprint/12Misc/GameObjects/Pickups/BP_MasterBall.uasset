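; BP_MasterBall is a Master Ball pickup that BP_Spike collects by overlapping its hit sphere.
; On BeginPlay it runs parent logic, pops upward with a randomized left or right impulse under gravity, and picks one of two pickup sounds.
; Unless Spike is in one excluded state, overlap adds Value to the player's count and the GameInstance total, then calls CollisionLogic.
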(event OnComponentBeginOverlap(SpriteHitSphere)
  (params (OverlappedComponent :type Primitive%20Component%20Object%20Reference) (OtherActor :type Actor%20Object%20Reference) (OtherComp :type Primitive%20Component%20Object%20Reference) (OtherBodyIndex :type Integer) (bFromSweep :type Boolean) (SweepResult :type Hit%20Result%20Structure%20%28by%20ref%29))
  ;[1 1 1] Collision Logic
  (bind _asbp_spike (Utilities|Casting|CastToBP_Spike OtherActor))
  (if (Utilities|Enum|NotEqual(Enum) (Variables|/Game/SetchOnLegs/00Blueprint/07Spike/BP_Spike.BP_Spike_C|GetState _asbp_spike) "NewEnumerator5")
    (Variables|/Game/SetchOnLegs/00Blueprint/07Spike/BP_Spike.BP_Spike_C|SetMasterBalls (Variables|Default|GetPlayer) (+ (Variables|/Game/SetchOnLegs/00Blueprint/07Spike/BP_Spike.BP_Spike_C|GetMasterBalls (Variables|Default|GetPlayer)) (Variables|Default|GetValue)))
    (CallFunction|SetMasterBalls)
    (CallFunction|CollisionLogic)))

(event Custom|SetMasterBalls
  ;[1 1 1] Add to total master balls
  (Variables|/Game/SetchOnLegs/00Blueprint/12Misc/Core/BP_GameInstance.BP_GameInstance_C|SetTotalMasterBalls (Variables|Default|GetGameInstance) (+ (Variables|/Game/SetchOnLegs/00Blueprint/12Misc/Core/BP_GameInstance.BP_GameInstance_C|GetTotalMasterBalls (Variables|Default|GetGameInstance)) (Variables|Default|GetValue))))

(event Custom|SetImpulse
  (bind _returnvalue (Math|Random|RandomFloatinRange 5e+02 7.5e+02))
  ;[1 1 1] Set Impulse of Master Ball
  (Variables|/Script/Engine.ProjectileMovementComponent|SetProjectileGravityScale (Variables|Default|GetProjectileMovement) 1.0)
  (if (== (Math|Random|RandomInteger 2) 0)
    (Physics|AddImpulse (Variables|Default|GetSprite) (Math|Vector|MakeVector (Math|Random|RandomFloatinRange -3e+02 -2e+02) 0.0 _returnvalue) "None" true)
    (else
      (Physics|AddImpulse (Variables|Default|GetSprite) (Math|Vector|MakeVector (Math|Random|RandomFloatinRange 2e+02 3e+02) 0.0 _returnvalue) "None" true))))

(event EventBeginPlay
  ;[1 1 1] Begin Play
  (|CallParentFunction)
  (CallFunction|SetImpulse)
  (switch int (Math|Random|RandomIntegerinRange 0 1)
    (:0
      (Variables|Default|SetPickupSound "/Game/SetchOnLegs/03Audio/08Misc/Pickup1.Pickup1"))
    (:1
      (Variables|Default|SetPickupSound "/Game/SetchOnLegs/03Audio/08Misc/Pickup2.Pickup2"))))

(fn ConstructionScript)
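; BP_BasePickup is a base pickup that plays a sound and destroys itself when BP_Spike, the player character, overlaps it.
; On BeginPlay it caches the player and BP_GameInstance references, though this graph does not use them further.
; Separate sprite and flipbook hit spheres both filter overlaps by a BP_Spike cast and feed the shared CollisionLogic event.
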(event OnComponentBeginOverlap(SpriteHitSphere)
  (params (OverlappedComponent :type Primitive%20Component%20Object%20Reference) (OtherActor :type Actor%20Object%20Reference) (OtherComp :type Primitive%20Component%20Object%20Reference) (OtherBodyIndex :type Integer) (bFromSweep :type Boolean) (SweepResult :type Hit%20Result%20Structure%20%28by%20ref%29))
  ;[1 1 1] Collision Logic
  (Utilities|Casting|CastToBP_Spike OtherActor)
  (CallFunction|CollisionLogic))

(event OnComponentBeginOverlap(FlipbookHitSphere)
  (params (OverlappedComponent :type Primitive%20Component%20Object%20Reference) (OtherActor :type Actor%20Object%20Reference) (OtherComp :type Primitive%20Component%20Object%20Reference) (OtherBodyIndex :type Integer) (bFromSweep :type Boolean) (SweepResult :type Hit%20Result%20Structure%20%28by%20ref%29))
  ;[1 1 1] Collision Logic
  (Utilities|Casting|CastToBP_Spike OtherActor)
  (CallFunction|CollisionLogic))

(event Custom|CollisionLogic
  ;[1 1 1] Collision Logic
  (Audio|PlaySound2D (Variables|Default|GetPickupSound) 1.0 1.0 0.0 0 0)
  (Actor|DestroyActor))

(event EventBeginPlay
  ;[1 1 1] Find Player & Game Instance
  (bind _asbp_spike (Utilities|Casting|CastToBP_Spike (Game|GetPlayerCharacter 0)))
  (Variables|Default|SetPlayer _asbp_spike)
  (bind _asbp_game_instance (Utilities|Casting|CastToBP_GameInstance (Game|GetGameInstance)))
  (Variables|Default|SetGameInstance _asbp_game_instance))

(fn ConstructionScript)
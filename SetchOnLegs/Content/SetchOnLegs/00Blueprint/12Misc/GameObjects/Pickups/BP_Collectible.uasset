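; BP_Collectible is a pickup that records its collection in the GameInstance when BP_Spike touches it.
; On HitSphere overlap, it ignores BP_Spike in one specific state, otherwise increments the collectible count and flags its CollectibleID in the CollectibleIDs array.
; It then calls CollisionLogic, which is defined outside this file.
; BeginPlay runs the parent logic and shows or hides the point light according to IsLit.
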(event OnComponentBeginOverlap(HitSphere)
  (params (OverlappedComponent :type Primitive%20Component%20Object%20Reference) (OtherActor :type Actor%20Object%20Reference) (OtherComp :type Primitive%20Component%20Object%20Reference) (OtherBodyIndex :type Integer) (bFromSweep :type Boolean) (SweepResult :type Hit%20Result%20Structure%20%28by%20ref%29))
  ;[1 1 1] Collision Logic
  (bind _asbp_spike (Utilities|Casting|CastToBP_Spike OtherActor))
  (if (Utilities|Enum|NotEqual(Enum) (Variables|/Game/SetchOnLegs/00Blueprint/07Spike/BP_Spike.BP_Spike_C|GetState _asbp_spike) "NewEnumerator5")
    (CallFunction|SetCollectibles)
    (CallFunction|CollisionLogic)))

(event Custom|SetCollectibles
  ;[1 1 1] Set Level Collectible to Collected Based on Collectible ID
  (Variables|/Game/SetchOnLegs/00Blueprint/12Misc/Core/BP_GameInstance.BP_GameInstance_C|SetCollectibleCount (Variables|Default|GetGameInstance) (+ (Variables|/Game/SetchOnLegs/00Blueprint/12Misc/Core/BP_GameInstance.BP_GameInstance_C|GetCollectibleCount (Variables|Default|GetGameInstance)) 1))
  (Utilities|Array|SetArrayElem (Variables|/Game/SetchOnLegs/00Blueprint/12Misc/Core/BP_GameInstance.BP_GameInstance_C|GetCollectibleIDs (Variables|Default|GetGameInstance)) (Variables|Default|GetCollectibleID) true true))

(event EventBeginPlay
  ;[1 1 1] Begin Play
  (|CallParentFunction)
  (Rendering|SetVisibility (Variables|Default|GetPointLight) (Variables|Default|GetIsLit) false))

(fn ConstructionScript)
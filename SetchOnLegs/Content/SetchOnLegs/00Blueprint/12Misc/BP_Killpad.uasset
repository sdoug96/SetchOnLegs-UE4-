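; BP_Killpad is a moving, optionally spinning actor, apparently meant as a spike hazard, though its Box overlap event contains no damage logic.
; On BeginPlay, a timeline lerps it from its start location to an X/Z offset, flipping TimeFactor on each finish to ping-pong indefinitely.
; When Rotator is set, Tick sets an absolute pitch from accumulated time multiplied by Rotation, zeroing roll and yaw.
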(event OnComponentBeginOverlap(Box)
  (params (OverlappedComponent :type Primitive%20Component%20Object%20Reference) (OtherActor :type Actor%20Object%20Reference) (OtherComp :type Primitive%20Component%20Object%20Reference) (OtherBodyIndex :type Integer) (bFromSweep :type Boolean) (SweepResult :type Hit%20Result%20Structure%20%28by%20ref%29))
  ;[1 1 1] Hurt Spike
)

(event EventBeginPlay
  ;[1 1 1] Movement
  (bind _output_get (Variables|Default|SetInitialLocation (Transformation|GetActorLocation)))
  (Variables|Default|SetEndLocation (+ _output_get (Math|Vector|MakeVector (Variables|Default|GetPosDiffX) 0.0 (Variables|Default|GetPosDiffZ))))
  (bind _newtrack_0 (Timeline|Timeline_0 Play)
    (:Update
      (Transformation|SetActorLocation (Math|Vector|Lerp(Vector) (Variables|Default|GetInitialLocation) (Variables|Default|GetEndLocation) _newtrack_0) false false))
    (:Finished
      (if (Variables|Default|GetTimeFactor)
        (Variables|Default|SetTimeFactor false)
        (Timeline|Timeline_0 ReverseFromEnd)
        (else
          (Variables|Default|SetTimeFactor true)
          (Timeline|Timeline_0 PlayFromStart))))))

(event EventTick
  (params (DeltaSeconds :type Float%20%28single-precision%29))
  ;[1 1 1] Rotate
  (if (Variables|Default|GetRotator)
    (Variables|Default|SetTimer (+ DeltaSeconds (Variables|Default|GetTimer)))
    (Transformation|SetActorRotation (Math|Rotator|MakeRotator 0.0 (* (Variables|Default|GetTimer) (Variables|Default|GetRotation)) 0.0))))

(fn ConstructionScript)
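; Trigger volume that locks the player's camera boom on some axes while BP_Spike is inside its box.
; On overlap it detaches the boom from the player, and on exit reattaches it to the capsule and resets its relative location.
; While active with XLock set, Tick moves the boom only in Z to match the player.
; An alternative X-follow update exists but is never executed.
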(event OnComponentBeginOverlap(Box)
  (params (OverlappedComponent :type Primitive%20Component%20Object%20Reference) (OtherActor :type Actor%20Object%20Reference) (OtherComp :type Primitive%20Component%20Object%20Reference) (OtherBodyIndex :type Integer) (bFromSweep :type Boolean) (SweepResult :type Hit%20Result%20Structure%20%28by%20ref%29))
  (Utilities|Casting|CastToBP_Spike OtherActor)
  (Transformation|DetachFromComponent (Variables|Default|GetCamBoom) "KeepWorld" "KeepWorld" "KeepWorld" true)
  (Variables|Default|SetActive true))

(event OnComponentEndOverlap(Box)
  (params (OverlappedComponent :type Primitive%20Component%20Object%20Reference) (OtherActor :type Actor%20Object%20Reference) (OtherComp :type Primitive%20Component%20Object%20Reference) (OtherBodyIndex :type Integer))
  (bind _asbp_spike (Utilities|Casting|CastToBP_Spike OtherActor))
  (Transformation|AttachComponentToComponent (Variables|Default|GetCamBoom) (Variables|/Script/Engine.Character|GetCapsuleComponent _asbp_spike) "None" "KeepWorld" "KeepWorld" "KeepWorld" true)
  (Variables|Default|SetActive false)
  (Transformation|SetRelativeLocation (Variables|Default|GetCamBoom) "0, 0,0.000000" false false))

(event EventBeginPlay
  (bind _asbp_spike (Utilities|Casting|CastToBP_Spike (Game|GetPlayerCharacter 0)))
  (bind _output_get (Variables|Default|SetPlayer _asbp_spike))
  (Variables|Default|SetCamBoom (Variables|/Game/SetchOnLegs/00Blueprint/07Spike/BP_Spike.BP_Spike_C|GetCameraBoom _output_get)))

(event EventTick
  (params (DeltaSeconds :type Float%20%28single-precision%29))
  (bind _camboom (Variables|Default|GetCamBoom))
  (bind _returnvalue (Transformation|GetWorldLocation _camboom))
  (bind (_x _y) (Math|Vector|BreakVector _returnvalue))
  ;[1 1 1] Fix camera movement based on lock type
  (if (Variables|Default|GetActive)
    (if (Variables|Default|GetXLock)
      (Transformation|SetWorldLocation (Variables|Default|GetCamBoom) (Math|Vector|MakeVector _x _y (.Z (Math|Vector|BreakVector (Transformation|GetActorLocation (Variables|Default|GetPlayer))))) false false))))

(fn ConstructionScript)
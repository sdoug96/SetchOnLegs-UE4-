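; Map boundary volume that bounces BP_WickedWitch back when the witch overlaps its box.
; A BoundaryType setting selects the response, reflecting vertical speed for Top and Bottom and horizontal X speed for Left and Right through SetSpeed.
; Left and Right also set a fixed actor rotation for each side and move the HeadLight to the matching Y offset.
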(event OnComponentBeginOverlap(Box)
  (params (OverlappedComponent :type Primitive%20Component%20Object%20Reference) (OtherActor :type Actor%20Object%20Reference) (OtherComp :type Primitive%20Component%20Object%20Reference) (OtherBodyIndex :type Integer) (bFromSweep :type Boolean) (SweepResult :type Hit%20Result%20Structure%20%28by%20ref%29))
  (bind _asbp_wicked_witch (Utilities|Casting|CastToBP_WickedWitch OtherActor))
  (bind _output_get (Variables|Default|SetWitch _asbp_wicked_witch))
  (Variables|Default|SetWitchMovement (Variables|/Script/Engine.Character|GetCharacterMovement _output_get))
  (switch Utilities|FlowControl|Switch|SwitchonBoundaryType (Variables|Default|GetBoundaryType)
    (:NewEnumerator0
      (Default|SetSpeed (Variables|Default|GetWitch) (.x (Variables|/Script/Engine.MovementComponent|GetVelocity (Variables|Default|GetWitchMovement))) (* (.z (Variables|/Script/Engine.MovementComponent|GetVelocity (Variables|Default|GetWitchMovement))) -1.0) :!label _label))
    (:NewEnumerator1
      (goto _label))
    (:NewEnumerator2
      (Transformation|SetActorRotation (Variables|Default|GetWitch))
      (Transformation|SetRelativeLocation (Variables|/Game/SetchOnLegs/00Blueprint/04AWitchesWelcome/BP_WickedWitch.BP_WickedWitch_C|GetHeadLight (Variables|Default|GetWitch)) "90.000000,100.000000,115.000000" false false)
      (Default|SetSpeed (Variables|Default|GetWitch) (* (.x (Variables|/Script/Engine.MovementComponent|GetVelocity (Variables|Default|GetWitchMovement))) -1.0) (.z (Variables|/Script/Engine.MovementComponent|GetVelocity (Variables|Default|GetWitchMovement))) :!label _label_2))
    (:NewEnumerator3
      (Transformation|SetActorRotation (Variables|Default|GetWitch) "0.000000,180.000000, 0")
      (Transformation|SetRelativeLocation (Variables|/Game/SetchOnLegs/00Blueprint/04AWitchesWelcome/BP_WickedWitch.BP_WickedWitch_C|GetHeadLight (Variables|Default|GetWitch)) "90.000000,-100.000000,115.000000" false false)
      (goto _label_2))))

(event OnComponentEndOverlap(Box)
  (params (OverlappedComponent :type Primitive%20Component%20Object%20Reference) (OtherActor :type Actor%20Object%20Reference) (OtherComp :type Primitive%20Component%20Object%20Reference) (OtherBodyIndex :type Integer)))

(fn ConstructionScript)
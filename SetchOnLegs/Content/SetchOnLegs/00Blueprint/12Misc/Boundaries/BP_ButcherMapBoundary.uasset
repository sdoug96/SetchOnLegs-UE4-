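; BP_ButcherMapBoundary is a boundary trigger that turns the Butcher around at the edges of its map.
; When its Box overlaps BP_TheButcher, it switches on BoundaryType (Left or Right) to set a fixed facing rotation.
; Both sides then share a step that negates the movement component's X velocity, reversing horizontal travel.
; Only the Left case also repositions the Butcher's CleaverSpawn component.
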(event OnComponentBeginOverlap(Box)
  (params (OverlappedComponent :type Primitive%20Component%20Object%20Reference) (OtherActor :type Actor%20Object%20Reference) (OtherComp :type Primitive%20Component%20Object%20Reference) (OtherBodyIndex :type Integer) (bFromSweep :type Boolean) (SweepResult :type Hit%20Result%20Structure%20%28by%20ref%29))
  (bind _asbp_the_butcher (Utilities|Casting|CastToBP_TheButcher OtherActor))
  (bind _output_get (Variables|Default|SetButcher _asbp_the_butcher))
  (Variables|Default|SetButcherMovement (Variables|/Script/Engine.Character|GetCharacterMovement _output_get))
  (switch Utilities|FlowControl|Switch|SwitchonBoundaryType (Variables|Default|GetBoundaryType)
    (:NewEnumerator2
      (Transformation|SetActorRotation (Variables|Default|GetButcher) "0,180.000000, 0")
      (Transformation|SetRelativeLocation (Variables|/Game/SetchOnLegs/00Blueprint/03TheButcher/BP_TheButcher.BP_TheButcher_C|GetCleaverSpawn (Variables|Default|GetButcher)) "-352.000000,0.100000,6.000000" false false))
    (:NewEnumerator3
      (Transformation|SetActorRotation (Variables|Default|GetButcher) "0.000000,0.000000, 0")))
  (Variables|/Script/Engine.MovementComponent|SetVelocity (Variables|Default|GetButcherMovement) (Math|Vector|MakeVector (* (.x (Variables|/Script/Engine.MovementComponent|GetVelocity (Variables|Default|GetButcherMovement))) -1.0) (.y (Variables|/Script/Engine.MovementComponent|GetVelocity (Variables|Default|GetButcherMovement))) (.z (Variables|/Script/Engine.MovementComponent|GetVelocity (Variables|Default|GetButcherMovement))))))

(fn ConstructionScript)
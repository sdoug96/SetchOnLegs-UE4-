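; BP_DestroyableWall is a wall that the player breaks by shooting it, with its destroyed state remembered in the game instance.
; Each BP_Bullet entering the HitBox is destroyed, lowers health by one and plays a hit sound.
; Tick watches for depleted health, then flags the wall's ID in the WallsDestroyed array, plays a sound and destroys it.
; On BeginPlay, a wall already flagged in that array removes itself.
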(event OnComponentBeginOverlap(HitBox)
  (params (OverlappedComponent :type Primitive%20Component%20Object%20Reference) (OtherActor :type Actor%20Object%20Reference) (OtherComp :type Primitive%20Component%20Object%20Reference) (OtherBodyIndex :type Integer) (bFromSweep :type Boolean) (SweepResult :type Hit%20Result%20Structure%20%28by%20ref%29))
  (bind _asbp_bullet (Utilities|Casting|CastToBP_Bullet OtherActor))
  (Actor|DestroyActor _asbp_bullet)
  (Variables|Default|SetCurrentHealth (- (Variables|Default|GetCurrentHealth) 1.0))
  (Audio|PlaySound2D "/Game/SetchOnLegs/03Audio/08Misc/ChestHit.ChestHit" 1.0 1.0 0.0 0 0))

(event EventTick
  (params (DeltaSeconds :type Float%20%28single-precision%29))
  (if (<= (Variables|Default|GetCurrentHealth) 0.0)
    (Utilities|Array|SetArrayElem (Variables|/Game/SetchOnLegs/00Blueprint/12Misc/BP_GameInstance.BP_GameInstance_C|GetWallsDestroyed (Variables|Default|GetGameInstance)) (Variables|Default|GetID) true true)
    (Audio|PlaySound2D "/Game/SetchOnLegs/03Audio/08Misc/UnusedAtTheMoment/FoundingFatherEssenceHit.FoundingFatherEssenceHit" 1.0 1.0 0.0 0 0)
    (Actor|DestroyActor)))

(event EventBeginPlay
  (bind _asbp_game_instance (Utilities|Casting|CastToBP_GameInstance (Game|GetGameInstance)))
  (bind _output_get (Variables|Default|SetGameInstance _asbp_game_instance))
  (for (_array_element _array_index) (Variables|/Game/SetchOnLegs/00Blueprint/12Misc/BP_GameInstance.BP_GameInstance_C|GetWallsDestroyed _output_get)
    (if (== _array_index (Variables|Default|GetID))
      (if _array_element
        (Actor|DestroyActor)))))

(fn ConstructionScript)
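; BP_MapBoundary is a map edge that bounces characters from its CharacterList back into play when they overlap its Box.
; Each Tick it checks overlaps and, by BoundaryType, negates Z velocity for top/bottom or negates X and turns yaw 180 degrees for left/right, zeroing Y velocity.
; A shared Active flag pauses the boundary for one second after a bounce.
; BeginPlay caches movement components, but the bounce logic never reads that cache.
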(event Custom|ReverseCharacterMovement
  (if (Variables|Default|GetActive)
    (for _array_element (Variables|Default|GetCharacterList)
      (if (Collision|IsOverlappingActor (Variables|Default|GetBox) _array_element :!class /Script/Engine.PrimitiveComponent)
        (switch Utilities|FlowControl|Switch|SwitchonBoundaryType (Variables|Default|GetBoundaryType)
          (:NewEnumerator0
            (Variables|/Script/Engine.MovementComponent|SetVelocity (Variables|/Script/Engine.Character|GetCharacterMovement _array_element) (Math|Vector|MakeVector (.x (Variables|/Script/Engine.MovementComponent|GetVelocity (Variables|/Script/Engine.Character|GetCharacterMovement _array_element))) 0.0 (* (.z (Variables|/Script/Engine.MovementComponent|GetVelocity (Variables|/Script/Engine.Character|GetCharacterMovement _array_element))) -1.0))))
          (:NewEnumerator1
            (Transformation|SetActorRotation _array_element (Math|Rotator|MakeRotator (.roll (Transformation|GetActorRotation _array_element)) (.pitch (Transformation|GetActorRotation _array_element)) (- (.yaw (Transformation|GetActorRotation _array_element)) 1.8e+02)))
            (Variables|/Script/Engine.MovementComponent|SetVelocity (Variables|/Script/Engine.Character|GetCharacterMovement _array_element) (Math|Vector|MakeVector (* (.x (Variables|/Script/Engine.MovementComponent|GetVelocity (Variables|/Script/Engine.Character|GetCharacterMovement _array_element))) -1.0) 0.0 (.z (Variables|/Script/Engine.MovementComponent|GetVelocity (Variables|/Script/Engine.Character|GetCharacterMovement _array_element)))))))
        (Variables|Default|SetActive false)
        (Utilities|FlowControl|Delay 1.0)
        (Variables|Default|SetActive true)))))

(event EventBeginPlay
  (for (_array_element _array_index) (Variables|Default|GetCharacterList)
    (Utilities|Array|SetArrayElem (Variables|Default|GetCharacterMovementList) _array_index (Variables|/Script/Engine.Character|GetCharacterMovement _array_element))))

(event EventTick
  (params (DeltaSeconds :type Float%20%28single-precision%29))
  (CallFunction|ReverseCharacterMovement))

(fn ConstructionScript)
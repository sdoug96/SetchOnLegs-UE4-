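; BP_NewAreaFade is a trigger box that moves the player character, BP_Spike, to a new area behind a screen fade.
; On overlap it disables input, shows the fade-out/fade-in widget and saves NewSpawn to the game instance's SpawnLocation.
; Tick auto-walks the player along world X, in the direction set by Left, during a short delay.
; The player then jumps to NewSpawn and regains input.
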(event OnComponentBeginOverlap(Box)
  (params (OverlappedComponent :type Primitive%20Component%20Object%20Reference) (OtherActor :type Actor%20Object%20Reference) (OtherComp :type Primitive%20Component%20Object%20Reference) (OtherBodyIndex :type Integer) (bFromSweep :type Boolean) (SweepResult :type Hit%20Result%20Structure%20%28by%20ref%29))
  ;[1 1 1] Exit Level Logic
  (bind _asbp_spike (Utilities|Casting|CastToBP_Spike OtherActor))
  (Variables|Default|SetPlayer _asbp_spike)
  (bind _asbp_game_instance (Utilities|Casting|CastToBP_GameInstance (Game|GetGameInstance)))
  (Variables|Default|SetGameInstance _asbp_game_instance)
  (Variables|Default|SetHit true)
  (Input|DisableInput (Variables|Default|GetPlayer) 0)
  (bind _returnvalue (UserInterface|CreateWidget "/Game/SetchOnLegs/00Blueprint/12Misc/Fades/Widget_QuickFadeOutFadeIn.Widget_QuickFadeOutFadeIn_C"))
  (UserInterface|Viewport|AddtoViewport _returnvalue 0)
  (Utilities|FlowControl|Sequence
    (:then_0
      (Variables|/Game/SetchOnLegs/00Blueprint/12Misc/BP_GameInstance.BP_GameInstance_C|SetSpawnLocation (Variables|Default|GetGameInstance) (Variables|Default|GetNewSpawn)))
    (:then_1
      (Utilities|FlowControl|Delay 2.0)
      (Transformation|SetActorLocation (Variables|Default|GetPlayer) (Variables|Default|GetNewSpawn) false false)
      (Variables|Default|SetHit false)
      (Input|EnableInput (Variables|Default|GetPlayer) 0))))

(event EventTick
  (params (DeltaSeconds :type Float%20%28single-precision%29))
  ;[1 1 1] Exit Level Logic
  ;;[1 1 1] Move Spike
  (if (Variables|Default|GetHit)
    (bind _asbp_spike (Utilities|Casting|CastToBP_Spike (Game|GetPlayerCharacter 0)))
    (if (Variables|Default|GetLeft)
      (Pawn|Input|AddMovementInput _asbp_spike (Math|Vector|MakeVector -1.0 0.0 0.0) 1.0 false)
      (else
        (Pawn|Input|AddMovementInput _asbp_spike (Math|Vector|MakeVector 1.0 0.0 0.0) 1.0 false)))))

(fn ConstructionScript)
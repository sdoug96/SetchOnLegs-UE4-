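; BP_CorruptionGate is a barrier that knocks BP_Spike back when it touches the gate, unless the character is in one specific state.
; On HitBox overlap it compares X positions and launches the character horizontally away from the gate, overriding current velocity, and plays a 2D sound.
; Falling lateral friction is raised briefly to damp the launch, then set to zero after a short delay.
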(event OnComponentBeginOverlap(HitBox)
  (params (OverlappedComponent :type Primitive%20Component%20Object%20Reference) (OtherActor :type Actor%20Object%20Reference) (OtherComp :type Primitive%20Component%20Object%20Reference) (OtherBodyIndex :type Integer) (bFromSweep :type Boolean) (SweepResult :type Hit%20Result%20Structure%20%28by%20ref%29))
  (bind _asbp_spike (Utilities|Casting|CastToBP_Spike OtherActor))
  (bind _output_get (Variables|Default|SetPlayer _asbp_spike))
  (if (not (Utilities|Enum|Equal(Enum) (Variables|/Game/SetchOnLegs/00Blueprint/07Spike/BP_Spike.BP_Spike_C|GetState _output_get) "NewEnumerator14"))
    (if (> (.x (Transformation|GetActorLocation (Variables|Default|GetPlayer))) (.x (Transformation|GetActorLocation)))
      (Character|LaunchCharacter (Variables|Default|GetPlayer) "1750.000000,0.000000, 0" true true)
      (Variables|/Script/Engine.CharacterMovementComponent|SetFallingLateralFriction (Variables|/Script/Engine.Character|GetCharacterMovement (Variables|Default|GetPlayer)) 7.0)
      (Audio|PlaySound2D "/Game/SetchOnLegs/03Audio/08Misc/CorruptionGate.CorruptionGate" 1.0 1.0 0.0 0 0)
      (Utilities|FlowControl|Delay 0.3)
      (Variables|/Script/Engine.CharacterMovementComponent|SetFallingLateralFriction (Variables|/Script/Engine.Character|GetCharacterMovement (Variables|Default|GetPlayer)) 0.0)
      (else
        (Character|LaunchCharacter (Variables|Default|GetPlayer) "-1750.000000, 0, 0" true true)
        (Variables|/Script/Engine.CharacterMovementComponent|SetFallingLateralFriction (Variables|/Script/Engine.Character|GetCharacterMovement (Variables|Default|GetPlayer)) 7.0)
        (Audio|PlaySound2D "/Game/SetchOnLegs/03Audio/08Misc/CorruptionGate.CorruptionGate" 1.0 1.0 0.0 0 0)
        (Utilities|FlowControl|Delay 0.3)
        (Variables|/Script/Engine.CharacterMovementComponent|SetFallingLateralFriction (Variables|/Script/Engine.Character|GetCharacterMovement (Variables|Default|GetPlayer)) 0.0)))))

(fn ConstructionScript)
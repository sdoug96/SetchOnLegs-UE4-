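; BP_Gate is a locked gate that the player, BP_Spike, opens by spending a key.
; Entering the PromptBox while grounded halts the player and shows an open or locked prompt widget, depending on keys held.
; OpenGate slides the gate up or down on a timeline with sound and camera shake, then removes a key and destroys the actor.
; Opened state is saved by ID in the GameInstance's GatesOpened array, so opened gates self-destroy on BeginPlay.
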(event OnComponentBeginOverlap(PromptBox)
  (params (OverlappedComponent :type Primitive%20Component%20Object%20Reference) (OtherActor :type Actor%20Object%20Reference) (OtherComp :type Primitive%20Component%20Object%20Reference) (OtherBodyIndex :type Integer) (bFromSweep :type Boolean) (SweepResult :type Hit%20Result%20Structure%20%28by%20ref%29))
  (bind _asbp_spike (Utilities|Casting|CastToBP_Spike OtherActor))
  (if (not (AI|Components|NavMovement|IsFalling (Variables|/Script/Engine.Character|GetCharacterMovement _asbp_spike)))
    (Input|DisableInput (Variables|Default|GetPlayer) 0)
    (Sprite|SetFlipbook (Variables|/Script/Paper2D.PaperCharacter|GetSprite (Variables|Default|GetPlayer)) "/Game/SetchOnLegs/01Sprites/07Spike/Character/A_Idle.A_Idle")
    (Pawn|Components|CharacterMovement|DisableMovement (Variables|/Script/Engine.Character|GetCharacterMovement (Variables|Default|GetPlayer)))
    (Pawn|Components|CharacterMovement|SetMovementMode (Variables|/Script/Engine.Character|GetCharacterMovement (Variables|Default|GetPlayer)) "MOVE_Walking" 0)
    (if (> (Variables|/Game/SetchOnLegs/00Blueprint/07Spike/BP_Spike.BP_Spike_C|GetKeys (Variables|Default|GetPlayer)) 0)
      (bind _returnvalue (UserInterface|CreateWidget "/Game/SetchOnLegs/00Blueprint/12Misc/Gate/Widget_OpenGatePrompt.Widget_OpenGatePrompt_C"))
      (Variables|/Game/SetchOnLegs/00Blueprint/12Misc/Gate/Widget_OpenGatePrompt.Widget_OpenGatePrompt_C|SetGateToOpen _returnvalue self)
      (UserInterface|Viewport|AddtoViewport _returnvalue 0)
      (else
        (bind _returnvalue_2 (UserInterface|CreateWidget "/Game/SetchOnLegs/00Blueprint/12Misc/Gate/Widget_LockedGatePrompt.Widget_LockedGatePrompt_C"))
        (UserInterface|Viewport|AddtoViewport _returnvalue_2 0)))))

(event Custom|OpenGate
  (bind _player (Variables|Default|GetPlayer))
  (Utilities|FlowControl|Sequence
    (:then_0
      (Audio|PlaySound2D "/Game/SetchOnLegs/03Audio/08Misc/GateUnlock.GateUnlock" 1.0 1.0 0.0 0 0)
      (Collision|SetCollisionEnabled (Variables|Default|GetGate) "NoCollision")
      (Utilities|FlowControl|Delay 0.75)
      (bind _defaulttrack (Timeline|OpenGateTimeline PlayFromStart)
        (:Update
          (Transformation|SetWorldLocation (Variables|Default|GetGate) (Math|Vector|Lerp(Vector) (Variables|Default|GetStartLocation) (Variables|Default|GetEndLocation) _defaulttrack) false false))))
    (:then_1
      (Utilities|FlowControl|Delay 0.75)
      (Camera|PlayWorldCameraShake "/Game/SetchOnLegs/00Blueprint/12Misc/Gate/BP_GateShake.BP_GateShake_C" (Transformation|GetWorldLocation (Variables|/Game/SetchOnLegs/00Blueprint/07Spike/BP_Spike.BP_Spike_C|GetSideViewCameraComponent (Variables|Default|GetPlayer))) 0.0 2e+02)
      (Utilities|Array|SetArrayElem (Variables|/Game/SetchOnLegs/00Blueprint/12Misc/BP_GameInstance.BP_GameInstance_C|GetGatesOpened (Variables|Default|GetGameInstance)) (Variables|Default|GetID) true true)
      (Audio|PlaySound2D "/Game/SetchOnLegs/03Audio/08Misc/GateRumble.GateRumble" 1.0 1.0 0.0 0 0)
      (Input|DisableInput _player 0)
      (Sprite|SetFlipbook (Variables|/Script/Paper2D.PaperCharacter|GetSprite _player) "/Game/SetchOnLegs/01Sprites/07Spike/Character/A_Idle.A_Idle")
      (Utilities|FlowControl|Delay 2.0)
      (Input|EnableInput (Variables|Default|GetPlayer) 0)
      (Math|Integer|DecrementInt (Variables|/Game/SetchOnLegs/00Blueprint/07Spike/BP_Spike.BP_Spike_C|GetKeys (Variables|Default|GetPlayer))
        (:%20%20
          (Actor|DestroyActor))))))

(event EventBeginPlay
  (bind _asbp_spike (Utilities|Casting|CastToBP_Spike (Game|GetPlayerCharacter 0)))
  (Variables|Default|SetPlayer _asbp_spike)
  (bind _asbp_game_instance (Utilities|Casting|CastToBP_GameInstance (Game|GetGameInstance)))
  (bind _output_get (Variables|Default|SetGameInstance _asbp_game_instance))
  (Utilities|FlowControl|Sequence
    (:then_0
      (Variables|Default|SetStartLocation (Transformation|GetWorldLocation (Variables|Default|GetGate)))
      (if (Variables|Default|GetMoveUp)
        (Variables|Default|SetEndLocation (+ (Transformation|GetWorldLocation (Variables|Default|GetGate)) "0, 0,385.000000"))
        (else
          (Variables|Default|SetEndLocation (- (Transformation|GetWorldLocation (Variables|Default|GetGate)) "0.000000, 0,385.000000")))))
    (:then_1
      (for (_array_element _array_index) (Variables|/Game/SetchOnLegs/00Blueprint/12Misc/BP_GameInstance.BP_GameInstance_C|GetGatesOpened _output_get)
        (if (== _array_index (Variables|Default|GetID))
          (if _array_element
            (Actor|DestroyActor)))))))

(fn ConstructionScript)
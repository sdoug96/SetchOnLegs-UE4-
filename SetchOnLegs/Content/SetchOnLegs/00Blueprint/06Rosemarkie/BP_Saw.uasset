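; Saw hazard that damages the BP_Spike player by 1 on overlap, unless the player is in one specific state.
; It either ping-pongs along X/Z between start and offset points on a slow, medium or fast timeline, or moves at constant projectile velocity.
; As a fall trap it fades the screen and teleports a living player to SpawnLocation.
; Otherwise it can launch the player with briefly raised falling friction.
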(event OnComponentBeginOverlap(CollisionSphere)
  (params (OverlappedComponent :type Primitive%20Component%20Object%20Reference) (OtherActor :type Actor%20Object%20Reference) (OtherComp :type Primitive%20Component%20Object%20Reference) (OtherBodyIndex :type Integer) (bFromSweep :type Boolean) (SweepResult :type Hit%20Result%20Structure%20%28by%20ref%29))
  ;[1 1 1] Player Collision
  (bind _asbp_spike (Utilities|Casting|CastToBP_Spike OtherActor))
  (if (Utilities|Enum|NotEqual(Enum) (Variables|/Game/SetchOnLegs/00Blueprint/07Spike/BP_Spike.BP_Spike_C|GetState _asbp_spike) "NewEnumerator5")
    (Default|DamageSystem _asbp_spike 1)
    (if (Variables|Default|GetFallTrap)
      (if (not (Variables|/Game/SetchOnLegs/00Blueprint/07Spike/BP_Spike.BP_Spike_C|GetIsDead (Variables|Default|GetPlayer)))
        (bind _returnvalue (UserInterface|CreateWidget "/Game/SetchOnLegs/00Blueprint/12Misc/Fades/Widget_FallTrapFade.Widget_FallTrapFade_C"))
        (UserInterface|Viewport|AddtoViewport _returnvalue 0)
        (Pawn|Components|CharacterMovement|DisableMovement (Variables|/Script/Engine.Character|GetCharacterMovement (Variables|Default|GetPlayer)))
        (Utilities|FlowControl|Delay 1.0)
        (Transformation|SetActorLocation (Variables|Default|GetPlayer) (Variables|Default|GetSpawnLocation) false false)
        (Pawn|Components|CharacterMovement|SetMovementMode (Variables|/Script/Engine.Character|GetCharacterMovement (Variables|Default|GetPlayer)) "MOVE_Walking" 0)
        (Variables|/Game/SetchOnLegs/00Blueprint/07Spike/BP_Spike.BP_Spike_C|SetState (Variables|Default|GetPlayer) "NewEnumerator0")
        (Default|UpdateAnimation (Variables|Default|GetPlayer))
        (Variables|/Game/SetchOnLegs/00Blueprint/07Spike/BP_Spike.BP_Spike_C|SetJumpCount (Variables|Default|GetPlayer) 0))
      (elif (Variables|Default|GetLaunch)
        (Character|LaunchCharacter (Variables|Default|GetPlayer) (Math|Vector|MakeVector (Variables|Default|GetLaunchForce) 0.0 0.0) false false)
        (Variables|/Script/Engine.CharacterMovementComponent|SetFallingLateralFriction (Variables|/Script/Engine.Character|GetCharacterMovement (Variables|Default|GetPlayer)) 8.0)
        (Utilities|FlowControl|Delay 0.4)
        (Variables|/Script/Engine.CharacterMovementComponent|SetFallingLateralFriction (Variables|/Script/Engine.Character|GetCharacterMovement (Variables|Default|GetPlayer)) 0.0)))))

(event Custom|SetLerpSpeed
  ;[1 1 1] Set Lerp Speed
  (switch Utilities|FlowControl|Switch|SwitchonBladeLerpSpeed (Variables|Default|GetLerpSpeed)
    (:NewEnumerator0
      (bind _newtrack_0 (Timeline|SlowLerpTimeline Play)
        (:Update
          (Transformation|SetActorLocation (Math|Vector|Lerp(Vector) (Variables|Default|GetInitialLocation) (Variables|Default|GetEndLocation) _newtrack_0) false false))
        (:Finished
          (if (Variables|Default|GetTimeFactor)
            (Variables|Default|SetTimeFactor false)
            (Timeline|SlowLerpTimeline ReverseFromEnd)
            (else
              (Variables|Default|SetTimeFactor true)
              (Timeline|SlowLerpTimeline PlayFromStart))))))
    (:NewEnumerator1
      (bind _newtrack_0_2 (Timeline|MediumLerpTimeline Play)
        (:Update
          (Transformation|SetActorLocation (Math|Vector|Lerp(Vector) (Variables|Default|GetInitialLocation) (Variables|Default|GetEndLocation) _newtrack_0_2) false false))
        (:Finished
          (if (Variables|Default|GetTimeFactor)
            (Variables|Default|SetTimeFactor false)
            (Timeline|MediumLerpTimeline ReverseFromEnd)
            (else
              (Variables|Default|SetTimeFactor true)
              (Timeline|MediumLerpTimeline PlayFromStart))))))
    (:NewEnumerator2
      (bind _newtrack_0_3 (Timeline|QuickLerpTimeline Play)
        (:Update
          (Transformation|SetActorLocation (Math|Vector|Lerp(Vector) (Variables|Default|GetInitialLocation) (Variables|Default|GetEndLocation) _newtrack_0_3) false false))
        (:Finished
          (if (Variables|Default|GetTimeFactor)
            (Variables|Default|SetTimeFactor false)
            (Timeline|QuickLerpTimeline ReverseFromEnd)
            (else
              (Variables|Default|SetTimeFactor true)
              (Timeline|QuickLerpTimeline PlayFromStart))))))))

(event EventBeginPlay
  ;[1 1 1] Movement
  (bind _asbp_spike (Utilities|Casting|CastToBP_Spike (Game|GetPlayerCharacter 0)))
  (Variables|Default|SetPlayer _asbp_spike)
  (if (Variables|Default|GetLerp)
    (bind _output_get (Variables|Default|SetInitialLocation (Transformation|GetActorLocation)))
    (Variables|Default|SetEndLocation (+ _output_get (Math|Vector|MakeVector (Variables|Default|GetPosDiffX) 0.0 (Variables|Default|GetPosDiffZ))))
    (CallFunction|SetLerpSpeed)))

(event EventTick
  (params (DeltaSeconds :type Float%20%28single-precision%29))
  ;[1 1 1] Rotate or move
  (if (not (Variables|Default|GetLerp))
    (Variables|/Script/Engine.MovementComponent|SetVelocity (Variables|Default|GetProjectileMovement) (Math|Vector|MakeVector (Variables|Default|GetXVelocity) 0.0 (Variables|Default|GetZVelocity)))))

(fn ConstructionScript)
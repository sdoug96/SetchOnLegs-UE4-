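; BP_EnergyBall is a short-lived boss hazard in the Rosemarkie level that damages and knocks back the player, BP_Spike.
; On spawn it shakes the camera at the player's side-view camera, plays a low rumble, then destroys itself after a delay.
; Unless the player is in one exempt state, overlapping its HitSphere deals damage and launches them along X, away from the first BP_FoundingFatherScott found.
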(event OnComponentBeginOverlap(HitSphere)
  (params (OverlappedComponent :type Primitive%20Component%20Object%20Reference) (OtherActor :type Actor%20Object%20Reference) (OtherComp :type Primitive%20Component%20Object%20Reference) (OtherBodyIndex :type Integer) (bFromSweep :type Boolean) (SweepResult :type Hit%20Result%20Structure%20%28by%20ref%29))
  ;[1 1 1] Hitsphere
  (bind _asbp_spike (Utilities|Casting|CastToBP_Spike OtherActor))
  (bind _output_get (Variables|Default|SetPlayer _asbp_spike))
  (if (Utilities|Enum|NotEqual(Enum) (Variables|/Game/SetchOnLegs/00Blueprint/07Spike/BP_Spike.BP_Spike_C|GetState _output_get) "NewEnumerator5")
    (bind _outactors (Actor|GetAllActorsOfClass "/Game/SetchOnLegs/00Blueprint/06Rosemarkie/Boss/BP_FoundingFatherScott.BP_FoundingFatherScott_C"))
    (if (< (.x (Transformation|GetActorLocation (Variables|Default|GetPlayer))) (.x (Transformation|GetActorLocation (Utilities|Array|Get(acopy) _outactors))))
      (Variables|Default|SetKnockback -5e+03)
      (else
        (Variables|Default|SetKnockback 5e+03)))
    (Default|DamageSystem (Variables|Default|GetPlayer) 2)
    (Character|LaunchCharacter (Variables|Default|GetPlayer) (Math|Vector|MakeVector (Variables|Default|GetKnockback) 0.0 0.0) false false)))

(event EventBeginPlay
  ;[1 1 1] Initialise
  (bind _asbp_spike (Utilities|Casting|CastToBP_Spike (Game|GetPlayerCharacter 0)))
  (Camera|PlayWorldCameraShake "/Game/SetchOnLegs/00Blueprint/06Rosemarkie/Boss/BP_EnergyBallShake.BP_EnergyBallShake_C" (Transformation|GetWorldLocation (Variables|/Game/SetchOnLegs/00Blueprint/07Spike/BP_Spike.BP_Spike_C|GetSideViewCameraComponent _asbp_spike)) 0.0 5e+02)
  (Audio|PlaySound2D "/Game/SetchOnLegs/03Audio/06Rosemarkie/FoundingFatherScott/LowRumble.LowRumble" 1.0 1.0 0.0 0 0)
  (Utilities|FlowControl|Delay 2.7)
  (Actor|DestroyActor))

(fn ConstructionScript)
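; Boss-fight projectile for FoundingFatherScott that flies along X, then hides and fires timed radial bursts of mini thunder discs.
; Each burst spawns evenly pitched discs from the location captured after the initial delay, with alternate bursts offset half a step to stagger gaps.
; The boss's phase sets burst delay and count: three by default, four in Phase2, five in Phase3.
; Only the Phase3 path explicitly destroys the spawner.
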(event Custom|SetBurstDelay
  ;[1 1 1] Set Burst Delay
  (if (Variables|/Game/SetchOnLegs/00Blueprint/06Rosemarkie/Boss/BP_FoundingFatherScott.BP_FoundingFatherScott_C|GetPhase%202 (Variables|Default|GetFoundingFatherScott))
    (Variables|Default|SetBurstDelay 0.45)
    (elif (Variables|/Game/SetchOnLegs/00Blueprint/06Rosemarkie/Boss/BP_FoundingFatherScott.BP_FoundingFatherScott_C|GetPhase3 (Variables|Default|GetFoundingFatherScott))
      (Variables|Default|SetBurstDelay 0.4))))

(event Custom|SpawnDiscBurst
  (bind _spawnpoint (Variables|Default|GetSpawnPoint))
  (bind _returnvalue (Transformation|GetWorldTransform _spawnpoint))
  ;[1 1 1] Spawn mini disc function
  (Audio|PlaySound2D "/Game/SetchOnLegs/03Audio/06Rosemarkie/FoundingFatherScott/Spark.Spark" 1.0 1.0 0.0 0 0)
  (for _index (range 0 (- (Variables|Default|GetMiniDiscs) 1))
    (Game|SpawnActorfromClass "/Game/SetchOnLegs/00Blueprint/06Rosemarkie/Boss/BP_MiniThunderDisc.BP_MiniThunderDisc_C" (Math|Transform|MakeTransform (Variables|Default|GetMiniDiscSpawnLocation) (Math|Rotator|MakeRotator (.roll (.rotation _returnvalue)) (+ (.pitch (.rotation _returnvalue)) (Variables|Default|GetRotationIncrement)) (.yaw (.rotation _returnvalue))) "1,1,1") "Undefined" 0 0)
    (Variables|Default|SetRotationIncrement (+ (Variables|Default|GetRotationIncrement) (Math|Conversions|ToFloat(Integer) (/ 360 (Variables|Default|GetMiniDiscs))))))
  (Variables|Default|SetRotationIncrement 0.0))

(event EventBeginPlay
  ;[1 1 1] Initialise
  (bind _outactors (Actor|GetAllActorsOfClass "/Game/SetchOnLegs/00Blueprint/06Rosemarkie/Boss/BP_FoundingFatherScott.BP_FoundingFatherScott_C"))
  (Variables|Default|SetFoundingFatherScott (Utilities|Array|Get(acopy) _outactors))
  (Utilities|FlowControl|Sequence
    (:then_0
      (CallFunction|SetBurstDelay))
    (:then_1
      (Audio|PlaySound2D "/Game/SetchOnLegs/03Audio/06Rosemarkie/FoundingFatherScott/Spark.Spark" 1.0 1.0 0.0 0 0)
      (Variables|/Script/Engine.MovementComponent|SetVelocity (Variables|Default|GetProjectileMovement) (Math|Vector|MakeVector (Variables|Default|GetXVelocity) 0.0 0.0))
      (Utilities|FlowControl|Delay 0.65)
      (Variables|Default|SetMiniDiscSpawnLocation (Transformation|GetWorldLocation (Variables|Default|GetSpawnPoint)))
      (Rendering|SetVisibility (Variables|Default|GetThunderDisc) false false)
      (CallFunction|SpawnDiscBurst)
      (Utilities|FlowControl|Delay (Variables|Default|GetBurstDelay))
      (Variables|Default|SetRotationIncrement (/ (Math|Conversions|ToFloat(Integer) (/ 360 (Variables|Default|GetMiniDiscs))) 2.0))
      (CallFunction|SpawnDiscBurst)
      (Utilities|FlowControl|Delay (Variables|Default|GetBurstDelay))
      (CallFunction|SpawnDiscBurst)
      (if (or (Variables|/Game/SetchOnLegs/00Blueprint/06Rosemarkie/Boss/BP_FoundingFatherScott.BP_FoundingFatherScott_C|GetPhase%202 (Variables|Default|GetFoundingFatherScott)) (Variables|/Game/SetchOnLegs/00Blueprint/06Rosemarkie/Boss/BP_FoundingFatherScott.BP_FoundingFatherScott_C|GetPhase3 (Variables|Default|GetFoundingFatherScott)))
        (Utilities|FlowControl|Delay (Variables|Default|GetBurstDelay))
        (Variables|Default|SetRotationIncrement (/ (Math|Conversions|ToFloat(Integer) (/ 360 (Variables|Default|GetMiniDiscs))) 2.0))
        (CallFunction|SpawnDiscBurst)
        (if (Variables|/Game/SetchOnLegs/00Blueprint/06Rosemarkie/Boss/BP_FoundingFatherScott.BP_FoundingFatherScott_C|GetPhase3 (Variables|Default|GetFoundingFatherScott))
          (Utilities|FlowControl|Delay (Variables|Default|GetBurstDelay))
          (CallFunction|SpawnDiscBurst)
          (Utilities|FlowControl|Delay (Variables|Default|GetBurstDelay))
          (Actor|DestroyActor))))))

(fn ConstructionScript)
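; BP_Thunder is a short-lived lightning strike hazard, filed under the Rosemarkie boss, that damages BP_Spike.
; On spawn it waits, switches a Paper2D flipbook to the white lightning animation, briefly enables its hitbox, then destroys itself, all timed with chained delays.
; Overlapping the hitbox calls BP_Spike's DamageSystem unless Spike is in one particular exempt state.
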(event OnComponentBeginOverlap(HitBox)
  (params (OverlappedComponent :type Primitive%20Component%20Object%20Reference) (OtherActor :type Actor%20Object%20Reference) (OtherComp :type Primitive%20Component%20Object%20Reference) (OtherBodyIndex :type Integer) (bFromSweep :type Boolean) (SweepResult :type Hit%20Result%20Structure%20%28by%20ref%29))
  ;[1 1 1] Hitsphere
  (bind _asbp_spike (Utilities|Casting|CastToBP_Spike OtherActor))
  (if (Utilities|Enum|NotEqual(Enum) (Variables|/Game/SetchOnLegs/00Blueprint/07Spike/BP_Spike.BP_Spike_C|GetState _asbp_spike) "NewEnumerator5")
    (Default|DamageSystem _asbp_spike 2)))

(event EventBeginPlay
  ;[1 1 1] Initialise
  (Collision|SetCollisionEnabled (Variables|Default|GetHitBox) "NoCollision")
  (Utilities|FlowControl|Delay 0.5)
  (Sprite|SetFlipbook (Variables|Default|GetWhiteLightning) "/Game/SetchOnLegs/01Sprites/06Rosemarkie/FoundingFatherScott/Attacks/WhiteLightning/A_WhiteLightning.A_WhiteLightning")
  (Utilities|FlowControl|Delay 0.4)
  (Collision|SetCollisionEnabled (Variables|Default|GetHitBox) "QueryAndPhysics")
  (Utilities|FlowControl|Delay 0.1)
  (Collision|SetCollisionEnabled (Variables|Default|GetHitBox) "NoCollision")
  (Utilities|FlowControl|Delay 0.3)
  (Actor|DestroyActor))

(fn ConstructionScript)
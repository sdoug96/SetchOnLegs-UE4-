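; BP_Thunder is a timed lightning strike attack, filed among the Rosemarkie boss attacks, that damages BP_Spike.
; A delay chain from BeginPlay shows the lightning flipbook, briefly enables HitBox collision with optional thunder sound, then destroys the actor.
; HitBox overlaps that cast to BP_Spike call DamagePlayer, so damage lands only during that short collision window.
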(event OnComponentBeginOverlap(HitBox)
  (params (OverlappedComponent :type Primitive%20Component%20Object%20Reference) (OtherActor :type Actor%20Object%20Reference) (OtherComp :type Primitive%20Component%20Object%20Reference) (OtherBodyIndex :type Integer) (bFromSweep :type Boolean) (SweepResult :type Hit%20Result%20Structure%20%28by%20ref%29))
  ;[1 1 1] Hitsphere
  (bind _asbp_spike (Utilities|Casting|CastToBP_Spike OtherActor))
  (CallFunction|DamagePlayer _asbp_spike))

(event EventBeginPlay
  ;[1 1 1] Initialise
  (Collision|SetCollisionEnabled (Variables|Default|GetHitBox) "NoCollision")
  (Utilities|FlowControl|Delay 0.5)
  (Sprite|SetFlipbook (Variables|Default|GetPaperFlipbook) "/Game/SetchOnLegs/01Sprites/06Rosemarkie/FoundingFatherScott/Attacks/WhiteLightning/A_WhiteLightning.A_WhiteLightning")
  (Utilities|FlowControl|Delay 0.4)
  (Collision|SetCollisionEnabled (Variables|Default|GetHitBox) "QueryAndPhysics")
  (if (Variables|Default|GetPlaySound)
    (Audio|PlaySound2D "/Game/SetchOnLegs/03Audio/06Rosemarkie/FoundingFatherScott/Thunder.Thunder" 1.0 1.0 0.0 0 0))
  (Utilities|FlowControl|Delay 0.1)
  (Collision|SetCollisionEnabled (Variables|Default|GetHitBox) "NoCollision")
  (Utilities|FlowControl|Delay 0.3)
  (Actor|DestroyActor))

(fn ConstructionScript)
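; Energy beam projectile for the Founding Father Scott boss fight that damages the player, BP_Spike, on contact.
; On spawn it plays a sound and flies along negative X, taking a faster speed if the first Scott actor found is in Phase 2 or 3.
; HitBox overlap calls Spike's DamageSystem except in two exempt states.
; The beam then destroys itself, unless Spike has ShadowDash and is in one particular state.
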(event OnComponentBeginOverlap(HitBox)
  (params (OverlappedComponent :type Primitive%20Component%20Object%20Reference) (OtherActor :type Actor%20Object%20Reference) (OtherComp :type Primitive%20Component%20Object%20Reference) (OtherBodyIndex :type Integer) (bFromSweep :type Boolean) (SweepResult :type Hit%20Result%20Structure%20%28by%20ref%29))
  ;[1 1 1] Collide with player
  (bind _asbp_spike (Utilities|Casting|CastToBP_Spike OtherActor))
  (if (and (Utilities|Enum|NotEqual(Enum) (Variables|/Game/SetchOnLegs/00Blueprint/07Spike/BP_Spike.BP_Spike_C|GetState _asbp_spike) "NewEnumerator5") (Utilities|Enum|NotEqual(Enum) (Variables|/Game/SetchOnLegs/00Blueprint/07Spike/BP_Spike.BP_Spike_C|GetState _asbp_spike) "NewEnumerator14"))
    (Default|DamageSystem _asbp_spike 2)
    (if (Variables|/Game/SetchOnLegs/00Blueprint/07Spike/BP_Spike.BP_Spike_C|GetShadowDash _asbp_spike)
      (if (Utilities|Enum|NotEqual(Enum) (Variables|/Game/SetchOnLegs/00Blueprint/07Spike/BP_Spike.BP_Spike_C|GetState _asbp_spike) "NewEnumerator8")
        (Actor|DestroyActor :!label _label))
      (else
        (goto _label)))))

(event EventBeginPlay
  ;[1 1 1] Initialise
  (Audio|PlaySound2D "/Game/SetchOnLegs/03Audio/06Rosemarkie/FoundingFatherScott/EnergyBeam.EnergyBeam" 1.0 1.0 0.0 0 0)
  (Variables|/Script/Engine.MovementComponent|SetVelocity (Variables|Default|GetProjectileMovement) "-1200.000000,0.0,0.0")
  (bind _outactors (Actor|GetAllActorsOfClass "/Game/SetchOnLegs/00Blueprint/06Rosemarkie/Boss/BP_FoundingFatherScott.BP_FoundingFatherScott_C"))
  (bind _output_get (Variables|Default|SetFoundingFatherScott (Utilities|Array|Get(acopy) _outactors)))
  (if (Variables|/Game/SetchOnLegs/00Blueprint/06Rosemarkie/Boss/BP_FoundingFatherScott.BP_FoundingFatherScott_C|GetPhase%202 _output_get)
    (Variables|/Script/Engine.MovementComponent|SetVelocity (Variables|Default|GetProjectileMovement) "-1500.000000,0.0,0.0")
    (elif (Variables|/Game/SetchOnLegs/00Blueprint/06Rosemarkie/Boss/BP_FoundingFatherScott.BP_FoundingFatherScott_C|GetPhase3 (Variables|Default|GetFoundingFatherScott))
      (Variables|/Script/Engine.MovementComponent|SetVelocity (Variables|Default|GetProjectileMovement) "-2000.000000,0.0,0.0"))))

(fn ConstructionScript)